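; TipDesignController shows the widget of the DesignTip actor nearest the player and lets the K key toggle visibility of all tips.
; A looping timer, rather than Tick, scans every DesignTip for the closest one within a short radius.
; It swaps the on-screen widget and Closer flag as the player's CurrentTip changes, clearing them when out of range.
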(event `NearestDesignTip`
  (bind _playerref (`self.PlayerRef`))
  (bind _newtip (`self.NewTip`))
  (bind _playerref_2 (`self.PlayerRef`))
  (bind _currenttip (`/Game/Blueprints/Player/Player_BP.CurrentTip` (`self.PlayerRef`)))
  ;[1 1 0] Show DesignTip
  (set `self.TipIndex` 0)
  (bind _outactors (`GameplayStatics.GetAllActorsOfClass` "/Game/Blueprints/NPCs/DesignTip.DesignTip_C"))
  (bind _returnvalue (`KismetArrayLibrary.Array_Length` _outactors))
  (if (> _returnvalue 0)
    (bind _output (`|GetArrayItem` _outactors (`self.TipIndex`)))
    (if (< (`self.GetDistanceTo` _output (`self.PlayerRef`)) 100.0) :!label _label
      (`/Engine/EditorBlueprintResources/StandardMacros.IsValid` (`self.NewTip`)
        (:`Is Valid`
          _)
        (:`Is Not Valid`
          (set `self.NewTip` _output)))
      (if (< (`self.GetDistanceTo` _output _playerref) (`self.GetDistanceTo` _playerref (`self.NewTip`)))
        (set `self.NewTip` _output)))
    (if (< (`self.TipIndex`) (- _returnvalue 1))
      (set `self.TipIndex` (+ (`self.TipIndex`) 1))
      (goto _label)
      (else
        (`/Engine/EditorBlueprintResources/StandardMacros.IsValid` _newtip
          (:`Is Valid`
            (if (< (`self.GetDistanceTo` _newtip (`self.PlayerRef`)) 100.0)
              (if (!= (`self.NewTip`) (`/Game/Blueprints/Player/Player_BP.CurrentTip` (`self.PlayerRef`)))
                (`/Engine/EditorBlueprintResources/StandardMacros.IsValid` _currenttip
                  (:`Is Valid`
                    (set `/Game/Blueprints/NPCs/DesignTip.Closer` false _currenttip)
                    (bind _foundwidgets (`WidgetBlueprintLibrary.GetAllWidgetsOfClass` (`/Game/Blueprints/NPCs/DesignTip.WidgetRef` (`/Game/Blueprints/Player/Player_BP.CurrentTip` (`self.PlayerRef`)))))
                    (bind _output_2 (`|GetArrayItem` _foundwidgets))
                    (`/Engine/EditorBlueprintResources/StandardMacros.IsValid` _output_2
                      (:`Is Valid`
                        (`Widget.RemoveFromParent` _output_2))
                      (:`Is Not Valid`
                        _)))
                  (:`Is Not Valid`
                    _))
                (bind _output_get (set `/Game/Blueprints/Player/Player_BP.CurrentTip` (`self.NewTip`) (`self.PlayerRef`)))
                (bind _returnvalue_2 (`|CreateWidget` (`/Game/Blueprints/NPCs/DesignTip.WidgetRef` _output_get) (`GameplayStatics.GetPlayerController` 0)))
                (`UserWidget.AddToViewport` _returnvalue_2 0)
                (set `/Game/Blueprints/NPCs/DesignTip.Closer` true (`/Game/Blueprints/Player/Player_BP.CurrentTip` (`self.PlayerRef`))))
              (else
                (`/Engine/EditorBlueprintResources/StandardMacros.IsValid` (`/Game/Blueprints/Player/Player_BP.CurrentTip` (`self.PlayerRef`))
                  (:`Is Valid`
                    (bind _foundwidgets_2 (`WidgetBlueprintLibrary.GetAllWidgetsOfClass` (`/Game/Blueprints/NPCs/DesignTip.WidgetRef` (`/Game/Blueprints/Player/Player_BP.CurrentTip` (`self.PlayerRef`)))))
                    (bind _output_3 (`|GetArrayItem` _foundwidgets_2))
                    (`/Engine/EditorBlueprintResources/StandardMacros.IsValid` _output_3
                      (:`Is Valid`
                        (`Widget.RemoveFromParent` _output_3)
                        (set `/Game/Blueprints/NPCs/DesignTip.Closer` false (`/Game/Blueprints/Player/Player_BP.CurrentTip` _playerref_2))
                        (set `/Game/Blueprints/Player/Player_BP.CurrentTip` null _playerref_2)))))))))))))

(event `Key|K`
  (params (Key :type "Key Structure"))
  ;[1 1 0] Show DesignTip
  (:`Pressed`
    (`/Engine/EditorBlueprintResources/StandardMacros.FlipFlop`
      (:`A`
        (set `self.TipIndex` 0)
        (bind _outactors (`GameplayStatics.GetAllActorsOfClass` "/Game/Blueprints/NPCs/DesignTip.DesignTip_C"))
        (`self.SetActorHiddenInGame` (`|GetArrayItem` _outactors (`self.TipIndex`)) false :!label _label_2)
        (if (< (`self.TipIndex`) (- (`KismetArrayLibrary.Array_Length` _outactors) 1))
          (set `self.TipIndex` (+ (`self.TipIndex`) 1))
          (goto _label_2)))
      (:`B`
        (set `self.TipIndex` 0)
        (bind _outactors_2 (`GameplayStatics.GetAllActorsOfClass` "/Game/Blueprints/NPCs/DesignTip.DesignTip_C"))
        (`self.SetActorHiddenInGame` (`|GetArrayItem` _outactors_2 (`self.TipIndex`)) true :!label _label_3)
        (if (< (`self.TipIndex`) (- (`KismetArrayLibrary.Array_Length` _outactors_2) 1))
          (set `self.TipIndex` (+ (`self.TipIndex`) 1))
          (goto _label_3))))))

(event `self.ReceiveBeginPlay`
  (bind _asplayer_bp (cast `/Game/Blueprints/Player/Player_BP` (`GameplayStatics.GetPlayerCharacter` 0)))
  (set `self.PlayerRef` _asplayer_bp)
  (`KismetSystemLibrary.K2_SetTimerDelegate` (delegate `NearestDesignTip`) 0.1 true))

(event `self.ReceiveTick`
  (params (DeltaSeconds :type "Float (single-precision)")))

(fn `UserConstructionScript`)