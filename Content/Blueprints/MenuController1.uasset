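; World map controller that toggles the pause menu, finding the player pawn and music controller at BeginPlay.
; Tick polls Escape, F10 and gamepad Start, feeding a DoOnce that creates or removes the menu widget with sound, then resets after a short delay.
; Game pause and music volume change only outside paused dialogue; IsCalling swallows a Start press.
; Separate events clear the player's text-skip flag and set a delayed pause-permission flag.
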(event `SkipText`
  (if (`PlayerController.WasInputKeyJustPressed` (`GameplayStatics.GetPlayerController` 0) "Enter")
    (`/Engine/EditorBlueprintResources/StandardMacros.IsValid` (`self.WMPlayerRef`) :!label _label
      (:`Is Valid`
        (if (not (`/Game/Blueprints/WorldMap/WorldMap_Player.IsMenuOn?` (`self.WMPlayerRef`)))
          (set `/Game/Blueprints/WorldMap/WorldMap_Player.IsSkipText` false (`self.WMPlayerRef`)))))
    (elif (`PlayerController.WasInputKeyJustPressed` (`GameplayStatics.GetPlayerController` 0) "Gamepad_FaceButton_Right")
      (goto _label))))

(event `self.ReceiveBeginPlay`
  (bind _asworld_map_player (cast `/Game/Blueprints/WorldMap/WorldMap_Player` (`GameplayStatics.GetPlayerPawn` 0))
    (:`then`
      (set `self.WMPlayerRef` _asworld_map_player))
    (:`CastFailed`
      (`KismetSystemLibrary.PrintString` "MenuController: Player Missing" true true (struct :`R` 1.0 :`B` 0.014804 :`A` 1.0))))
  (bind _outactors (`GameplayStatics.GetAllActorsOfClass` "/Game/Blueprints/MusicController.MusicController_C"))
  (bind _output (`|GetArrayItem` _outactors))
  (`/Engine/EditorBlueprintResources/StandardMacros.IsValid` _output
    (:`Is Valid`
      (set `self.MusicControllerRef` _output))
    (:`Is Not Valid`
      (`KismetSystemLibrary.PrintString` "MenuController: MusicController Missing" true true (struct :`R` 1.0 :`A` 1.0)))))

(event `PauseDelayer`
  (`/Engine/EditorBlueprintResources/StandardMacros.DoOnce` false
    (:`Completed`
      (`KismetSystemLibrary.Delay` 0.05)
      (set `self.CanPauseInPausedCall` true))))

(event `self.ReceiveTick`
  (params (DeltaSeconds :type "Float (single-precision)"))
  (`self.Menu`))

(event `ResetMenu`
  (goto _label_2 :!via `Reset`))

(event `Menu`
  (if (`PlayerController.WasInputKeyJustPressed` (`GameplayStatics.GetPlayerController` 0) "Escape")
    (`/Engine/EditorBlueprintResources/StandardMacros.DoOnce` false :!label _label_2
      (:`Completed`
        (set `self.isCalling` false)
        (if (`/Game/Blueprints/WorldMap/WorldMap_Player.IsMenuOn?` (`self.WMPlayerRef`))
          (if (not (`/Game/Blueprints/WorldMap/WorldMap_Player.IsTalkingPaused` (`self.WMPlayerRef`)))
            (`GameplayStatics.SetGamePaused` false)
            (`/Game/Blueprints/MusicController.inGameVolume` (`self.MusicControllerRef`)))
          (set `/Game/Blueprints/WorldMap/WorldMap_Player.IsMenuOn?` false (`self.WMPlayerRef`))
          (`GameplayStatics.PlaySound2D` "/Game/Sound/SFXs/sfx_pauseOut_Cue.sfx_pauseOut_Cue" 1.0 1.0 0.0 null null)
          (bind _foundwidgets (`WidgetBlueprintLibrary.GetAllWidgetsOfClass` "/Game/Widgets/PauseMenu_HUD1.PauseMenu_HUD1_C"))
          (`Widget.RemoveFromParent` (`|GetArrayItem` _foundwidgets))
          (else
            (if (not (`/Game/Blueprints/WorldMap/WorldMap_Player.IsTalkingPaused` (`self.WMPlayerRef`)))
              (`GameplayStatics.SetGamePaused` true)
              (`/Game/Blueprints/MusicController.PauseVolume` (`self.MusicControllerRef`)))
            (set `/Game/Blueprints/WorldMap/WorldMap_Player.IsMenuOn?` true (`self.WMPlayerRef`))
            (`GameplayStatics.PlaySound2D` "/Game/Sound/SFXs/sfx_PauseIn_Cue.sfx_PauseIn_Cue" 1.0 1.0 0.0 null null)
            (bind _returnvalue (`|CreateWidget` "/Game/Widgets/PauseMenu_HUD1.PauseMenu_HUD1_C"))
            (`UserWidget.AddToViewport` _returnvalue 0)))
        (`KismetSystemLibrary.Delay` 0.2)
        (`self.ResetMenu`)))
    (elif (`PlayerController.WasInputKeyJustPressed` (`GameplayStatics.GetPlayerController` 0) "F10")
      (goto _label_2)
      (elif (`PlayerController.WasInputKeyJustPressed` (`GameplayStatics.GetPlayerController` 0) "Gamepad_Special_Right")
        (if (`self.isCalling`)
          (set `self.isCalling` false)
          (else
            (goto _label_2)))))))

(fn `UserConstructionScript`)