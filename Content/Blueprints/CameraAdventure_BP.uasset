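; Side-scrolling follow camera for adventure gameplay that tracks Player_BP along X and Z.
; On BeginPlay it becomes the view target, or in the PreBoss state hands the view to CameraCorridor_BP and switches ScreenCollider_BP to fixed-cam.
; Tick applies dead-zone following while the player lives: horizontal distance drives X, and, if CanMoveZ, separate up/down thresholds drive Z, with descent clamped at ZMin.
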(event `self.ReceiveBeginPlay`
  ;[1 1 1] Default
  (`KismetSystemLibrary.Delay` 0.05)
  (bind _asplayer_bp (cast `/Game/Blueprints/Player/Player_BP` (`GameplayStatics.GetPlayerCharacter` 0)))
  (bind _output_get (set `self.PlayerRef` _asplayer_bp))
  (if (`/Game/Blueprints/Player/Player_BP.PreBoss?` _output_get)
    ;[1 1 1] PreBoss Cam (Corridor)
    (bind _outactors (`GameplayStatics.GetAllActorsOfClass` "/Game/Blueprints/CameraCorridor_BP.CameraCorridor_BP_C"))
    (bind _output (`|GetArrayItem` _outactors))
    (`PlayerController.SetViewTargetWithBlend` (`GameplayStatics.GetPlayerController` 0) _output 0.0 "VTBlend_Linear" 0.0 false)
    (bind _outactors_2 (`GameplayStatics.GetAllActorsOfClass` "/Game/Blueprints/Level/ScreenCollider_BP.ScreenCollider_BP_C"))
    (`/Game/Blueprints/Level/ScreenCollider_BP.ToFixedCam` (`|GetArrayItem` _outactors_2) (`self.K2_GetActorLocation` _output))
    (else
      (bind (_returnvalue_x _returnvalue_y _returnvalue_z) (`KismetMathLibrary.BreakVector` (`self.K2_GetActorLocation` _output_get)))
      (`self.K2_SetActorLocation` (`KismetMathLibrary.MakeVector` _returnvalue_x _returnvalue_y (`self.ZCurrent`)))
      (`PlayerController.SetViewTargetWithBlend` (`GameplayStatics.GetPlayerController` 0) self 0.0 "VTBlend_Linear" 0.0 false)
      (`KismetSystemLibrary.Delay` 3.0)
      (`KismetSystemLibrary.PrintString` (`KismetStringLibrary.Concat_StrStr` "Zcurrent: " (`KismetStringLibrary.Conv_DoubleToString` (`self.ZCurrent`))) true true (struct :`G` 0.66 :`B` 1.0 :`A` 1.0) 10.0)
      (`KismetSystemLibrary.PrintString` (`KismetStringLibrary.Concat_StrStr` "ZDistanceDownAllowed: " (`KismetStringLibrary.Conv_DoubleToString` (`self.ZDistanceDownAllowed`))) true true (struct :`G` 0.66 :`B` 1.0 :`A` 1.0) 10.0)
      (`KismetSystemLibrary.PrintString` (`KismetStringLibrary.Concat_StrStr` "ZMin: " (`KismetStringLibrary.Conv_DoubleToString` (`self.ZMin`))) true true (struct :`G` 0.66 :`B` 1.0 :`A` 1.0) 10.0))))

(event `self.ReceiveTick`
  (params (DeltaSeconds :type "Float (single-precision)"))
  ;[1 1 1] Default
  (`/Engine/EditorBlueprintResources/StandardMacros.IsValid` (`self.PlayerRef`)
    (:`Is Valid`
      (if (not (`/Game/Blueprints/Player/Player_BP.isDead` (`self.PlayerRef`)))
        (`self.CameraX`)
        (if (`self.CanMoveZ?`)
          (`self.CameraZ`))))))

(event `CameraX`
  (bind _returnvalue_x (`KismetMathLibrary.BreakVector` (`self.K2_GetActorLocation`)))
  (bind _returnvalue_x_2 (`KismetMathLibrary.BreakVector` (`self.K2_GetActorLocation` (`self.PlayerRef`))))
  (bind _returnvalue_x_3 (`KismetMathLibrary.BreakVector` (`self.K2_GetActorLocation` (`self.PlayerRef`))))
  (bind _returnvalue_x_4 (`KismetMathLibrary.BreakVector` (`self.K2_GetActorLocation` (`self.PlayerRef`))))
  ;[1 1 1] Camera X moving
  (if (> _returnvalue_x_2 _returnvalue_x)
    (if (>= (`self.GetHorizontalDistanceTo` (`self.PlayerRef`)) (`self.XDistanceAllowed`))
      (bind _output_get (set `self.XCurrent` (- _returnvalue_x_3 (`self.XDistanceAllowed`))))
      (`self.K2_SetActorLocation` (`KismetMathLibrary.MakeVector` _output_get 0.0 (`self.ZCurrent`))))
    (elif (>= (`self.GetHorizontalDistanceTo` (`self.PlayerRef`)) (`self.XDistanceAllowed`))
      (bind _output_get_2 (set `self.XCurrent` (+ _returnvalue_x_4 (`self.XDistanceAllowed`))))
      (`self.K2_SetActorLocation` (`KismetMathLibrary.MakeVector` _output_get_2 0.0 (`self.ZCurrent`))))))

(event `CameraZ`
  (bind (_returnvalue_x _returnvalue_y _returnvalue_z) (`KismetMathLibrary.BreakVector` (`self.K2_GetActorLocation`)))
  (bind (_returnvalue_x_2 _returnvalue_y_2 _returnvalue_z_2) (`KismetMathLibrary.BreakVector` (`self.K2_GetActorLocation`)))
  (bind (_returnvalue_x_3 _returnvalue_y_3 _returnvalue_z_3) (`KismetMathLibrary.BreakVector` (`self.K2_GetActorLocation` (`self.PlayerRef`))))
  (bind (_returnvalue_x_4 _returnvalue_y_4 _returnvalue_z_4) (`KismetMathLibrary.BreakVector` (`self.K2_GetActorLocation` (`self.PlayerRef`))))
  (bind (_returnvalue_x_5 _returnvalue_y_5 _returnvalue_z_5) (`KismetMathLibrary.BreakVector` (`self.K2_GetActorLocation` (`self.PlayerRef`))))
  (bind (_returnvalue_x_6 _returnvalue_y_6 _returnvalue_z_6) (`KismetMathLibrary.BreakVector` (`self.K2_GetActorLocation` (`self.PlayerRef`))))
  (bind (_returnvalue_x_7 _returnvalue_y_7 _returnvalue_z_7) (`KismetMathLibrary.BreakVector` (`self.K2_GetActorLocation` (`self.PlayerRef`))))
  (bind (_returnvalue_x_8 _returnvalue_y_8 _returnvalue_z_8) (`KismetMathLibrary.BreakVector` (`self.K2_GetActorLocation` (`self.PlayerRef`))))
  ;[1 1 1] Camera Z moving
  (if (> (+ _returnvalue_z_4 36.0) (+ (`self.ZCurrent`) (`self.ZDistanceUpAllowed`)))
    (if (>= (- (+ _returnvalue_z_8 36.0) _returnvalue_z_2) (`self.ZDistanceUpAllowed`))
      (bind _output_get (set `self.ZCurrent` (- (+ _returnvalue_z_7 36.0) (`self.ZDistanceUpAllowed`))))
      (`self.K2_SetActorLocation` (`KismetMathLibrary.MakeVector` (`self.XCurrent`) 0.0 _output_get)))
    (elif (< _returnvalue_z_6 (`self.ZCurrent`))
      (if (< (- (+ _returnvalue_z_3 36.0) _returnvalue_z) (`self.ZDistanceDownAllowed`))
        (set `self.ZCurrent` _returnvalue_z_5)
        (if (< (`self.ZCurrent`) (`self.ZMin`))
          (set `self.ZCurrent` (`self.ZMin`)))
        (`self.K2_SetActorLocation` (`KismetMathLibrary.MakeVector` (`self.XCurrent`) 0.0 (`self.ZCurrent`)))))))

(fn `UserConstructionScript`)