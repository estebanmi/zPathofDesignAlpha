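; CamPush is an auto-scrolling camera that, when ActiveCam is set, becomes the view target and moves via ProjectileMovement.
; Tick checks optional position thresholds that turn it diagonal, straighten it, then stop it at XMax.
; Its lateral and falling colliders kill the player with effects, save, and reload the level after a delay.
; The falling collider also destroys enemies, but only while the camera's height is near ZToStraight.
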(event `self.ReceiveBeginPlay`
  ;[1 1 1] Default
  (bind _returnvalue (`GameplayStatics.GetCurrentLevelName` true))
  (set `self.CurrentLevel` (`KismetStringLibrary.Conv_StringToName` _returnvalue))
  (`KismetSystemLibrary.Delay` 0.05)
  (bind _asplayer_bp (cast `/Game/Blueprints/Player/Player_BP` (`GameplayStatics.GetPlayerCharacter` 0)))
  (set `self.PlayerRef` _asplayer_bp)
  (if (`self.ActiveCam`)
    (`PlayerController.SetViewTargetWithBlend` (`GameplayStatics.GetPlayerController` 0) self 0.0 "VTBlend_Linear" 0.0 false)
    (`ProjectileMovementComponent.SetVelocityInLocalSpace` (`self.ProjectileMovement`) (`self.Velocity`))
    (bind _outactors (`GameplayStatics.GetAllActorsOfClass` "/Game/Blueprints/Level/ScreenCollider_BP.ScreenCollider_BP_C"))
    (set `/Game/Blueprints/Level/ScreenCollider_BP.FollowingCam` "NewEnumerator1" (`|GetArrayItem` _outactors))))

(event `PlayerFallingDeath`
  (bind (_returnvalue_x _returnvalue_y _returnvalue_z) (`KismetMathLibrary.BreakVector` (`self.K2_GetActorLocation`)))
  (bind _returnvalue_x_2 (`KismetMathLibrary.BreakVector` (`self.K2_GetActorLocation` (`self.PlayerRef`))))
  (`|SpawnActorFromClass` "/Game/Blueprints/FX/PlayerDeathFalling_FX.PlayerDeathFalling_FX_C" (`KismetMathLibrary.MakeTransform` (`KismetMathLibrary.MakeVector` _returnvalue_x_2 (`KismetMathLibrary.RandomFloatInRange` 3.0 4.0) (- _returnvalue_z 115.0)) (struct :`Roll` 180.0)) "Undefined" "OverrideRootScale" null null))

(event `self.ReceiveTick`
  (params (DeltaSeconds :type "Float (single-precision)"))
  ;[1 1 1] Default
  (`self.CheckXtoDiagonal`)
  (`self.CheckZtoStraight`)
  (`self.CheckXMax`))

(event `CheckXtoDiagonal`
  (bind _returnvalue_x (`KismetMathLibrary.BreakVector` (`self.K2_GetActorLocation`)))
  ;[1 1 1] Default
  (if (!= (`self.XToDiagonal`) 0.0)
    (if (>= _returnvalue_x (`self.XToDiagonal`))
      (`/Engine/EditorBlueprintResources/StandardMacros.DoOnce` false
        (:`Completed`
          (bind _output_get (set `self.Velocity` (20.0 0.0 20.0)))
          (`ProjectileMovementComponent.SetVelocityInLocalSpace` (`self.ProjectileMovement`) _output_get))))))

(event `PlayerLateralDeath`
  (bind (_returnvalue_x _returnvalue_y _returnvalue_z) (`KismetMathLibrary.BreakVector` (`self.K2_GetActorLocation` (`self.PlayerRef`))))
  (`|SpawnActorFromClass` "/Game/Blueprints/FX/PlayerDeathFalling_FX.PlayerDeathFalling_FX_C" (`KismetMathLibrary.MakeTransform` (`KismetMathLibrary.MakeVector` _returnvalue_x _returnvalue_y _returnvalue_z) (struct :`Roll` 180.0)) "Undefined" "OverrideRootScale" null null))

(event `CheckZtoStraight`
  (bind (_returnvalue_x _returnvalue_y _returnvalue_z) (`KismetMathLibrary.BreakVector` (`self.K2_GetActorLocation`)))
  ;[1 1 1] Default
  (if (!= (`self.ZToStraight`) 0.0)
    (if (>= _returnvalue_z (`self.ZToStraight`))
      (`/Engine/EditorBlueprintResources/StandardMacros.DoOnce` false
        (:`Completed`
          (bind _output_get (set `self.Velocity` (20.0 0.0 0.0)))
          (`ProjectileMovementComponent.SetVelocityInLocalSpace` (`self.ProjectileMovement`) _output_get))))))

(event `CheckXMax`
  (bind _returnvalue_x (`KismetMathLibrary.BreakVector` (`self.K2_GetActorLocation`)))
  (bind _projectilemovement (`self.ProjectileMovement`))
  ;[1 1 1] Default
  (if (!= (`self.XMax`) 0.0)
    (if (>= _returnvalue_x (`self.XMax`))
      (`/Engine/EditorBlueprintResources/StandardMacros.DoOnce` false
        (:`Completed`
          (bind _output_get (set `self.Velocity` (0.0 0.0 0.0)))
          (`ProjectileMovementComponent.SetVelocityInLocalSpace` _projectilemovement _output_get)
          (`MovementComponent.StopMovementImmediately` _projectilemovement)
          (`PrimitiveComponent.SetConstraintMode` (`self.Root`) "YZPlane"))))))

(event `self.DeathFallingCollider.OnComponentBeginOverlap`
  (params (OverlappedComponent :type "PrimitiveComponent Object Reference") (OtherActor :type "Actor Object Reference") (OtherComp :type "PrimitiveComponent Object Reference") (OtherBodyIndex :type Integer) (bFromSweep :type Boolean) (SweepResult :type "HitResult Structure (by ref)"))
  (bind _returnvalue_x (`KismetMathLibrary.BreakVector` (`self.K2_GetActorLocation` OtherActor)))
  (bind (_returnvalue_x_2 _returnvalue_y _returnvalue_z) (`KismetMathLibrary.BreakVector` (`self.K2_GetActorLocation`)))
  ;[0 0 0] Death By Falling
  (if (`self.ActorHasTag` OtherActor "Enemy")
    (bind _outactors (`GameplayStatics.GetAllActorsOfClass` "CamPush_C"))
    (bind _output (`|GetArrayItem` _outactors))
    (bind (_returnvalue_x_3 _returnvalue_y_2 _returnvalue_z_2) (`KismetMathLibrary.BreakVector` (`self.K2_GetActorLocation` _output)))
    (if (`KismetMathLibrary.NearlyEqual_FloatFloat` (`/Game/Blueprints/CamPush.ZToStraight` _output) _returnvalue_z_2 5.0)
      (`GameplayStatics.PlaySound2D` "/Game/Sound/SFXs/sfx_BlopDeath_Cue.sfx_BlopDeath_Cue" (`KismetMathLibrary.RandomFloatInRange` 0.1 0.3) (`KismetMathLibrary.RandomFloatInRange` 0.8 1.2) 0.0 null null)
      (`|SpawnActorFromClass` "/Game/Blueprints/FX/DeathFallingExplosion_FX.DeathFallingExplosion_FX_C" (`KismetMathLibrary.MakeTransform` (`KismetMathLibrary.MakeVector` _returnvalue_x (`KismetMathLibrary.RandomFloatInRange` 3.0 4.0) (- _returnvalue_z 115.0)) (struct :`Roll` 180.0)) "Undefined" "OverrideRootScale" null null)
      (`self.K2_DestroyActor` OtherActor))
    (else
      (bind _asplayer_bp (cast `/Game/Blueprints/Player/Player_BP` OtherActor))
      (if (not (`/Game/Blueprints/Player/Player_BP.isDead` _asplayer_bp))
        (`/Engine/EditorBlueprintResources/StandardMacros.DoOnce` false
          (:`Completed`
            (`/Game/Blueprints/Player/Player_BP.SaveGame` _asplayer_bp)
            (`self.SetActorHiddenInGame` _asplayer_bp true)
            (`self.PlayerFallingDeath`)
            (set `/Game/Blueprints/Player/Player_BP.isDead` true _asplayer_bp)
            (set `/Game/Blueprints/Player/Player_BP.InputDisabled` false _asplayer_bp)
            (set `/Game/Blueprints/Player/Player_BP.HPCurrent` 0.0 _asplayer_bp)
            (`GameplayStatics.PlaySound2D` "/Game/Sound/SFXs/sfx_PlayerDeath_Cue.sfx_PlayerDeath_Cue" 1.0 1.0 0.0 null null)
            (`self.DisableInput` _asplayer_bp (`GameplayStatics.GetPlayerController` 0))
            (`KismetSystemLibrary.Delay` 2.0)
            (`GameplayStatics.OpenLevel` (`self.CurrentLevel`))))))))

(event `self.DeathCollider.OnComponentBeginOverlap`
  (params (OverlappedComponent :type "PrimitiveComponent Object Reference") (OtherActor :type "Actor Object Reference") (OtherComp :type "PrimitiveComponent Object Reference") (OtherBodyIndex :type Integer) (bFromSweep :type Boolean) (SweepResult :type "HitResult Structure (by ref)"))
  ;[0 0 0] Death By Falling
  (bind _asplayer_bp (cast `/Game/Blueprints/Player/Player_BP` OtherActor))
  (if (not (`/Game/Blueprints/Player/Player_BP.isDead` _asplayer_bp))
    (`/Engine/EditorBlueprintResources/StandardMacros.DoOnce` false
      (:`Completed`
        (`/Game/Blueprints/Player/Player_BP.SaveGame` _asplayer_bp)
        (`self.SetActorHiddenInGame` _asplayer_bp true)
        (`self.PlayerLateralDeath`)
        (set `/Game/Blueprints/Player/Player_BP.isDead` true _asplayer_bp)
        (set `/Game/Blueprints/Player/Player_BP.InputDisabled` false _asplayer_bp)
        (set `/Game/Blueprints/Player/Player_BP.HPCurrent` 0.0 _asplayer_bp)
        (`GameplayStatics.PlaySound2D` "/Game/Sound/SFXs/sfx_PlayerDeath_Cue.sfx_PlayerDeath_Cue" 1.0 1.0 0.0 null null)
        (`self.DisableInput` _asplayer_bp (`GameplayStatics.GetPlayerController` 0))
        (`KismetSystemLibrary.Delay` 2.0)
        (`GameplayStatics.OpenLevel` (`self.CurrentLevel`))))))

(fn `UserConstructionScript`)