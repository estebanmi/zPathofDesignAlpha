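; Radio controller that plays world-map call dialogs themed on computer components such as HDD, RAM and Core.
; StartTalk creates the call HUD and picks lines by WorldType, skipping some components already switched on.
; ScrollingText types letters with sound via a delay loop, pausing during menus and between lines, then advances a stage capped by a count of filled dialogs.
; ResetCall clears progress and removes the HUD.
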(event `ScrollingText`
  (params (SetTextTarget :type "MultiLineEditableTextBox Object Reference") (TextString :type "Array of String") (TextSpeed :type "Float (double-precision)"))
  (bind _textarrayindex (`self.TextArrayIndex`))
  (bind _letterindex (`self.LetterIndex`))
  (bind _output (`|GetArrayItem` TextString _textarrayindex))
  (`KismetSystemLibrary.Delay` 0.2)
  (`/Engine/EditorBlueprintResources/StandardMacros.IsValid` (`self.WidgetRefff`) :!label _label
    (:`Is Valid`
      (if (`/Game/Blueprints/WorldMap/WorldMap_Player.IsMenuOn?` (`self.PlayerRef`))
        (`KismetSystemLibrary.Delay` 0.2)
        (goto _label)
        (else
          (bind _output_get (set `self.AppendTextString` (`KismetStringLibrary.Concat_StrStr` (`self.AppendTextString`) (`|GetArrayItem` (`KismetStringLibrary.GetCharacterArrayFromString` _output) _letterindex))))
          (`GameplayStatics.PlaySound2D` "/Game/Sound/SFXs/sfx_ScrollText_Cue.sfx_ScrollText_Cue" 1.0 1.0 0.0 null null)
          (`MultiLineEditableTextBox.SetText` SetTextTarget (`KismetTextLibrary.Conv_StringToText` _output_get))
          (set `self.isTalking` true)
          (`KismetSystemLibrary.Delay` TextSpeed)
          (if (>= _letterindex (- (`KismetStringLibrary.Len` _output) 1))
            (set `self.AppendTextString` "")
            (set `self.LetterIndex` 0)
            (if (< _textarrayindex (- (`KismetArrayLibrary.Array_Length` TextString) 1))
              (set `self.TextArrayIndex` (+ (`self.TextArrayIndex`) 1))
              (set `self.isTalking` false)
              (`KismetSystemLibrary.Delay` 1.5)
              (`/Engine/EditorBlueprintResources/StandardMacros.IsValid` (`self.WidgetRefff`)
                (:`Is Valid`
                  (goto _label)))
              (else
                (set `self.TextArrayIndex` 0)
                (if (< (`self.StageIndex`) (`self.DialogsNumber`))
                  (set `self.StageIndex` (+ (`self.StageIndex`) 1))
                  (set `self.isTalking` false)
                  (set `self.IsWaitingForPlayer` true))))
            (else
              (set `self.LetterIndex` (+ _letterindex 1))
              (goto _label))))))))

(event `self.ReceiveBeginPlay`
  (bind _asworld_map_player (cast `/Game/Blueprints/WorldMap/WorldMap_Player` (`GameplayStatics.GetPlayerPawn` 0)))
  (set `self.PlayerRef` _asworld_map_player))

(event `Reset Call`
  (set `self.TextArrayIndex` 0)
  (set `self.LetterIndex` 0)
  (set `self.StageIndex` 0)
  (set `self.AppendTextString` "")
  (set `self.WidgetRefff` null)
  (bind _foundwidgets (`WidgetBlueprintLibrary.GetAllWidgetsOfClass` "/Game/Widgets/NPCs/WorldMapCall_HUD.WorldMapCall_HUD_C"))
  (bind _output (`|GetArrayItem` _foundwidgets))
  (`/Engine/EditorBlueprintResources/StandardMacros.IsValid` _output
    (:`Is Valid`
      (`Widget.RemoveFromParent` _output))))

(event `StartTalk`
  (params (WorldType :type "/Game/Blueprints/WorldMap/CurrentWorld Enum" :default "NewEnumerator0"))
  (bind _playerref (`self.PlayerRef`))
  (switch `/Game/Blueprints/WorldMap/CurrentWorld` WorldType
    (:`NewEnumerator0`
      (`self.DialogsNumberCalculator` :!label _label_2)
      (bind _returnvalue (`|CreateWidget` "/Game/Widgets/NPCs/WorldMapCall_HUD.WorldMapCall_HUD_C"))
      (`UserWidget.AddToViewport` _returnvalue 0)
      (set `self.WidgetRefff` _returnvalue)
      (`self.ScrollingText` (`/Game/Widgets/NPCs/WorldMapCall_HUD.DialogText` (`self.WidgetRefff`)) (select `/Game/Blueprints/WorldMap/CurrentWorld` WorldType :`NewEnumerator0` (`self.DialogMother`) :`NewEnumerator1` (`self.DialogHDD`) :`NewEnumerator2` (`self.DialogVideo`) :`NewEnumerator3` (`self.DialogSound`) :`NewEnumerator4` (`self.DialogPower`) :`NewEnumerator5` (`self.DialogCooling`) :`NewEnumerator6` (`self.DialogRAM`) :`NewEnumerator7` (`self.DialogCore`)) (`self.TextSpeed`)))
    (:`NewEnumerator1`
      (if (not (`/Game/Blueprints/WorldMap/WorldMap_Player.HDDON` _playerref))
        (goto _label_2)))
    (:`NewEnumerator2`
      (if (not (`/Game/Blueprints/WorldMap/WorldMap_Player.VideoCardON` _playerref))
        (goto _label_2)))
    (:`NewEnumerator3`
      (if (not (`/Game/Blueprints/WorldMap/WorldMap_Player.SoundCardON` _playerref))
        (goto _label_2)))
    (:`NewEnumerator4`
      (if (not (`/Game/Blueprints/WorldMap/WorldMap_Player.PowerSupplyON` _playerref))
        (goto _label_2)))
    (:`NewEnumerator5`
      (if (not (`/Game/Blueprints/WorldMap/WorldMap_Player.CoolingSystemON` _playerref))
        (goto _label_2)))
    (:`NewEnumerator6`
      (goto _label_2))
    (:`NewEnumerator7`
      (goto _label_2))))

(event `DialogsNumberCalculator`
  ;[1 1 1] Dialog Number Calculator
  (if (`KismetStringLibrary.NotEqual_StrStr` (`|GetArrayItem` (`KismetStringLibrary.GetCharacterArrayFromString` (`|GetArrayItem` (`self.DialogMother`)))))
    (set `self.DialogsNumber` (+ (`self.DialogsNumber`) 1))
    (if (`KismetStringLibrary.NotEqual_StrStr` (`|GetArrayItem` (`KismetStringLibrary.GetCharacterArrayFromString` (`|GetArrayItem` (`self.DialogHDD`)))))
      (set `self.DialogsNumber` (+ (`self.DialogsNumber`) 1))
      (if (`KismetStringLibrary.NotEqual_StrStr` (`|GetArrayItem` (`KismetStringLibrary.GetCharacterArrayFromString` (`|GetArrayItem` (`self.DialogVideo`)))))
        (set `self.DialogsNumber` (+ (`self.DialogsNumber`) 1))
        (if (`KismetStringLibrary.NotEqual_StrStr` (`|GetArrayItem` (`KismetStringLibrary.GetCharacterArrayFromString` (`|GetArrayItem` (`self.DialogSound`)))))
          (set `self.DialogsNumber` (+ (`self.DialogsNumber`) 1))
          (if (`KismetStringLibrary.NotEqual_StrStr` (`|GetArrayItem` (`KismetStringLibrary.GetCharacterArrayFromString` (`|GetArrayItem` (`self.DialogPower`)))))
            (set `self.DialogsNumber` (+ (`self.DialogsNumber`) 1))))))))

(fn `UserConstructionScript`)