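; NPC that turns to face the player on a looping timer and talks when the player overlaps its box collider.
; Overlap sets the player's InputDisabled flag, opens Dialog_HUD and runs ScrollingText, a Delay-driven loop typing each string letter by letter with sound.
; Finishing switches StageIndex to the second dialogue array for later visits, then Tick waits for any key to remove the widget and restore input.
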(event `self.ReceiveTick`
  (params (DeltaSeconds :type "Float (single-precision)"))
  (if (`self.WaitingForPlayer`)
    (if (`PlayerController.WasInputKeyJustPressed` (`GameplayStatics.GetPlayerController` 0) "AnyKey")
      (set `self.WaitingForPlayer` false)
      (set `/Game/Blueprints/Player/Player_BP.InputDisabled` false (`self.PlayerRef`))
      (bind _foundwidgets (`WidgetBlueprintLibrary.GetAllWidgetsOfClass` "/Game/Widgets/Dialog_HUD.Dialog_HUD_C"))
      (`Widget.RemoveFromParent` _foundwidgets))))

(event `FacingPlayer`
  (bind _returnvalue_x (`KismetMathLibrary.BreakVector` (`self.K2_GetActorLocation`)))
  (bind _returnvalue_x_2 (`KismetMathLibrary.BreakVector` (`self.K2_GetActorLocation` (`self.PlayerRef`))))
  ;[1 1 1] Facing Player
  (if (< _returnvalue_x_2 _returnvalue_x)
    (`self.K2_SetActorRotation` (struct :`Yaw` 180.0))
    (else
      (`self.K2_SetActorRotation` (struct)))))

(event `self.ReceiveBeginPlay`
  (bind _asplayer_bp (cast `/Game/Blueprints/Player/Player_BP` (`GameplayStatics.GetPlayerCharacter` 0)))
  (set `self.PlayerRef` _asplayer_bp)
  (`KismetSystemLibrary.K2_SetTimerDelegate` (delegate `FacingPlayer`) 1.0 true))

(event `self.BoxCollider.OnComponentBeginOverlap`
  (params (OverlappedComponent :type "PrimitiveComponent Object Reference") (OtherActor :type "Actor Object Reference") (OtherComp :type "PrimitiveComponent Object Reference") (OtherBodyIndex :type Integer) (bFromSweep :type Boolean) (SweepResult :type "HitResult Structure (by ref)"))
  (bind _asplayer_bp (cast `/Game/Blueprints/Player/Player_BP` OtherActor))
  (set `/Game/Blueprints/Player/Player_BP.InputDisabled` true _asplayer_bp)
  (bind _returnvalue (`|CreateWidget` "/Game/Widgets/Dialog_HUD.Dialog_HUD_C"))
  (`UserWidget.AddToViewport` _returnvalue 0)
  (set `self.WidgetRef` _returnvalue)
  (`self.ScrollingText` (`/Game/Widgets/Dialog_HUD.MultiLineEditableTextBox_72` (`self.WidgetRef`)) (select `int` (`self.StageIndex`) :`0` (`self.DialogArray_0`) :`1` (`self.DialogArray_1`)) (`self.TextSpeed`)))

(fn `UserConstructionScript`)