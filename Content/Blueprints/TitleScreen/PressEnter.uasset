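; Title-screen "Press Enter" prompt that appears after a short delay and gates access to the main menu buttons.
; While idle, Tick randomly cycles its flipbook variants through a DoOnce that resets when each animation ends.
; The first Enter press plays a sound, blinks and hides the prompt, reveals DesignPlay-flagged MenuButton_BP actors and enables player selection.
; EnterPress calls made after that forward to the player's current button.
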(event `EnterPress`
  (bind _paperflipbook (`self.PaperFlipbook`))
  (bind _playerref (`self.PlayerRef`))
  (bind _paperflipbook_2 (`self.PaperFlipbook`))
  (bind _paperflipbook_3 (`self.PaperFlipbook`))
  (if (`self.EnterPressed`)
    (`/Game/Blueprints/TitleScreen/MenuButton_BP.ButtonPressed` (`/Game/Blueprints/TitleScreen/PlayerTitleScreen_BP.CurrentButton` (`self.PlayerRef`)))
    (else
      (`GameplayStatics.PlaySound2D` "/Game/Sound/SFXs/sfx_AllPassterisksCollected_Cue.sfx_AllPassterisksCollected_Cue" 1.0 1.0 0.0 null null)
      (set `self.EnterPressed` true)
      (`self.DisableInput` null)
      (`/Engine/EditorBlueprintResources/StandardMacros.FlipFlop` :!label _label
        (:`A`
          (`PaperFlipbookComponent.SetFlipbook` _paperflipbook_3 "/Game/Sprites/HUD/PressEnter/PressEnter0.PressEnter0"))
        (:`B`
          (`PaperFlipbookComponent.SetFlipbook` _paperflipbook_3 "/Game/Sprites/HUD/PressEnter/PressEnter1.PressEnter1")))
      (`KismetSystemLibrary.Delay` 0.3)
      (if (< (`self.Index`) 6)
        (set `self.Index` (+ (`self.Index`) 1))
        (goto _label)
        (else
          (`PaperFlipbookComponent.SetFlipbook` _paperflipbook "/Game/Sprites/HUD/PressEnter/PressEnterG1.PressEnterG1")
          (`KismetSystemLibrary.Delay` (`PaperFlipbookComponent.GetFlipbookLength` _paperflipbook))
          (`SceneComponent.SetVisibility` _paperflipbook_2 false false)
          (`PaperFlipbookComponent.SetFlipbook` _paperflipbook_2 "/Game/Sprites/HUD/PressEnter/PressEnter1.PressEnter1")
          (set `self.Index` 0)
          (bind _outactors (`GameplayStatics.GetAllActorsOfClass` "/Game/Blueprints/TitleScreen/MenuButton_BP.MenuButton_BP_C"))
          (bind _output (`|GetArrayItem` _outactors (`self.Index`)))
          (if (`/Game/Blueprints/TitleScreen/MenuButton_BP.DesignPlay?` _output) :!label _label_2
            (`SceneComponent.SetVisibility` (`/Game/Blueprints/TitleScreen/MenuButton_BP.PaperFlipbook` _output) true false))
          (if (< (`self.Index`) (- (`KismetArrayLibrary.Array_Length` _outactors) 1))
            (set `self.Index` (+ (`self.Index`) 1))
            (goto _label_2)
            (else
              (`/Engine/EditorBlueprintResources/StandardMacros.IsValid` _playerref
                (:`Is Valid`
                  (set `/Game/Blueprints/TitleScreen/PlayerTitleScreen_BP.CanSelect` true _playerref))))))))))

(event `self.ReceiveBeginPlay`
  (bind _paperflipbook (`self.PaperFlipbook`))
  (bind _asplayer_title_screen_bp (cast `/Game/Blueprints/TitleScreen/PlayerTitleScreen_BP` (`GameplayStatics.GetPlayerPawn` 0)))
  (set `self.PlayerRef` _asplayer_title_screen_bp)
  (`SceneComponent.SetVisibility` (`self.PaperFlipbook`) false false)
  (bind _outactors (`GameplayStatics.GetAllActorsOfClass` "/Game/Blueprints/Level/MusicController_BP.MusicController_BP_C"))
  (set `self.BinaryBumperRef` (`|GetArrayItem` _outactors))
  (`KismetSystemLibrary.Delay` 2.0)
  (`SceneComponent.SetVisibility` (`self.PaperFlipbook`) true false)
  (`PaperFlipbookComponent.SetFlipbook` _paperflipbook "/Game/Sprites/HUD/PressEnter/PressEnterG1.PressEnterG1")
  (`KismetSystemLibrary.Delay` (`PaperFlipbookComponent.GetFlipbookLength` _paperflipbook))
  (set `self.EnterPressed` false))

(event `self.ReceiveTick`
  (params (DeltaSeconds :type "Float (single-precision)"))
  (bind _returnvalue (`KismetMathLibrary.RandomFloatInRange` 0.0 100.0))
  (bind _paperflipbook (`self.PaperFlipbook`))
  (if (not (`self.EnterPressed`))
    (`/Engine/EditorBlueprintResources/StandardMacros.DoOnce` false :!label _label_3
      (:`Completed`
        (if (> _returnvalue 10.0)
          (`PaperFlipbookComponent.SetFlipbook` _paperflipbook "/Game/Sprites/HUD/PressEnter/PressEnter1.PressEnter1")
          (`KismetSystemLibrary.Delay` (`PaperFlipbookComponent.GetFlipbookLength` _paperflipbook))
          (goto _label_3 :!via `Reset`)
          (elif (> _returnvalue 30.0)
            (`PaperFlipbookComponent.SetFlipbook` _paperflipbook "/Game/Sprites/HUD/PressEnter/PressEnter0.PressEnter0")
            (`KismetSystemLibrary.Delay` (`PaperFlipbookComponent.GetFlipbookLength` _paperflipbook))
            (goto _label_3 :!via `Reset`)
            (else
              (`/Engine/EditorBlueprintResources/StandardMacros.FlipFlop`
                (:`A`
                  (`PaperFlipbookComponent.SetFlipbook` _paperflipbook "/Game/Sprites/HUD/PressEnter/PressEnterG1.PressEnterG1")
                  (`KismetSystemLibrary.Delay` (`PaperFlipbookComponent.GetFlipbookLength` _paperflipbook))
                  (goto _label_3 :!via `Reset`))
                (:`B`
                  (`PaperFlipbookComponent.SetFlipbook` _paperflipbook "/Game/Sprites/HUD/PressEnter/PressEnterG2.PressEnterG2")
                  (`KismetSystemLibrary.Delay` (`PaperFlipbookComponent.GetFlipbookLength` _paperflipbook))
                  (goto _label_3 :!via `Reset`))))))))))

(fn `UserConstructionScript`)