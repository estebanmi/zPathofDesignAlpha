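; MenuButton_BP is a Paper2D title-screen menu button that handles navigation between Main, Design, Play and Options pages.
; Tick swaps its flipbook between idle, over and pressed sprites from state flags.
; Enter and Back pass focus to linked buttons via PlayerTitleScreen_BP, then show only buttons of that page's type and toggle the PlayerPreview actor.
; Enter on a level button spawns a Binary Bumper HUD transition before opening the level.
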(event `self.ReceiveBeginPlay`
  ;[1 1 1] Default
  (`SceneComponent.SetVisibility` (`self.PaperFlipbook`) false false)
  (bind _asplayer_title_screen_bp (cast `/Game/Blueprints/TitleScreen/PlayerTitleScreen_BP` (`GameplayStatics.GetPlayerPawn` 0)))
  (set `self.PlayerRef` _asplayer_title_screen_bp))

(event `BinaryBumper`
  ;[1 1 1] Binary Bumper
  (bind _returnvalue (`|CreateWidget` "/Game/Widgets/BinaryBumper_HUD.BinaryBumper_HUD_C"))
  (`UserWidget.AddToViewport` _returnvalue 0)
  (bind _outactors (`GameplayStatics.GetAllActorsOfClass` "/Game/Blueprints/Level/BinaryController_BP.BinaryController_BP_C"))
  (`/Game/Blueprints/Level/BinaryController_BP.Adding01` (`|GetArrayItem` _outactors)))

(event `self.ReceiveTick`
  (params (DeltaSeconds :type "Float (single-precision)"))
  ;[1 1 1] Button Sprite Controller
  (if (`self.isButtonPressed`)
    (`PaperFlipbookComponent.SetFlipbook` (`self.PaperFlipbook`) (`self.Selected_Sprite`))
    (elif (`self.isPlayerHere`)
      (`PaperFlipbookComponent.SetFlipbook` (`self.PaperFlipbook`) (`self.Over_Sprite`))
      (else
        (`PaperFlipbookComponent.SetFlipbook` (`self.PaperFlipbook`) (`self.Idle_Sprite`))))))

(event `ButtonVisibilities`
  ;[1 1 1] Button Visibilities
  (if (`self.isPlayerHere`)
    (switch `/Game/Blueprints/TitleScreen/ButtonTypes` (`self.ButtonType`)
      (:`NewEnumerator0`
        (set `self.Index` 0)
        (bind _outactors (`GameplayStatics.GetAllActorsOfClass` "MenuButton_BP_C" :!label _label))
        (bind _output (`|GetArrayItem` _outactors (`self.Index`)))
        (`SceneComponent.SetVisibility` (`/Game/Blueprints/TitleScreen/MenuButton_BP.PaperFlipbook` _output) (`|EnumEquality` (`/Game/Blueprints/TitleScreen/MenuButton_BP.ButtonType` _output) "NewEnumerator0") false)
        (if (< (`self.Index`) (- (`KismetArrayLibrary.Array_Length` _outactors) 1))
          (set `self.Index` (+ (`self.Index`) 1))
          (goto _label)
          (else
            ;[1 1 1] Player Preview Visibilities
            (bind _outactors_2 (`GameplayStatics.GetAllActorsOfClass` "/Game/Blueprints/TitleScreen/PlayerPreview.PlayerPreview_C"))
            (`self.SetActorHiddenInGame` (`|GetArrayItem` _outactors_2) true))))
      (:`NewEnumerator1`
        (set `self.Index` 0)
        (bind _outactors_3 (`GameplayStatics.GetAllActorsOfClass` "MenuButton_BP_C" :!label _label_2))
        (bind _output_2 (`|GetArrayItem` _outactors_3 (`self.Index`)))
        (`SceneComponent.SetVisibility` (`/Game/Blueprints/TitleScreen/MenuButton_BP.PaperFlipbook` _output_2) (`|EnumEquality` (`/Game/Blueprints/TitleScreen/MenuButton_BP.ButtonType` _output_2) "NewEnumerator1") false)
        (if (< (`self.Index`) (- (`KismetArrayLibrary.Array_Length` _outactors_3) 1))
          (set `self.Index` (+ (`self.Index`) 1))
          (goto _label_2)
          (else
            (bind _outactors_4 (`GameplayStatics.GetAllActorsOfClass` "/Game/Blueprints/TitleScreen/PlayerPreview.PlayerPreview_C"))
            (bind _output_3 (`|GetArrayItem` _outactors_4))
            (`self.SetActorHiddenInGame` _output_3 false)
            (`PaperFlipbookComponent.PlayFromStart` (`/Game/Blueprints/TitleScreen/PlayerPreview.PaperFlipbook` _output_3)))))
      (:`NewEnumerator2`
        (set `self.Index` 0)
        (bind _outactors_5 (`GameplayStatics.GetAllActorsOfClass` "MenuButton_BP_C" :!label _label_3))
        (bind _output_4 (`|GetArrayItem` _outactors_5 (`self.Index`)))
        (`SceneComponent.SetVisibility` (`/Game/Blueprints/TitleScreen/MenuButton_BP.PaperFlipbook` _output_4) (`|EnumEquality` (`/Game/Blueprints/TitleScreen/MenuButton_BP.ButtonType` _output_4) "NewEnumerator2") false)
        (if (< (`self.Index`) (- (`KismetArrayLibrary.Array_Length` _outactors_5) 1))
          (set `self.Index` (+ (`self.Index`) 1))
          (goto _label_3)
          (else
            (bind _outactors_6 (`GameplayStatics.GetAllActorsOfClass` "/Game/Blueprints/TitleScreen/PlayerPreview.PlayerPreview_C"))
            (bind _output_5 (`|GetArrayItem` _outactors_6))
            (`self.SetActorHiddenInGame` _output_5 false)
            (`PaperFlipbookComponent.PlayFromStart` (`/Game/Blueprints/TitleScreen/PlayerPreview.PaperFlipbook` _output_5)))))
      (:`NewEnumerator3`
        (set `self.Index` 0)
        (bind _outactors_7 (`GameplayStatics.GetAllActorsOfClass` "MenuButton_BP_C" :!label _label_4))
        (bind _output_6 (`|GetArrayItem` _outactors_7 (`self.Index`)))
        (`SceneComponent.SetVisibility` (`/Game/Blueprints/TitleScreen/MenuButton_BP.PaperFlipbook` _output_6) (`|EnumEquality` (`/Game/Blueprints/TitleScreen/MenuButton_BP.ButtonType` _output_6) "NewEnumerator3") false)
        (if (< (`self.Index`) (- (`KismetArrayLibrary.Array_Length` _outactors_7) 1))
          (set `self.Index` (+ (`self.Index`) 1))
          (goto _label_4)
          (else
            (bind _outactors_8 (`GameplayStatics.GetAllActorsOfClass` "/Game/Blueprints/TitleScreen/PlayerPreview.PlayerPreview_C"))
            (`self.SetActorHiddenInGame` (`|GetArrayItem` _outactors_8) true)))))))

(event `ButtonEnterPressed`
  (bind _pressedbutton_enter (`self.PressedButton_Enter`))
  ;[1 1 1] Button Enter Pressed
  (if (`self.isPlayerHere`)
    (if (!= (`self.LevelToOpen`) "None")
      (`self.BinaryBumper`)
      (`KismetSystemLibrary.Delay` 0.3)
      (`GameplayStatics.OpenLevel` (`self.LevelToOpen`))
      (else
        (set `self.isPlayerHere` false)
        (`/Engine/EditorBlueprintResources/StandardMacros.IsValid` _pressedbutton_enter
          (:`Is Valid`
            (set `/Game/Blueprints/TitleScreen/PlayerTitleScreen_BP.CurrentButton` _pressedbutton_enter (`self.PlayerRef`))
            (set `/Game/Blueprints/TitleScreen/MenuButton_BP.isPlayerHere` true _pressedbutton_enter)
            (`self.ButtonVisibilities` _pressedbutton_enter)))))))

(event `ButtonBackPressed`
  (bind _pressedbutton_back (`self.PressedButton_Back`))
  ;[1 1 1] Button Back Pressed
  (if (`self.isPlayerHere`)
    (set `self.isPlayerHere` false)
    (set `/Game/Blueprints/TitleScreen/PlayerTitleScreen_BP.CurrentButton` _pressedbutton_back (`self.PlayerRef`))
    (set `/Game/Blueprints/TitleScreen/MenuButton_BP.isPlayerHere` true _pressedbutton_back)
    (`self.ButtonVisibilities` _pressedbutton_back)))

(event `PreviewPlayerVisibilities`
  (bind _outactors (`GameplayStatics.GetAllActorsOfClass` "/Game/Blueprints/TitleScreen/PlayerPreview.PlayerPreview_C"))
  (bind _output (`|GetArrayItem` _outactors))
  (`/Engine/EditorBlueprintResources/StandardMacros.IsValid` _output
    (:`Is Valid`
      (set `/Game/Blueprints/TitleScreen/PlayerPreview.PlayerPreview` (`self.PlayerPreview`) _output))
    (:`Is Not Valid`
      (`KismetSystemLibrary.PrintString` "MenuButton_BP: PlayerPreview_BP missing" true true (struct :`R` 1.0 :`A` 1.0)))))

(fn `UserConstructionScript`)