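; Title screen intro Blueprint that briefly locks player input and plays a sound on confirm.
; BeginPlay calls an empty LoadGame event, disables input, then re-enables it after a short delay with a debug print.
; Keyboard and gamepad confirm inputs share a DoOnce, so the sound plays only once.
; Cancel inputs share another DoOnce with the same sound, but it starts closed and is never reset.
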(event `self.ReceiveBeginPlay`
  ;[1 1 1] Default
  (`self.LoadGame`)
  (`self.DisableInput` (`GameplayStatics.GetPlayerController` 0))
  (`KismetSystemLibrary.Delay` 3.0)
  (`self.EnableInput` (`GameplayStatics.GetPlayerController` 0))
  (`KismetSystemLibrary.PrintString` "Input Enabled"))

(event `LoadGame`
  ;[1 1 1] Default
)

(event `InputAction|Enter`
  (params (Key :type "Key Structure"))
  (:`Pressed`
    (`/Engine/EditorBlueprintResources/StandardMacros.DoOnce` false :!label _label
      (:`Completed`
        (`GameplayStatics.PlaySound2D` "/Game/Sound/SFXs/DesignMap/sfx_EnterPOI.sfx_EnterPOI" 1.0 1.0 0.0 null null)))))

(event `Key|Gamepad_Special_Right`
  (params (Key :type "Key Structure"))
  (:`Pressed`
    (goto _label)))

(event `Key|Gamepad_FaceButton_Bottom`
  (params (Key :type "Key Structure"))
  (:`Pressed`
    (goto _label)))

(event `Key|Escape`
  (params (Key :type "Key Structure"))
  (:`Pressed`
    (`/Engine/EditorBlueprintResources/StandardMacros.DoOnce` true :!label _label_2
      (:`Completed`
        (`GameplayStatics.PlaySound2D` "/Game/Sound/SFXs/DesignMap/sfx_EnterPOI.sfx_EnterPOI" 1.0 1.0 0.0 null null)))))

(event `Key|Z`
  (params (Key :type "Key Structure"))
  (:`Pressed`
    (goto _label_2)))

(event `Key|BackSpace`
  (params (Key :type "Key Structure"))
  (:`Pressed`
    (goto _label_2)))

(event `Key|Gamepad_FaceButton_Left`
  (params (Key :type "Key Structure"))
  (:`Pressed`
    (goto _label_2)))

(event `Key|Gamepad_DPad_Up`
  (params (Key :type "Key Structure")))

(event `Key|Gamepad_LeftStick_Up`
  (params (Key :type "Key Structure")))

(event `Key|W`
  (params (Key :type "Key Structure")))

(event `Key|Gamepad_DPad_Down`
  (params (Key :type "Key Structure")))

(event `Key|Gamepad_LeftStick_Down`
  (params (Key :type "Key Structure")))

(event `Key|S`
  (params (Key :type "Key Structure")))

(event `Key|Gamepad_DPad_Left`
  (params (Key :type "Key Structure")))

(event `Key|Gamepad_LeftStick_Left`
  (params (Key :type "Key Structure")))

(event `Key|A`
  (params (Key :type "Key Structure")))

(event `Key|Gamepad_DPad_Right`
  (params (Key :type "Key Structure")))

(event `Key|Gamepad_LeftStick_Right`
  (params (Key :type "Key Structure")))

(event `Key|D`
  (params (Key :type "Key Structure")))

(fn `UserConstructionScript`)