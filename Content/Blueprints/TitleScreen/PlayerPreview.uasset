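; Title screen actor that previews the hero variant for the selected mode.
; On BeginPlay it caches the title screen player pawn.
; Each Tick, while that pawn allows selection, it switches on its PlayerPreview enum and sets the sword, gun or horror flipbook on its Paper2D component.
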(event `self.ReceiveBeginPlay`
  (bind _asplayer_title_screen_bp (cast `/Game/Blueprints/TitleScreen/PlayerTitleScreen_BP` (`GameplayStatics.GetPlayerPawn` 0)))
  (set `self.PlayerRef` _asplayer_title_screen_bp))

(event `self.ReceiveTick`
  (params (DeltaSeconds :type "Float (single-precision)"))
  (if (`/Game/Blueprints/TitleScreen/PlayerTitleScreen_BP.CanSelect` (`self.PlayerRef`))
    (switch `/Game/Blueprints/TitleScreen/PlayerPreviewType` (`self.PlayerPreview`)
      (:`NewEnumerator2`
        (`PaperFlipbookComponent.SetFlipbook` (`self.PaperFlipbook`) "/Game/Sprites/Player/PlayerSword/HeroSwordPreview.HeroSwordPreview"))
      (:`NewEnumerator3`
        (`PaperFlipbookComponent.SetFlipbook` (`self.PaperFlipbook`) "/Game/Sprites/Player/PlayerGun/HeroGunPreview.HeroGunPreview"))
      (:`NewEnumerator4`
        (`PaperFlipbookComponent.SetFlipbook` (`self.PaperFlipbook`) "/Game/Sprites/Player/PlayerUnarmed/HorrorHeroPreview.HorrorHeroPreview")))))

(fn `UserConstructionScript`)