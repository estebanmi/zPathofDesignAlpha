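; Title screen player Blueprint that handles keyboard navigation and selection of menu buttons.
; On BeginPlay it adds the title HUD, blocks input briefly, then highlights the starting button.
; WASD follows each button's directional neighbor links, moving the IsPlayerHere flag with move or blocked sounds.
; Enter triggers the PressEnter actor and, when CanSelect is true, selects the current button; L prints CanSelect for debugging.
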(event `InputAction|Enter`
  (params (Key :type "Key Structure"))
  (:`Pressed`
    (bind _outactors (`GameplayStatics.GetAllActorsOfClass` "/Game/Blueprints/TitleScreen/PressEnter.PressEnter_C"))
    (`/Game/Blueprints/TitleScreen/PressEnter.EnterPress` (`|GetArrayItem` _outactors))))

(event `self.ReceiveBeginPlay`
  (bind _startingbutton (`self.StartingButton`))
  (`self.DisableInput` (`GameplayStatics.GetPlayerController` 0))
  (bind _returnvalue (`|CreateWidget` "/Game/Widgets/TitleScreen_HUD.TitleScreen_HUD_C"))
  (`UserWidget.AddToPlayerScreen` _returnvalue 0)
  (`KismetSystemLibrary.Delay` 3.0)
  (`self.EnableInput` (`GameplayStatics.GetPlayerController` 0))
  (`/Engine/EditorBlueprintResources/StandardMacros.IsValid` _startingbutton
    (:`Is Valid`
      (set `/Game/Blueprints/TitleScreen/MenuButton_BP.isPlayerHere` true _startingbutton)
      (set `self.CurrentButton` _startingbutton))))

(event `Key|W`
  (params (Key :type "Key Structure"))
  (bind _currentbutton (`self.CurrentButton`))
  (bind _upbutton (`/Game/Blueprints/TitleScreen/MenuButton_BP.UpButton` _currentbutton))
  (:`Pressed`
    (if (`self.CanSelect`)
      (`/Engine/EditorBlueprintResources/StandardMacros.IsValid` _upbutton
        (:`Is Valid`
          (set `/Game/Blueprints/TitleScreen/MenuButton_BP.isPlayerHere` false _currentbutton)
          (set `/Game/Blueprints/TitleScreen/MenuButton_BP.isPlayerHere` true _upbutton)
          (set `self.CurrentButton` _upbutton)
          (`GameplayStatics.PlaySound2D` "/Game/Sound/SFXs/DesignMap/sfx_DMMove_Cue.sfx_DMMove_Cue" 1.0 1.0 0.0 null null))
        (:`Is Not Valid`
          (`GameplayStatics.PlaySound2D` "/Game/Sound/SFXs/DesignMap/sfx_DMMoveNot_Cue.sfx_DMMoveNot_Cue" 1.0 1.0 0.0 null null))))))

(event `Key|L`
  (params (Key :type "Key Structure"))
  (:`Pressed`
    (`KismetSystemLibrary.PrintString` (`KismetStringLibrary.Conv_BoolToString` (`self.CanSelect`)))))

(event `Key|S`
  (params (Key :type "Key Structure"))
  (bind _currentbutton (`self.CurrentButton`))
  (bind _downbutton (`/Game/Blueprints/TitleScreen/MenuButton_BP.DownButton` _currentbutton))
  (:`Pressed`
    (if (`self.CanSelect`)
      (`/Engine/EditorBlueprintResources/StandardMacros.IsValid` _downbutton
        (:`Is Valid`
          (set `/Game/Blueprints/TitleScreen/MenuButton_BP.isPlayerHere` false _currentbutton)
          (set `/Game/Blueprints/TitleScreen/MenuButton_BP.isPlayerHere` true _downbutton)
          (set `self.CurrentButton` _downbutton)
          (`GameplayStatics.PlaySound2D` "/Game/Sound/SFXs/DesignMap/sfx_DMMove_Cue.sfx_DMMove_Cue" 1.0 1.0 0.0 null null))
        (:`Is Not Valid`
          (`GameplayStatics.PlaySound2D` "/Game/Sound/SFXs/DesignMap/sfx_DMMoveNot_Cue.sfx_DMMoveNot_Cue" 1.0 1.0 0.0 null null))))))

(event `Key|A`
  (params (Key :type "Key Structure"))
  (bind _currentbutton (`self.CurrentButton`))
  (bind _leftbutton (`/Game/Blueprints/TitleScreen/MenuButton_BP.LeftButton` _currentbutton))
  (:`Pressed`
    (if (`self.CanSelect`)
      (`/Engine/EditorBlueprintResources/StandardMacros.IsValid` _leftbutton
        (:`Is Valid`
          (set `/Game/Blueprints/TitleScreen/MenuButton_BP.isPlayerHere` false _currentbutton)
          (set `/Game/Blueprints/TitleScreen/MenuButton_BP.isPlayerHere` true _leftbutton)
          (set `self.CurrentButton` _leftbutton)
          (`GameplayStatics.PlaySound2D` "/Game/Sound/SFXs/DesignMap/sfx_DMMove_Cue.sfx_DMMove_Cue" 1.0 1.0 0.0 null null))
        (:`Is Not Valid`
          (`GameplayStatics.PlaySound2D` "/Game/Sound/SFXs/DesignMap/sfx_DMMoveNot_Cue.sfx_DMMoveNot_Cue" 1.0 1.0 0.0 null null))))))

(event `Key|D`
  (params (Key :type "Key Structure"))
  (bind _currentbutton (`self.CurrentButton`))
  (bind _rightbutton (`/Game/Blueprints/TitleScreen/MenuButton_BP.RightButton` _currentbutton))
  (:`Pressed`
    (if (`self.CanSelect`)
      (`/Engine/EditorBlueprintResources/StandardMacros.IsValid` _rightbutton
        (:`Is Valid`
          (set `/Game/Blueprints/TitleScreen/MenuButton_BP.isPlayerHere` false _currentbutton)
          (set `/Game/Blueprints/TitleScreen/MenuButton_BP.isPlayerHere` true _rightbutton)
          (set `self.CurrentButton` _rightbutton)
          (`GameplayStatics.PlaySound2D` "/Game/Sound/SFXs/DesignMap/sfx_DMMove_Cue.sfx_DMMove_Cue" 1.0 1.0 0.0 null null))
        (:`Is Not Valid`
          (`GameplayStatics.PlaySound2D` "/Game/Sound/SFXs/DesignMap/sfx_DMMoveNot_Cue.sfx_DMMoveNot_Cue" 1.0 1.0 0.0 null null))))))

(event `InputAction|Enter`
  (params (Key :type "Key Structure"))
  (:`Pressed`
    (if (`self.CanSelect`)
      (`/Game/Blueprints/TitleScreen/MenuButton_BP.ButtonSelected` (`self.CurrentButton`))
      (`GameplayStatics.PlaySound2D` "/Game/Sound/SFXs/DesignMap/sfx_EnterPOI.sfx_EnterPOI" 1.0 1.0 0.0 null null))))

(fn `UserConstructionScript`)