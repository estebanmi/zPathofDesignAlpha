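; Corridor camera actor for a boss encounter with BossBlop, providing camera shake.
; CameraShake fires Shake and Recover together: timelines add offsets to the actor's location while others lerp it back to its BeginPlay position.
; The boss's Furious state selects the timeline pair, defaulting to the furious pair without a valid boss.
; Tick calls CameraX and CameraZ while the player lives, but both are empty, their dead-zone follow logic left disconnected.
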(event `self.ReceiveBeginPlay`
  ;[1 1 1] Default
  (set `self.StartLocation` (`self.K2_GetActorLocation`))
  (bind _outactors (`GameplayStatics.GetAllActorsOfClass` "/Game/Blueprints/Bosses/BossBlop/BossBlop_BP.BossBlop_BP_C"))
  (set `self.BossBlopRef` (`|GetArrayItem` _outactors))
  (bind _asplayer_bp (cast `/Game/Blueprints/Player/Player_BP` (`GameplayStatics.GetPlayerCharacter` 0)))
  (bind _output_get (set `self.PlayerRef` _asplayer_bp))
  (bind (_returnvalue_x _returnvalue_y _returnvalue_z) (`KismetMathLibrary.BreakVector` (`self.K2_GetActorLocation` _output_get)))
  (bind _output_get_2 (set `self.ZMin` _returnvalue_z))
  (bind _output_get_3 (set `self.ZCurrent` _output_get_2)))

(event `Recover`
  (`/Engine/EditorBlueprintResources/StandardMacros.IsValid` (`self.BossBlopRef`)
    (:`Is Valid`
      (if (`/Game/Blueprints/Bosses/BossBlop/BossBlop_BP.Furious` (`self.BossBlopRef`))
        (bind (_direction _newtrack_0) (`Timeline|Alpha` :!via `PlayFromStart` :!label _label)
          (:`Update`
            (`self.K2_SetActorRelativeLocation` (`KismetMathLibrary.VLerp` (`self.K2_GetActorLocation`) (`self.StartLocation`) _newtrack_0))))
        (else
          (bind (_direction_2 _newtrack_0_2) (`Timeline|Timeline_2` :!via `PlayFromStart`)
            (:`Update`
              (`self.K2_SetActorRelativeLocation` (`KismetMathLibrary.VLerp` (`self.K2_GetActorLocation`) (`self.StartLocation`) _newtrack_0_2)))))))
    (:`Is Not Valid`
      (goto _label :!via `PlayFromStart`))))

(event `self.ReceiveTick`
  (params (DeltaSeconds :type "Float (single-precision)"))
  ;[1 1 1] Default
  (`/Engine/EditorBlueprintResources/StandardMacros.IsValid` (`self.PlayerRef`)
    (:`Is Valid`
      (if (not (`/Game/Blueprints/Player/Player_BP.isDead` (`self.PlayerRef`)))
        (`self.CameraX`)
        (if (`self.CanMoveZ?`)
          (`self.CameraZ`))))))

(event `CameraShake`
  (`self.Shake`)
  (`self.Recover`))

(event `Shake`
  (bind _returnvalue (`self.K2_GetActorLocation`))
  (bind _bossblopref (`self.BossBlopRef`))
  (`/Engine/EditorBlueprintResources/StandardMacros.IsValid` _bossblopref
    (:`Is Valid`
      (if (`/Game/Blueprints/Bosses/BossBlop/BossBlop_BP.Furious` _bossblopref)
        (bind (_direction _shakebig _newtrack_0) (`Timeline|Timeline_0` :!via `PlayFromStart` :!label _label_2)
          (:`Update`
            (`self.K2_SetActorRelativeLocation` (+ _newtrack_0 _returnvalue))))
        (else
          (bind (_direction_2 _shakesmall _newtrack_0_2) (`Timeline|Timeline_1` :!via `PlayFromStart`)
            (:`Update`
              (`self.K2_SetActorRelativeLocation` (+ _returnvalue _newtrack_0_2)))))))
    (:`Is Not Valid`
      (goto _label_2 :!via `PlayFromStart`))))

(event `CameraX`
  ;[1 1 1] Camera X moving
)

(event `CameraZ`
  ;[1 1 1] Camera Z moving
)

(fn `UserConstructionScript`)