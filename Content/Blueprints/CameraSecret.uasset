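; Secret-area camera that takes over the player's view inside a hidden zone, registering the secret with a sound on first entry.
; Entering TriggerIN blends to this camera; leaving TriggerOUT loops through CameraFree actors to blend back to the active one.
; Both transitions lock input and briefly auto-walk the player via Tick, using RightEqualIn for direction.
; Unlocking resumes shooting if the fire key or button is still held.
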(event `self.ReceiveBeginPlay`)

(event `self.ReceiveTick`
  (params (DeltaSeconds :type "Float (single-precision)"))
  (bind _playerref (`self.PlayerRef`))
  (if (`self.AutoMovePlayer`)
    (if (`/Game/Blueprints/Player/Player_BP.isFacingRight` _playerref)
      (`Pawn.AddMovementInput` _playerref (1.0 0.0 0.0) 1.0 false)
      (else
        (`Pawn.AddMovementInput` _playerref (-1.0 0.0 0.0) 1.0 false)))))

(event `self.TriggerIN.OnComponentBeginOverlap`
  (params (OverlappedComponent :type "PrimitiveComponent Object Reference") (OtherActor :type "Actor Object Reference") (OtherComp :type "PrimitiveComponent Object Reference") (OtherBodyIndex :type Integer) (bFromSweep :type Boolean) (SweepResult :type "HitResult Structure (by ref)"))
  ;[1 1 1] In / Out
  (bind _asplayer_bp (cast `/Game/Blueprints/Player/Player_BP` OtherActor))
  (set `self.PlayerRef` _asplayer_bp)
  (`PlayerController.SetViewTargetWithBlend` (`GameplayStatics.GetPlayerController` 0) self 1.0 "VTBlend_Linear" 0.0 false)
  (`|ExecutionSequence`
    (:`then_0`
      (`/Engine/EditorBlueprintResources/StandardMacros.DoOnce` false
        (:`Completed`
          (`GameplayStatics.PlaySound2D` "/Game/Sound/SFXs/sfx_LetterCompleted_Cue.sfx_LetterCompleted_Cue" 1.0 1.0 0.0 null null)
          (`/Game/Blueprints/Player/Player_BP.SecretFound` (`self.PlayerRef`)))))
    (:`then_1`
      (`self.LockPlayer`)
      (`self.MovingIN`)
      (`KismetSystemLibrary.Delay` 1.0)
      (`self.FreePlayer`))))

(event `self.TriggerOUT.OnComponentEndOverlap`
  (params (OverlappedComponent :type "PrimitiveComponent Object Reference") (OtherActor :type "Actor Object Reference") (OtherComp :type "PrimitiveComponent Object Reference") (OtherBodyIndex :type Integer))
  ;[1 1 1] In / Out
  (cast `/Game/Blueprints/Player/Player_BP` OtherActor)
  (set `self.Index` 0)
  (bind _outactors (`GameplayStatics.GetAllActorsOfClass` "/Game/Blueprints/CameraFree.CameraFree_C" :!label _label))
  (bind _output (`|GetArrayItem` _outactors (`self.Index`)))
  (if (`/Game/Blueprints/CameraFree.ActiveCam` _output)
    (`PlayerController.SetViewTargetWithBlend` (`GameplayStatics.GetPlayerController` 0) _output 1.0 "VTBlend_Linear" 0.0 false)
    (`self.LockPlayer`)
    (`self.MovingOUT`)
    (`KismetSystemLibrary.Delay` 1.0)
    (`self.FreePlayer`)
    (else
      (set `self.Index` (+ (`self.Index`) 1))
      (goto _label))))

(event `MovingIN`
  (bind _playerref (`self.PlayerRef`))
  ;[1 1 1] Moving Player
  (set `self.AutoMovePlayer` true)
  (if (`self.Right_equal_In?`)
    (set `/Game/Blueprints/Player/Player_BP.isFacingRight` true _playerref)
    (else
      (set `/Game/Blueprints/Player/Player_BP.isFacingRight` false _playerref)))
  (`KismetSystemLibrary.Delay` 0.3 :!label _label_2)
  (set `self.AutoMovePlayer` false))

(event `MovingOUT`
  (bind _playerref (`self.PlayerRef`))
  ;[1 1 1] Moving Player
  (set `self.AutoMovePlayer` true)
  (if (`self.Right_equal_In?`)
    (set `/Game/Blueprints/Player/Player_BP.isFacingRight` false _playerref)
    (goto _label_2)
    (else
      (set `/Game/Blueprints/Player/Player_BP.isFacingRight` true _playerref)
      (goto _label_2))))

(event `LockPlayer`
  (bind _playerref (`self.PlayerRef`))
  ;[1 1 1] Lock Player
  (`self.DisableInput` _playerref (`GameplayStatics.GetPlayerController` 0))
  (set `/Game/Blueprints/Player/Player_BP.InputDisabled` true _playerref)
  (set `/Game/Blueprints/Player/Player_BP.ShootButtonDown` false _playerref))

(event `FreePlayer`
  ;[1 1 1] Free Player
  (`self.EnableInput` (`self.PlayerRef`) (`GameplayStatics.GetPlayerController` 0))
  (set `/Game/Blueprints/Player/Player_BP.InputDisabled` false (`self.PlayerRef`))
  (if (`PlayerController.IsInputKeyDown` (`GameplayStatics.GetPlayerController` 0) "RightControl")
    (`/Game/Blueprints/Player/Player_BP.ContinueShooting` (`self.PlayerRef`) :!label _label_3)
    (elif (`PlayerController.IsInputKeyDown` (`GameplayStatics.GetPlayerController` 0) "Gamepad_FaceButton_Left")
      (goto _label_3))))

(fn `UserConstructionScript`)