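; World map camera actor that makes itself the player's view target on BeginPlay and caches the WorldMap_Player pawn.
; It otherwise does nothing at runtime, as Tick is empty.
; Leftover side-scroller logic for forward-only X follow, a left-edge player blocker and banded Z follow remains in custom events.
; Their dispatch chain is disconnected and reads PlayerRef, not the cached WMPlayerRef.
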(event `self.ReceiveBeginPlay`
  ;[1 1 1] Default
  (bind _asworld_map_player (cast `/Game/Blueprints/WorldMap/WorldMap_Player` (`GameplayStatics.GetPlayerPawn` 0)))
  (set `self.WMPlayerRef` _asworld_map_player)
  (`PlayerController.SetViewTargetWithBlend` (`GameplayStatics.GetPlayerController` 0) self 0.0 "VTBlend_Linear" 0.0 false))

(event `self.ReceiveTick`
  (params (DeltaSeconds :type "Float (single-precision)"))
  ;[1 1 1] Default
)

(event `ReplacingPlayerX`
  (bind _returnvalue_x (`KismetMathLibrary.BreakVector` (`self.K2_GetActorLocation`)))
  (bind (_returnvalue_x_2 _returnvalue_y _returnvalue_z) (`KismetMathLibrary.BreakVector` (`self.K2_GetActorLocation` (`self.PlayerRef`))))
  (bind _returnvalue (- _returnvalue_x 180.0))
  ;[1 1 1] Left Border Blocker
  (if (< _returnvalue_x_2 _returnvalue)
    (`self.K2_SetActorLocation` (`self.PlayerRef`) (`KismetMathLibrary.MakeVector` _returnvalue _returnvalue_y _returnvalue_z) false false)))

(event `CameraX`
  (bind (_returnvalue_x _returnvalue_y _returnvalue_z) (`KismetMathLibrary.BreakVector` (`self.K2_GetActorLocation`)))
  (bind _returnvalue_x_2 (`KismetMathLibrary.BreakVector` (`self.K2_GetActorLocation` (`self.PlayerRef`))))
  (bind _returnvalue_x_3 (`KismetMathLibrary.BreakVector` (`self.K2_GetActorLocation` (`self.PlayerRef`))))
  (bind _returnvalue_x_4 (`KismetMathLibrary.BreakVector` (`self.K2_GetActorLocation` (`self.PlayerRef`))))
  ;[1 1 1] Camera X moving
  (if (< _returnvalue_x_2 (`self.XMax`))
    (if (> _returnvalue_x_4 _returnvalue_x)
      (`self.K2_SetActorLocation` (`KismetMathLibrary.MakeVector` _returnvalue_x_3 _returnvalue_y _returnvalue_z)))))

(event `CameraZ`
  (bind (_returnvalue_x _returnvalue_y _returnvalue_z) (`KismetMathLibrary.BreakVector` (`self.K2_GetActorLocation`)))
  (bind (_returnvalue_x_2 _returnvalue_y_2 _returnvalue_z_2) (`KismetMathLibrary.BreakVector` (`self.K2_GetActorLocation`)))
  (bind (_returnvalue_x_3 _returnvalue_y_3 _returnvalue_z_3) (`KismetMathLibrary.BreakVector` (`self.K2_GetActorLocation` (`self.PlayerRef`))))
  (bind (_returnvalue_x_4 _returnvalue_y_4 _returnvalue_z_4) (`KismetMathLibrary.BreakVector` (`self.K2_GetActorLocation` (`self.PlayerRef`))))
  (bind (_returnvalue_x_5 _returnvalue_y_5 _returnvalue_z_5) (`KismetMathLibrary.BreakVector` (`self.K2_GetActorLocation` (`self.PlayerRef`))))
  (bind (_returnvalue_x_6 _returnvalue_y_6 _returnvalue_z_6) (`KismetMathLibrary.BreakVector` (`self.K2_GetActorLocation` (`self.PlayerRef`))))
  (bind (_returnvalue_x_7 _returnvalue_y_7 _returnvalue_z_7) (`KismetMathLibrary.BreakVector` (`self.K2_GetActorLocation` (`self.PlayerRef`))))
  (bind (_returnvalue_x_8 _returnvalue_y_8 _returnvalue_z_8) (`KismetMathLibrary.BreakVector` (`self.K2_GetActorLocation` (`self.PlayerRef`))))
  ;[1 1 1] Camera Z moving
  (if (> (+ _returnvalue_z_4 36.0) (+ (`self.ZCurrent`) (`self.ZDistanceUpAllowed`)))
    (if (>= (- (+ _returnvalue_z_8 36.0) _returnvalue_z_2) (`self.ZDistanceUpAllowed`))
      (bind _output_get (set `self.ZCurrent` (- (+ _returnvalue_z_7 36.0) (`self.ZDistanceUpAllowed`))))
      (`self.K2_SetActorLocation` (`KismetMathLibrary.MakeVector` (`self.XCurrent`) 0.0 _output_get)))
    (elif (< _returnvalue_z_6 (`self.ZCurrent`))
      (if (< (- (+ _returnvalue_z_3 36.0) _returnvalue_z) (`self.ZDistanceDownAllowed`))
        (set `self.ZCurrent` _returnvalue_z_5)
        (if (< (`self.ZCurrent`) (`self.ZMin`))
          (set `self.ZCurrent` (`self.ZMin`)))
        (`self.K2_SetActorLocation` (`KismetMathLibrary.MakeVector` (`self.XCurrent`) 0.0 (`self.ZCurrent`)))))))

(fn `UserConstructionScript`)