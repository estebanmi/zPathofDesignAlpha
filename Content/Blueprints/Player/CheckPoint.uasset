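; Checkpoint trigger that saves the player's progress when Player_BP overlaps its box collider.
; On overlap it creates a fresh PODSaveGame, stores the player's transform, current level name and gamepad-usage flag, then writes it to Slot1 and prints a confirmation.
; The existing save is never loaded, so each checkpoint overwrites the slot with only those fields set.
; Its Paper sprite is destroyed on BeginPlay.
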(event `self.ReceiveBeginPlay`
  (`ActorComponent.K2_DestroyComponent` (`self.PaperSprite`)))

(event `self.BoxCollider.OnComponentBeginOverlap`
  (params (OverlappedComponent :type "PrimitiveComponent Object Reference") (OtherActor :type "Actor Object Reference") (OtherComp :type "PrimitiveComponent Object Reference") (OtherBodyIndex :type Integer) (bFromSweep :type Boolean) (SweepResult :type "HitResult Structure (by ref)"))
  (bind _asplayer_bp (cast `/Game/Blueprints/Player/Player_BP` OtherActor))
  (set `self.PlayerRef` _asplayer_bp)
  (bind _returnvalue (`GameplayStatics.CreateSaveGameObject` "/Game/Blueprints/SaveGame/PODSaveGame.PODSaveGame_C"))
  (bind _output_get (set `self.SaveGameRef` _returnvalue))
  (set `/Game/Blueprints/SaveGame/PODSaveGame.LastCheckPoint` (`self.GetTransform` _asplayer_bp) _output_get)
  (bind _returnvalue_2 (`GameplayStatics.GetCurrentLevelName` true))
  (set `/Game/Blueprints/SaveGame/PODSaveGame.CurrentLevel` _returnvalue_2 (`self.SaveGameRef`))
  (set `/Game/Blueprints/SaveGame/PODSaveGame.IsUsingGamepad` (`/Game/Blueprints/Player/Player_BP.IsUsingGamepad` (`self.PlayerRef`)) (`self.SaveGameRef`))
  (`GameplayStatics.SaveGameToSlot` (`self.SaveGameRef`) "Slot1")
  (`KismetSystemLibrary.PrintString` "Checkpoint Saved"))

(fn `UserConstructionScript`)