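; Player projectile for a 2D Paper2D character that flies horizontally in the player's movement direction and damages what it hits.
; On spawn it reads IsMovingRight to set velocity and flipbook rotation, then self-destructs after a short lifetime.
; A looping timer spawns one of two random trail actors behind it, with slight random Y depth.
; Sphere hits on anything but the player apply damage, spawn an explosion and destroy the bullet.
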(event `self.ReceiveBeginPlay`
  (bind _paperflipbook (`self.PaperFlipbook`))
  (bind _asplayer_bp (cast `/Game/Blueprints/Player/Player_BP` (`GameplayStatics.GetPlayerCharacter` 0)))
  (set `self.PlayerRef` _asplayer_bp)
  (`KismetSystemLibrary.K2_SetTimerDelegate` (delegate `BulletTrail`) 0.05 true)
  (if (`/Game/Blueprints/Player/Player_BP.isMovingRight` (`self.PlayerRef`))
    (set `MovementComponent.Velocity` (300.0 0.0 0.0) (`self.ProjectileMovement`))
    (`SceneComponent.K2_SetWorldRotation` :`self` _paperflipbook)
    (else
      (set `MovementComponent.Velocity` (-300.0 0.0 0.0) (`self.ProjectileMovement`))
      (`SceneComponent.K2_SetWorldRotation` _paperflipbook (struct :`Yaw` 180.0) false false)))
  (`KismetSystemLibrary.Delay` 2.0)
  (`self.K2_DestroyActor`))

(event `BulletTrail`
  (bind _returnvalue (`KismetMathLibrary.RandomFloatInRange` 0.0 1.0))
  (bind (_returnvalue_x _returnvalue_y _returnvalue_z) (`KismetMathLibrary.BreakVector` (`self.K2_GetActorLocation`)))
  (`KismetSystemLibrary.Delay` 0.0)
  (if (== (`KismetMathLibrary.RandomIntegerInRange` 0 1) 0)
    (`|SpawnActorFromClass` "/Game/Blueprints/Player/ActionPlayer/PlayerBulletTrail0.PlayerBulletTrail0_C" (`KismetMathLibrary.MakeTransform` (`KismetMathLibrary.MakeVector` _returnvalue_x _returnvalue _returnvalue_z)) "Undefined" "OverrideRootScale" null null)
    (else
      (`|SpawnActorFromClass` "/Game/Blueprints/Player/ActionPlayer/PlayerBulletTrail1.PlayerBulletTrail1_C" (`KismetMathLibrary.MakeTransform` (`KismetMathLibrary.MakeVector` _returnvalue_x _returnvalue _returnvalue_z)) "Undefined" "OverrideRootScale" null null))))

(event `self.Sphere.OnComponentHit`
  (params (HitComponent :type "PrimitiveComponent Object Reference") (OtherActor :type "Actor Object Reference") (OtherComp :type "PrimitiveComponent Object Reference") (NormalImpulse :type "Vector Structure") (Hit :type "HitResult Structure (by ref)"))
  (if (!= OtherActor "/Game/Blueprints/Player/Player_BP.Player_BP")
    (`GameplayStatics.ApplyDamage` OtherActor (`self.Damage`))
    (`|SpawnActorFromClass` "/Game/Blueprints/Player/ActionPlayer/PlayerBulletExplosion_BP.PlayerBulletExplosion_BP_C" (`KismetMathLibrary.MakeTransform` (`self.K2_GetActorLocation`)) "Undefined" "OverrideRootScale" null null)
    (`self.K2_DestroyActor`)))

(event `self.Sphere.OnComponentBeginOverlap`
  (params (OverlappedComponent :type "PrimitiveComponent Object Reference") (OtherActor :type "Actor Object Reference") (OtherComp :type "PrimitiveComponent Object Reference") (OtherBodyIndex :type Integer) (bFromSweep :type Boolean) (SweepResult :type "HitResult Structure (by ref)")))

(fn `UserConstructionScript`)