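; PlayerShotFlame_BP is a short-lived shot flame effect for the player, drawn with a Paper2D flipbook.
; On BeginPlay it casts the player pawn to Player_BP and rotates the flipbook to match the facing direction from IsMovingRight.
; It destroys itself after a delay equal to the flipbook's length.
; Logic to follow the upper body's GunAttackSocket exists but is unconnected, so it never runs.
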(event `self.ReceiveBeginPlay`
  (bind _paperflipbook (`self.PaperFlipbook`))
  (bind _asplayer_bp (cast `/Game/Blueprints/Player/Player_BP` (`GameplayStatics.GetPlayerCharacter` 0)))
  (set `self.PlayerRef` _asplayer_bp)
  (if (`/Game/Blueprints/Player/Player_BP.isMovingRight` (`self.PlayerRef`))
    (`SceneComponent.K2_SetWorldRotation` :`self` _paperflipbook)
    (else
      (`SceneComponent.K2_SetWorldRotation` _paperflipbook (struct :`Yaw` 180.0) false false)))
  (`KismetSystemLibrary.Delay` (`PaperFlipbookComponent.GetFlipbookLength` (`self.PaperFlipbook`)))
  (`self.K2_DestroyActor`))

(event `self.ReceiveTick`
  (params (DeltaSeconds :type "Float (single-precision)")))

(fn `UserConstructionScript`)