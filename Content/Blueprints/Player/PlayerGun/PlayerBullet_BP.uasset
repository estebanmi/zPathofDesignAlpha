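; PlayerBullet_BP is the player gun's projectile, a Paper2D flipbook bullet that damages actors it overlaps.
; On BeginPlay it casts the player character to PlayerGun_BP and uses its facing to set horizontal velocity and flipbook rotation, then destroys itself after a short delay.
; The sphere's overlap applies damage to any actor except the player, crediting the player as causer, without destroying the bullet.
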(event `self.ReceiveBeginPlay`
  (bind _paperflipbook (`self.PaperFlipbook`))
  (bind _asplayer_gun_bp (cast `/Game/Blueprints/Player/PlayerGun/PlayerGun_BP` (`GameplayStatics.GetPlayerCharacter` 0)))
  (set `self.PlayerGunRef` _asplayer_gun_bp)
  (if (`/Game/Blueprints/Player/PlayerGun/PlayerGun_BP.isMovingRight` (`self.PlayerGunRef`))
    (set `MovementComponent.Velocity` (300.0 0.0 0.0) (`self.ProjectileMovement`))
    (`SceneComponent.K2_SetWorldRotation` :`self` _paperflipbook)
    (else
      (set `MovementComponent.Velocity` (-300.0 0.0 0.0) (`self.ProjectileMovement`))
      (`SceneComponent.K2_SetWorldRotation` _paperflipbook (struct :`Yaw` 180.0) false false)))
  (`KismetSystemLibrary.Delay` 2.0)
  (`self.K2_DestroyActor`))

(event `self.Sphere.OnComponentBeginOverlap`
  (params (OverlappedComponent :type "PrimitiveComponent Object Reference") (OtherActor :type "Actor Object Reference") (OtherComp :type "PrimitiveComponent Object Reference") (OtherBodyIndex :type Integer) (bFromSweep :type Boolean) (SweepResult :type "HitResult Structure (by ref)"))
  (bind _playergunref (`self.PlayerGunRef`))
  (if (!= OtherActor _playergunref)
    (`GameplayStatics.ApplyDamage` OtherActor (`self.Damage`) null _playergunref)))

(fn `UserConstructionScript`)