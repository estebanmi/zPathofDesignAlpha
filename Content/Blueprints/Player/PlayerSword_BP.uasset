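; Paper2D side-scrolling player character with sword attack, jumping, damage and death, which also creates the HUD.
; Tick derives a PlayerStates value from flags to set flipbooks and facing, firing Slash to spawn the attack at a sprite socket.
; DoOnce-gated damage applies knockback, stun and blinking invulnerability.
; It loads the save on BeginPlay, saves when entering open ArmoredDoors, and has hotkeys for a double-jump test and binary-puzzle controllers.
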(event `Key|LeftMouseButton`
  (params (Key :type "Key Structure"))
  ;[1 1 1] Attack (Sword)
  (:`Pressed`
    (if (`self.InputDisabled`)
      _
      (elif (`self.isDead`)
        _
        (elif (`self.isPlayerHit`)
          _
          (elif (not (`self.isAttacking`))
            (set `self.isAttacking` true)))))))

(event `Slash`
  ;[1 1 1] Attack (Sword)
  (set `self.InputDisabled` true)
  (`/Engine/EditorBlueprintResources/StandardMacros.DoOnce` false :!label _label
    (:`Completed`
      (`GameplayStatics.PlaySound2D` "/Game/Sound/SFXs/sfx_Sword_Cue.sfx_Sword_Cue" 1.0 1.0 0.0 null null)
      (`|SpawnActorFromClass` "/Game/Blueprints/Player/Slash_BP.Slash_BP_C" (`KismetMathLibrary.MakeTransform` (`SceneComponent.GetSocketLocation` (`self.Sprite`) "SwordAttackSocket")) "Undefined" "OverrideRootScale" null null)
      (`KismetSystemLibrary.Delay` 0.4)
      (set `self.isAttacking` false)
      (if (not (`self.isDead`))
        (if (not (`self.isTalking`))
          (set `self.InputDisabled` false))
        (`self.ControlAnimation`)
        (goto _label :!via `Reset`)))))

(event `OnLandedSafety`
  ;[1 1 1] Attack (Sword)
  (goto _label :!via `Reset`))

(event `self.ReceiveBeginPlay`
  ;[1 1 1] Default
  (`ActorComponent.SetIsReplicated` (`self.Sprite`) true)
  (bind _returnvalue (`|CreateWidget` "/Game/Widgets/Player_HUD.Player_HUD_C"))
  (`UserWidget.AddToPlayerScreen` _returnvalue 0)
  (`self.LoadGame`))

(event `ControlAnimation`
  (bind _returnvalue_x (`KismetMathLibrary.BreakVector` (`self.GetVelocity`)))
  ;[1 1 1] Control Animations
  (if (`self.isDead`)
    (set `self.PlayerStates` "NewEnumerator5")
    (elif (`self.isPlayerHit`)
      (set `self.PlayerStates` "NewEnumerator1")
      (elif (`self.isAttacking`)
        (if (`self.isOnAir`)
          (set `self.PlayerStates` "NewEnumerator6")
          (else
            (set `self.PlayerStates` "NewEnumerator2")))
        (`self.Slash`)
        (elif (`NavMovementComponent.IsFalling` (`self.CharacterMovement`))
          (set `self.PlayerStates` "NewEnumerator3" :!label _label_2)
          (elif (`self.isOnAir`)
            (goto _label_2)
            (elif (!= _returnvalue_x 0.0)
              (set `self.PlayerStates` "NewEnumerator4")
              (else
                (set `self.PlayerStates` "NewEnumerator0")))))))))

(event `self.ReceiveTick`
  (params (DeltaSeconds :type "Float (single-precision)"))
  ;[1 1 1] Default
  (`self.ControlAnimation`)
  (`self.UpdateAnimations`)
  (`self.TurnControl`))

(event `InputAxis|MoveRight`
  (params (AxisValue :type "Float (single-precision)"))
  ;[1 1 1] Handle movement
  (if (`self.isDead`)
    _
    (elif (not (`self.InputDisabled`))
      (if (> AxisValue 0.0)
        (set `self.isMovingRight` true)
        (elif (< AxisValue 0.0)
          (set `self.isMovingRight` false)))
      (`self.AddMovementInput` (1.0 0.0 0.0) AxisValue))))

(event `TurnControl`
  ;[1 1 1] Turn Control
  (if (`self.isPlayerHit`)
    _
    (elif (`self.isMovingRight`)
      (`Controller.SetControlRotation` (`self.GetController`) (`KismetMathLibrary.MakeRotator` 0.0))
      (else
        (`Controller.SetControlRotation` (`self.GetController`) (`KismetMathLibrary.MakeRotator` 0.0 0.0 180.0))))))

(event `Key|H`
  (params (Key :type "Key Structure"))
  (:`Pressed`
    (`self.BinaryBumper`)))

(event `BinaryBumper`
  ;[1 1 1] Binary Bumper
  (bind _returnvalue (`|CreateWidget` "/Game/Widgets/BinaryBumper_HUD.BinaryBumper_HUD_C"))
  (`UserWidget.AddToViewport` _returnvalue 0)
  (bind _outactors (`GameplayStatics.GetAllActorsOfClass` "/Game/Blueprints/Level/BinaryBumperController_BP.BinaryBumperController_BP_C"))
  (`/Game/Blueprints/Level/BinaryBumperController_BP.Adding01` (`|GetArrayItem` _outactors))
  (`KismetSystemLibrary.Delay` 0.3))

(event `UpdateAnimations`
  (bind _sprite (`self.Sprite`))
  ;[1 1 1] Update Animations
  (switch `/Game/Blueprints/Player/PlayerSwordStates` (`self.PlayerStates`)
    (:`NewEnumerator0`
      (`PaperFlipbookComponent.SetFlipbook` _sprite "/Game/Sprites/Player/PlayerSword/Idle/HeroTestIdle.HeroTestIdle"))
    (:`NewEnumerator1`
      (`PaperFlipbookComponent.SetFlipbook` _sprite "/Game/Sprites/Player/PlayerSword/Hit/HeroHit_Flipbook.HeroHit_Flipbook"))
    (:`NewEnumerator7`
      (`PaperFlipbookComponent.SetFlipbook` _sprite "/Game/Sprites/Player/PlayerSword/Slash/HeroPreSlash1.HeroPreSlash1"))
    (:`NewEnumerator2`
      (`PaperFlipbookComponent.SetFlipbook` _sprite "/Game/Sprites/Player/PlayerSword/Sword/HeroSwordNew1.HeroSwordNew1"))
    (:`NewEnumerator8`
      (`PaperFlipbookComponent.SetFlipbook` _sprite "/Game/Sprites/Player/PlayerSword/Slash/HeroPreSlashOnAir.HeroPreSlashOnAir"))
    (:`NewEnumerator6`
      (`PaperFlipbookComponent.SetFlipbook` _sprite "/Game/Sprites/Player/PlayerSword/Slash/HeroSlashOnAir1.HeroSlashOnAir1"))
    (:`NewEnumerator3`
      (`PaperFlipbookComponent.SetFlipbook` _sprite "/Game/Sprites/Player/PlayerSword/Jump/HeroTestJump_Flipbook.HeroTestJump_Flipbook"))
    (:`NewEnumerator4`
      (`PaperFlipbookComponent.SetFlipbook` _sprite "/Game/Sprites/Player/PlayerSword/Walk/HeroTestWalk1.HeroTestWalk1"))
    (:`NewEnumerator5`
      (`PaperFlipbookComponent.SetFlipbook` _sprite "/Game/Sprites/Player/PlayerSword/Death/HeroDeath_1.HeroDeath_1")
      (`/Engine/EditorBlueprintResources/StandardMacros.DoOnce` false
        (:`Completed`
          (`KismetSystemLibrary.Delay` 1.0)
          (`PaperFlipbookComponent.Stop` (`self.Sprite`)))))))

(event `InputAction|Jump`
  (params (Key :type "Key Structure"))
  ;[1 1 1] Handle Jump
  (:`Pressed`
    (if (`self.isDead`)
      _
      (elif (not (`self.InputDisabled`))
        (`self.Jump`)
        (if (not (`self.isOnAir`))
          (`GameplayStatics.PlaySound2D` "/Game/Sound/SFXs/sfx_PlayerJump_Cue.sfx_PlayerJump_Cue" 1.0 1.0 0.0 null null)
          (set `self.isOnAir` true)))))
  (:`Released`
    (`self.StopJumping`)))

(event `Key|J`
  (params (Key :type "Key Structure"))
  ;[1 1 1] DobleJump Test
  (:`Pressed`
    (`/Engine/EditorBlueprintResources/StandardMacros.Do N` 2 :!label _label_3
      (:`Exit`
        (if true
          (`PaperFlipbookComponent.SetFlipbook` (`self.Sprite`) "/Game/Sprites/Player/PlayerSword/Hit/HeroHit_Flipbook.HeroHit_Flipbook")
          (`self.DobleJumpAnim`))
        (`self.LaunchCharacter` (0.0 0.0 400.0))
        (set `self.isOnAir` true)))))

(event `ResetJumps`
  ;[1 1 1] DobleJump Test
  (goto _label_3 :!via `Reset`))

(event `DobleJumpAnim`
  ;[1 1 1] DobleJump Test
  (`KismetSystemLibrary.Delay` 0.1)
  (`PaperFlipbookComponent.SetFlipbook` (`self.Sprite`) "/Game/Sprites/Player/PlayerSword/Jump/HeroTestJump_Flipbook.HeroTestJump_Flipbook"))

(event `self.OnLanded`
  (params (Hit :type "HitResult Structure (by ref)"))
  ;[1 1 1] On Landed (Trigger Invul)
  (`self.ResetJumps`)
  (set `self.isOnAir` false)
  (set `self.isAttacking` false)
  (`GameplayStatics.PlaySound2D` "/Game/Sound/SFXs/sfx_PlayerLanding_Cue.sfx_PlayerLanding_Cue" 1.0 1.0 0.0 null null)
  (if (`self.isPlayerHit`)
    (if (> (`self.HP`) 0.0)
      (set `self.isPlayerHit` false)
      (set `self.isInvulnerable` true)
      (`self.Invulnerable`)
      (if (not (`self.isDead`))
        (set `self.InputDisabled` false)
        (`KismetSystemLibrary.Delay` 2.0)
        (set `self.isInvulnerable` false))
      (else
        (set `self.isDead` true)))
    (elif (not (`self.isTalking`))
      (set `self.InputDisabled` false)
      (`self.OnLandedSafety`))))

(event `Key|L`
  (params (Key :type "Key Structure"))
  (:`Pressed`
    (bind _outactors (`GameplayStatics.GetAllActorsOfClass` "/Game/Blueprints/Player/BinaryWordsController_BP.BinaryWordsController_BP_C"))
    (bind _output (`|GetArrayItem` _outactors))
    (`/Engine/EditorBlueprintResources/StandardMacros.IsValid` _output
      (:`Is Valid`
        (`/Game/Blueprints/Player/BinaryWordsController_BP.GetBinaryCoin` _output false)))))

(event `InvulnerableOver`
  (bind (_hitimpulse_x _hitimpulse_y _hitimpulse_z) (`KismetMathLibrary.BreakVector` (`self.HitImpulse`)))
  ;[1 1 1] Player Hit
  (goto _label_4 :!via `Reset`))

(event `self.ReceiveAnyDamage`
  (params (Damage :type "Float (single-precision)") (DamageType :type "DamageType Object Reference") (InstigatedBy :type "Controller Object Reference") (DamageCauser :type "Actor Object Reference"))
  (bind (_hitimpulse_x _hitimpulse_y _hitimpulse_z) (`KismetMathLibrary.BreakVector` (`self.HitImpulse`)))
  (bind _returnvalue_x (`KismetMathLibrary.BreakVector` (`KismetMathLibrary.GetDirectionUnitVector` (`self.K2_GetActorLocation`) (`self.K2_GetActorLocation` DamageCauser))))
  ;[1 1 1] Player Hit
  (`/Engine/EditorBlueprintResources/StandardMacros.DoOnce` false :!label _label_4
    (:`Completed`
      (set `self.HP` (- (`self.HP`) Damage))
      (`PrimitiveComponent.SetCollisionResponseToChannel` (`self.CapsuleComponent`) "ECC_WorldDynamic" "ECR_Ignore")
      (set `self.InputDisabled` true)
      (`GameplayStatics.PlaySound2D` "/Game/Sound/SFXs/sfx_PlayerHit_Cue.sfx_PlayerHit_Cue" 1.0 1.0 0.0 null null)
      (`MovementComponent.StopMovementImmediately` (`self.CharacterMovement`))
      (set `self.isPlayerHit` true)
      (if (> _returnvalue_x 0.0)
        (`CharacterMovementComponent.AddForce` (`self.CharacterMovement`) (`KismetMathLibrary.MakeVector` (* _hitimpulse_x -1.0) _hitimpulse_y _hitimpulse_z))
        (set `self.isMovingRight` true)
        (else
          (`CharacterMovementComponent.AddForce` (`self.CharacterMovement`) (`self.HitImpulse`))
          (set `self.isMovingRight` false)))
      (`KismetSystemLibrary.Delay` (`self.MaxStunDuration`))
      (if (`self.isDead`)
        (`PrimitiveComponent.SetCollisionEnabled` (`self.CapsuleComponent`) "NoCollision")
        (`GameplayStatics.PlaySound2D` "/Game/Sound/SFXs/sfx_PlayerDeath_Cue.sfx_PlayerDeath_Cue" 1.0 1.0 0.0 null null)
        (set `self.InputDisabled` true)
        (else
          (set `self.isPlayerHit` false)
          (set `self.isInvulnerable` true)
          (`self.Invulnerable`)
          (if (not (`self.isDead`))
            (set `self.InputDisabled` false)))))))

(event `InputAction|UpAction`
  (params (Key :type "Key Structure"))
  ;[1 1 1] Enter Door
  (:`Pressed`
    (if (`self.InputDisabled`)
      _
      (elif (`self.isDead`)
        _
        (elif (not (`self.isOnAir`))
          (`self.EnterDoor`))))))

(event `Invulnerable`
  ;[1 1 1] Invulnerable
  (`/Engine/EditorBlueprintResources/StandardMacros.FlipFlop` :!label _label_5
    (:`A`
      (`SceneComponent.SetVisibility` (`self.Sprite`) false false))
    (:`B`
      (`SceneComponent.SetVisibility` (`self.Sprite`) true false)))
  (`KismetSystemLibrary.Delay` 0.1)
  (if (`self.isInvulnerable`)
    (goto _label_5)
    (else
      (`SceneComponent.SetVisibility` (`self.Sprite`) true false)
      (`PrimitiveComponent.SetCollisionResponseToChannel` (`self.CapsuleComponent`) "ECC_WorldDynamic" "ECR_Block")
      (`self.InvulnerableOver`))))

(event `EnterDoor`
  ;[1 1 1] Enter Door
  (bind _outactors (`GameplayStatics.GetAllActorsOfClass` "/Game/Blueprints/Level/ArmoredDoor_BP.ArmoredDoor_BP_C"))
  (bind _output (`|GetArrayItem` _outactors))
  (if (`/Game/Blueprints/Level/ArmoredDoor_BP.inRange` _output)
    (if (`/Game/Blueprints/Level/ArmoredDoor_BP.isOpen` _output)
      (`self.SaveGame`)
      (`self.BinaryBumper`)
      (`KismetSystemLibrary.Delay` 0.3)
      (`GameplayStatics.OpenLevel` (`/Game/Blueprints/Level/ArmoredDoor_BP.NextLevel` _output)))))

(event `SaveGame`
  ;[1 1 1] SaveGame
  (bind _returnvalue (`GameplayStatics.CreateSaveGameObject` "/Game/Blueprints/MySaveGame.MySaveGame_C"))
  (set `self.MySaveGameRef` _returnvalue)
  (`|ExecutionSequence`
    (:`then_0`
      (set `/Game/Blueprints/MySaveGame.LevelUpSaved` (`/Game/Blueprints/Level/ArmoredDoor_BP.LevelUp` (`|GetArrayItem` (stale `EnterDoor` _outactors))) (`self.MySaveGameRef`)))
    (:`then_2`
      (`GameplayStatics.SaveGameToSlot` (`self.MySaveGameRef`) "GameSlotSaved")
      (`KismetSystemLibrary.PrintString` (`KismetStringLibrary.Concat_StrStr` "Game Saved (CurrentPOI: " (`KismetSystemLibrary.GetDisplayName` (`/Game/Blueprints/MySaveGame.CurrentPOISaved` (`self.MySaveGameRef`))) ")") true true (struct :`G` 0.66 :`B` 1.0 :`A` 1.0) 6.0))))

(event `LoadGame`
  ;[1 1 1] Load Game
  (bind _returnvalue (`GameplayStatics.DoesSaveGameExist` "GameSlotSaved"))
  (if _returnvalue
    (bind _returnvalue_2 (`GameplayStatics.LoadGameFromSlot` "GameSlotSaved"))
    (bind _asmy_save_game (cast `/Game/Blueprints/MySaveGame` _returnvalue_2))
    (bind _output_get (set `self.MySaveGameRef` _asmy_save_game))
    (`KismetSystemLibrary.PrintString` (`KismetStringLibrary.Concat_StrStr` "Game Loaded (CurrentPOI: " (`KismetSystemLibrary.GetDisplayName` (`/Game/Blueprints/MySaveGame.CurrentPOISaved` _output_get)) ")") true true (struct :`G` 0.66 :`B` 1.0 :`A` 1.0) 6.0)))

(fn `UserConstructionScript`)