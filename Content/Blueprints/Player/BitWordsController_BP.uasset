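; Player-side controller for a binary spelling puzzle where collected 1/0 coins spell a target word bit by bit.
; Each coin is checked against the current letter's code from BinaryWordsTable, advancing the displayed bit string on a match and playing right/wrong sounds based on the player's SoundCardON.
; Eight correct bits complete a letter, refreshing the PlayerRAMWord widget and underscore-masked word.
; Completing the word sets the player's RAM flag.
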(event `self.ReceiveTick`
  (params (DeltaSeconds :type "Float (single-precision)")))

(event `self.ReceiveBeginPlay`
  (bind _asplayer_bp (cast `/Game/Blueprints/Player/Player_BP` (`GameplayStatics.GetPlayerCharacter` 0)))
  (set `self.PlayerRef` _asplayer_bp)
  (`self.WordSet`))

(event `WordSet`
  (`self.WordTransform`)
  (set `self.WordLastIndex` (- (`KismetStringLibrary.Len` (`self.WordEspaced`)) 1))
  (set `self.CurrentWord` (`KismetStringLibrary.Concat_StrStr` (`self.CurrentWord`) "_ ") :!label _label)
  (if (> (`self.WordLastIndex`) (`self.WordIndex`))
    (set `self.WordIndex` (+ (`self.WordIndex`) 2))
    (goto _label)))

(event `LetterCompleted`
  ;[1 1 1] Letter Completed
  (bind _foundwidgets (`WidgetBlueprintLibrary.GetAllWidgetsOfClass` "/Game/Widgets/PlayerHUD/PlayerRAMWord.PlayerRAMWord_C"))
  (bind _output (`|GetArrayItem` _foundwidgets))
  (`/Engine/EditorBlueprintResources/StandardMacros.IsValid` _output
    (:`Is Valid`
      (`Widget.RemoveFromParent` _output))
    (:`Is Not Valid`
      _))
  (bind _returnvalue (`|CreateWidget` "/Game/Widgets/PlayerHUD/PlayerRAMWord.PlayerRAMWord_C" (`GameplayStatics.GetPlayerController` 0)))
  (`UserWidget.AddToViewport` _returnvalue 0)
  (`GameplayStatics.PlaySound2D` "/Game/Sound/SFXs/sfx_LetterCompleted_Cue.sfx_LetterCompleted_Cue" 1.0 1.0 0.0 null null)
  (if (>= (`self.WordCompletedIndex`) (`KismetStringLibrary.Len` (`self.WordEspaced`)))
    (`KismetSystemLibrary.PrintString` "ALL LETTERS DONE")
    (else
      (bind _output_get (set `self.WordCompletedIndex` (+ (`self.WordCompletedIndex`) 2)))
      (set `self.WordRestIndex` _output_get)
      (bind _output_get_2 (set `self.CurrentWord` (`KismetStringLibrary.Mid` (`self.WordEspaced`) 0 (`self.WordCompletedIndex`))))
      (if (< (`self.WordRestIndex`) (`self.WordLastIndex`)) :!label _label_2
        (set `self.CurrentWord` (`KismetStringLibrary.Concat_StrStr` _output_get_2 "_ "))
        (set `self.WordRestIndex` (+ (`self.WordRestIndex`) 2))
        (goto _label_2)
        (else
          (set `self.WordRestIndex` _output_get)
          (if (>= (`self.WordCompletedIndex`) (`KismetStringLibrary.Len` (`self.WordEspaced`)))
            (set `/Game/Blueprints/Player/Player_BP.RAM?` true (`self.PlayerRef`))
            (`KismetSystemLibrary.PrintString` "WORD COMPLETED")))))))

(event `WordTransform`
  (set `self.WordTransLastIndex` (`KismetStringLibrary.Len` (`self.Word`)))
  (if (< (`self.WordTransIndex`) (`self.WordTransLastIndex`)) :!label _label_3
    (set `self.WordEspaced` (`KismetStringLibrary.Concat_StrStr` (`self.WordEspaced`) (`KismetStringLibrary.Mid` (`self.Word`) (`self.WordTransIndex`) 1) " "))
    (set `self.WordTransIndex` (+ (`self.WordTransIndex`) 1))
    (goto _label_3)))

(event `RightCoin`
  (`KismetSystemLibrary.PrintString` "Right Coin")
  (set `self.BitCodeIndex` (+ (`self.BitCodeIndex`) 1))
  (set `self.BitCode` (`KismetStringLibrary.Concat_StrStr` (`KismetStringLibrary.Mid` (`.Code_38_E7ED30EA46310EC9C2953C9D2FFEA782` (break `/Game/Blueprints/Player/BinaryWordsStruct` (stale `GetBinaryCoin` _returnvalue))) 0 (+ (`self.BitCodeIndex`) 0)) "--------"))
  (if (== (`self.BitCodeIndex`) 8)
    (`self.LetterCompleted`)
    (set `self.BitCodeIndex` 0)
    (set `self.GetCoinLetterIndex` (+ (`self.GetCoinLetterIndex`) 1))
    (set `self.BitCode` "--------")))

(event `GetBinaryCoin`
  (params (CoinBool :type Boolean))
  (bind _soundcardon (`/Game/Blueprints/Player/Player_BP.SoundCardON` (`self.PlayerRef`)))
  (bind _returnvalue (`|GetDataTableRow` "/Game/Blueprints/Player/BinaryWordsTable.BinaryWordsTable" (`KismetStringLibrary.Conv_StringToName` (`KismetStringLibrary.Mid` (`self.Word`) (`self.GetCoinLetterIndex`) 1)))
    (:`then`
      (if (`KismetStringLibrary.EqualEqual_StrStr` (`KismetStringLibrary.Mid` (`.Code_38_E7ED30EA46310EC9C2953C9D2FFEA782` (break `/Game/Blueprints/Player/BinaryWordsStruct` _returnvalue)) (`self.BitCodeIndex`) 1) "1")
        (if CoinBool
          (`self.RightCoin` :!label _label_4)
          (if _soundcardon
            (`GameplayStatics.PlaySound2D` "/Game/Sound/SFXs/sfx_coin_Right_Cue.sfx_coin_Right_Cue" 1.0 1.0 0.0 null null)
            (else
              (`GameplayStatics.PlaySound2D` "/Game/Sound/SFXs/sfx_coin_Wrong_Cue.sfx_coin_Wrong_Cue" 1.0 1.0 0.0 null null :!label _label_5)))
          (else
            (`self.WrongCoin` :!label _label_6)
            (if _soundcardon
              (goto _label_5)
              (else
                (goto _label_5)))))
        (elif CoinBool
          (goto _label_6)
          (else
            (goto _label_4)))))
    (:`RowNotFound`
      (`KismetSystemLibrary.PrintString` "Invalid Character" true true (struct :`R` 1.0 :`B` 0.025802 :`A` 1.0) 5.0))))

(event `WrongCoin`
  (`KismetSystemLibrary.PrintString` "Wrong Coin"))

(fn `UserConstructionScript`)