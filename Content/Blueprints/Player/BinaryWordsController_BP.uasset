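; Controller for a binary spelling mechanic in which collected true/false coins spell a target word bit by bit.
; On BeginPlay it builds an underscore placeholder from the word, stepping two indices per letter.
; GetBinaryCoin checks each coin against the current letter's code in BinaryWordsTable; correct coins advance the displayed code, wrong ones only print.
; Every eighth correct bit reveals a letter and rebuilds the masked word.
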(event `self.ReceiveTick`
  (params (DeltaSeconds :type "Float (single-precision)")))

(event `self.ReceiveBeginPlay`
  (`self.WordSet`))

(event `WordSet`
  (`self.WordTransform`)
  (set `self.WordLastIndex` (- (`KismetStringLibrary.Len` (`self.WordEspaced`)) 1))
  (set `self.CurrentWord` (`KismetStringLibrary.Concat_StrStr` (`self.CurrentWord`) "_ ") :!label _label)
  (if (> (`self.WordLastIndex`) (`self.WordIndex`))
    (set `self.WordIndex` (+ (`self.WordIndex`) 2))
    (goto _label)))

(event `WordTransform`
  (set `self.WordTransLastIndex` (`KismetStringLibrary.Len` (`self.Word`)))
  (if (< (`self.WordTransIndex`) (`self.WordTransLastIndex`)) :!label _label_2
    (set `self.WordEspaced` (`KismetStringLibrary.Concat_StrStr` (`self.WordEspaced`) (`KismetStringLibrary.Mid` (`self.Word`) (`self.WordTransIndex`) 1) " "))
    (set `self.WordTransIndex` (+ (`self.WordTransIndex`) 1))
    (goto _label_2)))

(event `RightCoin`
  (`KismetSystemLibrary.PrintString` "Right Coin")
  (set `self.BinaryCodeIndex` (+ (`self.BinaryCodeIndex`) 1))
  (set `self.BinaryCode` (`KismetStringLibrary.Concat_StrStr` (`KismetStringLibrary.Mid` (`.Code_38_E7ED30EA46310EC9C2953C9D2FFEA782` (break `/Game/Blueprints/Player/BinaryWordsStruct` (stale `GetBinaryCoin` _returnvalue))) 0 (+ (`self.BinaryCodeIndex`) 0)) "--------"))
  (if (== (`self.BinaryCodeIndex`) 8)
    (`self.LetterCompleted`)
    (set `self.BinaryCodeIndex` 0)
    (set `self.GetCoinLetterIndex` (+ (`self.GetCoinLetterIndex`) 1))
    (set `self.BinaryCode` "--------")))

(event `GetBinaryCoin`
  (params (CoinBool :type Boolean))
  (bind _returnvalue (`|GetDataTableRow` "/Game/Blueprints/Player/BinaryWordsTable.BinaryWordsTable" (`KismetStringLibrary.Conv_StringToName` (`KismetStringLibrary.Mid` (`self.Word`) (`self.GetCoinLetterIndex`) 1)))
    (:`then`
      (if (`KismetStringLibrary.EqualEqual_StrStr` (`KismetStringLibrary.Mid` (`.Code_38_E7ED30EA46310EC9C2953C9D2FFEA782` (break `/Game/Blueprints/Player/BinaryWordsStruct` _returnvalue)) (`self.BinaryCodeIndex`) 1) "1")
        (if CoinBool
          (`self.RightCoin` :!label _label_3)
          (else
            (`self.WrongCoin` :!label _label_4)))
        (elif CoinBool
          (goto _label_4)
          (else
            (goto _label_3)))))
    (:`RowNotFound`
      (`KismetSystemLibrary.PrintString` "Invalid Character" true true (struct :`R` 1.0 :`B` 0.025802 :`A` 1.0) 5.0))))

(event `WrongCoin`
  (`KismetSystemLibrary.PrintString` "Wrong Coin"))

(event `LetterCompleted`
  (if (>= (`self.WordCompletedIndex`) (`KismetStringLibrary.Len` (`self.WordEspaced`)))
    (`KismetSystemLibrary.PrintString` "ALL LETTERS DONE")
    (else
      (bind _output_get (set `self.WordCompletedIndex` (+ (`self.WordCompletedIndex`) 2)))
      (set `self.WordRestIndex` _output_get)
      (bind _output_get_2 (set `self.CurrentWord` (`KismetStringLibrary.Mid` (`self.WordEspaced`) 0 (`self.WordCompletedIndex`))))
      (if (< (`self.WordRestIndex`) (`self.WordLastIndex`)) :!label _label_5
        (set `self.CurrentWord` (`KismetStringLibrary.Concat_StrStr` _output_get_2 "_ "))
        (set `self.WordRestIndex` (+ (`self.WordRestIndex`) 2))
        (goto _label_5)
        (else
          (set `self.WordRestIndex` _output_get)
          (if (>= (`self.WordCompletedIndex`) (`KismetStringLibrary.Len` (`self.WordEspaced`)))
            (`KismetSystemLibrary.PrintString` "WORD COMPLETED")))))))

(fn `UserConstructionScript`)