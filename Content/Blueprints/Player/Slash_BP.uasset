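; Short-lived sword slash hitbox actor that deals damage during the player's attack.
; On BeginPlay it caches the Player_BP reference and destroys itself after a brief delay.
; Each tick it snaps to the SwordAttackSocket on the player's sprite, so the hitbox follows the sword.
; Its Sphere overlap applies damage to any actor other than the player, with the player as damage causer.
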(event `self.ReceiveBeginPlay`
  (bind _asplayer_bp (cast `/Game/Blueprints/Player/Player_BP` (`GameplayStatics.GetPlayerCharacter` 0)))
  (set `self.PlayerRef` _asplayer_bp)
  (`KismetSystemLibrary.Delay` 0.1)
  (`self.K2_DestroyActor`))

(event `self.ReceiveTick`
  (params (DeltaSeconds :type "Float (single-precision)"))
  (bind _playerref (`self.PlayerRef`))
  (`/Engine/EditorBlueprintResources/StandardMacros.IsValid` _playerref
    (:`Is Valid`
      (`self.K2_SetActorLocation` (`SceneComponent.GetSocketLocation` (`PaperCharacter.Sprite` _playerref) "SwordAttackSocket")))))

(event `self.Sphere.OnComponentBeginOverlap`
  (params (OverlappedComponent :type "PrimitiveComponent Object Reference") (OtherActor :type "Actor Object Reference") (OtherComp :type "PrimitiveComponent Object Reference") (OtherBodyIndex :type Integer) (bFromSweep :type Boolean) (SweepResult :type "HitResult Structure (by ref)"))
  (bind _playerref (`self.PlayerRef`))
  (if (!= OtherActor _playerref)
    (`GameplayStatics.ApplyDamage` OtherActor (`self.Damage`) null _playerref)))

(fn `UserConstructionScript`)