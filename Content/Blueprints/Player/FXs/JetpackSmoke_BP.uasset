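; JetpackSmoke_BP is a short-lived Paper2D flipbook effect for the player's jetpack smoke.
; On BeginPlay it randomly chooses between a zero and a 180-degree rotation for visual variety and nudges itself by a tiny random amount along Y.
; It then waits until just before the flipbook ends and destroys itself, with no Tick logic.
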(event `self.ReceiveBeginPlay`
  (bind (_returnvalue_x _returnvalue_y _returnvalue_z) (`KismetMathLibrary.BreakVector` (`self.K2_GetActorLocation`)))
  (`self.K2_SetActorRotation` (select `bool` (`KismetMathLibrary.RandomBool`) :`true` (struct :`Yaw` 180.0) :!type "Rotator Structure"))
  (`self.K2_SetActorLocation` (`KismetMathLibrary.MakeVector` _returnvalue_x (+ _returnvalue_y (`KismetMathLibrary.RandomFloatInRange` 0.0 0.1)) _returnvalue_z))
  (`KismetSystemLibrary.Delay` (- (`PaperFlipbookComponent.GetFlipbookLength` (`self.PaperFlipbook`)) 0.1))
  (`self.K2_DestroyActor`))

(fn `UserConstructionScript`)