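; Paper2D player character playable as a sword-slashing Adventure Hero or a gun-firing Action Hero, selected by PlayerType.
; Tick drives turning and per-type state-to-flipbook animation; the Action Hero layers a socket-following upper body over the legs and changes walk speed while shooting.
; Damage applies knockback, stun, then blinking invulnerability or death, with DoOnce gates limiting attacks and hits.
; Entering an open ArmoredDoor saves level progress and loads the next level.
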(event `Slash`
  ;[1 1 1] Attack (Sword)
  (set `self.InputDisabled` true)
  (`/Engine/EditorBlueprintResources/StandardMacros.DoOnce` false :!label _label
    (:`Completed`
      (`GameplayStatics.PlaySound2D` "/Game/Sound/SFXs/sfx_Sword_Cue.sfx_Sword_Cue" 1.0 1.0 0.0 null null)
      (`|SpawnActorFromClass` "/Game/Blueprints/Player/AdventurePlayer/PlayerSlash_BP.PlayerSlash_BP_C" (`KismetMathLibrary.MakeTransform` (`SceneComponent.GetSocketLocation` (`self.Sprite`) "SwordAttackSocket")) "Undefined" "OverrideRootScale" null null)
      (`KismetSystemLibrary.Delay` 0.4)
      (set `self.isAttacking` false)
      (if (not (`self.isDead`))
        (if (not (`self.isTalking`))
          (set `self.InputDisabled` false))
        (`self.AdventureControlAnimation`)
        (goto _label :!via `Reset`)))))

(event `OnLandedSafety`
  ;[1 1 1] Attack (Sword)
  (goto _label :!via `Reset`))

(event `ControlAnimationLegs`
  (bind _returnvalue_x (`KismetMathLibrary.BreakVector` (`self.GetVelocity`)))
  ;[1 1 1] Control Animations
  (if (`self.isDead`)
    (set `self.ActionPlayerStates` "NewEnumerator5")
    (elif (`self.isPlayerHit`)
      (set `self.ActionPlayerStates` "NewEnumerator1")
      (elif (`NavMovementComponent.IsFalling` (`self.CharacterMovement`))
        (set `self.ActionPlayerStates` "NewEnumerator3" :!label _label_2)
        (elif (`self.isOnAir`)
          (goto _label_2)
          (elif (!= _returnvalue_x 0.0)
            (set `self.ActionPlayerStates` "NewEnumerator4")
            (else
              (set `self.ActionPlayerStates` "NewEnumerator0"))))))))

(event `AttackingTimeCounter`
  ;[1 1 1] Attacking Time Counter
  (if (`self.isAttacking`)
    (set `self.AttackingTimePassed` (+ (`self.AttackingTimePassed`) (`GameplayStatics.GetWorldDeltaSeconds`)))
    (if (>= (`self.AttackingTimePassed`) 0.5)
      (set `self.isAttacking` false)
      (set `self.AttackingTimePassed` 0.0 :!label _label_3)
      (set `CharacterMovementComponent.MaxWalkSpeed` (`self.NonShoothingSpeed`) (`self.CharacterMovement`)))))

(event `ActionControlAnimationsBody`
  ;[1 1 1] Control Animations
  ;;[1 1 1] Control Animations Body
  (if (`self.isDead`)
    (`SceneComponent.SetVisibility` (`self.HeroUpperBody`) false false :!label _label_4)
    (elif (`self.isPlayerHit`)
      (goto _label_4)
      (else
        (`SceneComponent.SetVisibility` (`self.HeroUpperBody`) true false)
        (if (`self.isAttacking`)
          (`PaperFlipbookComponent.SetFlipbook` (`self.HeroUpperBody`) "/Game/Sprites/Player/PlayerGun/Body/HeroGunBody_Shoot.HeroGunBody_Shoot")
          (else
            (`PaperFlipbookComponent.SetFlipbook` (`self.HeroUpperBody`) "/Game/Sprites/Player/PlayerGun/Body/HeroGunBody_Idle_Flipbook.HeroGunBody_Idle_Flipbook")))))))

(event `ResetSpeedOnLanding`
  ;[1 1 1] Attacking Time Counter
  (goto _label_3))

(event `Key|LeftMouseButton`
  (params (Key :type "Key Structure"))
  (:`Pressed`
    (switch `/Game/Blueprints/Player/PlayerTypes` (`self.PlayerType`)
      (:`NewEnumerator0`
        ;[1 1 1] Attack (Sword)
        (if (`self.InputDisabled`)
          _
          (elif (`self.isDead`)
            _
            (elif (`self.isPlayerHit`)
              _
              (elif (not (`self.isAttacking`))
                (set `self.isAttacking` true))))))
      (:`NewEnumerator1`
        ;[1 1 1] Attack (Gun)
        (if (`self.InputDisabled`)
          _
          (elif (`self.isDead`)
            _
            (elif (not (`self.isPlayerHit`))
              (set `self.isAttacking` true)
              (`self.GunFire`)
              (set `self.AttackingTimePassed` 0.0)
              (set `CharacterMovementComponent.MaxWalkSpeed` (`self.ShoothingSpeed`) (`self.CharacterMovement`)))))))))

(event `GunFire`
  (bind _returnvalue (`SceneComponent.GetSocketLocation` (`self.HeroUpperBody`) "GunAttackSocket"))
  ;[1 1 1] Attack (Gun)
  (`/Engine/EditorBlueprintResources/StandardMacros.DoOnce` false :!label _label_5
    (:`Completed`
      (`PaperFlipbookComponent.PlayFromStart` (`self.HeroUpperBody`))
      (`GameplayStatics.PlaySound2D` "/Game/Sound/SFXs/sfx_Sword_Cue.sfx_Sword_Cue" 1.0 1.0 0.0 null null)
      (`|SpawnActorFromClass` "/Game/Blueprints/Player/ActionPlayer/PlayerBullet_BP.PlayerBullet_BP_C" (`KismetMathLibrary.MakeTransform` _returnvalue) "Undefined" "OverrideRootScale" null null)
      (`|SpawnActorFromClass` "/Game/Blueprints/Player/ActionPlayer/PlayerShotFlame_BP.PlayerShotFlame_BP_C" (`KismetMathLibrary.MakeTransform` _returnvalue) "Undefined" "OverrideRootScale" null null)
      (`KismetSystemLibrary.Delay` 0.1)
      (if (not (`self.isDead`))
        (if (not (`self.isTalking`))
          (set `self.InputDisabled` false))
        (`self.ActionControlAnimationsBody`)
        (goto _label_5 :!via `Reset`)))))

(event `self.ReceiveBeginPlay`
  ;[1 1 1] Default
  (`ActorComponent.SetIsReplicated` (`self.Sprite`) true)
  (bind _returnvalue (`|CreateWidget` "/Game/Widgets/Player_HUD.Player_HUD_C"))
  (`UserWidget.AddToPlayerScreen` _returnvalue 0)
  (if (`|EnumInequality` (`self.PlayerType`) "NewEnumerator1")
    (`ActorComponent.K2_DestroyComponent` (`self.HeroUpperBody`))))

(event `self.ReceiveTick`
  (params (DeltaSeconds :type "Float (single-precision)"))
  ;[1 1 1] Default
  (`self.TurnControl`)
  (switch `/Game/Blueprints/Player/PlayerTypes` (`self.PlayerType`)
    (:`NewEnumerator0`
      (`self.AdventureControlAnimation`)
      (`self.AdventureUpdateAnimations`))
    (:`NewEnumerator1`
      (`self.ControlAnimationLegs`)
      (`self.ActionUpdateAnimations`)
      (`self.ActionBodyFollowsLegs`)
      (`self.ActionControlAnimationsBody`)
      (`self.AttackingTimeCounter`))))

(event `AdventureControlAnimation`
  (bind _returnvalue_x (`KismetMathLibrary.BreakVector` (`self.GetVelocity`)))
  ;[1 1 1] Control Animations
  (if (`self.isDead`)
    (set `self.AdventurePlayerStates` "NewEnumerator5")
    (elif (`self.isPlayerHit`)
      (set `self.AdventurePlayerStates` "NewEnumerator1")
      (elif (`self.isAttacking`)
        (if (`self.isOnAir`)
          (set `self.AdventurePlayerStates` "NewEnumerator6")
          (else
            (set `self.AdventurePlayerStates` "NewEnumerator2")))
        (`self.Slash`)
        (elif (`NavMovementComponent.IsFalling` (`self.CharacterMovement`))
          (set `self.AdventurePlayerStates` "NewEnumerator3" :!label _label_6)
          (elif (`self.isOnAir`)
            (goto _label_6)
            (elif (!= _returnvalue_x 0.0)
              (set `self.AdventurePlayerStates` "NewEnumerator4")
              (else
                (set `self.AdventurePlayerStates` "NewEnumerator0")))))))))

(event `ActionBodyFollowsLegs`
  (bind (_returnvalue_x _returnvalue_y _returnvalue_z) (`KismetMathLibrary.BreakVector` (`SceneComponent.GetSocketLocation` (`self.Sprite`) "SocketBody")))
  ;[1 1 1] Action Body Follows Legs
  (if (`self.isMovingRight`)
    (`SceneComponent.K2_SetWorldLocation` (`self.HeroUpperBody`) (`SceneComponent.GetSocketLocation` (`self.Sprite`) "SocketBody") false false)
    (else
      (`SceneComponent.K2_SetWorldLocation` (`self.HeroUpperBody`) (`KismetMathLibrary.MakeVector` _returnvalue_x (+ _returnvalue_y 2.0) _returnvalue_z) false false))))

(event `InputAxis|MoveRight`
  (params (AxisValue :type "Float (single-precision)"))
  ;[1 1 1] Handle movement
  (if (`self.isDead`)
    _
    (elif (not (`self.InputDisabled`))
      (if (> AxisValue 0.0)
        (set `self.isMovingRight` true)
        (elif (< AxisValue 0.0)
          (set `self.isMovingRight` false)))
      (`self.AddMovementInput` (1.0 0.0 0.0) AxisValue))))

(event `TurnControl`
  ;[1 1 1] Turn Control
  (if (`self.isPlayerHit`)
    _
    (elif (`self.isMovingRight`)
      (`Controller.SetControlRotation` (`self.GetController`) (`KismetMathLibrary.MakeRotator` 0.0))
      (else
        (`Controller.SetControlRotation` (`self.GetController`) (`KismetMathLibrary.MakeRotator` 0.0 0.0 180.0))))))

(event `Key|H`
  (params (Key :type "Key Structure"))
  (:`Pressed`
    (`self.BinaryBumper`)))

(event `BinaryBumper`
  ;[1 1 1] Binary Bumper
  (bind _returnvalue (`|CreateWidget` "/Game/Widgets/BinaryBumper_HUD.BinaryBumper_HUD_C"))
  (`UserWidget.AddToViewport` _returnvalue 0)
  (bind _outactors (`GameplayStatics.GetAllActorsOfClass` "/Game/Blueprints/Level/BinaryBumperController_BP.BinaryBumperController_BP_C"))
  (`/Game/Blueprints/Level/BinaryBumperController_BP.Adding01` (`|GetArrayItem` _outactors))
  (`KismetSystemLibrary.Delay` 0.3))

(event `ActionUpdateAnimations`
  (bind _sprite (`self.Sprite`))
  ;[1 1 1] Action Update Animations
  (switch `/Game/Blueprints/Player/ActionPlayer/ActionPlayerStates` (`self.ActionPlayerStates`)
    (:`NewEnumerator0`
      (`PaperFlipbookComponent.SetFlipbook` _sprite "/Game/Sprites/Player/PlayerGun/Legs/HeroSwordLegsIdlet1.HeroSwordLegsIdlet1"))
    (:`NewEnumerator1`
      (`PaperFlipbookComponent.SetFlipbook` _sprite "/Game/Sprites/Player/PlayerGun/Hit/HeroGunHit1.HeroGunHit1"))
    (:`NewEnumerator2`
      (`PaperFlipbookComponent.SetFlipbook` _sprite "/Game/Sprites/Player/PlayerGun/Fire/HeroGunFireStand1.HeroGunFireStand1"))
    (:`NewEnumerator6`
      (`PaperFlipbookComponent.SetFlipbook` _sprite "/Game/Sprites/Player/PlayerSword/Slash/HeroSlashOnAir1.HeroSlashOnAir1"))
    (:`NewEnumerator3`
      (`PaperFlipbookComponent.SetFlipbook` _sprite "/Game/Sprites/Player/PlayerGun/Legs/HeroGunLegsJump1.HeroGunLegsJump1"))
    (:`NewEnumerator4`
      (`PaperFlipbookComponent.SetFlipbook` _sprite "/Game/Sprites/Player/PlayerGun/Legs/HeroGunLegsWalk.HeroGunLegsWalk"))
    (:`NewEnumerator5`
      (`PaperFlipbookComponent.SetFlipbook` _sprite "/Game/Sprites/Player/PlayerGun/Death/HeroGunDeath1.HeroGunDeath1")
      (`/Engine/EditorBlueprintResources/StandardMacros.DoOnce` false
        (:`Completed`
          (`KismetSystemLibrary.Delay` 1.0)
          (`PaperFlipbookComponent.Stop` (`self.Sprite`)))))))

(event `AdventureUpdateAnimations`
  (bind _sprite (`self.Sprite`))
  ;[1 1 1] Adventure Update Animations
  (switch `/Game/Blueprints/Player/AdventurePlayer/PlayerSwordStates` (`self.AdventurePlayerStates`)
    (:`NewEnumerator0`
      (`PaperFlipbookComponent.SetFlipbook` _sprite "/Game/Sprites/Player/PlayerSword/Idle/HeroTestIdle.HeroTestIdle"))
    (:`NewEnumerator1`
      (`PaperFlipbookComponent.SetFlipbook` _sprite "/Game/Sprites/Player/PlayerSword/Hit/HeroHit_Flipbook.HeroHit_Flipbook"))
    (:`NewEnumerator7`
      (`PaperFlipbookComponent.SetFlipbook` _sprite "/Game/Sprites/Player/PlayerSword/Slash/HeroPreSlash1.HeroPreSlash1"))
    (:`NewEnumerator2`
      (`PaperFlipbookComponent.SetFlipbook` _sprite "/Game/Sprites/Player/PlayerSword/Sword/HeroSwordNew1.HeroSwordNew1"))
    (:`NewEnumerator8`
      (`PaperFlipbookComponent.SetFlipbook` _sprite "/Game/Sprites/Player/PlayerSword/Slash/HeroPreSlashOnAir.HeroPreSlashOnAir"))
    (:`NewEnumerator6`
      (`PaperFlipbookComponent.SetFlipbook` _sprite "/Game/Sprites/Player/PlayerSword/Slash/HeroSlashOnAir1.HeroSlashOnAir1"))
    (:`NewEnumerator3`
      (`PaperFlipbookComponent.SetFlipbook` _sprite "/Game/Sprites/Player/PlayerSword/Jump/HeroTestJump_Flipbook.HeroTestJump_Flipbook"))
    (:`NewEnumerator4`
      (`PaperFlipbookComponent.SetFlipbook` _sprite "/Game/Sprites/Player/PlayerSword/Walk/HeroTestWalk1.HeroTestWalk1"))
    (:`NewEnumerator5`
      (`PaperFlipbookComponent.SetFlipbook` _sprite "/Game/Sprites/Player/PlayerSword/Death/HeroDeath_1.HeroDeath_1")
      (`/Engine/EditorBlueprintResources/StandardMacros.DoOnce` false
        (:`Completed`
          (`KismetSystemLibrary.Delay` 1.0)
          (`PaperFlipbookComponent.Stop` (`self.Sprite`)))))))

(event `InputAction|Jump`
  (params (Key :type "Key Structure"))
  ;[1 1 1] Handle Jump
  (:`Pressed`
    (if (`self.isDead`) :!label _label_7
      _
      (elif (not (`self.InputDisabled`))
        (`self.Jump`)
        (if (not (`self.isOnAir`))
          (`GameplayStatics.PlaySound2D` "/Game/Sound/SFXs/sfx_PlayerJump_Cue.sfx_PlayerJump_Cue" 1.0 1.0 0.0 null null)
          (set `self.isOnAir` true)))))
  (:`Released`
    (`self.StopJumping`)))

(event `JumpEvent`
  ;[1 1 1] Handle Jump
  (goto _label_7))

(event `self.OnLanded`
  (params (Hit :type "HitResult Structure (by ref)"))
  ;[1 1 1] On Landed (Trigger Invul)
  (set `self.isOnAir` false)
  (set `self.isAttacking` false)
  (`GameplayStatics.PlaySound2D` "/Game/Sound/SFXs/sfx_PlayerLanding_Cue.sfx_PlayerLanding_Cue" 1.0 1.0 0.0 null null)
  (if (`self.isPlayerHit`)
    (if (> (`self.HP`) 0.0)
      (set `self.isPlayerHit` false)
      (set `self.isInvulnerable` true)
      (`self.Invulnerable`)
      (if (not (`self.isDead`))
        (set `self.InputDisabled` false)
        (`KismetSystemLibrary.Delay` 2.0)
        (set `self.isInvulnerable` false))
      (else
        (set `self.isDead` true)))
    (elif (not (`self.isTalking`))
      (set `self.InputDisabled` false)
      (`self.OnLandedSafety`)
      (`self.ResetSpeedOnLanding`))))

(event `Key|L`
  (params (Key :type "Key Structure"))
  (:`Pressed`
    (bind _outactors (`GameplayStatics.GetAllActorsOfClass` "/Game/Blueprints/Player/BinaryWordsController_BP.BinaryWordsController_BP_C"))
    (bind _output (`|GetArrayItem` _outactors))
    (`/Engine/EditorBlueprintResources/StandardMacros.IsValid` _output
      (:`Is Valid`
        (`/Game/Blueprints/Player/BinaryWordsController_BP.GetBinaryCoin` _output false)))))

(event `InvulnerableOver`
  (bind (_hitimpulse_x _hitimpulse_y _hitimpulse_z) (`KismetMathLibrary.BreakVector` (`self.HitImpulse`)))
  ;[1 1 1] Player Hit
  (goto _label_8 :!via `Reset`))

(event `self.ReceiveAnyDamage`
  (params (Damage :type "Float (single-precision)") (DamageType :type "DamageType Object Reference") (InstigatedBy :type "Controller Object Reference") (DamageCauser :type "Actor Object Reference"))
  (bind (_hitimpulse_x _hitimpulse_y _hitimpulse_z) (`KismetMathLibrary.BreakVector` (`self.HitImpulse`)))
  (bind _returnvalue_x (`KismetMathLibrary.BreakVector` (`KismetMathLibrary.GetDirectionUnitVector` (`self.K2_GetActorLocation`) (`self.K2_GetActorLocation` DamageCauser))))
  ;[1 1 1] Player Hit
  (`/Engine/EditorBlueprintResources/StandardMacros.DoOnce` false :!label _label_8
    (:`Completed`
      (set `self.HP` (- (`self.HP`) Damage))
      (`PrimitiveComponent.SetCollisionResponseToChannel` (`self.CapsuleComponent`) "ECC_WorldDynamic" "ECR_Ignore")
      (set `self.InputDisabled` true)
      (`GameplayStatics.PlaySound2D` "/Game/Sound/SFXs/sfx_PlayerHit_Cue.sfx_PlayerHit_Cue" 1.0 1.0 0.0 null null)
      (`MovementComponent.StopMovementImmediately` (`self.CharacterMovement`))
      (set `self.isPlayerHit` true)
      (if (> _returnvalue_x 0.0)
        (`CharacterMovementComponent.AddForce` (`self.CharacterMovement`) (`KismetMathLibrary.MakeVector` (* _hitimpulse_x -1.0) _hitimpulse_y _hitimpulse_z))
        (set `self.isMovingRight` true)
        (else
          (`CharacterMovementComponent.AddForce` (`self.CharacterMovement`) (`self.HitImpulse`))
          (set `self.isMovingRight` false)))
      (`KismetSystemLibrary.Delay` (`self.MaxStunDuration`))
      (if (`self.isDead`)
        (`PrimitiveComponent.SetCollisionEnabled` (`self.CapsuleComponent`) "NoCollision")
        (`GameplayStatics.PlaySound2D` "/Game/Sound/SFXs/sfx_PlayerDeath_Cue.sfx_PlayerDeath_Cue" 1.0 1.0 0.0 null null)
        (set `self.InputDisabled` true)
        (else
          (set `self.isPlayerHit` false)
          (set `self.isInvulnerable` true)
          (`self.Invulnerable`)
          (if (not (`self.isDead`))
            (set `self.InputDisabled` false)))))))

(event `InputAction|UpAction`
  (params (Key :type "Key Structure"))
  ;[1 1 1] Enter Door
  (:`Pressed`
    (if (`self.InputDisabled`)
      _
      (elif (`self.isDead`)
        _
        (elif (not (`self.isOnAir`))
          (`self.EnterDoor`))))))

(event `Invulnerable`
  ;[1 1 1] Invulnerable
  (`/Engine/EditorBlueprintResources/StandardMacros.FlipFlop` :!label _label_9
    (:`A`
      (`SceneComponent.SetVisibility` (`self.Sprite`) false false)
      (if (`|EnumEquality` (`self.PlayerType`) "NewEnumerator1")
        (`SceneComponent.SetHiddenInGame` (`self.HeroUpperBody`) true false)))
    (:`B`
      (`SceneComponent.SetVisibility` (`self.Sprite`) true false)
      (if (`|EnumEquality` (`self.PlayerType`) "NewEnumerator1")
        (`SceneComponent.SetHiddenInGame` (`self.HeroUpperBody`) false false))))
  (`KismetSystemLibrary.Delay` 0.15)
  (if (`self.isInvulnerable`)
    (goto _label_9)
    (else
      (`SceneComponent.SetVisibility` (`self.Sprite`) true true)
      (if (`|EnumEquality` (`self.PlayerType`) "NewEnumerator1")
        (`SceneComponent.SetHiddenInGame` (`self.HeroUpperBody`) false false))
      (`PrimitiveComponent.SetCollisionResponseToChannel` (`self.CapsuleComponent`) "ECC_WorldDynamic" "ECR_Block")
      (`self.InvulnerableOver`))))

(event `EnterDoor`
  ;[1 1 1] Enter Door
  (bind _outactors (`GameplayStatics.GetAllActorsOfClass` "/Game/Blueprints/Level/ArmoredDoor_BP.ArmoredDoor_BP_C"))
  (bind _output (`|GetArrayItem` _outactors))
  (if (`/Game/Blueprints/Level/ArmoredDoor_BP.inRange` _output)
    (if (`/Game/Blueprints/Level/ArmoredDoor_BP.isOpen` _output)
      (`self.SaveLevelUp`)
      (`self.BinaryBumper`)
      (`KismetSystemLibrary.Delay` 0.3)
      (`GameplayStatics.OpenLevel` (`/Game/Blueprints/Level/ArmoredDoor_BP.NextLevel` _output)))))

(event `SaveGame`
  ;[1 1 1] SaveGame
  (bind _returnvalue (`GameplayStatics.CreateSaveGameObject` "/Game/Blueprints/MySaveGame.MySaveGame_C"))
  (set `self.MySaveGameRef` _returnvalue)
  (`|ExecutionSequence`
    (:`then_0`
      (set `/Game/Blueprints/MySaveGame.LevelUpSaved` (`/Game/Blueprints/Level/ArmoredDoor_BP.LevelUp` (`|GetArrayItem` (stale `EnterDoor` _outactors))) (`self.MySaveGameRef`)))
    (:`then_2`
      (`GameplayStatics.SaveGameToSlot` (`self.MySaveGameRef`) "GameSlotSaved")
      (`KismetSystemLibrary.PrintString` (`KismetStringLibrary.Concat_StrStr` "Game Saved (CurrentPOI: " (`KismetSystemLibrary.GetDisplayName` (`/Game/Blueprints/MySaveGame.CurrentPOISaved` (`self.MySaveGameRef`))) ")") true true (struct :`G` 0.66 :`B` 1.0 :`A` 1.0) 6.0))))

(event `SaveLevelUp`
  (bind _returnvalue (`GameplayStatics.CreateSaveGameObject` "/Game/Blueprints/MySaveGameLevelUp.MySaveGameLevelUp_C"))
  (bind _output_get (set `self.SaveGameLevelUpRef` _returnvalue))
  (bind _output_get_2 (set `/Game/Blueprints/MySaveGameLevelUp.LevelUpSaved` (`/Game/Blueprints/Level/ArmoredDoor_BP.LevelUp` (`|GetArrayItem` (stale `EnterDoor` _outactors))) _output_get))
  (`GameplayStatics.SaveGameToSlot` _output_get "1")
  (`KismetSystemLibrary.PrintString` (`|GetEnumeratorNameAsString` _output_get_2) true true (struct :`R` 1.0 :`A` 1.0)))

(fn `UserConstructionScript`)