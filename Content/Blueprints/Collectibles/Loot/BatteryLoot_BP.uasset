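; BatteryLoot_BP is a health pickup that pops upward with a physics impulse on spawn.
; When the player overlaps its box collider, it plays a sound, adds HP capped at the maximum, or prints an overcharge message if already full, then destroys itself either way.
; Unless flagged to last forever, it waits out its lifetime, then blinks its flipbook through a FlipFlop delay loop before despawning.
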(event `self.ReceiveBeginPlay`
  (`PrimitiveComponent.AddImpulse` (`self.Box Collider`) (0.0 0.0 100.0) "None" false)
  (if (not (`self.LastsForever?`))
    (`self.DestroyDelay`)))

(event `self.Box Collider.OnComponentBeginOverlap`
  (params (OverlappedComponent :type "PrimitiveComponent Object Reference") (OtherActor :type "Actor Object Reference") (OtherComp :type "PrimitiveComponent Object Reference") (OtherBodyIndex :type Integer) (bFromSweep :type Boolean) (SweepResult :type "HitResult Structure (by ref)"))
  (bind _asplayer_bp (cast `/Game/Blueprints/Player/Player_BP` OtherActor))
  (`GameplayStatics.PlaySound2D` "/Game/Sound/SFXs/sfx_HPLoot_Cue1.sfx_HPLoot_Cue1" 1.0 1.0 0.0 null null)
  (bind _hpcurrent (`/Game/Blueprints/Player/Player_BP.HPCurrent` _asplayer_bp))
  (if (< _hpcurrent (`/Game/Blueprints/Player/Player_BP.HPMax` _asplayer_bp))
    (set `/Game/Blueprints/Player/Player_BP.HPCurrent` (+ _hpcurrent (`self.HP+`)) _asplayer_bp)
    (if (> (`/Game/Blueprints/Player/Player_BP.HPCurrent` _asplayer_bp) (`/Game/Blueprints/Player/Player_BP.HPMax` _asplayer_bp))
      (set `/Game/Blueprints/Player/Player_BP.HPCurrent` (`/Game/Blueprints/Player/Player_BP.HPMax` _asplayer_bp) _asplayer_bp))
    (else
      (`KismetSystemLibrary.PrintString` "OVERCHARGED!!!" true true (struct :`R` 1.0 :`A` 1.0))))
  (`self.K2_DestroyActor`))

(event `DestroyDelay`
  (`KismetSystemLibrary.Delay` (`self.LifeTime`))
  (`/Engine/EditorBlueprintResources/StandardMacros.FlipFlop` :!label _label
    (:`A`
      (`SceneComponent.SetVisibility` (`self.PaperFlipbook`) false false))
    (:`B`
      (`SceneComponent.SetVisibility` (`self.PaperFlipbook`) true false)))
  (`KismetSystemLibrary.Delay` 0.3)
  (if (< (`self.Index`) 5)
    (set `self.Index` (+ (`self.Index`) 1))
    (goto _label)
    (else
      (`self.K2_DestroyActor`))))

(fn `UserConstructionScript`)