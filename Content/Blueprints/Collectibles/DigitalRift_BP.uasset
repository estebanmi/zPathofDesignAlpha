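; Destructible digital rift collectible that bursts into a shower of Bitcoin loot when its health runs out.
; BeginPlay picks one of six flipbooks and a random flipped or rotated orientation, then starts a looping timer that randomly flickers the sprite.
; Damage depletes HP; near zero, it disables collision, plays a sound and runs BinaryRain, a delayed loop spawning BitCoinLoot_BP pickups at the rift before destroying it.
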(event `Flickering`
  (if (`self.isVisible`)
    (if (< (`KismetMathLibrary.RandomFloatInRange` 0.0 100.0) 30.0)
      (`SceneComponent.SetVisibility` (`self.PaperFlipbook`) false false)
      (else
        (`SceneComponent.SetVisibility` (`self.PaperFlipbook`) true false :!label _label)))
    (else
      (goto _label))))

(event `self.ReceiveBeginPlay`
  (set `self.index` (`KismetMathLibrary.RandomIntegerInRange` 0 5))
  (`PaperFlipbookComponent.SetFlipbook` (`self.PaperFlipbook`) (select `int` (`self.index`) :`0` "/Game/Sprites/Collectibles/DigitalRift/DigitalRift1.DigitalRift1" :`1` "/Game/Sprites/Collectibles/DigitalRift/DigitalRift2.DigitalRift2" :`2` "/Game/Sprites/Collectibles/DigitalRift/DigitalRift3.DigitalRift3" :`3` "/Game/Sprites/Collectibles/DigitalRift/DigitalRift4.DigitalRift4" :`4` "/Game/Sprites/Collectibles/DigitalRift/DigitalRift5.DigitalRift5" :`5` "/Game/Sprites/Collectibles/DigitalRift/DigitalRift6.DigitalRift6" :!type "PaperFlipbook Object Reference"))
  (set `self.index` (`KismetMathLibrary.RandomIntegerInRange` 0 1))
  (`self.K2_SetActorRotation` (`KismetMathLibrary.MakeRotator` 0.0 0.0 (select `int` (`self.index`) :`0` 0.0 :`1` 180.0 :!type "Float (single-precision)")))
  (set `self.index` (`KismetMathLibrary.RandomIntegerInRange` 0 5))
  (`self.K2_SetActorRotation` (`KismetMathLibrary.MakeRotator` 0.0 (select `int` (`self.index`) :`0` 0.0 :`1` 90.0 :`2` 180.0 :`3` 270.0 :!type "Float (single-precision)")))
  (`KismetSystemLibrary.K2_SetTimerDelegate` (delegate `Flickering`) 0.05 true))

(event `BinaryRain`
  (bind (_returnvalue_x _returnvalue_y _returnvalue_z) (`KismetMathLibrary.BreakVector` (`self.K2_GetActorLocation`)))
  (if (< (`self.index`) 20) :!label _label_2
    (`|SpawnActorFromClass` "/Game/Blueprints/Collectibles/Loot/BitCoinLoot_BP.BitCoinLoot_BP_C" (`KismetMathLibrary.MakeTransform` (`KismetMathLibrary.MakeVector` _returnvalue_x 1.0 _returnvalue_z)) "Undefined" "OverrideRootScale" null null)
    (set `self.index` (+ (`self.index`) 1))
    (`KismetSystemLibrary.Delay` (`KismetMathLibrary.RandomFloatInRange` 0.0 0.1))
    (goto _label_2)
    (else
      (`self.K2_DestroyActor`))))

(event `self.ReceiveAnyDamage`
  (params (Damage :type "Float (single-precision)") (DamageType :type "DamageType Object Reference") (InstigatedBy :type "Controller Object Reference") (DamageCauser :type "Actor Object Reference"))
  (set `self.HP` (- (`self.HP`) Damage))
  (if (<= (`self.HP`) 1.0)
    (`PrimitiveComponent.SetCollisionEnabled` (`self.BoxCollider`) "NoCollision")
    (`self.BinaryRain`)
    (`GameplayStatics.PlaySound2D` null 1.0 1.0 0.0 null null)))

(fn `UserConstructionScript`)