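; Tip trigger actor that shows up to five stages of tutorial-style dialog in a TipCoin_HUD, started by player overlap or automatically, optionally pausing the game.
; The ScrollingText macro types each string letter by letter with sound, honoring the player's skip flag.
; Tick polls Enter between stages while EnterKey blinks the prompt.
; After the last stage it notifies the player and optionally sets LaunchEvent, plays an explosion and destroys itself.
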(event `self.ReceiveBeginPlay`
  ;[1 1 1] Default
  (bind _asplayer_bp (cast `/Game/Blueprints/Player/Player_BP` (`GameplayStatics.GetPlayerCharacter` 0)))
  (set `self.PlayerRef` _asplayer_bp)
  (if (`self.AutoStart`)
    (`KismetSystemLibrary.Delay` 1.5)
    (`self.StartTalk`)
    (set `self.isActive` false)))

(event `self.BoxCollider.OnComponentBeginOverlap`
  (params (OverlappedComponent :type "PrimitiveComponent Object Reference") (OtherActor :type "Actor Object Reference") (OtherComp :type "PrimitiveComponent Object Reference") (OtherBodyIndex :type Integer) (bFromSweep :type Boolean) (SweepResult :type "HitResult Structure (by ref)"))
  ;[1 1 1] Start Talk
  (if (`self.isActive`)
    (cast `/Game/Blueprints/Player/Player_BP` OtherActor)
    (`/Engine/EditorBlueprintResources/StandardMacros.DoOnce` false :!label _label
      (:`Completed`
        (set `self.isRunning` true)
        (bind _foundwidgets (`WidgetBlueprintLibrary.GetAllWidgetsOfClass` "/Game/Widgets/NPCs/zDesignerOff_HUD.zDesignerOff_HUD_C"))
        (`Widget.RemoveFromParent` _foundwidgets)
        (set `/Game/Blueprints/Player/Player_BP.isSkipText` false (`self.PlayerRef`))
        (if (`self.PausesTheGame?`)
          (`GameplayStatics.SetGamePaused` true))
        (bind _returnvalue (`|CreateWidget` "/Game/Widgets/TipCoin_HUD.TipCoin_HUD_C"))
        (`UserWidget.AddToViewport` _returnvalue 0)
        (set `self.WidgetRef` _returnvalue)
        (`self.ScrollingText` (`/Game/Widgets/TipCoin_HUD.DialogText` (`self.WidgetRef`)) (select `int` (`self.StageIndex`) :`0` (`self.DialogArray_0`) :`1` (`self.DialogArray_1`) :`2` (`self.DialogArray_2`) :`3` (`self.DialogArray_3`) :`4` (`self.DialogArray_4`)) (`self.TextSpeed`))))))

(event `StartTalk`
  ;[1 1 1] Start Talk
  (goto _label))

(event `self.ReceiveTick`
  (params (DeltaSeconds :type "Float (single-precision)"))
  (bind _playerref (`self.PlayerRef`))
  (bind _paperflipbook (`self.PaperFlipbook`))
  ;[1 1 1] Waiting for Input to free player
  (if (`self.isWaitingForPlayer`)
    (`self.EnterKey`)
    (if (`PlayerController.WasInputKeyJustPressed` (`GameplayStatics.GetPlayerController` 0) "Enter")
      (`Widget.SetVisibility` (`/Game/Widgets/TipCoin_HUD.EnterKey` (`self.WidgetRef`)) "Hidden")
      (if (`self.PausesTheGame?`)
        (`GameplayStatics.SetGamePaused` false))
      (if (< (`self.StageIndex`) (`self.DialogsNumber`))
        (set `self.isWaitingForPlayer` false)
        (set `/Game/Blueprints/Player/Player_BP.isSkipText` false (`self.PlayerRef`))
        (`self.ScrollingText` (`/Game/Widgets/TipCoin_HUD.DialogText` (`self.WidgetRef`)) (select `int` (`self.StageIndex`) :`0` (`self.DialogArray_0`) :`1` (`self.DialogArray_1`) :`2` (`self.DialogArray_2`) :`3` (`self.DialogArray_3`) :`4` (`self.DialogArray_4`)) (`self.TextSpeed`))
        (else
          (set `self.isWaitingForPlayer` false)
          (if (not (`self.StayForever?`))
            (bind _foundwidgets (`WidgetBlueprintLibrary.GetAllWidgetsOfClass` "/Game/Widgets/TipCoin_HUD.TipCoin_HUD_C"))
            (`Widget.RemoveFromParent` _foundwidgets))
          (set `self.isRunning` false)
          (set `/Game/Blueprints/Player/Player_BP.isSkipText` false _playerref)
          (`/Game/Blueprints/Player/Player_BP.TipDesignWatched` _playerref)
          (if (`self.HasEvent?`)
            (set `self.LaunchEvent` true)
            (`GameplayStatics.PlaySound2D` "/Game/Sound/SFXs/sfx_CodeBlockExplosion.sfx_CodeBlockExplosion" 1.0 1.0 0.0 null null)
            (`PaperFlipbookComponent.SetFlipbook` _paperflipbook "/Game/Sprites/Collectibles/CodeBlock/CodeBlockExplosion2.CodeBlockExplosion2")
            (`KismetSystemLibrary.Delay` (`PaperFlipbookComponent.GetFlipbookLength` _paperflipbook))
            (`self.K2_DestroyActor`)))))))

(event `EnterKey`
  (bind _enterkey (`/Game/Widgets/TipCoin_HUD.EnterKey` (`self.WidgetRef`)))
  ;[1 1 1] EnterKey
  (if (< (`self.StageIndex`) (`self.DialogsNumber`))
    (`/Engine/EditorBlueprintResources/StandardMacros.DoOnce` false :!label _label_2
      (:`Completed`
        (if (`self.isWaitingForPlayer`)
          (`/Engine/EditorBlueprintResources/StandardMacros.FlipFlop`
            (:`A`
              (`Widget.SetVisibility` _enterkey "Visible"))
            (:`B`
              (`Widget.SetVisibility` _enterkey "Hidden")))
          (`KismetSystemLibrary.Delay` 0.5)
          (goto _label_2 :!via `Reset`))))
    (elif (`self.HasEvent?`)
      (goto _label_2))))

(fn `UserConstructionScript`)