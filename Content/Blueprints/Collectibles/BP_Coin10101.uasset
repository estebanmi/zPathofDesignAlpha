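; BP_Coin10101 is a collectible coin pickup for the 2D side scroller, themed on binary digits.
; On BeginPlay it randomly sets its Paper2D flipbook to either the zero or the one variant.
; When a 2DSideScrollerCharacter overlaps its Box, it plays one of two coin sounds, rolled independently of the visual, then destroys itself.
; The Blueprint itself updates no score or counter.
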(event `self.ReceiveBeginPlay`
  (if (== (`KismetMathLibrary.RandomIntegerInRange` 0 1) 0)
    (`PaperFlipbookComponent.SetFlipbook` (`self.PaperFlipbook`) "/Game/Sprites/Collectibles/10101/101_Zero.101_Zero")
    (else
      (`PaperFlipbookComponent.SetFlipbook` (`self.PaperFlipbook`) "/Game/Sprites/Collectibles/10101/101_One.101_One"))))

(event `self.Box.OnComponentBeginOverlap`
  (params (OverlappedComponent :type "PrimitiveComponent Object Reference") (OtherActor :type "Actor Object Reference") (OtherComp :type "PrimitiveComponent Object Reference") (OtherBodyIndex :type Integer) (bFromSweep :type Boolean) (SweepResult :type "HitResult Structure (by ref)"))
  (cast `/Game/Blueprints/Player/2DSideScrollerCharacter` OtherActor)
  (if (== (`KismetMathLibrary.RandomIntegerInRange` 0 1) 0)
    (`GameplayStatics.PlaySound2D` "/Game/Sound/SFXs/sfx_coin_0_Cue.sfx_coin_0_Cue" 1.0 1.0 0.0 null null)
    (else
      (`GameplayStatics.PlaySound2D` "/Game/Sound/SFXs/sfx_coin_1_Cue.sfx_coin_1_Cue" 1.0 1.0 0.0 null null)))
  (`self.K2_DestroyActor`))

(fn `UserConstructionScript`)