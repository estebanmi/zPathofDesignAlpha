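; BinaryCoin_BP is a collectible 2D coin that represents a binary 0 or 1.
; On BeginPlay it optionally randomizes its value, then sets the Paper2D flipbook to match.
; When its box collider overlaps PlayerSword_BP, it finds the first BinaryWordsController_BP in the level, passes it the bit via GetBinaryCoin, and destroys itself.
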(event `self.ReceiveBeginPlay`
  (if (`self.isRandom`)
    (if (== (`KismetMathLibrary.RandomIntegerInRange` 0 1) 0)
      (set `self.BinaryValue` false)
      (else
        (set `self.BinaryValue` true))))
  (if (`self.BinaryValue`)
    (`PaperFlipbookComponent.SetFlipbook` (`self.PaperFlipbook`) "/Game/Sprites/Login/BinaryCoinsOne.BinaryCoinsOne")
    (else
      (`PaperFlipbookComponent.SetFlipbook` (`self.PaperFlipbook`) "/Game/Sprites/Login/BinaryCoinsZero.BinaryCoinsZero"))))

(event `self.Box Collider.OnComponentBeginOverlap`
  (params (OverlappedComponent :type "PrimitiveComponent Object Reference") (OtherActor :type "Actor Object Reference") (OtherComp :type "PrimitiveComponent Object Reference") (OtherBodyIndex :type Integer) (bFromSweep :type Boolean) (SweepResult :type "HitResult Structure (by ref)"))
  (cast `/Game/Blueprints/Player/PlayerSword_BP` OtherActor)
  (bind _outactors (`GameplayStatics.GetAllActorsOfClass` "/Game/Blueprints/Player/BinaryWordsController_BP.BinaryWordsController_BP_C"))
  (`/Game/Blueprints/Player/BinaryWordsController_BP.GetBinaryCoin` (`|GetArrayItem` _outactors) (`self.BinaryValue`))
  (`self.K2_DestroyActor`))

(fn `UserConstructionScript`)