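; NewLife is a short-lived sprite effect, apparently an extra-life indicator, that plays the all-Passterisks-collected sound when spawned.
; On BeginPlay it tints its sprite with the active color scheme's player color, looked up via ColorController and a data table, if the player's VideoCardON is set.
; A timeline floats the actor upward, then delayed visibility toggles blink the sprite before the actor destroys itself.
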(event `ColorControl`
  ;[0 1 1] Color Control
  (if (`/Game/Blueprints/Player/Player_BP.VideoCardON` (`self.PlayerRef`))
    (bind _outactors (`GameplayStatics.GetAllActorsOfClass` "/Game/Blueprints/Art/ColorController.ColorController_C"))
    (bind _returnvalue (`|GetDataTableRow` "/Game/Blueprints/Art/ColorSchemeTable.ColorSchemeTable" (`/Game/Blueprints/Art/ColorController.ColorScheme` (`|GetArrayItem` _outactors)))
      (:`then`
        (`PaperSpriteComponent.SetSpriteColor` (`self.PaperSprite`) (break `/Game/Blueprints/Art/ColorScheme` _returnvalue))))))

(event `self.ReceiveBeginPlay`
  (bind (_returnvalue_x _returnvalue_y _returnvalue_z) (`KismetMathLibrary.BreakVector` (`self.K2_GetActorLocation`)))
  (bind _asplayer_bp (cast `/Game/Blueprints/Player/Player_BP` (`GameplayStatics.GetPlayerCharacter` 0)))
  (set `self.PlayerRef` _asplayer_bp)
  (`self.ColorControl`)
  (`GameplayStatics.PlaySound2D` "/Game/Sound/SFXs/sfx_AllPassterisksCollected_Cue.sfx_AllPassterisksCollected_Cue" 1.0 1.0 0.0 null null)
  (bind (_direction _newtrack_0) (`Timeline|FloatingUp` :!via `PlayFromStart`)
    (:`Update`
      (`self.K2_SetActorLocation` (`KismetMathLibrary.MakeVector` _returnvalue_x _returnvalue_y (+ _returnvalue_z _newtrack_0))))
    (:`Finished`
      (`KismetSystemLibrary.Delay` 0.2)
      (`SceneComponent.SetVisibility` (`self.PaperSprite`) false false)
      (`KismetSystemLibrary.Delay` 0.2)
      (`SceneComponent.SetVisibility` (`self.PaperSprite`) true false)
      (`KismetSystemLibrary.Delay` 0.2)
      (`SceneComponent.SetVisibility` (`self.PaperSprite`) false false)
      (`KismetSystemLibrary.Delay` 0.2)
      (`SceneComponent.SetVisibility` (`self.PaperSprite`) true false)
      (`KismetSystemLibrary.Delay` 0.2)
      (`self.K2_DestroyActor`))))

(fn `UserConstructionScript`)