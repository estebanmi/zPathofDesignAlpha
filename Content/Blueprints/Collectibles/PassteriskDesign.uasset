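; Passterisk collectible, a hidden flipbook pickup that opens the configured level when the player collects it.
; It spawns and idles once the player enters its Trigger, unless DesignerOff has an event, or when ActivePassterisk is called.
; While active, box overlap or a Tick check runs a one-shot collection with sound and explosion.
; If BeforeRecap is set, it calls the player's BinaryBumper before the level change.
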(event `self.ReceiveBeginPlay`
  (`SceneComponent.SetVisibility` (`self.PaperFlipbook`) false false))

(event `ActivePassterisk`
  (bind _paperflipbook (`self.PaperFlipbook`))
  (`SceneComponent.SetVisibility` (`self.PaperFlipbook`) true false)
  (set `self.Active` true)
  (`PaperFlipbookComponent.SetFlipbook` _paperflipbook "/Game/Sprites/Collectibles/Passterisk/PassterikSpawn.PassterikSpawn")
  (`KismetSystemLibrary.Delay` (`PaperFlipbookComponent.GetFlipbookLength` _paperflipbook))
  (`PaperFlipbookComponent.SetFlipbook` (`self.PaperFlipbook`) "/Game/Sprites/Collectibles/Passterisk/PassterikIdle.PassterikIdle"))

(event `Passterisk Collected`)

(event `OverPassterisk`
  (bind _paperflipbook (`self.PaperFlipbook`))
  (bind _leveltoopen (`self.LevelToOpen`))
  (`/Engine/EditorBlueprintResources/StandardMacros.DoOnce` false :!label _label
    (:`Completed`
      (set `self.Active` false)
      (`GameplayStatics.PlaySound2D` "/Game/Sound/SFXs/sfx_PassteriskCollected_Cue.sfx_PassteriskCollected_Cue" 1.0 1.0 0.0 null null)
      (`PaperFlipbookComponent.SetFlipbook` _paperflipbook "/Game/Sprites/Collectibles/Passterisk/PassterikExplosion1.PassterikExplosion1")
      (`KismetSystemLibrary.Delay` (`PaperFlipbookComponent.GetFlipbookLength` _paperflipbook))
      (`SceneComponent.SetVisibility` (`self.PaperFlipbook`) false false)
      (`KismetSystemLibrary.Delay` 1.0)
      (if (`self.BeforeRecap?`)
        (bind _asplayer_bp (cast `/Game/Blueprints/Player/Player_BP` (`GameplayStatics.GetPlayerCharacter` 0)))
        (`/Game/Blueprints/Player/Player_BP.BinaryBumper` _asplayer_bp)
        (`KismetSystemLibrary.Delay` 0.3))
      (if (!= _leveltoopen "None")
        (`GameplayStatics.OpenLevel` _leveltoopen)))))

(event `self.BoxCollider.OnComponentBeginOverlap`
  (params (OverlappedComponent :type "PrimitiveComponent Object Reference") (OtherActor :type "Actor Object Reference") (OtherComp :type "PrimitiveComponent Object Reference") (OtherBodyIndex :type Integer) (bFromSweep :type Boolean) (SweepResult :type "HitResult Structure (by ref)"))
  (if (`self.Active`)
    (cast `/Game/Blueprints/Player/Player_BP` OtherActor)
    (goto _label)))

(event `self.Trigger.OnComponentBeginOverlap`
  (params (OverlappedComponent :type "PrimitiveComponent Object Reference") (OtherActor :type "Actor Object Reference") (OtherComp :type "PrimitiveComponent Object Reference") (OtherBodyIndex :type Integer) (bFromSweep :type Boolean) (SweepResult :type "HitResult Structure (by ref)"))
  (bind _paperflipbook (`self.PaperFlipbook`))
  (bind _outactors (`GameplayStatics.GetAllActorsOfClass` "/Game/Blueprints/NPCs/DesignerOff.DesignerOff_C"))
  (if (not (`/Game/Blueprints/NPCs/DesignerOff.HasEvent?` (`|GetArrayItem` _outactors)))
    (cast `/Game/Blueprints/Player/Player_BP` OtherActor)
    (`/Engine/EditorBlueprintResources/StandardMacros.DoOnce` false
      (:`Completed`
        (set `self.Active` true)
        (`GameplayStatics.PlaySound2D` "/Game/Sound/SFXs/sfx_PassteriskSpawn_Cue.sfx_PassteriskSpawn_Cue" 1.0 1.0 0.0 null null)
        (`SceneComponent.SetVisibility` (`self.PaperFlipbook`) true false)
        (`PaperFlipbookComponent.SetFlipbook` _paperflipbook "/Game/Sprites/Collectibles/Passterisk/PassterikSpawn.PassterikSpawn")
        (`KismetSystemLibrary.Delay` (`PaperFlipbookComponent.GetFlipbookLength` _paperflipbook))
        (if (`self.Active`)
          (`PaperFlipbookComponent.SetFlipbook` (`self.PaperFlipbook`) "/Game/Sprites/Collectibles/Passterisk/PassterikIdle.PassterikIdle"))))))

(event `self.ReceiveTick`
  (params (DeltaSeconds :type "Float (single-precision)"))
  (if (`self.Active`)
    (`/Engine/EditorBlueprintResources/StandardMacros.IsValid` (`|GetArrayItem` (`PrimitiveComponent.GetOverlappingActors` (`self.BoxCollider`) "/Game/Blueprints/Player/Player_BP.Player_BP_C"))
      (:`Is Valid`
        (`self.OverPassterisk`)))))

(fn `UserConstructionScript`)