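; BitCoin is a collectible coin that shows a binary one or zero flipbook based on its BitValue.
; On overlap with Player_BP it notifies the player, passes its bit to BitWordsController_BP or plays a wrong-coin sound if none exists, then spawns an explosion and destroys itself.
; When the player's VideoCardON is set, a timeline blends the coin between the active ColorScheme's item color and black, and the explosion takes that color.
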(event `ColorControl`
  ;[0 1 1] Color Control
  (if (`/Game/Blueprints/Player/Player_BP.VideoCardON` (`self.PlayerRef`))
    (bind _outactors (`GameplayStatics.GetAllActorsOfClass` "/Game/Blueprints/Art/ColorController.ColorController_C"))
    (bind _returnvalue (`|GetDataTableRow` "/Game/Blueprints/Art/ColorSchemeTable.ColorSchemeTable" (`/Game/Blueprints/Art/ColorController.ColorScheme` (`|GetArrayItem` _outactors)))
      (:`then`
        (bind (_direction _newtrack_0) (`Timeline|Timeline_0`)
          (:`Update`
            (`PaperFlipbookComponent.SetSpriteColor` (`self.PaperFlipbook`) (`KismetMathLibrary.LinearColorLerp` (`.Items_29_2BC6507E48F0D0D31E739786CFADAD7C` (break `/Game/Blueprints/Art/ColorScheme` _returnvalue)) (struct :`A` 1.0) _newtrack_0))))))))

(event `self.Box Collider.OnComponentBeginOverlap`
  (params (OverlappedComponent :type "PrimitiveComponent Object Reference") (OtherActor :type "Actor Object Reference") (OtherComp :type "PrimitiveComponent Object Reference") (OtherBodyIndex :type Integer) (bFromSweep :type Boolean) (SweepResult :type "HitResult Structure (by ref)"))
  ;[1 1 1] Pick Up
  (bind _asplayer_bp (cast `/Game/Blueprints/Player/Player_BP` OtherActor))
  (`/Game/Blueprints/Player/Player_BP.GetBitCoin` _asplayer_bp)
  (bind _outactors (`GameplayStatics.GetAllActorsOfClass` "/Game/Blueprints/Player/BitWordsController_BP.BitWordsController_BP_C"))
  (bind _output (`|GetArrayItem` _outactors))
  (`/Engine/EditorBlueprintResources/StandardMacros.IsValid` _output
    (:`Is Valid`
      (`/Game/Blueprints/Player/BitWordsController_BP.GetBinaryCoin` _output (`self.BitValue`)))
    (:`Is Not Valid`
      (`GameplayStatics.PlaySound2D` "/Game/Sound/SFXs/sfx_coin_Wrong_Cue.sfx_coin_Wrong_Cue" 1.0 1.0 0.0 null null)))
  (bind _returnvalue (`|SpawnActorFromClass` "/Game/Blueprints/Player/ActionPlayer/PlayerBulletExplosion_BP.PlayerBulletExplosion_BP_C" (`self.GetTransform`) "Undefined" "OverrideRootScale" null null))
  (if (`/Game/Blueprints/Player/Player_BP.VideoCardON` (`self.PlayerRef`))
    (`PaperFlipbookComponent.SetSpriteColor` (`/Game/Blueprints/Player/ActionPlayer/PlayerBulletExplosion_BP.PaperFlipbook` _returnvalue) (`.Items_29_2BC6507E48F0D0D31E739786CFADAD7C` (break `/Game/Blueprints/Art/ColorScheme` (stale `ColorControl` _returnvalue)))))
  (`self.K2_DestroyActor`))

(event `self.ReceiveBeginPlay`
  ;[1 0.4264 0] Defaullt
  (`KismetSystemLibrary.Delay` 0.1)
  (bind _asplayer_bp (cast `/Game/Blueprints/Player/Player_BP` (`GameplayStatics.GetPlayerCharacter` 0)))
  (set `self.PlayerRef` _asplayer_bp)
  (`self.ColorControl`)
  (if (`self.BitValue`)
    (`PaperFlipbookComponent.SetFlipbook` (`self.PaperFlipbook`) "/Game/Sprites/Login/BinaryCoinsOne.BinaryCoinsOne")
    (else
      (`PaperFlipbookComponent.SetFlipbook` (`self.PaperFlipbook`) "/Game/Sprites/Login/BinaryCoinsZero.BinaryCoinsZero"))))

(fn `UserConstructionScript`)