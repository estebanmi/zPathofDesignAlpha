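; Passterisk collectible, a flipbook-animated pickup that starts hidden and reports to the LoginController_BP when the player collects it.
; The player's first Trigger overlap reveals it with a sound and spawn flipbook, then switches to idle.
; A player overlap on BoxCollider plays a coin sound, calls PassteriskCollected on the first controller found, then destroys the actor after the explosion flipbook's length.
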(event `self.ReceiveBeginPlay`
  (`SceneComponent.SetVisibility` (`self.PaperFlipbook`) false false))

(event `self.BoxCollider.OnComponentBeginOverlap`
  (params (OverlappedComponent :type "PrimitiveComponent Object Reference") (OtherActor :type "Actor Object Reference") (OtherComp :type "PrimitiveComponent Object Reference") (OtherBodyIndex :type Integer) (bFromSweep :type Boolean) (SweepResult :type "HitResult Structure (by ref)"))
  (bind _paperflipbook (`self.PaperFlipbook`))
  (cast `/Game/Blueprints/Player/Player_BP` OtherActor)
  (`GameplayStatics.PlaySound2D` "/Game/Sound/SFXs/sfx_coin_1_Cue.sfx_coin_1_Cue" 1.0 1.0 0.0 null null)
  (bind _outactors (`GameplayStatics.GetAllActorsOfClass` "/Game/Blueprints/Level/LoginController_BP.LoginController_BP_C"))
  (bind _output (`|GetArrayItem` _outactors))
  (`/Engine/EditorBlueprintResources/StandardMacros.IsValid` _output
    (:`Is Valid`
      (`/Game/Blueprints/Level/LoginController_BP.Passterisk Collected` _output))
    (:`Is Not Valid`
      _))
  (`PaperFlipbookComponent.SetFlipbook` _paperflipbook "/Game/Sprites/Collectibles/Passterisk/PassterikExplosion1.PassterikExplosion1")
  (`KismetSystemLibrary.Delay` (`PaperFlipbookComponent.GetFlipbookLength` _paperflipbook))
  (`self.K2_DestroyActor`))

(event `self.Trigger.OnComponentBeginOverlap`
  (params (OverlappedComponent :type "PrimitiveComponent Object Reference") (OtherActor :type "Actor Object Reference") (OtherComp :type "PrimitiveComponent Object Reference") (OtherBodyIndex :type Integer) (bFromSweep :type Boolean) (SweepResult :type "HitResult Structure (by ref)"))
  (bind _paperflipbook (`self.PaperFlipbook`))
  (cast `/Game/Blueprints/Player/Player_BP` OtherActor)
  (`/Engine/EditorBlueprintResources/StandardMacros.DoOnce` false
    (:`Completed`
      (`GameplayStatics.PlaySound2D` "/Game/Sound/SFXs/sfx_PassteriskSpawn_Cue.sfx_PassteriskSpawn_Cue" 1.0 1.0 0.0 null null)
      (`SceneComponent.SetVisibility` (`self.PaperFlipbook`) true false)
      (`PaperFlipbookComponent.SetFlipbook` _paperflipbook "/Game/Sprites/Collectibles/Passterisk/PassterikSpawn.PassterikSpawn")
      (`KismetSystemLibrary.Delay` (`PaperFlipbookComponent.GetFlipbookLength` _paperflipbook))
      (`PaperFlipbookComponent.SetFlipbook` (`self.PaperFlipbook`) "/Game/Sprites/Collectibles/Passterisk/PassterikIdle.PassterikIdle"))))

(fn `UserConstructionScript`)