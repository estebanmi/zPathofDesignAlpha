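; Collectible binary coin that shows a 0 or 1 flipbook, optionally randomized at start, and is picked up when Player_BP overlaps it.
; Pickup calls GetBitCoin on the player, spawns an explosion effect, and destroys the coin.
; Dynamic coins loop on a random delay, flickering before flipping their bit.
; With the player's VideoCard on, a timeline lerps the sprite between the scheme's item color and black, and tints the explosion.
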(event `ColorControl`
  ;[0 1 1] Color Control
  (if (`/Game/Blueprints/Player/Player_BP.VideoCardON` (`self.PlayerRef`))
    (bind _outactors (`GameplayStatics.GetAllActorsOfClass` "/Game/Blueprints/Art/ColorController.ColorController_C"))
    (bind _returnvalue (`|GetDataTableRow` "/Game/Blueprints/Art/ColorSchemeTable.ColorSchemeTable" (`/Game/Blueprints/Art/ColorController.ColorScheme` (`|GetArrayItem` _outactors)))
      (:`then`
        (bind (_direction _newtrack_0) (`Timeline|Timeline_0`)
          (:`Update`
            (`PaperFlipbookComponent.SetSpriteColor` (`self.PaperFlipbook`) (`KismetMathLibrary.LinearColorLerp` (`KismetMathLibrary.Conv_ColorToLinearColor` (`.Items_4_2BC6507E48F0D0D31E739786CFADAD7C` (break `/Game/Blueprints/Art/ColorScheme` _returnvalue))) (struct :`A` 1.0) _newtrack_0))))))))

(event `self.Box Collider.OnComponentBeginOverlap`
  (params (OverlappedComponent :type "PrimitiveComponent Object Reference") (OtherActor :type "Actor Object Reference") (OtherComp :type "PrimitiveComponent Object Reference") (OtherBodyIndex :type Integer) (bFromSweep :type Boolean) (SweepResult :type "HitResult Structure (by ref)"))
  ;[1 1 1] Pick Up
  (bind _asplayer_bp (cast `/Game/Blueprints/Player/Player_BP` OtherActor))
  (`/Game/Blueprints/Player/Player_BP.GetBitCoin` _asplayer_bp)
  (bind _returnvalue (`|SpawnActorFromClass` "/Game/Blueprints/Player/ActionPlayer/PlayerBulletExplosion_BP.PlayerBulletExplosion_BP_C" (`self.GetTransform`) "Undefined" "OverrideRootScale" null null))
  (if (`/Game/Blueprints/Player/Player_BP.VideoCardON` (`self.PlayerRef`))
    (`PaperFlipbookComponent.SetSpriteColor` (`/Game/Blueprints/Player/ActionPlayer/PlayerBulletExplosion_BP.PaperFlipbook` _returnvalue) (`KismetMathLibrary.Conv_ColorToLinearColor` (`.Items_4_2BC6507E48F0D0D31E739786CFADAD7C` (break `/Game/Blueprints/Art/ColorScheme` (stale `ColorControl` _returnvalue))))))
  (`self.K2_DestroyActor`))

(event `self.ReceiveBeginPlay`
  ;[1 1 1] Defaullt
  (bind _asplayer_bp (cast `/Game/Blueprints/Player/Player_BP` (`GameplayStatics.GetPlayerCharacter` 0)))
  (set `self.PlayerRef` _asplayer_bp)
  (`self.ColorControl`)
  (if (`self.isRandom`)
    (if (== (`KismetMathLibrary.RandomIntegerInRange` 0 1) 0)
      (set `self.BitValue` false)
      (else
        (set `self.BitValue` true))))
  (if (`self.BitValue`)
    (`PaperFlipbookComponent.SetFlipbook` (`self.PaperFlipbook`) "/Game/Sprites/Login/BinaryCoinsOne.BinaryCoinsOne")
    (else
      (`PaperFlipbookComponent.SetFlipbook` (`self.PaperFlipbook`) "/Game/Sprites/Login/BinaryCoinsZero.BinaryCoinsZero")))
  (if (`self.Dynamic`)
    (`self.BitChange`)))

(event `BitChange`
  ;[1 1 1] Dynamic Change
  (bind _output_get (set `self.RandomDelay` (`KismetMathLibrary.RandomFloatInRange` 6.0 12.0) :!label _label))
  (`KismetSystemLibrary.Delay` _output_get)
  (set `self.FlickeringTimes` 0.0)
  (`SceneComponent.SetVisibility` (`self.PaperFlipbook`) false false :!label _label_2)
  (`KismetSystemLibrary.Delay` (`self.FlickeringTime`))
  (`SceneComponent.SetVisibility` (`self.PaperFlipbook`) true false)
  (`KismetSystemLibrary.Delay` (`self.FlickeringTime`))
  (if (< (`self.FlickeringTimes`) 8.0)
    (set `self.FlickeringTimes` (+ (`self.FlickeringTimes`) 1.0))
    (goto _label_2)
    (else
      (`SceneComponent.SetVisibility` (`self.PaperFlipbook`) false false)
      (`KismetSystemLibrary.Delay` (`self.FlickeringTime`))
      (`SceneComponent.SetVisibility` (`self.PaperFlipbook`) true false)
      (if (`self.BitValue`)
        (`PaperFlipbookComponent.SetFlipbook` (`self.PaperFlipbook`) "/Game/Sprites/Login/BinaryCoinsZero.BinaryCoinsZero")
        (set `self.BitValue` false)
        (goto _label)
        (else
          (`PaperFlipbookComponent.SetFlipbook` (`self.PaperFlipbook`) "/Game/Sprites/Login/BinaryCoinsOne.BinaryCoinsOne")
          (set `self.BitValue` true)
          (goto _label))))))

(fn `UserConstructionScript`)