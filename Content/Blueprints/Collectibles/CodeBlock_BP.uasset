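; Destructible 2D code block collectible that drops bitcoin or battery health loot when broken.
; A looping timer, started after a random delay, occasionally swaps in glitch flipbooks.
; Damage lowers HP and plays a timeline shake, whose update triggers one-time destruction at low HP.
; Destruction disables collision, spawns either a random roll (possibly nothing) or the configured Loot, then plays an explosion flipbook before destroying the actor.
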(event `Glitch`
  ;[1 1 1] Glitch
  (if (`self.isDestroyed`)
    _
    (elif (< (`KismetMathLibrary.RandomFloatInRange` 0.0 100.0) 10.0)
      (if (< (`KismetMathLibrary.RandomFloatInRange` 0.0 100.0) 40.0)
        (`PaperFlipbookComponent.SetFlipbook` (`self.PaperFlipbook`) "/Game/Sprites/Collectibles/CodeBlock/CodeBlockGlitch1.CodeBlockGlitch1")
        (else
          (`PaperFlipbookComponent.SetFlipbook` (`self.PaperFlipbook`) "/Game/Sprites/Collectibles/CodeBlock/CodeBlockGlitch2.CodeBlockGlitch2")))
      (else
        (`PaperFlipbookComponent.SetFlipbook` (`self.PaperFlipbook`) "/Game/Sprites/Collectibles/CodeBlock/CodeBlock1.CodeBlock1")))))

(event `self.ReceiveBeginPlay`
  ;[1 1 1] Default
  (`KismetSystemLibrary.Delay` (`KismetMathLibrary.RandomFloatInRange` 0.0 2.0))
  (`KismetSystemLibrary.K2_SetTimerDelegate` (delegate `Glitch`) 0.1 true))

(event `self.ReceiveAnyDamage`
  (params (Damage :type "Float (single-precision)") (DamageType :type "DamageType Object Reference") (InstigatedBy :type "Controller Object Reference") (DamageCauser :type "Actor Object Reference"))
  (bind _paperflipbook (`self.PaperFlipbook`))
  (bind _paperflipbook_2 (`self.PaperFlipbook`))
  (bind (_relativelocation_x _relativelocation_y _relativelocation_z) (`KismetMathLibrary.BreakVector` (`SceneComponent.RelativeLocation` _paperflipbook)))
  ;[1 1 1] Receive Damage
  (set `self.HP` (- (`self.HP`) Damage))
  (`GameplayStatics.PlaySound2D` "/Game/Sound/SFXs/sfx_BlopHit_Cue.sfx_BlopHit_Cue" 1.0 1.0 0.0 null null)
  (bind (_direction _horizontalshake) (`Timeline|Timeline_0` :!via `PlayFromStart`)
    (:`Update`
      (`SceneComponent.K2_SetRelativeLocation` _paperflipbook (`KismetMathLibrary.MakeVector` _horizontalshake _relativelocation_y _relativelocation_z) false false)
      (if (<= (`self.HP`) 1.0)
        (`/Engine/EditorBlueprintResources/StandardMacros.DoOnce` false
          (:`Completed`
            (`PrimitiveComponent.SetCollisionEnabled` (`self.BoxCollider`) "NoCollision")
            (if (`self.RandomLoot?`)
              (`self.RandomLoot`)
              (else
                (`self.DropLoot`)))
            (`GameplayStatics.PlaySound2D` "/Game/Sound/SFXs/sfx_CodeBlockExplosion_Cue.sfx_CodeBlockExplosion_Cue" 1.0 1.0 0.0 null null)
            (set `self.isDestroyed` true)
            (`PaperFlipbookComponent.SetFlipbook` _paperflipbook_2 "/Game/Sprites/Collectibles/CodeBlock/CodeBlockExplosion2.CodeBlockExplosion2")
            (`KismetSystemLibrary.Delay` (`PaperFlipbookComponent.GetFlipbookLength` _paperflipbook_2))
            (`self.K2_DestroyActor`)))))))

(event `RandomLoot`
  (set `self.Roll` (`KismetMathLibrary.RandomFloatInRange` 0.0 100.0))
  (`KismetSystemLibrary.PrintString` (`KismetStringLibrary.Concat_StrStr` "Loot Roll: " (`KismetStringLibrary.Conv_DoubleToString` (`self.Roll`))) true true (struct :`R` 1.0 :`B` 0.74359 :`A` 1.0))
  (if (> (`self.Roll`) 80.0)
    _
    (elif (> (`self.Roll`) 40.0)
      (`self.DropBitcoin`)
      (elif (> (`self.Roll`) 10.0)
        (`self.DropHP`)
        (else
          (`self.Drop5Bitcoins`))))))

(event `DropLoot`
  ;[1 1 1] Drop Loot
  (switch `/Game/Blueprints/Collectibles/CodeBlockLoots` (`self.Loot`)
    (:`NewEnumerator0`
      (`self.DropBitcoin`))
    (:`NewEnumerator1`
      (`self.DropHP`))
    (:`NewEnumerator2`
      (`self.Drop5Bitcoins`))))

(event `DropBitcoin`
  (bind (_returnvalue_x _returnvalue_y _returnvalue_z) (`KismetMathLibrary.BreakVector` (`self.K2_GetActorLocation`)))
  (`|SpawnActorFromClass` "/Game/Blueprints/Collectibles/BitCoinLootBlock.BitCoinLootBlock_C" (`KismetMathLibrary.MakeTransform` (`KismetMathLibrary.MakeVector` _returnvalue_x 1.0 _returnvalue_z)) "Undefined" "OverrideRootScale" null null))

(event `Drop5Bitcoins`
  (bind (_returnvalue_x _returnvalue_y _returnvalue_z) (`KismetMathLibrary.BreakVector` (`self.K2_GetActorLocation`)))
  (if (< (`self.index`) 5) :!label _label
    (`|SpawnActorFromClass` "/Game/Blueprints/Collectibles/BitCoinLootBlock.BitCoinLootBlock_C" (`KismetMathLibrary.MakeTransform` (`KismetMathLibrary.MakeVector` _returnvalue_x 1.0 _returnvalue_z)) "Undefined" "OverrideRootScale" null null)
    (set `self.index` (+ (`self.index`) 1))
    (`KismetSystemLibrary.Delay` (`KismetMathLibrary.RandomFloatInRange` 0.0 0.1))
    (goto _label)))

(event `DropHP`
  (bind (_returnvalue_x _returnvalue_y _returnvalue_z) (`KismetMathLibrary.BreakVector` (`self.K2_GetActorLocation`)))
  (`|SpawnActorFromClass` "/Game/Blueprints/Collectibles/Loot/BatteryLoot_BP.BatteryLoot_BP_C" (`KismetMathLibrary.MakeTransform` (`KismetMathLibrary.MakeVector` _returnvalue_x 1.0 _returnvalue_z)) "Undefined" "OverrideRootScale" null null))

(fn `UserConstructionScript`)