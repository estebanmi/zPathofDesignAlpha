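; BinaryCoinLoot is a collectible coin worth a binary 0 or 1, either preset or randomized, shown with a matching flipbook.
; It pops upward with an impulse on its box collider at spawn.
; Player_BP overlap passes the value to the first BinaryWordsController_BP found in the level and destroys the coin.
; Uncollected coins blink briefly through a FlipFlop delay loop once their lifetime ends, then destroy themselves.
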(event `self.ReceiveBeginPlay`
  (`PrimitiveComponent.AddImpulse` (`self.Box Collider`) (0.0 0.0 100.0) "None" false)
  (if (`self.isRandom`)
    (if (== (`KismetMathLibrary.RandomIntegerInRange` 0 1) 0)
      (set `self.BinaryValue` false)
      (else
        (set `self.BinaryValue` true))))
  (if (`self.BinaryValue`)
    (`PaperFlipbookComponent.SetFlipbook` (`self.PaperFlipbook`) "/Game/Sprites/Collectibles/BinaryCoin/BinaryCoin1.BinaryCoin1")
    (else
      (`PaperFlipbookComponent.SetFlipbook` (`self.PaperFlipbook`) "/Game/Sprites/Player/PlayerGun/Bullet/BinaryCoin0.BinaryCoin0")))
  (`self.DestroyDelay`))

(event `self.Box Collider.OnComponentBeginOverlap`
  (params (OverlappedComponent :type "PrimitiveComponent Object Reference") (OtherActor :type "Actor Object Reference") (OtherComp :type "PrimitiveComponent Object Reference") (OtherBodyIndex :type Integer) (bFromSweep :type Boolean) (SweepResult :type "HitResult Structure (by ref)"))
  (cast `/Game/Blueprints/Player/Player_BP` OtherActor)
  (bind _outactors (`GameplayStatics.GetAllActorsOfClass` "/Game/Blueprints/Player/BinaryWordsController_BP.BinaryWordsController_BP_C"))
  (`/Game/Blueprints/Player/BinaryWordsController_BP.GetBinaryCoin` (`|GetArrayItem` _outactors) (`self.BinaryValue`))
  (`self.K2_DestroyActor`))

(event `DestroyDelay`
  (`KismetSystemLibrary.Delay` (`self.LifeTime`))
  (`/Engine/EditorBlueprintResources/StandardMacros.FlipFlop` :!label _label
    (:`A`
      (`SceneComponent.SetVisibility` (`self.PaperFlipbook`) false false))
    (:`B`
      (`SceneComponent.SetVisibility` (`self.PaperFlipbook`) true false)))
  (`KismetSystemLibrary.Delay` 0.3)
  (if (< (`self.Index`) 5)
    (set `self.Index` (+ (`self.Index`) 1))
    (goto _label)
    (else
      (`self.K2_DestroyActor`))))

(fn `UserConstructionScript`)