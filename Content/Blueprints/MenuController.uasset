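; MenuController is a Blueprint that polls keyboard input for text skipping and a menu hotkey.
; On BeginPlay it caches the Player_BP character, printing an error if the cast fails.
; Each Tick, Enter sets the player's IsSkipText flag, while Escape or Z only prints a "MENU" placeholder.
; Keys are read directly from the player controller rather than through input bindings.
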(event `self.ReceiveBeginPlay`
  (bind _asplayer_bp (cast `/Game/Blueprints/Player/Player_BP` (`GameplayStatics.GetPlayerCharacter` 0))
    (:`then`
      (set `self.PlayerRef` _asplayer_bp))
    (:`CastFailed`
      (`KismetSystemLibrary.PrintString` "MenuController: Player Missing"))))

(event `self.ReceiveTick`
  (params (DeltaSeconds :type "Float (single-precision)"))
  (`self.SkipText`)
  (`self.Menu`))

(event `SkipText`
  (if (`PlayerController.WasInputKeyJustPressed` (`GameplayStatics.GetPlayerController` 0) "Enter")
    (set `/Game/Blueprints/Player/Player_BP.isSkipText` true (`self.PlayerRef`))))

(event `Menu`
  (if (`PlayerController.WasInputKeyJustPressed` (`GameplayStatics.GetPlayerController` 0) "Escape")
    (`KismetSystemLibrary.PrintString` "MENU" :!label _label)
    (elif (`PlayerController.WasInputKeyJustPressed` (`GameplayStatics.GetPlayerController` 0) "Z")
      (goto _label))))

(fn `UserConstructionScript`)