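; Music controller that switches the game's soundtrack between level, pre-boss, boss and victory tracks.
; Level music fades in on BeginPlay, and SetMusic crossfades to the selected track through CurrentMusic and NextMusic, with delays before reassigning the current one.
; Boss music skips the slow crossfade, starting immediately over a quick fade-out.
; Separate events duck volume for pause, restore it with a timeline, or fade out and stop playback.
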(event `self.ReceiveBeginPlay`
  (bind _output_get (set `self.CurrentMusic` (`self.sm_Level`)))
  (`AudioComponent.FadeIn` _output_get 3.0 1.0 0.0))

(event `SetMusic`
  (params (SelectMusic :type "/Game/Blueprints/SelectMusic Enum" :default "NewEnumerator0"))
  (switch `/Game/Blueprints/SelectMusic` SelectMusic
    (:`NewEnumerator0`
      (set `self.NextMusic` (`self.sm_Level`))
      (`AudioComponent.FadeOut` (`self.CurrentMusic`) 3.0 0.0 :!label _label)
      (`KismetSystemLibrary.Delay` 1.0)
      (`AudioComponent.FadeIn` (`self.NextMusic`) 1.0 1.0 0.0)
      (`KismetSystemLibrary.Delay` 2.0)
      (set `self.CurrentMusic` (`self.NextMusic`)))
    (:`NewEnumerator1`
      (set `self.NextMusic` (`self.sm_PreBoss`))
      (goto _label))
    (:`NewEnumerator2`
      (set `self.NextMusic` (`self.sm_Boss`))
      (`AudioComponent.FadeOut` (`self.CurrentMusic`) 0.5 0.0)
      (`AudioComponent.Play` (`self.NextMusic`) 0.0)
      (`KismetSystemLibrary.Delay` 0.2)
      (set `self.CurrentMusic` (`self.NextMusic`)))
    (:`NewEnumerator3`
      (set `self.NextMusic` (`self.sm_Victory`))
      (goto _label))))

(event `PauseVolume`
  (`AudioComponent.SetVolumeMultiplier` (`self.CurrentMusic`) 0.1))

(event `inGameVolume`
  (bind (_direction _risevolume) (`Timeline|RaiseVolumen` :!via `PlayFromStart`)
    (:`Update`
      (`AudioComponent.SetVolumeMultiplier` (`self.CurrentMusic`) _risevolume))))

(event `StopMusic`
  (bind _currentmusic (`self.CurrentMusic`))
  (`AudioComponent.FadeOut` _currentmusic 3.0 0.0)
  (`KismetSystemLibrary.Delay` 3.0)
  (`AudioComponent.Stop` _currentmusic))

(fn `UserConstructionScript`)