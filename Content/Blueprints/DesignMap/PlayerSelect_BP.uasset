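; PlayerSelect_BP is the player's selector on the design map, stepping between linked POIs, starting their dialog and opening their levels.
; Moves are gated by Adventure, Action and Horror levels, and each updates which emotion branch of POI sprites is visible.
; BeginPlay loads two save slots, current POI and levels, then applies pending level-ups that unlock matching POIs.
; Number keys trigger debug level-up, save, load and reset.
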(event `NoLevelUpStart`
  (bind (_returnvalue_x _returnvalue_y _returnvalue_z) (`KismetMathLibrary.BreakVector` (`self.K2_GetActorLocation` (`self.CurrentPOI`))))
  ;[1 1 1] Save Game
  ;;[1 1 1] No Level Up
  (`self.K2_SetActorLocation` (`KismetMathLibrary.MakeVector` _returnvalue_x 110.0 _returnvalue_z))
  (`/Game/Blueprints/DesignMap/POI.StartDialog` (`self.CurrentPOI`)))

(event `DeleteGame`
  ;[1 1 1] Save Game
  ;;[1 1 1] Reset Game
  (`GameplayStatics.DeleteGameInSlot` "0")
  (`GameplayStatics.DeleteGameInSlot` "1")
  (`KismetSystemLibrary.PrintString` "Game Reset"))

(event `SaveGame`
  ;[1 1 1] Save Game
  ;;[1 1 1] Save Game
  (bind _returnvalue (`GameplayStatics.CreateSaveGameObject` "/Game/Blueprints/MySaveGame.MySaveGame_C"))
  (set `self.MySaveGameRef` _returnvalue)
  (`|ExecutionSequence`
    (:`then_0`
      (bind _output_get (set `/Game/Blueprints/MySaveGame.CurrentPOISaved` (`self.CurrentPOI`) (`self.MySaveGameRef`)))
      (`KismetSystemLibrary.PrintString` (`KismetStringLibrary.Concat_StrStr` "POI saved: " (`KismetSystemLibrary.GetDisplayName` _output_get)) true true (struct :`R` 0.019484 :`G` 1.0 :`A` 1.0)))
    (:`then_3`
      (`GameplayStatics.SaveGameToSlot` (`self.MySaveGameRef`) "0")
      (`KismetSystemLibrary.PrintString` "Game Saved" true true (struct :`G` 1.0 :`B` 0.035872 :`A` 1.0)))
    (:`then_4`
      (`self.SaveLevelUp`))))

(event `SaveLevelUp`
  (bind _returnvalue (`GameplayStatics.CreateSaveGameObject` "/Game/Blueprints/MySaveGameLevelUp.MySaveGameLevelUp_C"))
  (bind _output_get (set `self.SaveGameLevelUpRef` _returnvalue))
  (bind _output_get_2 (set `/Game/Blueprints/MySaveGameLevelUp.LevelUpSaved` "NewEnumerator3" _output_get))
  (set `/Game/Blueprints/MySaveGameLevelUp.PlayerLevelsSaved` (`self.PlayerLevels`) _output_get)
  (`GameplayStatics.SaveGameToSlot` _output_get "1")
  (`KismetSystemLibrary.PrintString` (`|GetEnumeratorNameAsString` _output_get_2) true true (struct :`R` 1.0 :`A` 1.0)))

(event `LoadLevelUp`
  (bind _returnvalue (`GameplayStatics.DoesSaveGameExist` "1"))
  (if _returnvalue
    (bind _returnvalue_2 (`GameplayStatics.LoadGameFromSlot` "1"))
    (bind _asmy_save_game_level_up (cast `/Game/Blueprints/MySaveGameLevelUp` _returnvalue_2))
    (set `self.PlayerLevels` (`/Game/Blueprints/MySaveGameLevelUp.PlayerLevelsSaved` _asmy_save_game_level_up))
    (bind _output_get (set `self.LevelUp` (`/Game/Blueprints/MySaveGameLevelUp.LevelUpSaved` _asmy_save_game_level_up)))))

(event `LoadGame`
  ;[1 1 1] Save Game
  ;;[1 1 1] Load Game
  (bind _returnvalue (`GameplayStatics.DoesSaveGameExist` "0"))
  (if _returnvalue
    (bind _returnvalue_2 (`GameplayStatics.LoadGameFromSlot` "0"))
    (bind _asmy_save_game (cast `/Game/Blueprints/MySaveGame` _returnvalue_2))
    (set `self.MySaveGameRef` _asmy_save_game)
    (`|ExecutionSequence`
      (:`then_0`
        (bind _output_get (set `self.CurrentPOI` (`/Game/Blueprints/MySaveGame.CurrentPOISaved` (`self.MySaveGameRef`))))
        (`KismetSystemLibrary.PrintString` (`KismetStringLibrary.Concat_StrStr` "POI saved: " (`KismetSystemLibrary.GetDisplayName` _output_get)) true true (struct :`R` 0.019484 :`G` 1.0 :`A` 1.0)))
      (:`then_1`
        (`self.SetVisibilties`)))
    (else
      (set `self.CurrentPOI` (`self.StartingPOI`))
      (`self.SaveGame`)
      (`KismetSystemLibrary.PrintString` "Creating new saved game")
      (`self.StartVisibilities`)
      (`self.NoLevelUpStart`))))

(event `First Location`
  (switch `/Game/Blueprints/LevelUp` (stale `LoadLevelUp` _output_get)
    (:`NewEnumerator3`
      (`self.NoLevelUpStart`))
    (:`NewEnumerator0`
      (`self.LevelUpAdventure`))
    (:`NewEnumerator1`
      (`self.LevelUpAction`))
    (:`NewEnumerator2`
      (`self.LevelUpHorror`)))
  (`KismetSystemLibrary.PrintString` "Hello" true true (struct :`R` 1.0 :`A` 1.0))
  (`self.SaveLevelUp`))

(event `levelssss`
  (bind (_playerlevels_leveladventure _playerlevels_levelaction _playerlevels_levelhorror) (break `/Game/Blueprints/DesignMap/PlayerLevels` (`self.PlayerLevels`)))
  (`KismetSystemLibrary.PrintString` (`KismetStringLibrary.Concat_StrStr` (`KismetStringLibrary.Conv_IntToString` _playerlevels_leveladventure) " - " (`KismetStringLibrary.Conv_IntToString` _playerlevels_levelaction) " - " (`KismetStringLibrary.Conv_IntToString` _playerlevels_levelhorror)) true true (struct :`R` 1.0 :`G` 0.506951 :`A` 1.0) 0.01))

(event `LevelUpHorror`
  (bind (_playerlevels_leveladventure _playerlevels_levelaction _playerlevels_levelhorror) (break `/Game/Blueprints/DesignMap/PlayerLevels` (`self.PlayerLevels`)))
  (bind (_playerlevels_leveladventure_2 _playerlevels_levelaction_2 _playerlevels_levelhorror_2) (break `/Game/Blueprints/DesignMap/PlayerLevels` (`self.PlayerLevels`)))
  ;[1 1 1] LevelUp Horror
  (set `self.IndexPOI` 0)
  (bind _foundwidgets (`WidgetBlueprintLibrary.GetAllWidgetsOfClass` "/Game/Widgets/DialogOFF_HUD.DialogOFF_HUD_C"))
  (`Widget.RemoveFromParent` _foundwidgets)
  (set `self.PlayerLevels` (make `/Game/Blueprints/DesignMap/PlayerLevels` _playerlevels_leveladventure _playerlevels_levelaction (+ _playerlevels_levelhorror 1)))
  (bind _outactors (`GameplayStatics.GetAllActorsOfClass` "/Game/Blueprints/DesignMap/POI.POI_C"))
  (bind _output (`|GetArrayItem` _outactors (`self.IndexPOI`)))
  (`/Engine/EditorBlueprintResources/StandardMacros.IsValid` _output :!label _label
    (:`Is Valid`
      (switch `/Game/Blueprints/DesignMap/GameEmotion` (`/Game/Blueprints/DesignMap/POI.GameEmotion` _output)
        (:`NewEnumerator3`
          _)
        (:`NewEnumerator4`
          _)
        (:`NewEnumerator0`
          _)
        (:`NewEnumerator5`
          _)
        (:`NewEnumerator1`
          _)
        (:`NewEnumerator6`
          (bind (_levelneeded_leveladventure _levelneeded_levelaction _levelneeded_levelhorror) (break `/Game/Blueprints/DesignMap/PlayerLevels` (`/Game/Blueprints/DesignMap/POI.LevelNeeded` _output)))
          (if (== _playerlevels_levelhorror_2 _levelneeded_levelhorror) :!label _label_2
            (set `self.InputDisabled` true)
            (`/Game/Blueprints/DesignMap/POI.UnlockPOI` _output)))
        (:`NewEnumerator2`
          (goto _label_2)))
      (if (< (`self.IndexPOI`) (`KismetArrayLibrary.Array_Length` _outactors))
        (set `self.IndexPOI` (+ (`self.IndexPOI`) 1))
        (goto _label)))))

(event `Key|Enter`
  (params (Key :type "Key Structure"))
  (bind _playerlevelssaved_leveladventure (break `/Game/Blueprints/DesignMap/PlayerLevels` (`/Game/Blueprints/MySaveGameLevelUp.PlayerLevelsSaved` (`self.SaveGameLevelUpRef`))))
  ;[1 1 1] Enter POI
  (:`Pressed`
    (if (not (`self.InputDisabled`)) :!label _label_3
      (bind _foundwidgets (`WidgetBlueprintLibrary.GetAllWidgetsOfClass` "/Game/Widgets/DialogNPC_HUD.DialogNPC_HUD_C"))
      (`Widget.RemoveFromParent` _foundwidgets)
      (if (!= (`/Game/Blueprints/DesignMap/POI.LevelToOpen` (`self.CurrentPOI`)) "None")
        (set `self.InputDisabled` true)
        (`GameplayStatics.PlaySound2D` "/Game/Sound/SFXs/DesignMap/sfx_EnterPOI_Cue.sfx_EnterPOI_Cue" 1.0 1.0 0.0 null null)
        (`self.BinaryBumper`)
        (`self.SaveGame`)
        (`self.SaveLevelUp`)
        (`KismetSystemLibrary.PrintString` (`KismetStringLibrary.Conv_IntToString` _playerlevelssaved_leveladventure) true true (struct :`R` 0.978041 :`G` 0.976708 :`B` 1.0 :`A` 1.0))
        (else
          (`GameplayStatics.PlaySound2D` "/Game/Sound/SFXs/DesignMap/sfx_DMMoveNot_Cue.sfx_DMMoveNot_Cue" 1.0 1.0 0.0 null null))))))

(event `Key|LeftMouseButton`
  (params (Key :type "Key Structure"))
  ;[1 1 1] Enter POI
  (:`Pressed`
    (goto _label_3)))

(event `LevelUpAction`
  (bind (_playerlevels_leveladventure _playerlevels_levelaction _playerlevels_levelhorror) (break `/Game/Blueprints/DesignMap/PlayerLevels` (`self.PlayerLevels`)))
  (bind (_playerlevels_leveladventure_2 _playerlevels_levelaction_2) (break `/Game/Blueprints/DesignMap/PlayerLevels` (`self.PlayerLevels`)))
  ;[1 1 1] LevelUp Action
  (set `self.IndexPOI` 0)
  (bind _foundwidgets (`WidgetBlueprintLibrary.GetAllWidgetsOfClass` "/Game/Widgets/DialogOFF_HUD.DialogOFF_HUD_C"))
  (`Widget.RemoveFromParent` _foundwidgets)
  (set `self.PlayerLevels` (make `/Game/Blueprints/DesignMap/PlayerLevels` _playerlevels_leveladventure (+ _playerlevels_levelaction 1) _playerlevels_levelhorror))
  (bind _outactors (`GameplayStatics.GetAllActorsOfClass` "/Game/Blueprints/DesignMap/POI.POI_C"))
  (bind _output (`|GetArrayItem` _outactors (`self.IndexPOI`)))
  (`/Engine/EditorBlueprintResources/StandardMacros.IsValid` _output :!label _label_4
    (:`Is Valid`
      (switch `/Game/Blueprints/DesignMap/GameEmotion` (`/Game/Blueprints/DesignMap/POI.GameEmotion` _output)
        (:`NewEnumerator3`
          _)
        (:`NewEnumerator4`
          _)
        (:`NewEnumerator0`
          _)
        (:`NewEnumerator5`
          (bind (_levelneeded_leveladventure _levelneeded_levelaction) (break `/Game/Blueprints/DesignMap/PlayerLevels` (`/Game/Blueprints/DesignMap/POI.LevelNeeded` _output)))
          (if (== _playerlevels_levelaction_2 _levelneeded_levelaction) :!label _label_5
            (set `self.InputDisabled` true)
            (`/Game/Blueprints/DesignMap/POI.UnlockPOI` _output)))
        (:`NewEnumerator1`
          (goto _label_5))
        (:`NewEnumerator6`
          _)
        (:`NewEnumerator2`
          _))
      (if (< (`self.IndexPOI`) (`KismetArrayLibrary.Array_Length` _outactors))
        (set `self.IndexPOI` (+ (`self.IndexPOI`) 1))
        (goto _label_4)))))

(event `Key|SpaceBar`
  (params (Key :type "Key Structure"))
  (bind _currentpoi (`self.CurrentPOI`))
  ;[1 1 1] Skip Text
  (:`Pressed`
    (if (`/Game/Blueprints/DesignMap/POI.isTalking` _currentpoi)
      (set `/Game/Blueprints/DesignMap/POI.IsSkipText` true _currentpoi))))

(event `LevelUpAdventure`
  (bind (_playerlevels_leveladventure _playerlevels_levelaction _playerlevels_levelhorror) (break `/Game/Blueprints/DesignMap/PlayerLevels` (`self.PlayerLevels`)))
  (bind _playerlevels_leveladventure_2 (break `/Game/Blueprints/DesignMap/PlayerLevels` (`self.PlayerLevels`)))
  ;[1 1 1] LevelUp Adventure
  (set `self.IndexPOI` 0)
  (bind _foundwidgets (`WidgetBlueprintLibrary.GetAllWidgetsOfClass` "/Game/Widgets/DialogOFF_HUD.DialogOFF_HUD_C"))
  (`Widget.RemoveFromParent` _foundwidgets)
  (bind _output_get (set `self.PlayerLevels` (make `/Game/Blueprints/DesignMap/PlayerLevels` (+ _playerlevels_leveladventure 1) _playerlevels_levelaction _playerlevels_levelhorror)))
  (`KismetSystemLibrary.PrintString` (`KismetStringLibrary.Concat_StrStr` (`KismetStringLibrary.Conv_IntToString` _playerlevels_leveladventure) " + 1 = " (`KismetStringLibrary.Conv_IntToString` (break `/Game/Blueprints/DesignMap/PlayerLevels` _output_get))) true true (struct :`R` 1.0 :`B` 0.934574 :`A` 1.0))
  (bind _outactors (`GameplayStatics.GetAllActorsOfClass` "/Game/Blueprints/DesignMap/POI.POI_C"))
  (bind _output (`|GetArrayItem` _outactors (`self.IndexPOI`)))
  (`/Engine/EditorBlueprintResources/StandardMacros.IsValid` _output :!label _label_6
    (:`Is Valid`
      (switch `/Game/Blueprints/DesignMap/GameEmotion` (`/Game/Blueprints/DesignMap/POI.GameEmotion` _output)
        (:`NewEnumerator3`
          _)
        (:`NewEnumerator4`
          (bind _levelneeded_leveladventure (break `/Game/Blueprints/DesignMap/PlayerLevels` (`/Game/Blueprints/DesignMap/POI.LevelNeeded` _output)))
          (if (== _playerlevels_leveladventure_2 _levelneeded_leveladventure) :!label _label_7
            (set `self.InputDisabled` true)
            (`/Game/Blueprints/DesignMap/POI.UnlockPOI` _output)))
        (:`NewEnumerator0`
          (goto _label_7))
        (:`NewEnumerator5`
          _)
        (:`NewEnumerator1`
          _)
        (:`NewEnumerator6`
          _)
        (:`NewEnumerator2`
          _))
      (if (< (`self.IndexPOI`) (`KismetArrayLibrary.Array_Length` _outactors))
        (set `self.IndexPOI` (+ (`self.IndexPOI`) 1))
        (goto _label_6)))))

(event `BinaryBumper`
  ;[1 1 1] Binary Bumper
  (bind _returnvalue (`|CreateWidget` "/Game/Widgets/BinaryBumper_HUD.BinaryBumper_HUD_C"))
  (`UserWidget.AddToViewport` _returnvalue 0)
  (bind _outactors (`GameplayStatics.GetAllActorsOfClass` "/Game/Blueprints/Level/BinaryBumperController_BP.BinaryBumperController_BP_C"))
  (`/Game/Blueprints/Level/BinaryBumperController_BP.Adding01` (`|GetArrayItem` _outactors))
  (`KismetSystemLibrary.Delay` 0.3)
  (`GameplayStatics.OpenLevel` (`/Game/Blueprints/DesignMap/POI.LevelToOpen` (`self.CurrentPOI`))))

(event `Key|Four`
  (params (Key :type "Key Structure"))
  (:`Pressed`
    (`self.SaveGame`)))

(event `Key|One`
  (params (Key :type "Key Structure"))
  (:`Pressed`
    (`self.LevelUpAdventure`)))

(event `self.ReceiveBeginPlay`
  (`|ExecutionSequence`
    (:`then_0`
      (`self.LoadLevelUp`))
    (:`then_1`
      (`self.LoadGame`))
    (:`then_2`
      (set `self.InputDisabled` true))
    (:`then_4`
      (`self.First Location`))))

(event `Key|Two`
  (params (Key :type "Key Structure"))
  (:`Pressed`
    (`self.LevelUpAction`)))

(event `Key|Five`
  (params (Key :type "Key Structure"))
  (:`Pressed`
    (`self.LoadGame`)))

(event `self.ReceiveTick`
  (params (DeltaSeconds :type "Float (single-precision)"))
  (`self.levelssss`))

(event `Key|Three`
  (params (Key :type "Key Structure"))
  (:`Pressed`
    (`self.LevelUpHorror`)))

(event `Key|Six`
  (params (Key :type "Key Structure"))
  (:`Pressed`
    (`self.DeleteGame`)))

(event `Key|A`
  (params (Key :type "Key Structure"))
  (bind (_playerlevels_leveladventure _playerlevels_levelaction _playerlevels_levelhorror) (break `/Game/Blueprints/DesignMap/PlayerLevels` (`self.PlayerLevels`)))
  (bind _poileft (`/Game/Blueprints/DesignMap/POI.POIleft` (`self.CurrentPOI`)))
  (bind (_returnvalue_x _returnvalue_y _returnvalue_z) (`KismetMathLibrary.BreakVector` (`self.K2_GetActorLocation` _poileft)))
  (bind (_levelneeded_leveladventure _levelneeded_levelaction _levelneeded_levelhorror) (break `/Game/Blueprints/DesignMap/PlayerLevels` (`/Game/Blueprints/DesignMap/POI.LevelNeeded` _poileft)))
  ;[1 1 1] Moving through POIs
  (:`Pressed`
    (if (not (`self.InputDisabled`)) :!label _label_8
      (`/Engine/EditorBlueprintResources/StandardMacros.IsValid` _poileft
        (:`Is Valid`
          (if (>= _playerlevels_leveladventure _levelneeded_leveladventure)
            (bind _foundwidgets (`WidgetBlueprintLibrary.GetAllWidgetsOfClass` "/Game/Widgets/DialogNPC_HUD.DialogNPC_HUD_C" :!label _label_9))
            (`Widget.RemoveFromParent` _foundwidgets)
            (`self.K2_SetActorLocation` (`KismetMathLibrary.MakeVector` _returnvalue_x 110.0 _returnvalue_z))
            (`GameplayStatics.PlaySound2D` "/Game/Sound/SFXs/DesignMap/sfx_DMMove_Cue.sfx_DMMove_Cue" 1.0 1.0 0.0 null null)
            (bind _output_get (set `self.CurrentPOI` _poileft))
            (`/Game/Blueprints/DesignMap/POI.StartDialog` _output_get)
            (`self.SetVisibilties`)
            (`self.SaveGame`)
            (elif (>= _playerlevels_levelaction _levelneeded_levelaction)
              (goto _label_9)
              (elif (>= _playerlevels_levelhorror _levelneeded_levelhorror)
                (goto _label_9)
                (else
                  (`GameplayStatics.PlaySound2D` "/Game/Sound/SFXs/DesignMap/sfx_DMMoveNot_Cue.sfx_DMMoveNot_Cue" 1.0 1.0 0.0 null null :!label _label_10))))))
        (:`Is Not Valid`
          (goto _label_10))))))

(event `Key|Left`
  (params (Key :type "Key Structure"))
  ;[1 1 1] Moving through POIs
  (:`Pressed`
    (goto _label_8)))

(event `Key|D`
  (params (Key :type "Key Structure"))
  (bind (_playerlevels_leveladventure _playerlevels_levelaction _playerlevels_levelhorror) (break `/Game/Blueprints/DesignMap/PlayerLevels` (`self.PlayerLevels`)))
  (bind _poiright (`/Game/Blueprints/DesignMap/POI.POIright` (`self.CurrentPOI`)))
  (bind (_returnvalue_x _returnvalue_y _returnvalue_z) (`KismetMathLibrary.BreakVector` (`self.K2_GetActorLocation` _poiright)))
  (bind (_levelneeded_leveladventure _levelneeded_levelaction _levelneeded_levelhorror) (break `/Game/Blueprints/DesignMap/PlayerLevels` (`/Game/Blueprints/DesignMap/POI.LevelNeeded` _poiright)))
  ;[1 1 1] Moving through POIs
  (:`Pressed`
    (if (not (`self.InputDisabled`)) :!label _label_11
      (`/Engine/EditorBlueprintResources/StandardMacros.IsValid` _poiright
        (:`Is Valid`
          (if (>= _playerlevels_leveladventure _levelneeded_leveladventure)
            (bind _foundwidgets (`WidgetBlueprintLibrary.GetAllWidgetsOfClass` "/Game/Widgets/DialogNPC_HUD.DialogNPC_HUD_C" :!label _label_12))
            (`Widget.RemoveFromParent` _foundwidgets)
            (`self.K2_SetActorLocation` (`KismetMathLibrary.MakeVector` _returnvalue_x 110.0 _returnvalue_z))
            (`GameplayStatics.PlaySound2D` "/Game/Sound/SFXs/DesignMap/sfx_DMMove_Cue.sfx_DMMove_Cue" 1.0 1.0 0.0 null null)
            (bind _output_get (set `self.CurrentPOI` _poiright))
            (`/Game/Blueprints/DesignMap/POI.StartDialog` _output_get)
            (`self.SetVisibilties`)
            (`self.SaveGame`)
            (elif (>= _playerlevels_levelaction _levelneeded_levelaction)
              (goto _label_12)
              (elif (>= _playerlevels_levelhorror _levelneeded_levelhorror)
                (goto _label_12)
                (else
                  (`GameplayStatics.PlaySound2D` "/Game/Sound/SFXs/DesignMap/sfx_DMMoveNot_Cue.sfx_DMMoveNot_Cue" 1.0 1.0 0.0 null null :!label _label_13))))))
        (:`Is Not Valid`
          (goto _label_13))))))

(event `Key|Right`
  (params (Key :type "Key Structure"))
  ;[1 1 1] Moving through POIs
  (:`Pressed`
    (goto _label_11)))

(event `Key|W`
  (params (Key :type "Key Structure"))
  (bind (_playerlevels_leveladventure _playerlevels_levelaction _playerlevels_levelhorror) (break `/Game/Blueprints/DesignMap/PlayerLevels` (`self.PlayerLevels`)))
  (bind _poiup (`/Game/Blueprints/DesignMap/POI.POIup` (`self.CurrentPOI`)))
  (bind (_returnvalue_x _returnvalue_y _returnvalue_z) (`KismetMathLibrary.BreakVector` (`self.K2_GetActorLocation` _poiup)))
  (bind (_levelneeded_leveladventure _levelneeded_levelaction _levelneeded_levelhorror) (break `/Game/Blueprints/DesignMap/PlayerLevels` (`/Game/Blueprints/DesignMap/POI.LevelNeeded` _poiup)))
  ;[1 1 1] Moving through POIs
  (:`Pressed`
    (if (not (`self.InputDisabled`)) :!label _label_14
      (`/Engine/EditorBlueprintResources/StandardMacros.IsValid` _poiup
        (:`Is Valid`
          (if (>= _playerlevels_leveladventure _levelneeded_leveladventure)
            (bind _foundwidgets (`WidgetBlueprintLibrary.GetAllWidgetsOfClass` "/Game/Widgets/DialogNPC_HUD.DialogNPC_HUD_C" :!label _label_15))
            (`Widget.RemoveFromParent` _foundwidgets)
            (`self.K2_SetActorLocation` (`KismetMathLibrary.MakeVector` _returnvalue_x 110.0 _returnvalue_z))
            (`GameplayStatics.PlaySound2D` "/Game/Sound/SFXs/DesignMap/sfx_DMMove_Cue.sfx_DMMove_Cue" 1.0 1.0 0.0 null null)
            (bind _output_get (set `self.CurrentPOI` _poiup))
            (`/Game/Blueprints/DesignMap/POI.StartDialog` _output_get)
            (`self.SetVisibilties`)
            (`self.SaveGame`)
            (elif (>= _playerlevels_levelaction _levelneeded_levelaction)
              (goto _label_15)
              (elif (>= _playerlevels_levelhorror _levelneeded_levelhorror)
                (goto _label_15)
                (else
                  (`GameplayStatics.PlaySound2D` "/Game/Sound/SFXs/DesignMap/sfx_DMMoveNot_Cue.sfx_DMMoveNot_Cue" 1.0 1.0 0.0 null null :!label _label_16))))))
        (:`Is Not Valid`
          (goto _label_16))))))

(event `Key|Up`
  (params (Key :type "Key Structure"))
  ;[1 1 1] Moving through POIs
  (:`Pressed`
    (goto _label_14)))

(event `Key|S`
  (params (Key :type "Key Structure"))
  (bind (_playerlevels_leveladventure _playerlevels_levelaction _playerlevels_levelhorror) (break `/Game/Blueprints/DesignMap/PlayerLevels` (`self.PlayerLevels`)))
  (bind _poidown (`/Game/Blueprints/DesignMap/POI.POIdown` (`self.CurrentPOI`)))
  (bind (_returnvalue_x _returnvalue_y _returnvalue_z) (`KismetMathLibrary.BreakVector` (`self.K2_GetActorLocation` _poidown)))
  (bind (_levelneeded_leveladventure _levelneeded_levelaction _levelneeded_levelhorror) (break `/Game/Blueprints/DesignMap/PlayerLevels` (`/Game/Blueprints/DesignMap/POI.LevelNeeded` _poidown)))
  ;[1 1 1] Moving through POIs
  (:`Pressed`
    (if (not (`self.InputDisabled`)) :!label _label_17
      (`/Engine/EditorBlueprintResources/StandardMacros.IsValid` _poidown
        (:`Is Valid`
          (if (>= _playerlevels_leveladventure _levelneeded_leveladventure)
            (bind _foundwidgets (`WidgetBlueprintLibrary.GetAllWidgetsOfClass` "/Game/Widgets/DialogNPC_HUD.DialogNPC_HUD_C" :!label _label_18))
            (`Widget.RemoveFromParent` _foundwidgets)
            (`self.K2_SetActorLocation` (`KismetMathLibrary.MakeVector` _returnvalue_x 110.0 _returnvalue_z))
            (`GameplayStatics.PlaySound2D` "/Game/Sound/SFXs/DesignMap/sfx_DMMove_Cue.sfx_DMMove_Cue" 1.0 1.0 0.0 null null)
            (bind _output_get (set `self.CurrentPOI` _poidown))
            (`/Game/Blueprints/DesignMap/POI.StartDialog` _output_get)
            (`self.SetVisibilties`)
            (`self.SaveGame`)
            (elif (>= _playerlevels_levelaction _levelneeded_levelaction)
              (goto _label_18)
              (elif (>= _playerlevels_levelhorror _levelneeded_levelhorror)
                (goto _label_18)
                (else
                  (`GameplayStatics.PlaySound2D` "/Game/Sound/SFXs/DesignMap/sfx_DMMoveNot_Cue.sfx_DMMoveNot_Cue" 1.0 1.0 0.0 null null :!label _label_19))))))
        (:`Is Not Valid`
          (goto _label_19))))))

(event `Key|Down`
  (params (Key :type "Key Structure"))
  ;[1 1 1] Moving through POIs
  (:`Pressed`
    (goto _label_17)))

(event `SetAdvVis`
  ;[1 1 1] Set POI Visibilities
  (bind _outactors (`GameplayStatics.GetAllActorsOfClass` "/Game/Blueprints/DesignMap/POI.POI_C" :!label _label_20))
  (bind _output (`|GetArrayItem` _outactors (`self.IndexVis`)))
  (switch `/Game/Blueprints/DesignMap/GameEmotion` (`/Game/Blueprints/DesignMap/POI.GameEmotion` _output) :!label _label_21
    (:`NewEnumerator3`
      _)
    (:`NewEnumerator4`
      _)
    (:`NewEnumerator0`
      (bind _papersprite (`/Game/Blueprints/DesignMap/POI.PaperSprite` _output))
      (`SceneComponent.SetVisibility` _papersprite true true))
    (:`NewEnumerator5`
      _)
    (:`NewEnumerator1`
      (`SceneComponent.SetVisibility` _papersprite false true :!label _label_22))
    (:`NewEnumerator6`
      _)
    (:`NewEnumerator2`
      (goto _label_22)))
  (if (< (`self.IndexVis`) (- (`KismetArrayLibrary.Array_Length` _outactors) 1))
    (set `self.IndexVis` (+ (`self.IndexVis`) 1))
    (goto _label_21)
    (else
      (set `self.IndexVis` 0))))

(event `SetVisibilties`
  (bind _gameemotion (`/Game/Blueprints/DesignMap/POI.GameEmotion` (`self.CurrentPOI`)))
  ;[1 1 1] Set POI Visibilities
  (`KismetSystemLibrary.PrintString` (`KismetStringLibrary.Concat_StrStr` "Set Visibilities: " (`|GetEnumeratorNameAsString` _gameemotion)))
  (switch `/Game/Blueprints/DesignMap/GameEmotion` _gameemotion
    (:`NewEnumerator3`
      ;[1 1 1] Start Visibilities
      (bind _outactors (`GameplayStatics.GetAllActorsOfClass` "/Game/Blueprints/DesignMap/POI.POI_C" :!label _label_23))
      (bind _output (`|GetArrayItem` _outactors (`self.IndexVis`)))
      (switch `/Game/Blueprints/DesignMap/GameEmotion` (`/Game/Blueprints/DesignMap/POI.GameEmotion` _output) :!label _label_24
        (:`NewEnumerator3`
          _)
        (:`NewEnumerator4`
          _)
        (:`NewEnumerator0`
          (`SceneComponent.SetVisibility` (`/Game/Blueprints/DesignMap/POI.PaperSprite` _output) false true :!label _label_25))
        (:`NewEnumerator5`
          _)
        (:`NewEnumerator1`
          (goto _label_25))
        (:`NewEnumerator6`
          _)
        (:`NewEnumerator2`
          (goto _label_25)))
      (if (< (`self.IndexVis`) (- (`KismetArrayLibrary.Array_Length` _outactors) 1))
        (set `self.IndexVis` (+ (`self.IndexVis`) 1))
        (goto _label_24)
        (else
          (set `self.IndexVis` 0))))
    (:`NewEnumerator4`
      (goto _label_20))
    (:`NewEnumerator0`
      (goto _label_20))
    (:`NewEnumerator5`
      (bind _outactors_2 (`GameplayStatics.GetAllActorsOfClass` "/Game/Blueprints/DesignMap/POI.POI_C" :!label _label_26))
      (bind _output_2 (`|GetArrayItem` _outactors_2 (`self.IndexVis`)))
      (switch `/Game/Blueprints/DesignMap/GameEmotion` (`/Game/Blueprints/DesignMap/POI.GameEmotion` _output_2) :!label _label_27
        (:`NewEnumerator3`
          _)
        (:`NewEnumerator4`
          _)
        (:`NewEnumerator0`
          (bind _papersprite (`/Game/Blueprints/DesignMap/POI.PaperSprite` _output_2))
          (`SceneComponent.SetVisibility` _papersprite false true :!label _label_28))
        (:`NewEnumerator5`
          _)
        (:`NewEnumerator1`
          (`SceneComponent.SetVisibility` _papersprite true true))
        (:`NewEnumerator6`
          _)
        (:`NewEnumerator2`
          (goto _label_28)))
      (if (< (`self.IndexVis`) (- (`KismetArrayLibrary.Array_Length` _outactors_2) 1))
        (set `self.IndexVis` (+ (`self.IndexVis`) 1))
        (goto _label_27)
        (else
          (set `self.IndexVis` 0))))
    (:`NewEnumerator1`
      (goto _label_26))
    (:`NewEnumerator6`
      (bind _outactors_3 (`GameplayStatics.GetAllActorsOfClass` "/Game/Blueprints/DesignMap/POI.POI_C" :!label _label_29))
      (bind _output_3 (`|GetArrayItem` _outactors_3 (`self.IndexVis`)))
      (switch `/Game/Blueprints/DesignMap/GameEmotion` (`/Game/Blueprints/DesignMap/POI.GameEmotion` _output_3) :!label _label_30
        (:`NewEnumerator3`
          _)
        (:`NewEnumerator4`
          _)
        (:`NewEnumerator0`
          (bind _papersprite_2 (`/Game/Blueprints/DesignMap/POI.PaperSprite` _output_3))
          (`SceneComponent.SetVisibility` _papersprite_2 false true :!label _label_31))
        (:`NewEnumerator5`
          _)
        (:`NewEnumerator1`
          (goto _label_31))
        (:`NewEnumerator6`
          _)
        (:`NewEnumerator2`
          (`SceneComponent.SetVisibility` _papersprite_2 true true)))
      (if (< (`self.IndexVis`) (- (`KismetArrayLibrary.Array_Length` _outactors_3) 1))
        (set `self.IndexVis` (+ (`self.IndexVis`) 1))
        (goto _label_30)
        (else
          (set `self.IndexVis` 0))))
    (:`NewEnumerator2`
      (goto _label_29))))

(event `SetActionVis`
  ;[1 1 1] Set POI Visibilities
  (goto _label_26))

(event `SetHorrorVis`
  ;[1 1 1] Set POI Visibilities
  (goto _label_29))

(event `StartVisibilities`
  ;[1 1 1] Start Visibilities
  (goto _label_23))

(fn `UserConstructionScript`)