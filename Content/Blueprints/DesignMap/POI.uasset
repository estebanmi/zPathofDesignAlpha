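; Design-map point of interest that starts locked and, when unlocked, becomes the player selector's current location and plays its dialog.
; UnlockPOI flickers the sprite, opens and destroys the locker, moves the selector, saves, then updates Adventure, Action or Horror visuals and level by GameEmotion.
; BeginPlay removes the locker if any saved genre level meets LevelNeeded.
; Dialog uses a typewriter macro with per-letter sound, and Tick restores input on any key afterwards.
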(event `UnlockPOI`
  (bind (_returnvalue_x _returnvalue_y _returnvalue_z) (`KismetMathLibrary.BreakVector` (`self.K2_GetActorLocation`)))
  (bind _locker (`self.Locker`))
  (bind _playerselectref (`self.PlayerSelectRef`))
  (bind _playerselectref_2 (`self.PlayerSelectRef`))
  (bind _playerselectref_3 (`self.PlayerSelectRef`))
  ;[1 1 1] Unlock POI
  (`GameplayStatics.PlaySound2D` "/Game/Sound/SFXs/DesignMap/sfx_DMUnlockPOI_Cue.sfx_DMUnlockPOI_Cue" 1.0 1.0 0.0 null null)
  (`self.Flickering`)
  (`KismetSystemLibrary.Delay` (* (`self.FlickeringDelay`) 6.0))
  (`/Engine/EditorBlueprintResources/StandardMacros.IsValid` _locker
    (:`Is Valid`
      (`PaperSpriteComponent.SetSprite` _locker "/Game/Sprites/DesignMap/POI/truePOIs/POIs_LockerOpen.POIs_LockerOpen")
      (`GameplayStatics.PlaySound2D` "/Game/Sound/SFXs/DesignMap/sfx_DMLockerOpen_Cue.sfx_DMLockerOpen_Cue" 1.0 1.0 0.0 null null)
      (`KismetSystemLibrary.Delay` 0.5)
      (`self.K2_SetActorLocation` (`self.PlayerSelectRef`) (`KismetMathLibrary.MakeVector` _returnvalue_x 110.0 _returnvalue_z) false false)
      (set `/Game/Blueprints/DesignMap/PlayerSelect_BP.CurrentPOI` self (`self.PlayerSelectRef`))
      (`ActorComponent.K2_DestroyComponent` (`self.Locker`))
      (set `self.AlreadyOpened` true)
      (`/Game/Blueprints/DesignMap/PlayerSelect_BP.SaveGame` (`self.PlayerSelectRef`))
      (set `/Game/Blueprints/DesignMap/PlayerSelect_BP.InputDisabled` false _playerselectref_2)
      (`self.StartDialog` (`/Game/Blueprints/DesignMap/PlayerSelect_BP.CurrentPOI` _playerselectref_2))
      (switch `/Game/Blueprints/DesignMap/GameEmotion` (`self.GameEmotion`)
        (:`NewEnumerator4`
          (`/Game/Blueprints/DesignMap/PlayerSelect_BP.SetAdvVis` _playerselectref :!label _label))
        (:`NewEnumerator0`
          (goto _label))
        (:`NewEnumerator5`
          (`/Game/Blueprints/DesignMap/PlayerSelect_BP.SetActionVis` _playerselectref :!label _label_2))
        (:`NewEnumerator1`
          (goto _label_2))
        (:`NewEnumerator6`
          (`/Game/Blueprints/DesignMap/PlayerSelect_BP.SetHorrorVis` _playerselectref :!label _label_3))
        (:`NewEnumerator2`
          (goto _label_3)))
      (`/Game/Blueprints/DesignMap/PlayerSelect_BP.SetPlayerLevel` _playerselectref_3)
      (`/Game/Blueprints/DesignMap/PlayerSelect_BP.SaveGame` _playerselectref_3))))

(event `self.ReceiveBeginPlay`
  (bind (_levelneeded_leveladventure _levelneeded_levelaction _levelneeded_levelhorror) (break `/Game/Blueprints/DesignMap/PlayerLevels` (`self.LevelNeeded`)))
  ;[1 1 1] Begin Play
  (`PaperSpriteComponent.SetSprite` (`self.PaperSprite`) (`self.Sprite`))
  (bind _asplayer_select_bp (cast `/Game/Blueprints/DesignMap/PlayerSelect_BP` (`GameplayStatics.GetPlayerPawn` 0)))
  (set `self.PlayerSelectRef` _asplayer_select_bp)
  (if (`self.AlreadyOpened`)
    (`ActorComponent.K2_DestroyComponent` (`self.Locker`) :!label _label_4)
    (set `self.AlreadyOpened` true)
    (else
      (bind _returnvalue (`GameplayStatics.DoesSaveGameExist` "2"))
      (if _returnvalue
        (bind _returnvalue_2 (`GameplayStatics.LoadGameFromSlot` "2"))
        (bind _asmy_save_game_player_levels (cast `/Game/Blueprints/MySaveGamePlayerLevels` _returnvalue_2))
        (bind (_playerlevelssaved_leveladventure _playerlevelssaved_levelaction _playerlevelssaved_levelhorror) (break `/Game/Blueprints/DesignMap/PlayerLevels` (`/Game/Blueprints/MySaveGamePlayerLevels.PlayerLevelsSaved` _asmy_save_game_player_levels)))
        (if (>= _playerlevelssaved_leveladventure _levelneeded_leveladventure)
          (goto _label_4)
          (elif (>= _playerlevelssaved_levelaction _levelneeded_levelaction)
            (goto _label_4)
            (elif (>= _playerlevelssaved_levelhorror _levelneeded_levelhorror)
              (goto _label_4))))))))

(event `Flickering`
  ;[1 1 1] Flickering
  (if (not (`self.AlreadyOpened`))
    (`/Engine/EditorBlueprintResources/StandardMacros.FlipFlop` :!label _label_5
      (:`A`
        (`PaperSpriteComponent.SetSprite` (`self.PaperSprite`) (`self.SpriteB`)))
      (:`B`
        (`PaperSpriteComponent.SetSprite` (`self.PaperSprite`) (`self.Sprite`))))
    (`KismetSystemLibrary.Delay` (`self.FlickeringDelay`))
    (if (< (`self.flickeringIndex`) 6)
      (set `self.flickeringIndex` (+ (`self.flickeringIndex`) 1))
      (goto _label_5)
      (else
        (`PaperSpriteComponent.SetSprite` (`self.PaperSprite`) (`self.Sprite`))
        (set `self.flickeringIndex` 0)))))

(event `StartDialog`
  ;[1 1 1] Start Dialog
  (set `/Game/Blueprints/DesignMap/PlayerSelect_BP.InputDisabled` true (`self.PlayerSelectRef`))
  (bind _foundwidgets (`WidgetBlueprintLibrary.GetAllWidgetsOfClass` "/Game/Widgets/DialogOFF_HUD.DialogOFF_HUD_C"))
  (`Widget.RemoveFromParent` _foundwidgets)
  (bind _returnvalue (`|CreateWidget` "/Game/Widgets/DialogOFF_HUD.DialogOFF_HUD_C"))
  (`UserWidget.AddToViewport` _returnvalue 0)
  (set `self.WidgetRef` _returnvalue)
  (`self.ScrollingText` (`/Game/Widgets/DialogOFF_HUD.MultiLineEditableTextBox_72` (`self.WidgetRef`)) (select `int` (`self.StageIndex`) :`0` (`self.DialogArray_0`) :`1` (`self.DialogArray_1`)) (`self.TextSpeed`)))

(event `self.ReceiveTick`
  (params (DeltaSeconds :type "Float (single-precision)"))
  ;[1 1 1] Waiting for Player Input
  (if (`self.isWaitingForPlayer`)
    (if (`PlayerController.WasInputKeyJustPressed` (`GameplayStatics.GetPlayerController` 0) "AnyKey")
      (set `self.isWaitingForPlayer` false)
      (set `self.isTalking` false)
      (set `/Game/Blueprints/DesignMap/PlayerSelect_BP.InputDisabled` false (`self.PlayerSelectRef`)))))

(fn `UserConstructionScript`)