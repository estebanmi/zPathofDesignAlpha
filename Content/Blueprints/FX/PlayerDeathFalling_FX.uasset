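; One-shot flipbook effect actor for the player's falling death.
; On BeginPlay, if the player's VideoCardON flag is set, it tints the flipbook with the Player color from the ColorSchemeTable row named by the level's ColorController.
; It then waits for the flipbook's length and destroys itself, going straight to that step when the flag is off.
; A failed player cast or missing table row leaves the actor alive.
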(event `self.ReceiveBeginPlay`
  (bind _asplayer_bp (cast `/Game/Blueprints/Player/Player_BP` (`GameplayStatics.GetPlayerCharacter` 0)))
  (if (`/Game/Blueprints/Player/Player_BP.VideoCardON` _asplayer_bp)
    (bind _outactors (`GameplayStatics.GetAllActorsOfClass` "/Game/Blueprints/Art/ColorController.ColorController_C"))
    (bind _returnvalue (`|GetDataTableRow` "/Game/Blueprints/Art/ColorSchemeTable.ColorSchemeTable" (`/Game/Blueprints/Art/ColorController.ColorScheme` (`|GetArrayItem` _outactors)))
      (:`then`
        (`PaperFlipbookComponent.SetSpriteColor` (`self.PaperFlipbook`) (break `/Game/Blueprints/Art/ColorScheme` _returnvalue)))))
  (`KismetSystemLibrary.Delay` (`PaperFlipbookComponent.GetFlipbookLength` (`self.PaperFlipbook`)))
  (`self.K2_DestroyActor`))

(fn `UserConstructionScript`)