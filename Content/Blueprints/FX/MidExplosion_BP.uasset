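; MidExplosion_BP is a short-lived flipbook explosion effect that damages actors it overlaps.
; On BeginPlay it randomly picks one of two flipbook rotations and plays a 2D sound with randomized volume and pitch.
; A timed sphere radius change creates a brief damage window through overlap events, then shrinks and disables collision.
; A separate custom event destroys the actor after the flipbook's length.
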(event `DelayDestroy`
  (`KismetSystemLibrary.Delay` (`PaperFlipbookComponent.GetFlipbookLength` (`self.PaperFlipbook`)))
  (`self.K2_DestroyActor`))

(event `self.ReceiveBeginPlay`
  (bind _sphere (`self.Sphere`))
  (`SceneComponent.K2_SetRelativeRotation` (`self.PaperFlipbook`) (`KismetMathLibrary.SelectRotator` (struct) (struct :`Yaw` 180.0) (`KismetMathLibrary.RandomBool`)) false false)
  (`GameplayStatics.PlaySound2D` "/Game/Sound/SFXs/sfx_CodeBlockExplosion_Cue.sfx_CodeBlockExplosion_Cue" (`KismetMathLibrary.RandomFloatInRange` 0.8 1.2) (`KismetMathLibrary.RandomFloatInRange` 0.8 1.2) 0.0 null null)
  (`self.DelayDestroy`)
  (`KismetSystemLibrary.Delay` 0.1)
  (`SphereComponent.SetSphereRadius` (`self.Sphere`) 15.0 true)
  (`KismetSystemLibrary.Delay` 0.1)
  (`SphereComponent.SetSphereRadius` _sphere 1.0 true)
  (`PrimitiveComponent.SetCollisionEnabled` _sphere "NoCollision"))

(event `self.Sphere.OnComponentBeginOverlap`
  (params (OverlappedComponent :type "PrimitiveComponent Object Reference") (OtherActor :type "Actor Object Reference") (OtherComp :type "PrimitiveComponent Object Reference") (OtherBodyIndex :type Integer) (bFromSweep :type Boolean) (SweepResult :type "HitResult Structure (by ref)"))
  (`GameplayStatics.ApplyDamage` OtherActor 20.0 null self))

(fn `UserConstructionScript`)