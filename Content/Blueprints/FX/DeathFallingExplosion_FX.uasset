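; DeathFallingExplosion_FX is a one-shot flipbook explosion effect, named for falling deaths, that destroys itself after one flipbook length.
; On BeginPlay, if the player's VideoCardON flag is set, it reads the ColorController's scheme from ColorSchemeTable and tints the sprite with that Explosion color, randomly dimmed per RGB channel.
; With the flag off, it skips tinting; a failed player cast or missing row leaves the actor undestroyed.
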(event `self.ReceiveBeginPlay`
  (bind _returnvalue (`KismetMathLibrary.RandomFloatInRange` 0.6 1.0))
  (bind _asplayer_bp (cast `/Game/Blueprints/Player/Player_BP` (`GameplayStatics.GetPlayerCharacter` 0)))
  (if (`/Game/Blueprints/Player/Player_BP.VideoCardON` _asplayer_bp)
    (bind _outactors (`GameplayStatics.GetAllActorsOfClass` "/Game/Blueprints/Art/ColorController.ColorController_C"))
    (bind _returnvalue_2 (`|GetDataTableRow` "/Game/Blueprints/Art/ColorSchemeTable.ColorSchemeTable" (`/Game/Blueprints/Art/ColorController.ColorScheme` (`|GetArrayItem` _outactors)))
      (:`then`
        (`PaperFlipbookComponent.SetSpriteColor` (`self.PaperFlipbook`) (* (`.Explosion_34_AFEABEF2445912176FAE47AD02015058` (break `/Game/Blueprints/Art/ColorScheme` _returnvalue_2)) (make `LinearColor` _returnvalue _returnvalue _returnvalue 1.0))))))
  (`KismetSystemLibrary.Delay` (`PaperFlipbookComponent.GetFlipbookLength` (`self.PaperFlipbook`)))
  (`self.K2_DestroyActor`))

(fn `UserConstructionScript`)