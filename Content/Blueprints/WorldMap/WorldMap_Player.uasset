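; World map player pawn that moves between linked location nodes and loads its progress on BeginPlay.
; Directional input tweens it along N/E/S/W links with a timeline, auto-continuing through two-way path nodes and refusing non-isle targets whose level masters are locked.
; Jump on a level node plays an enter animation and sets a hardcoded progress flag, without opening the level.
; Debug keys save (omitting RAM and Core worlds) or delete slot SaveA.
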(event `InputAction|Jump`
  (params (Key :type "Key Structure"))
  (bind _returnvalue (+ 0 0))
  (:`Pressed`
    (if (not (`self.PlayerIsMoving`))
      (set `self.PlayerIsMoving` true)
      (if (!= (`/Game/Blueprints/WorldMap/WorldMap_Section.LevelName` (`self.CurrentLocation`)) "None")
        (`GameplayStatics.PlaySound2D` "/Game/Sound/SFXs/DesignMap/sfx_DMUnlockPOI_Cue.sfx_DMUnlockPOI_Cue" 1.0 1.0 0.0 null null)
        (`PaperFlipbookComponent.SetFlipbook` (`self.PaperFlipbook`) "/Game/Sprites/WorldMap/WMPlayer_Enter.WMPlayer_Enter")
        (bind _output_get (set `self.CurrentWorld` (select `/Game/Blueprints/WorldMap/CurrentWorld` (`self.CurrentWorldType`) :`NewEnumerator0` (`self.WorldMother`) :`NewEnumerator1` (`self.WorldHDD`) :`NewEnumerator2` (`self.WorldVideo`) :`NewEnumerator3` (`self.WorldSound`) :`NewEnumerator4` (`self.WorldPower`) :`NewEnumerator5` (`self.WorldCooling`) :`NewEnumerator6` (`self.WorldRAM`) :`NewEnumerator7` (`self.WorldCore`))))
        ;[1 1 1] Secret or not
        (if true
          (bind _output_get_2 (set `self.CurrentWorld` (make `/Game/Blueprints/WorldMap/WorldStruct` (break `/Game/Blueprints/WorldMap/WorldStruct` _output_get) (`|MakeArray` (select `bool` (== _returnvalue 0) :`false` (`|GetArrayItem` (`.Secrets_59_E5D92C3E440CB88324C8F8B2D62F1C0E` (break `/Game/Blueprints/WorldMap/WorldStruct` _output_get))) :`true` true) (select `bool` (== _returnvalue 1) :`false` (`|GetArrayItem` (`.Secrets_59_E5D92C3E440CB88324C8F8B2D62F1C0E` (break `/Game/Blueprints/WorldMap/WorldStruct` _output_get)) 1) :`true` true) (select `bool` (== _returnvalue 2) :`false` (`|GetArrayItem` (`.Secrets_59_E5D92C3E440CB88324C8F8B2D62F1C0E` (break `/Game/Blueprints/WorldMap/WorldStruct` _output_get)) 2) :`true` true)))))
          (switch `/Game/Blueprints/WorldMap/CurrentWorld` (`self.CurrentWorldType`)
            (:`NewEnumerator0`
              (set `self.WorldMother` _output_get_2))
            (:`NewEnumerator1`
              (set `self.WorldHDD` _output_get_2))
            (:`NewEnumerator2`
              (set `self.WorldVideo` _output_get_2))
            (:`NewEnumerator3`
              (set `self.WorldSound` _output_get_2))
            (:`NewEnumerator4`
              (set `self.WorldPower` _output_get_2))
            (:`NewEnumerator5`
              (set `self.WorldCooling` _output_get_2))
            (:`NewEnumerator6`
              (set `self.WorldRAM` _output_get_2))
            (:`NewEnumerator7`
              (set `self.WorldCore` _output_get_2)))
          (else
            (bind _output_get_3 (set `self.CurrentWorld` (make `/Game/Blueprints/WorldMap/WorldStruct` (`|MakeArray` (select `bool` (== _returnvalue 0) :`false` (`|GetArrayItem` (break `/Game/Blueprints/WorldMap/WorldStruct` _output_get)) :`true` true) (select `bool` (== _returnvalue 1) :`false` (`|GetArrayItem` (break `/Game/Blueprints/WorldMap/WorldStruct` _output_get) 1) :`true` true) (select `bool` (== _returnvalue 2) :`false` (`|GetArrayItem` (break `/Game/Blueprints/WorldMap/WorldStruct` _output_get) 2) :`true` true) (select `bool` (== _returnvalue 3) :`false` (`|GetArrayItem` (break `/Game/Blueprints/WorldMap/WorldStruct` _output_get) 3) :`true` true) (select `bool` (== _returnvalue 4) :`false` (`|GetArrayItem` (break `/Game/Blueprints/WorldMap/WorldStruct` _output_get) 4) :`true` true) (select `bool` (== _returnvalue 5) :`false` (`|GetArrayItem` (break `/Game/Blueprints/WorldMap/WorldStruct` _output_get) 5) :`true` true) (select `bool` (== _returnvalue 6) :`false` (`|GetArrayItem` (break `/Game/Blueprints/WorldMap/WorldStruct` _output_get) 6) :`true` true) (select `bool` (== _returnvalue 7) :`false` (`|GetArrayItem` (break `/Game/Blueprints/WorldMap/WorldStruct` _output_get) 7) :`true` true)) (`.Secrets_59_E5D92C3E440CB88324C8F8B2D62F1C0E` (break `/Game/Blueprints/WorldMap/WorldStruct` _output_get)))))
            (switch `/Game/Blueprints/WorldMap/CurrentWorld` (`self.CurrentWorldType`)
              (:`NewEnumerator0`
                (set `self.WorldMother` _output_get_3))
              (:`NewEnumerator1`
                (set `self.WorldHDD` _output_get_3))
              (:`NewEnumerator2`
                (set `self.WorldVideo` _output_get_3))
              (:`NewEnumerator3`
                (set `self.WorldSound` _output_get_3))
              (:`NewEnumerator4`
                (set `self.WorldPower` _output_get_3))
              (:`NewEnumerator5`
                (set `self.WorldCooling` _output_get_3))
              (:`NewEnumerator6`
                (set `self.WorldRAM` _output_get_3))
              (:`NewEnumerator7`
                (set `self.WorldCore` _output_get_3)))))
        (`KismetSystemLibrary.Delay` 1.0)
        (set `self.PlayerIsMoving` false)
        (`PaperFlipbookComponent.SetFlipbook` (`self.PaperFlipbook`) "/Game/Sprites/WorldMap/WMPlayer_Stand.WMPlayer_Stand")
        (else
          (`self.WrongInput`))))))

(event `InputAxis|MoveRight`
  (params (AxisValue :type "Float (single-precision)"))
  (bind _currentlocation (`self.CurrentLocation`))
  ;[1 1 1] Inputs
  (if (`self.PlayerIsMoving`)
    _
    (elif (> AxisValue 0.0)
      (`self.WMMove` (`/Game/Blueprints/WorldMap/WorldMap_Section.Destiny E` _currentlocation))
      (elif (< AxisValue 0.0)
        (`self.WMMove` (`/Game/Blueprints/WorldMap/WorldMap_Section.Destiny W` _currentlocation))))))

(event `InputAxis|MoveUp`
  (params (AxisValue :type "Float (single-precision)"))
  (bind _currentlocation (`self.CurrentLocation`))
  ;[1 1 1] Inputs
  (if (`self.PlayerIsMoving`)
    _
    (elif (> AxisValue 0.0)
      (`self.WMMove` (`/Game/Blueprints/WorldMap/WorldMap_Section.Destiny N` _currentlocation))
      (elif (< AxisValue 0.0)
        (`self.WMMove` (`/Game/Blueprints/WorldMap/WorldMap_Section.Destiny S` _currentlocation))))))

(event `WMMove`
  (params (Destiny :type "/Game/Blueprints/WorldMap/WorldMap_Section Object Reference"))
  (bind _currentlocation (`self.CurrentLocation`))
  (bind _destiny_n (`/Game/Blueprints/WorldMap/WorldMap_Section.Destiny N` _currentlocation))
  (bind _destiny_s (`/Game/Blueprints/WorldMap/WorldMap_Section.Destiny S` _currentlocation))
  (bind _destiny_e (`/Game/Blueprints/WorldMap/WorldMap_Section.Destiny E` _currentlocation))
  (bind _destiny_w (`/Game/Blueprints/WorldMap/WorldMap_Section.Destiny W` _currentlocation))
  ;[1 1 1] Movement
  (set `self.PlayerIsMoving` true)
  (`/Engine/EditorBlueprintResources/StandardMacros.IsValid` Destiny
    (:`Is Valid`
      (if (`|EnumEquality` (`/Game/Blueprints/WorldMap/WorldMap_Section.WM Type 1` Destiny) "NewEnumerator0")
        (`GameplayStatics.PlaySound2D` "/Game/Sound/SFXs/DesignMap/sfx_DMMove_Cue.sfx_DMMove_Cue" 1.0 1.0 0.0 null null :!label _label)
        (bind (_direction _newtrack_0) (`Timeline|Moving E` :!via `PlayFromStart`)
          (:`Update`
            (`self.K2_SetActorLocation` (`KismetMathLibrary.VLerp` (`self.K2_GetActorLocation` (`self.CurrentLocation`)) (`self.K2_GetActorLocation` Destiny) _newtrack_0)))
          (:`Finished`
            (set `self.lastLocation` (`self.CurrentLocation`))
            (bind _output_get (set `self.CurrentLocation` Destiny))
            (switch `/Game/Blueprints/WorldMap/WorldMap_Type` (`/Game/Blueprints/WorldMap/WorldMap_Section.WM Type 1` _output_get)
              (:`NewEnumerator0`
                (set `self.PlayerIsMoving` false :!label _label_2))
              (:`NewEnumerator1`
                (`self.CompareDestinies` _destiny_n _destiny_s))
              (:`NewEnumerator2`
                (`self.CompareDestinies` _destiny_e _destiny_w))
              (:`NewEnumerator3`
                (goto _label_2))
              (:`NewEnumerator4`
                (goto _label_2))
              (:`NewEnumerator5`
                (goto _label_2))
              (:`NewEnumerator6`
                (goto _label_2))
              (:`NewEnumerator7`
                (goto _label_2))
              (:`NewEnumerator8`
                (`self.CompareDestinies` _destiny_n _destiny_w))
              (:`NewEnumerator9`
                (`self.CompareDestinies` _destiny_n _destiny_e))
              (:`NewEnumerator10`
                (`self.CompareDestinies` _destiny_w _destiny_s))
              (:`NewEnumerator11`
                (`self.CompareDestinies` _destiny_e _destiny_s)))))
        (elif (`/Game/Blueprints/WorldMap/WorldMap_Section.Unlocked` (`/Game/Blueprints/WorldMap/WorldMap_Section.LevelMaster` Destiny))
          (goto _label)
          (elif (`/Game/Blueprints/WorldMap/WorldMap_Section.Unlocked` (`/Game/Blueprints/WorldMap/WorldMap_Section.LevelMaster2` Destiny))
            (goto _label)
            (else
              (`self.WrongInput` :!label _label_3))))))
    (:`Is Not Valid`
      (goto _label_3))))

(event `CompareDestinies`
  (params (`Destiny 1` :type "/Game/Blueprints/WorldMap/WorldMap_Section Object Reference") (`Destiny 2` :type "/Game/Blueprints/WorldMap/WorldMap_Section Object Reference"))
  ;[1 1 1] Movement
  (if (!= `Destiny 1` (`self.lastLocation`))
    (`self.WMMove` `Destiny 1`)
    (else
      (`self.WMMove` `Destiny 2`))))

(event `WrongInput`
  ;[1 1 1] Wrong Input
  (`GameplayStatics.PlaySound2D` "/Game/Sound/SFXs/DesignMap/sfx_DMMoveNot_Cue.sfx_DMMoveNot_Cue" 1.0 1.0 0.0 null null)
  (`KismetSystemLibrary.Delay` 0.2)
  (set `self.PlayerIsMoving` false))

(event `self.ReceiveBeginPlay`
  (bind _currentlocation (`self.CurrentLocation`))
  (bind _currentlocation_2 (`self.CurrentLocation`))
  (bind _startinglocation (`self.StartingLocation`))
  (`self.LoadGame`)
  (`/Engine/EditorBlueprintResources/StandardMacros.IsValid` _currentlocation
    (:`Is Valid`
      (`self.K2_SetActorLocation` (`self.K2_GetActorLocation` _currentlocation))
      (set `self.CurrentLocation` _currentlocation_2)
      (set `self.CurrentWorldType` (`/Game/Blueprints/WorldMap/WorldMap_Section.WorldType` _currentlocation_2)))
    (:`Is Not Valid`
      (`self.K2_SetActorLocation` (`self.K2_GetActorLocation` (`self.StartingLocation`)))
      (set `self.CurrentLocation` _startinglocation)
      (set `self.CurrentWorldType` (`/Game/Blueprints/WorldMap/WorldMap_Section.WorldType` _startinglocation)))))

(event `Key|Three`
  (params (Key :type "Key Structure"))
  (:`Pressed`
    (`GameplayStatics.DeleteGameInSlot` "SaveA")
    (`KismetSystemLibrary.PrintString` "SaveA Deleted")))

(event `Key|One`
  (params (Key :type "Key Structure"))
  (bind _savegameref (`self.SaveGameRef`))
  (bind _savegameref_2 (`self.SaveGameRef`))
  (:`Pressed`
    (bind _returnvalue (`GameplayStatics.CreateSaveGameObject` "/Game/Blueprints/SaveGame/PODSaveGame.PODSaveGame_C"))
    (bind _output_get (set `self.SaveGameRef` _returnvalue))
    (set `/Game/Blueprints/SaveGame/PODSaveGame.WorldMother` (`self.WorldMother`) _output_get)
    (set `/Game/Blueprints/SaveGame/PODSaveGame.WorldHDD` (`self.WorldHDD`) _output_get)
    (set `/Game/Blueprints/SaveGame/PODSaveGame.WorldVideo` (`self.WorldVideo`) _output_get)
    (set `/Game/Blueprints/SaveGame/PODSaveGame.WorldSound` (`self.WorldSound`) _output_get)
    (set `/Game/Blueprints/SaveGame/PODSaveGame.WorldPower` (`self.WorldPower`) _output_get)
    (set `/Game/Blueprints/SaveGame/PODSaveGame.WorldCooling` (`self.WorldCooling`) _output_get)
    (set `self.WorldRAM` (`self.WorldRAM`))
    (set `self.WorldCore` (`self.WorldCore`))
    (set `/Game/Blueprints/SaveGame/PODSaveGame.HDDONs` (`self.HDDON`) _savegameref)
    (set `/Game/Blueprints/SaveGame/PODSaveGame.VideoONs` (`self.VideoCardON`) _savegameref)
    (set `/Game/Blueprints/SaveGame/PODSaveGame.SoundONs` (`self.SoundCardON`) _savegameref)
    (set `/Game/Blueprints/SaveGame/PODSaveGame.PowerONs` (`self.PowerSupplyON`) _savegameref)
    (set `/Game/Blueprints/SaveGame/PODSaveGame.CoolingONs` (`self.CoolingSystemON`) _savegameref)
    (set `/Game/Blueprints/SaveGame/PODSaveGame.CurrentLocation` (`self.CurrentLocation`) _savegameref_2)
    (set `/Game/Blueprints/SaveGame/PODSaveGame.CurrentWorldType` (`self.CurrentWorldType`) _savegameref_2)
    (set `/Game/Blueprints/SaveGame/PODSaveGame.IsUsingGamepad` (`self.IsUsingGamePad`) _savegameref_2)
    (set `/Game/Blueprints/SaveGame/PODSaveGame.LastCheckPoint` (`self.LastCheckPoint`) _savegameref_2)
    (set `/Game/Blueprints/SaveGame/PODSaveGame.CurrentLevel` (`self.CurrentLevel`) _savegameref_2)
    (`GameplayStatics.SaveGameToSlot` (`self.SaveGameRef`) "SaveA")
    (`KismetSystemLibrary.PrintString` "Game Saved")))

(event `LoadGame`
  (bind _returnvalue (`GameplayStatics.DoesSaveGameExist` "SaveA"))
  (if _returnvalue
    (bind _returnvalue_2 (`GameplayStatics.LoadGameFromSlot` "SaveA"))
    (bind _aspodsave_game (cast `/Game/Blueprints/SaveGame/PODSaveGame` _returnvalue_2))
    (set `self.WorldMother` (`/Game/Blueprints/SaveGame/PODSaveGame.WorldMother` _aspodsave_game))
    (set `self.WorldHDD` (`/Game/Blueprints/SaveGame/PODSaveGame.WorldHDD` _aspodsave_game))
    (set `self.WorldVideo` (`/Game/Blueprints/SaveGame/PODSaveGame.WorldVideo` _aspodsave_game))
    (set `self.WorldSound` (`/Game/Blueprints/SaveGame/PODSaveGame.WorldSound` _aspodsave_game))
    (set `self.WorldPower` (`/Game/Blueprints/SaveGame/PODSaveGame.WorldPower` _aspodsave_game))
    (set `self.WorldCooling` (`/Game/Blueprints/SaveGame/PODSaveGame.WorldCooling` _aspodsave_game))
    (set `self.WorldRAM` (`/Game/Blueprints/SaveGame/PODSaveGame.WorldRAM` _aspodsave_game))
    (set `self.WorldCore` (`/Game/Blueprints/SaveGame/PODSaveGame.WorldCore` _aspodsave_game))
    (set `self.HDDON` (`/Game/Blueprints/SaveGame/PODSaveGame.HDDONs` _aspodsave_game))
    (set `self.VideoCardON` (`/Game/Blueprints/SaveGame/PODSaveGame.VideoONs` _aspodsave_game))
    (set `self.SoundCardON` (`/Game/Blueprints/SaveGame/PODSaveGame.SoundONs` _aspodsave_game))
    (set `self.PowerSupplyON` (`/Game/Blueprints/SaveGame/PODSaveGame.PowerONs` _aspodsave_game))
    (set `self.CoolingSystemON` (`/Game/Blueprints/SaveGame/PODSaveGame.CoolingONs` _aspodsave_game))
    (set `self.CurrentLocation` (`/Game/Blueprints/SaveGame/PODSaveGame.CurrentLocation` _aspodsave_game))
    (set `self.CurrentWorldType` (`/Game/Blueprints/SaveGame/PODSaveGame.CurrentWorldType` _aspodsave_game))
    (set `self.IsUsingGamePad` (`/Game/Blueprints/SaveGame/PODSaveGame.IsUsingGamepad` _aspodsave_game))
    (set `self.LastCheckPoint` (`/Game/Blueprints/SaveGame/PODSaveGame.LastCheckPoint` _aspodsave_game))
    (set `self.CurrentLevel` (`/Game/Blueprints/SaveGame/PODSaveGame.CurrentLevel` _aspodsave_game))
    (`KismetSystemLibrary.PrintString` "Game Loaded")
    (else
      (`KismetSystemLibrary.PrintString` "No Game Saved"))))

(fn `UserConstructionScript`)