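; World map tile for one section of the computer-themed overworld, either a level isle or a connecting path piece.
; Isles read their unlock state from the player's per-world level or secret arrays and report themselves as starting location when matching the current level.
; Paths choose sprite shapes from up to two LevelMaster unlock states, and locked secrets are hidden.
; Player hardware flags drive completion markers and video-card-dependent tinting.
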(event `ColorControl`
  ;[0 1 1] Color Control
  (if (`/Game/Blueprints/WorldMap/WorldMap_Player.VideoCardON` (`self.WMPlayerRef`))
    (bind _outactors (`GameplayStatics.GetAllActorsOfClass` "/Game/Blueprints/Art/ColorController.ColorController_C"))
    (`|GetDataTableRow` "/Game/Blueprints/Art/ColorSchemeTable.ColorSchemeTable" (`/Game/Blueprints/Art/ColorController.ColorScheme` (`|GetArrayItem` _outactors))
      (:`then`
        (`PaperSpriteComponent.SetSpriteColor` (`self.Sprite Type`) (struct :`R` 1.0 :`G` 0.575142 :`A` 1.0))
        (`PaperSpriteComponent.SetSpriteColor` (`self.Sprite Level`) (struct :`R` 1.0 :`A` 1.0))))))

(event `AmIUnlocked?`
  (bind _sprite_type (`self.Sprite Type`))
  ;[1 1 1] Am I Unlocked?
  (bind _asworld_map_player (cast `/Game/Blueprints/WorldMap/WorldMap_Player` (`GameplayStatics.GetPlayerPawn` 0)))
  (bind _output_get (set `self.CurrentWorld` (select `/Game/Blueprints/WorldMap/CurrentWorld` (`self.WorldType`) :`NewEnumerator0` (`/Game/Blueprints/WorldMap/WorldMap_Player.WorldMother` _asworld_map_player) :`NewEnumerator1` (`/Game/Blueprints/WorldMap/WorldMap_Player.WorldHDD` _asworld_map_player) :`NewEnumerator2` (`/Game/Blueprints/WorldMap/WorldMap_Player.WorldVideo` _asworld_map_player) :`NewEnumerator3` (`/Game/Blueprints/WorldMap/WorldMap_Player.WorldSound` _asworld_map_player) :`NewEnumerator4` (`/Game/Blueprints/WorldMap/WorldMap_Player.WorldPower` _asworld_map_player) :`NewEnumerator5` (`/Game/Blueprints/WorldMap/WorldMap_Player.WorldCooling` _asworld_map_player) :`NewEnumerator6` (`/Game/Blueprints/WorldMap/WorldMap_Player.WorldRAM` _asworld_map_player) :`NewEnumerator7` (`/Game/Blueprints/WorldMap/WorldMap_Player.WorldCore` _asworld_map_player))))
  (if (`self.Secret`)
    (if (`|GetArrayItem` (`.Secrets_59_E5D92C3E440CB88324C8F8B2D62F1C0E` (break `/Game/Blueprints/WorldMap/WorldStruct` _output_get)) (`self.Level`))
      (set `self.Unlocked` true)
      (else
        (set `self.Unlocked` false)))
    (elif (`|GetArrayItem` (break `/Game/Blueprints/WorldMap/WorldStruct` _output_get) (`self.Level`))
      (set `self.Unlocked` true)
      (else
        (set `self.Unlocked` false))))
  (if (`|EnumEquality` (`self.WM Type 1`) "NewEnumerator0")
    (`KismetSystemLibrary.PrintString` (`KismetStringLibrary.Concat_StrStr` "I am " (select `/Game/Blueprints/WorldMap/CurrentWorld` (`self.WorldType`) :`NewEnumerator0` "Bios" :`NewEnumerator1` "HDD" :`NewEnumerator2` "Video" :`NewEnumerator3` "Sound" :`NewEnumerator4` "Power" :`NewEnumerator5` "Cooling" :`NewEnumerator6` "RAM" :`NewEnumerator7` "Core") ", Unlocked = " "" "" "" (`KismetStringLibrary.Conv_BoolToString` (`self.Unlocked`))) true true (struct :`G` 0.66 :`B` 1.0 :`A` 1.0) 16.0)
    (if (`self.Secret`)
      (if (not (`self.Unlocked`))
        (`SceneComponent.SetVisibility` (`self.Sprite Type`) false true)))
    (switch `/Game/Blueprints/WorldMap/WorldMap_Type` (`self.WM Type 1`) :!label _label
      (:`NewEnumerator0`
        (`PaperSpriteComponent.SetSprite` _sprite_type "/Game/Sprites/WorldMap/WMPath_Isle.WMPath_Isle"))
      (:`NewEnumerator1`
        (`PaperSpriteComponent.SetSprite` _sprite_type "/Game/Sprites/WorldMap/WMPath_NS.WMPath_NS"))
      (:`NewEnumerator2`
        (`PaperSpriteComponent.SetSprite` _sprite_type "/Game/Sprites/WorldMap/WMPath_WE.WMPath_WE"))
      (:`NewEnumerator3`
        (`PaperSpriteComponent.SetSprite` _sprite_type "/Game/Sprites/WorldMap/WMPath_NWS.WMPath_NWS"))
      (:`NewEnumerator4`
        (`PaperSpriteComponent.SetSprite` _sprite_type "/Game/Sprites/WorldMap/WMPath_NES.WMPath_NES"))
      (:`NewEnumerator5`
        (`PaperSpriteComponent.SetSprite` _sprite_type "/Game/Sprites/WorldMap/WMPath_NWE.WMPath_NWE"))
      (:`NewEnumerator6`
        (`PaperSpriteComponent.SetSprite` _sprite_type "/Game/Sprites/WorldMap/WMPath_WES.WMPath_WES"))
      (:`NewEnumerator7`
        (`PaperSpriteComponent.SetSprite` _sprite_type "/Game/Sprites/WorldMap/WMPath_X.WMPath_X"))
      (:`NewEnumerator8`
        (`PaperSpriteComponent.SetSprite` _sprite_type "/Game/Sprites/WorldMap/WMPath_NW.WMPath_NW"))
      (:`NewEnumerator9`
        (`PaperSpriteComponent.SetSprite` _sprite_type "/Game/Sprites/WorldMap/WMPath_NE.WMPath_NE"))
      (:`NewEnumerator10`
        (`PaperSpriteComponent.SetSprite` _sprite_type "/Game/Sprites/WorldMap/WMPath_WS.WMPath_WS"))
      (:`NewEnumerator11`
        (`PaperSpriteComponent.SetSprite` _sprite_type "/Game/Sprites/WorldMap/WMPath_ES.WMPath_ES"))
      (:`NewEnumerator12`
        (`PaperSpriteComponent.SetSprite` _sprite_type "/Game/Sprites/WorldMap/WMPath_MouthN.WMPath_MouthN"))
      (:`NewEnumerator13`
        (`PaperSpriteComponent.SetSprite` _sprite_type "/Game/Sprites/WorldMap/WMPath_MouthS.WMPath_MouthS"))
      (:`NewEnumerator14`
        (`PaperSpriteComponent.SetSprite` _sprite_type "/Game/Sprites/WorldMap/WMPath_MouthW.WMPath_MouthW"))
      (:`NewEnumerator15`
        (`PaperSpriteComponent.SetSprite` _sprite_type "/Game/Sprites/WorldMap/WMPath_MouthE.WMPath_MouthE")))))

(event `IAmLastLevel?`
  (params (`Player World Type` :type "/Game/Blueprints/WorldMap/CurrentWorld Enum" :default "NewEnumerator0") (`Player Level` :type Integer))
  ;[1 1 1] I am Last Level
  (if (`|EnumEquality` `Player World Type` (`self.WorldType`))
    (if (== `Player Level` (`self.Level`))
      (`/Game/Blueprints/WorldMap/WorldMap_Player.StartingLocationEvent` (`self.WMPlayerRef`) self)
      (`KismetSystemLibrary.PrintString` (`KismetStringLibrary.Concat_StrStr` (`KismetSystemLibrary.GetDisplayName` self) ": I am last level") true true (struct :`R` 1.0 :`B` 0.385594 :`A` 1.0) 6.0))))

(event `self.ReceiveBeginPlay`
  (bind _levelmaster (`self.LevelMaster`))
  (bind _levelmaster2 (`self.LevelMaster2`))
  (bind _levelmaster2_2 (`self.LevelMaster2`))
  (`KismetSystemLibrary.Delay` 0.1)
  (bind _asworld_map_player (cast `/Game/Blueprints/WorldMap/WorldMap_Player` (`GameplayStatics.GetPlayerPawn` 0)))
  (bind _output_get (set `self.WMPlayerRef` _asworld_map_player))
  (`self.ColorControl`)
  (`self.AlreadyDone?`)
  (if (`|EnumEquality` (`self.WM Type 1`) "NewEnumerator0")
    (`self.IAmLastLevel?` (`/Game/Blueprints/WorldMap/WorldMap_Player.CurrentWorldType` _output_get) (`/Game/Blueprints/WorldMap/WorldMap_Player.CurrentWorldLevel` _output_get))
    (`self.AmIUnlocked?`)
    (else
      (`KismetSystemLibrary.Delay` 0.1)
      (`ActorComponent.K2_DestroyComponent` (`self.Sprite Level`))
      (`/Engine/EditorBlueprintResources/StandardMacros.IsValid` _levelmaster
        (:`Is Valid`
          (if (`/Game/Blueprints/WorldMap/WorldMap_Section.Unlocked` _levelmaster)
            (`/Engine/EditorBlueprintResources/StandardMacros.IsValid` _levelmaster2_2
              (:`Is Valid`
                (if (`/Game/Blueprints/WorldMap/WorldMap_Section.Unlocked` _levelmaster2_2)
                  (set `self.WM Type 1` (`self.WM Type 1 and 2`))
                  (goto _label)
                  (else
                    _)))
              (:`Is Not Valid`
                (goto _label)))
            (else
              (`/Engine/EditorBlueprintResources/StandardMacros.IsValid` _levelmaster2
                (:`Is Valid`
                  (if (`/Game/Blueprints/WorldMap/WorldMap_Section.Unlocked` _levelmaster2)
                    _
                    (else
                      (if (`self.Secret`) :!label _label_2
                        (`SceneComponent.SetVisibility` (`self.Sprite Type`) false true)
                        (goto _label)
                        (else
                          (goto _label))))))
                (:`Is Not Valid`
                  (goto _label_2)))))
          (set `self.WM Type 1` (`self.WM Type 2`))
          (goto _label))
        (:`Is Not Valid`
          (goto _label))))))

(event `AlreadyDone?`
  (bind _wmplayerref (`self.WMPlayerRef`))
  (switch `/Game/Blueprints/WorldMap/CurrentWorld` (`self.WorldType`)
    (:`NewEnumerator0`
      (if (== (`self.Level`) 1)
        (`PaperSpriteComponent.SetSprite` (`self.Sprite Level`) "/Game/Sprites/WorldMap/WMPath_PointB.WMPath_PointB" :!label _label_3)))
    (:`NewEnumerator1`
      (if (`/Game/Blueprints/WorldMap/WorldMap_Player.HDDON` _wmplayerref)
        (goto _label_3)))
    (:`NewEnumerator2`
      (if (`/Game/Blueprints/WorldMap/WorldMap_Player.VideoCardON` _wmplayerref)
        (goto _label_3)))
    (:`NewEnumerator3`
      (if (`/Game/Blueprints/WorldMap/WorldMap_Player.SoundCardON` _wmplayerref)
        (goto _label_3)))
    (:`NewEnumerator4`
      (if (`/Game/Blueprints/WorldMap/WorldMap_Player.PowerSupplyON` _wmplayerref)
        (goto _label_3)))
    (:`NewEnumerator5`
      (if (`/Game/Blueprints/WorldMap/WorldMap_Player.CoolingSystemON` _wmplayerref)
        (goto _label_3)))))

(fn `UserConstructionScript`)