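; World map icon that shows one hardware device (HDD, video, sound, power or cooling) and whether it is on.
; On BeginPlay it caches the WorldMap_Player, sets the sprite for its DeviceType and runs a one-time, briefly delayed status check.
; With the video card on, it tints the sprite Friendly or Explosion from the ColorController's scheme in ColorSchemeTable.
; With the video card off, devices that are off swap to alternate sprites instead.
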(event `ColorControl`
  (bind _wmplayerref (`self.WMPlayerRef`))
  ;[0 1 1] Color Control
  (`KismetSystemLibrary.Delay` 0.1)
  (if (`/Game/Blueprints/WorldMap/WorldMap_Player.VideoCardON` (`self.WMPlayerRef`))
    (bind _outactors (`GameplayStatics.GetAllActorsOfClass` "/Game/Blueprints/Art/ColorController.ColorController_C"))
    (bind _returnvalue (`|GetDataTableRow` "/Game/Blueprints/Art/ColorSchemeTable.ColorSchemeTable" (`/Game/Blueprints/Art/ColorController.ColorScheme` (`|GetArrayItem` _outactors)))
      (:`then`
        (switch `/Game/Blueprints/WorldMap/DeviceType` (`self.DeviceType`)
          (:`NewEnumerator0`
            (`PaperSpriteComponent.SetSpriteColor` (`self.Device`) (`KismetMathLibrary.SelectColor` (`.Friendly_28_A722989D438FB0BFB80A41832B39E11A` (break `/Game/Blueprints/Art/ColorScheme` _returnvalue)) (`.Explosion_34_AFEABEF2445912176FAE47AD02015058` (break `/Game/Blueprints/Art/ColorScheme` _returnvalue)) (`/Game/Blueprints/WorldMap/WorldMap_Player.HDDON` _wmplayerref))))
          (:`NewEnumerator1`
            (`PaperSpriteComponent.SetSpriteColor` (`self.Device`) (`KismetMathLibrary.SelectColor` (`.Friendly_28_A722989D438FB0BFB80A41832B39E11A` (break `/Game/Blueprints/Art/ColorScheme` _returnvalue)) (`.Explosion_34_AFEABEF2445912176FAE47AD02015058` (break `/Game/Blueprints/Art/ColorScheme` _returnvalue)) (`/Game/Blueprints/WorldMap/WorldMap_Player.VideoCardON` _wmplayerref))))
          (:`NewEnumerator2`
            (`PaperSpriteComponent.SetSpriteColor` (`self.Device`) (`KismetMathLibrary.SelectColor` (`.Friendly_28_A722989D438FB0BFB80A41832B39E11A` (break `/Game/Blueprints/Art/ColorScheme` _returnvalue)) (`.Explosion_34_AFEABEF2445912176FAE47AD02015058` (break `/Game/Blueprints/Art/ColorScheme` _returnvalue)) (`/Game/Blueprints/WorldMap/WorldMap_Player.SoundCardON` _wmplayerref))))
          (:`NewEnumerator3`
            (`PaperSpriteComponent.SetSpriteColor` (`self.Device`) (`KismetMathLibrary.SelectColor` (`.Friendly_28_A722989D438FB0BFB80A41832B39E11A` (break `/Game/Blueprints/Art/ColorScheme` _returnvalue)) (`.Explosion_34_AFEABEF2445912176FAE47AD02015058` (break `/Game/Blueprints/Art/ColorScheme` _returnvalue)) (`/Game/Blueprints/WorldMap/WorldMap_Player.PowerSupplyON` _wmplayerref))))
          (:`NewEnumerator4`
            (`PaperSpriteComponent.SetSpriteColor` (`self.Device`) (`KismetMathLibrary.SelectColor` (`.Friendly_28_A722989D438FB0BFB80A41832B39E11A` (break `/Game/Blueprints/Art/ColorScheme` _returnvalue)) (`.Explosion_34_AFEABEF2445912176FAE47AD02015058` (break `/Game/Blueprints/Art/ColorScheme` _returnvalue)) (`/Game/Blueprints/WorldMap/WorldMap_Player.CoolingSystemON` _wmplayerref)))))))
    (else
      (`self.VideoOffOff`))))

(event `VideoOffOff`
  (bind _device (`self.Device`))
  (bind _wmplayerref (`self.WMPlayerRef`))
  (switch `/Game/Blueprints/WorldMap/DeviceType` (`self.DeviceType`)
    (:`NewEnumerator0`
      (if (not (`/Game/Blueprints/WorldMap/WorldMap_Player.HDDON` _wmplayerref))
        (`PaperSpriteComponent.SetSprite` _device "/Game/Sprites/WorldMap/DeviceIcons/DevicesIcons_Sprite_5.DevicesIcons_Sprite_5")))
    (:`NewEnumerator1`
      (if (not (`/Game/Blueprints/WorldMap/WorldMap_Player.VideoCardON` _wmplayerref))
        (`PaperSpriteComponent.SetSprite` _device "/Game/Sprites/WorldMap/DeviceIcons/DevicesIcons_Sprite_6.DevicesIcons_Sprite_6")))
    (:`NewEnumerator2`
      (if (not (`/Game/Blueprints/WorldMap/WorldMap_Player.SoundCardON` _wmplayerref))
        (`PaperSpriteComponent.SetSprite` _device "/Game/Sprites/WorldMap/DeviceIcons/DevicesIcons_Sprite_7.DevicesIcons_Sprite_7")))
    (:`NewEnumerator3`
      (if (not (`/Game/Blueprints/WorldMap/WorldMap_Player.PowerSupplyON` _wmplayerref))
        (`PaperSpriteComponent.SetSprite` _device "/Game/Sprites/WorldMap/DeviceIcons/DevicesIcons_Sprite_8.DevicesIcons_Sprite_8")))
    (:`NewEnumerator4`
      (if (not (`/Game/Blueprints/WorldMap/WorldMap_Player.CoolingSystemON` _wmplayerref))
        (`PaperSpriteComponent.SetSprite` _device "/Game/Sprites/WorldMap/DeviceIcons/DevicesIcons_Sprite_9.DevicesIcons_Sprite_9")))))

(event `self.ReceiveBeginPlay`
  (bind _device (`self.Device`))
  (bind _asworld_map_player (cast `/Game/Blueprints/WorldMap/WorldMap_Player` (`GameplayStatics.GetPlayerPawn` 0)))
  (set `self.WMPlayerRef` _asworld_map_player)
  (`self.ColorControl`)
  (switch `/Game/Blueprints/WorldMap/DeviceType` (`self.DeviceType`)
    (:`NewEnumerator0`
      (`PaperSpriteComponent.SetSprite` _device "/Game/Sprites/WorldMap/DeviceIcons/DevicesIcons_Sprite_0.DevicesIcons_Sprite_0"))
    (:`NewEnumerator1`
      (`PaperSpriteComponent.SetSprite` _device "/Game/Sprites/WorldMap/DeviceIcons/DevicesIcons_Sprite_1.DevicesIcons_Sprite_1"))
    (:`NewEnumerator2`
      (`PaperSpriteComponent.SetSprite` _device "/Game/Sprites/WorldMap/DeviceIcons/DevicesIcons_Sprite_2.DevicesIcons_Sprite_2"))
    (:`NewEnumerator3`
      (`PaperSpriteComponent.SetSprite` _device "/Game/Sprites/WorldMap/DeviceIcons/DevicesIcons_Sprite_3.DevicesIcons_Sprite_3"))
    (:`NewEnumerator4`
      (`PaperSpriteComponent.SetSprite` _device "/Game/Sprites/WorldMap/DeviceIcons/DevicesIcons_Sprite_4.DevicesIcons_Sprite_4"))))

(fn `UserConstructionScript`)