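; Small decorative virus on the world map that infests one PC component world and disappears once that component is restored.
; On BeginPlay it randomizes orientation, bobbing and idle flipbooks, and tints itself from the color scheme table when the video card is on.
; ExplosionControl reads player flags, destroying it silently for earlier restorations or playing a delayed shake-and-pop for fresh ones.
; Core viruses check several components, including JustSound rather than SoundCardON, and explode later.
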(event `ExplosionControl`
  (bind _playerref (`self.PlayerRef`))
  (bind _playerref_2 (`self.PlayerRef`))
  (bind _playerref_3 (`self.PlayerRef`))
  (bind _playerref_4 (`self.PlayerRef`))
  (bind _playerref_5 (`self.PlayerRef`))
  (bind _playerref_6 (`self.PlayerRef`))
  (`KismetSystemLibrary.Delay` 0.1)
  (switch `/Game/Blueprints/WorldMap/World` (`self.InfestingWorld`)
    (:`NewEnumerator0`
      (if (`/Game/Blueprints/WorldMap/WorldMap_Player.HDDON` _playerref_2)
        (if (`/Game/Blueprints/WorldMap/WorldMap_Player.JustHDD` _playerref_2)
          (`KismetSystemLibrary.Delay` 2.0 :!label _label)
          (`self.Explode`)
          (else
            (`self.K2_DestroyActor`)))))
    (:`NewEnumerator1`
      (if (`/Game/Blueprints/WorldMap/WorldMap_Player.VideoCardON` _playerref_3)
        (if (`/Game/Blueprints/WorldMap/WorldMap_Player.JustVideo` _playerref_3)
          (goto _label)
          (else
            (`self.K2_DestroyActor`)))))
    (:`NewEnumerator2`
      (if (`/Game/Blueprints/WorldMap/WorldMap_Player.SoundCardON` _playerref_4)
        (if (`/Game/Blueprints/WorldMap/WorldMap_Player.JustSound` _playerref_4)
          (goto _label)
          (else
            (`self.K2_DestroyActor`)))))
    (:`NewEnumerator3`
      (if (`/Game/Blueprints/WorldMap/WorldMap_Player.PowerSupplyON` _playerref_5)
        (if (`/Game/Blueprints/WorldMap/WorldMap_Player.JustPower` _playerref_5)
          (goto _label)
          (else
            (`self.K2_DestroyActor`)))))
    (:`NewEnumerator4`
      (if (`/Game/Blueprints/WorldMap/WorldMap_Player.CoolingSystemON` _playerref)
        (if (`/Game/Blueprints/WorldMap/WorldMap_Player.JustCooling` _playerref)
          (goto _label)
          (else
            (`self.K2_DestroyActor`)))))
    (:`NewEnumerator5`
      (if (`/Game/Blueprints/WorldMap/WorldMap_Player.HDDON` _playerref_6)
        (if (`/Game/Blueprints/WorldMap/WorldMap_Player.VideoCardON` _playerref_6)
          (if (`/Game/Blueprints/WorldMap/WorldMap_Player.JustSound` _playerref_6)
            (if (`/Game/Blueprints/WorldMap/WorldMap_Player.PowerSupplyON` _playerref_6)
              (if (`/Game/Blueprints/WorldMap/WorldMap_Player.CoolingSystemON` _playerref_6)
                (if (`/Game/Blueprints/WorldMap/WorldMap_Player.JustHDD` _playerref_6)
                  (`KismetSystemLibrary.Delay` 5.0 :!label _label_2)
                  (goto _label)
                  (elif (`/Game/Blueprints/WorldMap/WorldMap_Player.JustVideo` _playerref_6)
                    (goto _label_2)
                    (elif (`/Game/Blueprints/WorldMap/WorldMap_Player.JustSound` _playerref_6)
                      (goto _label_2)
                      (elif (`/Game/Blueprints/WorldMap/WorldMap_Player.JustPower` _playerref_6)
                        (goto _label_2)
                        (elif (`/Game/Blueprints/WorldMap/WorldMap_Player.JustCooling` _playerref_6)
                          (goto _label_2)
                          (else
                            (`self.K2_DestroyActor`)))))))))))))))

(event `ColorControl`
  ;[0 1 1] Color Control
  (`KismetSystemLibrary.Delay` 0.1)
  (if (`/Game/Blueprints/WorldMap/WorldMap_Player.VideoCardON` (`self.PlayerRef`))
    (bind _outactors (`GameplayStatics.GetAllActorsOfClass` "/Game/Blueprints/Art/ColorController.ColorController_C"))
    (bind _returnvalue (`|GetDataTableRow` "/Game/Blueprints/Art/ColorSchemeTable.ColorSchemeTable" (`/Game/Blueprints/Art/ColorController.ColorScheme` (`|GetArrayItem` _outactors)))
      (:`then`
        (`PaperFlipbookComponent.SetSpriteColor` (`self.PaperFlipbook`) (`.Enemies_33_D3933F8042CE8CB253100FB32ECD27F6` (break `/Game/Blueprints/Art/ColorScheme` _returnvalue)))))))

(event `self.ReceiveBeginPlay`
  (bind _asworld_map_player (cast `/Game/Blueprints/WorldMap/WorldMap_Player` (`GameplayStatics.GetPlayerPawn` 0)))
  (set `self.PlayerRef` _asworld_map_player)
  (`self.RandomRotation`)
  (`self.ColorControl`)
  (`self.Floating`)
  (`self.Animation Control`)
  (`self.ExplosionControl`))

(event `Animation Control`
  (bind _paperflipbook (`self.PaperFlipbook`))
  (bind _paperflipbook_2 (`self.PaperFlipbook`))
  (if (not (`self.ToExplode`)) :!label _label_3
    (`PaperFlipbookComponent.SetFlipbook` (`self.PaperFlipbook`) "/Game/Sprites/WorldMap/Virus/WorldMapVirusSmall0.WorldMapVirusSmall0")
    (`KismetSystemLibrary.Delay` (`KismetMathLibrary.RandomFloatInRange` 0.0 8.0))
    (if (`self.ToExplode`)
      _
      (elif (`KismetMathLibrary.RandomBool`)
        (`PaperFlipbookComponent.SetFlipbook` _paperflipbook "/Game/Sprites/WorldMap/Virus/WorldMapVirusSmall1.WorldMapVirusSmall1")
        (`KismetSystemLibrary.Delay` (`PaperFlipbookComponent.GetFlipbookLength` _paperflipbook))
        (goto _label_3)
        (else
          (`PaperFlipbookComponent.SetFlipbook` _paperflipbook_2 "/Game/Sprites/WorldMap/Virus/WorldMapVirusSmall2.WorldMapVirusSmall2")
          (`KismetSystemLibrary.Delay` (`PaperFlipbookComponent.GetFlipbookLength` _paperflipbook_2))
          (goto _label_3))))))

(event `Floating`
  (`|ExecutionSequence`
    (:`then_0`
      (bind (_direction _floatz) (`Timeline|Timeline_0` :`NewTime` (`KismetMathLibrary.RandomFloatInRange` 0.0 7.0) :!via `SetNewTime` :!label _label_4)
        (:`Update`
          (`SceneComponent.K2_SetRelativeLocation` (`self.PaperFlipbook`) (`KismetMathLibrary.MakeVector` 0.0 0.0 _floatz) false false))))
    (:`then_1`
      (if (`KismetMathLibrary.RandomBool`)
        (goto _label_4)
        (else
          (goto _label_4 :!via `Reverse`))))))

(event `StopFloating`
  (goto _label_4 :!via `Stop`))

(event `Explode`
  (bind _paperflipbook (`self.PaperFlipbook`))
  (bind _paperflipbook_2 (`self.PaperFlipbook`))
  (bind (_relativelocation_x _relativelocation_y _relativelocation_z) (`KismetMathLibrary.BreakVector` (`SceneComponent.RelativeLocation` _paperflipbook_2)))
  (`KismetSystemLibrary.Delay` (`KismetMathLibrary.RandomFloatInRange` 0.0 2.0))
  (set `self.ToExplode` true)
  (`PaperFlipbookComponent.SetFlipbook` (`self.PaperFlipbook`) "/Game/Sprites/WorldMap/Virus/WorldMapVirusSmall3.WorldMapVirusSmall3")
  (`self.StopFloating`)
  (bind (_direction _horizontalshake) (`Timeline|Timeline_1` :!via `ReverseFromEnd`)
    (:`Update`
      (`SceneComponent.K2_SetRelativeLocation` _paperflipbook_2 (`KismetMathLibrary.MakeVector` _horizontalshake _relativelocation_y _relativelocation_z) false false))
    (:`Finished`
      (`PaperFlipbookComponent.SetFlipbook` _paperflipbook "/Game/Sprites/WorldMap/Virus/WorldMapVirusSmallExplosion.WorldMapVirusSmallExplosion")
      (if (`/Game/Blueprints/WorldMap/WorldMap_Player.VideoCardON` (`self.PlayerRef`))
        (`PaperFlipbookComponent.SetSpriteColor` _paperflipbook (`.Explosion_34_AFEABEF2445912176FAE47AD02015058` (break `/Game/Blueprints/Art/ColorScheme` (stale `ColorControl` _returnvalue)))))
      (`GameplayStatics.PlaySound2D` "/Game/Sound/SFXs/sfx_BlopDeath_Cue.sfx_BlopDeath_Cue" (`KismetMathLibrary.RandomFloatInRange` 0.6 1.0) (`KismetMathLibrary.RandomFloatInRange` 0.8 1.0) 0.0 null null)
      (`KismetSystemLibrary.Delay` (- (`PaperFlipbookComponent.GetFlipbookLength` _paperflipbook) 0.1))
      (`self.K2_DestroyActor`))))

(event `RandomRotation`
  (`SceneComponent.K2_SetWorldRotation` (`self.PaperFlipbook`) (`KismetMathLibrary.MakeRotator` (select `bool` (`KismetMathLibrary.RandomBool`) :`true` 180.0 :!type "Float (single-precision)") (select `bool` (`KismetMathLibrary.RandomBool`) :`true` 90.0 :!type "Float (single-precision)") (select `bool` (`KismetMathLibrary.RandomBool`) :`true` 180.0 :!type "Float (single-precision)")) false false))

(fn `UserConstructionScript`)