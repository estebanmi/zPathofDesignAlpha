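; CameraFree is a level camera that follows the player in X and Z within min/max bounds and doubles as a fall-death zone.
; When active, it becomes the view target, or hands off to the corridor camera and fixes the screen collider if PreBoss is set.
; Its DeathFallingCollider saves and kills a player on hit, then reloads the level.
; Overlapping enemies are destroyed with effects only while the camera sits near its lower Z limit.
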(event `self.ReceiveBeginPlay`
  ;[1 1 1] Default
  (bind _returnvalue (`GameplayStatics.GetCurrentLevelName` true))
  (set `self.CurrentLevel` (`KismetStringLibrary.Conv_StringToName` _returnvalue))
  (`KismetSystemLibrary.Delay` 0.05)
  (bind _asplayer_bp (cast `/Game/Blueprints/Player/Player_BP` (`GameplayStatics.GetPlayerCharacter` 0)))
  (bind _output_get (set `self.PlayerRef` _asplayer_bp))
  (if (`self.ActiveCam`)
    (if (`/Game/Blueprints/Player/Player_BP.PreBoss?` _output_get)
      ;[1 1 1] PreBoss Cam (Corridor)
      (bind _outactors (`GameplayStatics.GetAllActorsOfClass` "/Game/Blueprints/CameraCorridor_BP.CameraCorridor_BP_C"))
      (bind _output (`|GetArrayItem` _outactors))
      (`PlayerController.SetViewTargetWithBlend` (`GameplayStatics.GetPlayerController` 0) _output 0.0 "VTBlend_Linear" 0.0 false)
      (bind _outactors_2 (`GameplayStatics.GetAllActorsOfClass` "/Game/Blueprints/Level/ScreenCollider_BP.ScreenCollider_BP_C"))
      (`/Game/Blueprints/Level/ScreenCollider_BP.ToFixedCam` (`|GetArrayItem` _outactors_2) (`self.K2_GetActorLocation` _output))
      (else
        (`PlayerController.SetViewTargetWithBlend` (`GameplayStatics.GetPlayerController` 0) self 0.0 "VTBlend_Linear" 0.0 false)))))

(event `PlayerFallingDeath`
  (bind (_returnvalue_x _returnvalue_y _returnvalue_z) (`KismetMathLibrary.BreakVector` (`self.K2_GetActorLocation`)))
  (bind _returnvalue_x_2 (`KismetMathLibrary.BreakVector` (`self.K2_GetActorLocation` (`self.PlayerRef`))))
  (`|SpawnActorFromClass` "/Game/Blueprints/FX/PlayerDeathFalling_FX.PlayerDeathFalling_FX_C" (`KismetMathLibrary.MakeTransform` (`KismetMathLibrary.MakeVector` _returnvalue_x_2 (`KismetMathLibrary.RandomFloatInRange` 3.0 4.0) (- _returnvalue_z 115.0)) (struct :`Roll` 180.0)) "Undefined" "OverrideRootScale" null null))

(event `self.ReceiveTick`
  (params (DeltaSeconds :type "Float (single-precision)"))
  (bind _zmax (`self.ZMax`))
  (bind _xmax (`self.XMax`))
  (bind _playerref (`self.PlayerRef`))
  (bind _zmin (`self.ZMin`))
  (bind _xmin (`self.XMin`))
  (bind (_returnvalue_x _returnvalue_y _returnvalue_z) (`KismetMathLibrary.BreakVector` (`self.K2_GetActorLocation` _playerref)))
  ;[1 1 1] Default
  (if (`self.ActiveCam`)
    (`/Engine/EditorBlueprintResources/StandardMacros.IsValid` (`self.PlayerRef`)
      (:`Is Valid`
        (if (`/Game/Blueprints/Player/Player_BP.isDead` _playerref)
          _
          (elif (not (`/Game/Blueprints/Player/Player_BP.ExitingLevel?` (`self.PlayerRef`)))
            (`self.K2_SetActorLocation` (`KismetMathLibrary.MakeVector` (`KismetMathLibrary.SelectFloat` (`KismetMathLibrary.SelectFloat` _returnvalue_x _xmin (> _returnvalue_x _xmin)) _xmax (< _returnvalue_x _xmax)) 0.0 (`KismetMathLibrary.SelectFloat` (`KismetMathLibrary.SelectFloat` _returnvalue_z _zmin (> _returnvalue_z _zmin)) _zmax (< _returnvalue_z _zmax))))))))))

(event `self.DeathFallingCollider.OnComponentHit`
  (params (HitComponent :type "PrimitiveComponent Object Reference") (OtherActor :type "Actor Object Reference") (OtherComp :type "PrimitiveComponent Object Reference") (NormalImpulse :type "Vector Structure") (Hit :type "HitResult Structure (by ref)"))
  ;[0 0 0] Death By Falling
  (bind _asplayer_bp (cast `/Game/Blueprints/Player/Player_BP` OtherActor))
  (`/Game/Blueprints/Player/Player_BP.SaveGame` _asplayer_bp)
  (`self.SetActorHiddenInGame` _asplayer_bp true)
  (`self.PlayerFallingDeath`)
  (set `/Game/Blueprints/Player/Player_BP.isDead` true _asplayer_bp)
  (set `/Game/Blueprints/Player/Player_BP.InputDisabled` false _asplayer_bp)
  (set `/Game/Blueprints/Player/Player_BP.HPCurrent` 0.0 _asplayer_bp)
  (`GameplayStatics.PlaySound2D` "/Game/Sound/SFXs/sfx_PlayerDeath_Cue.sfx_PlayerDeath_Cue" 1.0 1.0 0.0 null null)
  (`self.DisableInput` _asplayer_bp (`GameplayStatics.GetPlayerController` 0))
  (`KismetSystemLibrary.Delay` 2.0)
  (`GameplayStatics.OpenLevel` (`self.CurrentLevel`)))

(event `self.DeathFallingCollider.OnComponentBeginOverlap`
  (params (OverlappedComponent :type "PrimitiveComponent Object Reference") (OtherActor :type "Actor Object Reference") (OtherComp :type "PrimitiveComponent Object Reference") (OtherBodyIndex :type Integer) (bFromSweep :type Boolean) (SweepResult :type "HitResult Structure (by ref)"))
  (bind _returnvalue_x (`KismetMathLibrary.BreakVector` (`self.K2_GetActorLocation` OtherActor)))
  (bind (_returnvalue_x_2 _returnvalue_y _returnvalue_z) (`KismetMathLibrary.BreakVector` (`self.K2_GetActorLocation`)))
  ;[0 0 0] Death By Falling
  (if (`self.ActorHasTag` OtherActor "Enemy")
    (bind _outactors (`GameplayStatics.GetAllActorsOfClass` "CameraFree_C"))
    (bind _output (`|GetArrayItem` _outactors))
    (bind (_returnvalue_x_3 _returnvalue_y_2 _returnvalue_z_2) (`KismetMathLibrary.BreakVector` (`self.K2_GetActorLocation` _output)))
    (if (`KismetMathLibrary.NearlyEqual_FloatFloat` (`/Game/Blueprints/CameraFree.ZMin` _output) _returnvalue_z_2 5.0)
      (`GameplayStatics.PlaySound2D` "/Game/Sound/SFXs/sfx_BlopDeath_Cue.sfx_BlopDeath_Cue" (`KismetMathLibrary.RandomFloatInRange` 0.2 0.6) (`KismetMathLibrary.RandomFloatInRange` 0.8 1.2) 0.0 null null)
      (`|SpawnActorFromClass` "/Game/Blueprints/FX/DeathFallingExplosion_FX.DeathFallingExplosion_FX_C" (`KismetMathLibrary.MakeTransform` (`KismetMathLibrary.MakeVector` _returnvalue_x (`KismetMathLibrary.RandomFloatInRange` 3.0 4.0) (- _returnvalue_z 115.0)) (struct :`Roll` 180.0)) "Undefined" "OverrideRootScale" null null)
      (`self.K2_DestroyActor` OtherActor))))

(fn `UserConstructionScript`)