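; Wounded hero NPC with a Paper2D flipbook that talks to the player on overlap, then dies and calls WoundedPlayerFound on the player.
; A looping timer turns it toward the player, and the inner box opens a dialogue HUD, optionally pausing the game.
; ScrollingText types staged dialogue letter by letter with skip support, while Tick awaits Enter or gamepad input under a blinking prompt.
; After death, leaving the outer box re-arms the final dialogue stage.
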(event `FacingPlayer`
  (bind _returnvalue_x (`KismetMathLibrary.BreakVector` (`self.K2_GetActorLocation`)))
  (bind _playerref (`self.PlayerRef`))
  (bind _returnvalue_x_2 (`KismetMathLibrary.BreakVector` (`self.K2_GetActorLocation` _playerref)))
  ;[1 1 1] Facing Player
  (if (`self.CanFacePlayer`)
    (`/Engine/EditorBlueprintResources/StandardMacros.IsValid` _playerref
      (:`Is Valid`
        (if (`self.isDeath`)
          _
          (elif (< _returnvalue_x_2 _returnvalue_x)
            (`self.K2_SetActorRotation` (struct :`Yaw` 180.0))
            (else
              (`self.K2_SetActorRotation` (struct)))))))))

(event `self.ReceiveBeginPlay`
  ;[1 1 1] Default
  (bind _asplayer_bp (cast `/Game/Blueprints/Player/Player_BP` (`GameplayStatics.GetPlayerCharacter` 0)))
  (set `self.PlayerRef` _asplayer_bp)
  (`KismetSystemLibrary.K2_SetTimerDelegate` (delegate `FacingPlayer`) 0.5 true))

(event `self.BoxColliderIN.OnComponentBeginOverlap`
  (params (OverlappedComponent :type "PrimitiveComponent Object Reference") (OtherActor :type "Actor Object Reference") (OtherComp :type "PrimitiveComponent Object Reference") (OtherBodyIndex :type Integer) (bFromSweep :type Boolean) (SweepResult :type "HitResult Structure (by ref)"))
  ;[1 1 1] Start Talk
  (if (`self.isActive`)
    (cast `/Game/Blueprints/Player/Player_BP` OtherActor)
    (`/Engine/EditorBlueprintResources/StandardMacros.DoOnce` false :!label _label
      (:`Completed`
        (set `self.isRunning` true)
        (bind _foundwidgets (`WidgetBlueprintLibrary.GetAllWidgetsOfClass` "/Game/Widgets/NPCs/zFallenPlayer_HUD.zFallenPlayer_HUD_C"))
        (`Widget.RemoveFromParent` _foundwidgets)
        (set `/Game/Blueprints/Player/Player_BP.isSkipText` false (`self.PlayerRef`))
        (if (`self.PausesTheGame?`)
          (`GameplayStatics.SetGamePaused` true)
          (set `/Game/Blueprints/Player/Player_BP.isTalkingPaused` true (`self.PlayerRef`)))
        (bind _returnvalue (`|CreateWidget` "/Game/Widgets/NPCs/zFallenPlayer_HUD.zFallenPlayer_HUD_C"))
        (`UserWidget.AddToViewport` _returnvalue 0)
        (set `self.WidgetRef` _returnvalue)
        (`self.ScrollingText` (`/Game/Widgets/NPCs/zFallenPlayer_HUD.DialogText` (`self.WidgetRef`)) (select `int` (`self.StageIndex`) :`0` (`self.DialogArray_0`) :`1` (`self.DialogArray_1`) :`2` (`self.DialogArray_2`) :`3` (`self.DialogArray_3`) :`4` (`self.DialogArray_4`)) (`self.TextSpeed`))))))

(event `self.BoxColliderOut.OnComponentEndOverlap`
  (params (OverlappedComponent :type "PrimitiveComponent Object Reference") (OtherActor :type "Actor Object Reference") (OtherComp :type "PrimitiveComponent Object Reference") (OtherBodyIndex :type Integer))
  ;[1 1 1] Start Talk
  ;;[1 1 1] Reactivate NPC
  (cast `/Game/Blueprints/Player/Player_BP` OtherActor)
  (if (`self.isDeath`)
    (set `self.StageIndex` (`self.DialogsNumber`))
    (set `self.isActive` true)
    (goto _label :!via `Reset`)))

(event `self.ReceiveTick`
  (params (DeltaSeconds :type "Float (single-precision)"))
  ;[1 1 1] Waiting for Input to free player
  (if (`self.isWaitingForPlayer`)
    (`self.EnterKey`)
    (if (`/Game/Blueprints/Player/Player_BP.isMenuOn?` (`self.PlayerRef`))
      _
      (elif (`PlayerController.WasInputKeyJustPressed` (`GameplayStatics.GetPlayerController` 0) "Enter")
        (set `/Game/Blueprints/Player/Player_BP.isSkipText` false (`self.PlayerRef`) :!label _label_2)
        (`Widget.SetVisibility` (`/Game/Widgets/NPCs/zFallenPlayer_HUD.EnterKey` (`self.WidgetRef`)) "Hidden")
        (if (< (`self.StageIndex`) (`self.DialogsNumber`))
          (set `self.isWaitingForPlayer` false)
          (set `/Game/Blueprints/Player/Player_BP.isSkipText` false (`self.PlayerRef`))
          (`self.ScrollingText` (`/Game/Widgets/NPCs/zFallenPlayer_HUD.DialogText` (`self.WidgetRef`)) (select `int` (`self.StageIndex`) :`0` (`self.DialogArray_0`) :`1` (`self.DialogArray_1`) :`2` (`self.DialogArray_2`) :`3` (`self.DialogArray_2`) :`4` (`self.DialogArray_4`)) (`self.TextSpeed`))
          (else
            (if (`self.PausesTheGame?`)
              (`GameplayStatics.SetGamePaused` false)
              (set `/Game/Blueprints/Player/Player_BP.isTalkingPaused` false (`self.PlayerRef`)))
            (set `self.isWaitingForPlayer` false)
            (bind _foundwidgets (`WidgetBlueprintLibrary.GetAllWidgetsOfClass` "/Game/Widgets/NPCs/zFallenPlayer_HUD.zFallenPlayer_HUD_C"))
            (`Widget.RemoveFromParent` _foundwidgets)
            (set `self.isRunning` false)
            (set `/Game/Blueprints/Player/Player_BP.isSkipText` false (`self.PlayerRef`))
            (if (not (`self.isDeath`))
              (`GameplayStatics.PlaySound2D` "/Game/Sound/SFXs/sfx_WoundedHeroDeath_Cue.sfx_WoundedHeroDeath_Cue" 1.0 1.0 0.0 null null)
              (set `self.CanFacePlayer` false)
              (`PaperFlipbookComponent.SetFlipbook` (`self.PaperFlipbook`) "/Game/Sprites/NPCs/WoundedHero/WoundedHeroDeath.WoundedHeroDeath")
              (`KismetSystemLibrary.Delay` 1.3)
              (set `self.isDeath` true)
              (`PaperFlipbookComponent.Stop` (`self.PaperFlipbook`))
              (`KismetSystemLibrary.Delay` 0.5)
              (`/Game/Blueprints/Player/Player_BP.WoundedPlayerFound` (`self.PlayerRef`)))))
        (elif (`PlayerController.WasInputKeyJustPressed` (`GameplayStatics.GetPlayerController` 0) "Gamepad_FaceButton_Right")
          (goto _label_2))))))

(event `EnterKey`
  (bind _facebuttonright (`/Game/Widgets/NPCs/zFallenPlayer_HUD.FaceButtonRight` (`self.WidgetRef`)))
  (bind _enterkey (`/Game/Widgets/NPCs/zFallenPlayer_HUD.EnterKey` (`self.WidgetRef`)))
  ;[1 1 1] EnterKey
  (`/Engine/EditorBlueprintResources/StandardMacros.DoOnce` false :!label _label_3
    (:`Completed`
      (if (`self.isWaitingForPlayer`)
        (if (`/Game/Blueprints/Player/Player_BP.IsUsingGamepad` (`self.PlayerRef`))
          (`/Engine/EditorBlueprintResources/StandardMacros.FlipFlop`
            (:`A`
              (`Widget.SetVisibility` _facebuttonright "Visible"))
            (:`B`
              (`Widget.SetVisibility` _facebuttonright "Hidden")))
          (`KismetSystemLibrary.Delay` 0.5)
          (goto _label_3 :!via `Reset`)
          (else
            (`/Engine/EditorBlueprintResources/StandardMacros.FlipFlop`
              (:`A`
                (`Widget.SetVisibility` _enterkey "Visible"))
              (:`B`
                (`Widget.SetVisibility` _enterkey "Hidden")))
            (`KismetSystemLibrary.Delay` 0.5)
            (goto _label_3 :!via `Reset`)))))))

(fn `UserConstructionScript`)