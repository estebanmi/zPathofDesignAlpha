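; DesignerOff dialogue actor that plays a one-shot, staged on-screen conversation, triggered by player overlap or delayed auto-start.
; Starting replaces open NPC dialogue widgets with its own HUD, flags the player as talking and optionally pauses the game.
; ScrollingText types the stage's string array letter by letter with sound, honoring the player's skip flag.
; Tick then polls Enter to unpause and either play the next stage or close dialogue and free the player.
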(event `self.ReceiveBeginPlay`
  ;[1 1 1] Default
  (bind _asplayer_bp (cast `/Game/Blueprints/Player/Player_BP` (`GameplayStatics.GetPlayerCharacter` 0)))
  (set `self.PlayerRef` _asplayer_bp)
  (if (`self.AutoStart`)
    (`KismetSystemLibrary.Delay` 1.5)
    (`self.StartTalk`)
    (set `self.isActive` false)))

(event `self.BoxCollider.OnComponentBeginOverlap`
  (params (OverlappedComponent :type "PrimitiveComponent Object Reference") (OtherActor :type "Actor Object Reference") (OtherComp :type "PrimitiveComponent Object Reference") (OtherBodyIndex :type Integer) (bFromSweep :type Boolean) (SweepResult :type "HitResult Structure (by ref)"))
  ;[1 1 1] Start Talk
  (if (`self.isActive`)
    (cast `/Game/Blueprints/Player/Player_BP` OtherActor)
    (`/Engine/EditorBlueprintResources/StandardMacros.DoOnce` false :!label _label
      (:`Completed`
        (bind _foundwidgets (`WidgetBlueprintLibrary.GetAllWidgetsOfClass` "/Game/Widgets/DialogNPC_HUD.DialogNPC_HUD_C"))
        (`Widget.RemoveFromParent` _foundwidgets)
        (set `/Game/Blueprints/Player/Player_BP.isSkipText` false (`self.PlayerRef`))
        (if (`self.PausesTheGame?`)
          (`GameplayStatics.SetGamePaused` true))
        (set `/Game/Blueprints/Player/Player_BP.isTalking` true (`self.PlayerRef`))
        (bind _returnvalue (`|CreateWidget` "/Game/Widgets/DialogDesignerOff_HUD.DialogDesignerOff_HUD_C"))
        (`UserWidget.AddToViewport` _returnvalue 0)
        (set `self.WidgetRef` _returnvalue)
        (`self.ScrollingText` (`/Game/Widgets/DialogDesignerOff_HUD.DialogText` (`self.WidgetRef`)) (select `int` (`self.StageIndex`) :`0` (`self.DialogArray_0`) :`1` (`self.DialogArray_1`)) (`self.TextSpeed`))))))

(event `StartTalk`
  ;[1 1 1] Start Talk
  (goto _label))

(event `self.ReceiveTick`
  (params (DeltaSeconds :type "Float (single-precision)"))
  ;[1 1 1] Waiting for Input to free player
  (if (`self.isWaitingForPlayer`)
    (if (`PlayerController.WasInputKeyJustPressed` (`GameplayStatics.GetPlayerController` 0) "Enter")
      (if (`self.PausesTheGame?`)
        (`GameplayStatics.SetGamePaused` false))
      (if (< (`self.StageIndex`) (`self.DialogsNumber`))
        (set `self.isWaitingForPlayer` false)
        (set `/Game/Blueprints/Player/Player_BP.isSkipText` false (`self.PlayerRef`))
        (`self.ScrollingText` (`/Game/Widgets/DialogDesignerOff_HUD.DialogText` (`self.WidgetRef`)) (select `int` (`self.StageIndex`) :`0` (`self.DialogArray_0`) :`1` (`self.DialogArray_1`)) (`self.TextSpeed`))
        (else
          (set `self.isWaitingForPlayer` false)
          (set `/Game/Blueprints/Player/Player_BP.isTalking` false (`self.PlayerRef`))
          (bind _foundwidgets (`WidgetBlueprintLibrary.GetAllWidgetsOfClass` "/Game/Widgets/DialogNPC_HUD.DialogNPC_HUD_C"))
          (`Widget.RemoveFromParent` _foundwidgets)
          (set `/Game/Blueprints/Player/Player_BP.isSkipText` false (`self.PlayerRef`)))))))

(fn `UserConstructionScript`)