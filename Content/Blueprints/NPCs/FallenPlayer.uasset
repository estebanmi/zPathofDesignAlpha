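; Fallen player NPC, a wounded hero who faces the player, talks on overlap, then dies and notifies the player.
; Overlap opens a dialogue HUD, optionally pausing the game, and a looping ScrollingText macro types staged string arrays letter by letter with sound.
; Enter skips typing or advances stages; Tick polls it while waiting.
; Leaving the outer collider after death re-arms the NPC at dialogue index DialogsNumber.
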(event `FacingPlayer`
  (bind _returnvalue_x (`KismetMathLibrary.BreakVector` (`self.K2_GetActorLocation`)))
  (bind _playerref (`self.PlayerRef`))
  (bind _returnvalue_x_2 (`KismetMathLibrary.BreakVector` (`self.K2_GetActorLocation` _playerref)))
  ;[1 1 1] Facing Player
  (if (`self.CanFacePlayer`)
    (`/Engine/EditorBlueprintResources/StandardMacros.IsValid` _playerref
      (:`Is Valid`
        (if (`self.isDeath`)
          _
          (elif (< _returnvalue_x_2 _returnvalue_x)
            (`self.K2_SetActorRotation` (struct :`Yaw` 180.0))
            (else
              (`self.K2_SetActorRotation` (struct)))))))))

(event `self.ReceiveBeginPlay`
  ;[1 1 1] Default
  (bind _asplayer_bp (cast `/Game/Blueprints/Player/Player_BP` (`GameplayStatics.GetPlayerCharacter` 0)))
  (set `self.PlayerRef` _asplayer_bp)
  (`KismetSystemLibrary.K2_SetTimerDelegate` (delegate `FacingPlayer`) 0.5 true))

(event `self.BoxColliderIN.OnComponentBeginOverlap`
  (params (OverlappedComponent :type "PrimitiveComponent Object Reference") (OtherActor :type "Actor Object Reference") (OtherComp :type "PrimitiveComponent Object Reference") (OtherBodyIndex :type Integer) (bFromSweep :type Boolean) (SweepResult :type "HitResult Structure (by ref)"))
  ;[1 1 1] Start Talk
  (if (`self.isActive`)
    (cast `/Game/Blueprints/Player/Player_BP` OtherActor)
    (`/Engine/EditorBlueprintResources/StandardMacros.DoOnce` false :!label _label
      (:`Completed`
        (set `self.isRunning` true)
        (bind _foundwidgets (`WidgetBlueprintLibrary.GetAllWidgetsOfClass` "/Game/Widgets/FallenPlayer_HUD.FallenPlayer_HUD_C"))
        (`Widget.RemoveFromParent` _foundwidgets)
        (set `/Game/Blueprints/Player/Player_BP.isSkipText` false (`self.PlayerRef`))
        (if (`self.PausesTheGame?`)
          (`GameplayStatics.SetGamePaused` true))
        (bind _returnvalue (`|CreateWidget` "/Game/Widgets/FallenPlayer_HUD.FallenPlayer_HUD_C"))
        (`UserWidget.AddToViewport` _returnvalue 0)
        (set `self.WidgetRef` _returnvalue)
        (`self.ScrollingText` (`/Game/Widgets/FallenPlayer_HUD.DialogText` (`self.WidgetRef`)) (select `int` (`self.StageIndex`) :`0` (`self.DialogArray_0`) :`1` (`self.DialogArray_1`) :`2` (`self.DialogArray_2`) :`3` (`self.DialogArray_3`) :`4` (`self.DialogArray_4`)) (`self.TextSpeed`))))))

(event `self.BoxColliderOut.OnComponentEndOverlap`
  (params (OverlappedComponent :type "PrimitiveComponent Object Reference") (OtherActor :type "Actor Object Reference") (OtherComp :type "PrimitiveComponent Object Reference") (OtherBodyIndex :type Integer))
  ;[1 1 1] Start Talk
  ;;[1 1 1] Reactivate NPC
  (cast `/Game/Blueprints/Player/Player_BP` OtherActor)
  (if (`self.isDeath`)
    (set `self.StageIndex` (`self.DialogsNumber`))
    (set `self.isActive` true)
    (goto _label :!via `Reset`)))

(event `self.ReceiveTick`
  (params (DeltaSeconds :type "Float (single-precision)"))
  ;[1 1 1] Waiting for Input to free player
  (if (`self.isWaitingForPlayer`)
    (`self.EnterKey`)
    (if (`PlayerController.WasInputKeyJustPressed` (`GameplayStatics.GetPlayerController` 0) "Enter")
      (`Widget.SetVisibility` (`/Game/Widgets/FallenPlayer_HUD.EnterKey` (`self.WidgetRef`)) "Hidden")
      (if (< (`self.StageIndex`) (`self.DialogsNumber`))
        (set `self.isWaitingForPlayer` false)
        (set `/Game/Blueprints/Player/Player_BP.isSkipText` false (`self.PlayerRef`))
        (`self.ScrollingText` (`/Game/Widgets/FallenPlayer_HUD.DialogText` (`self.WidgetRef`)) (select `int` (`self.StageIndex`) :`0` (`self.DialogArray_0`) :`1` (`self.DialogArray_1`) :`2` (`self.DialogArray_2`) :`3` (`self.DialogArray_2`) :`4` (`self.DialogArray_4`)) (`self.TextSpeed`))
        (else
          (if (`self.PausesTheGame?`)
            (`GameplayStatics.SetGamePaused` false))
          (set `self.isWaitingForPlayer` false)
          (bind _foundwidgets (`WidgetBlueprintLibrary.GetAllWidgetsOfClass` "/Game/Widgets/FallenPlayer_HUD.FallenPlayer_HUD_C"))
          (`Widget.RemoveFromParent` _foundwidgets)
          (set `self.isRunning` false)
          (set `/Game/Blueprints/Player/Player_BP.isSkipText` false (`self.PlayerRef`))
          (if (not (`self.isDeath`))
            (`GameplayStatics.PlaySound2D` "/Game/Sound/SFXs/sfx_WoundedHeroDeath_Cue.sfx_WoundedHeroDeath_Cue" 1.0 1.0 0.0 null null)
            (set `self.CanFacePlayer` false)
            (`PaperFlipbookComponent.SetFlipbook` (`self.PaperFlipbook`) "/Game/Sprites/NPCs/WoundedHero/WoundedHeroDeath.WoundedHeroDeath")
            (`KismetSystemLibrary.Delay` 1.3)
            (set `self.isDeath` true)
            (`PaperFlipbookComponent.Stop` (`self.PaperFlipbook`))
            (`KismetSystemLibrary.Delay` 0.5)
            (`/Game/Blueprints/Player/Player_BP.WoundedPlayerFound` (`self.PlayerRef`))))))))

(event `EnterKey`
  (bind _enterkey (`/Game/Widgets/FallenPlayer_HUD.EnterKey` (`self.WidgetRef`)))
  ;[1 1 1] EnterKey
  (if (>= (`self.StageIndex`) (`self.DialogsNumber`))
    (`/Engine/EditorBlueprintResources/StandardMacros.DoOnce` false :!label _label_2
      (:`Completed`
        (if (`self.isWaitingForPlayer`)
          (`/Engine/EditorBlueprintResources/StandardMacros.FlipFlop`
            (:`A`
              (`Widget.SetVisibility` _enterkey "Visible"))
            (:`B`
              (`Widget.SetVisibility` _enterkey "Hidden")))
          (`KismetSystemLibrary.Delay` 0.5)
          (goto _label_2 :!via `Reset`))))))

(event `Key|Enter` :paused true
  (params (Key :type "Key Structure"))
  (:`Pressed`
    (if (`self.isRunning`)
      (set `/Game/Blueprints/Player/Player_BP.isSkipText` true (`self.PlayerRef`)))))

(fn `UserConstructionScript`)