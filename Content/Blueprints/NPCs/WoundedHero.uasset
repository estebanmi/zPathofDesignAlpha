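; Wounded hero NPC in a Paper2D game that talks to the player, then dies after the first conversation.
; A looping timer turns it toward the player while alive.
; Trigger overlap locks input and opens a dialog widget, typing stage-selected lines letter by letter with sound.
; A key press closes the dialog, plays the death once and frees the player; leaving the outer box re-arms it for post-death dialog.
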(event `FacingPlayer`
  (bind _returnvalue_x (`KismetMathLibrary.BreakVector` (`self.K2_GetActorLocation`)))
  (bind _playerref (`self.PlayerRef`))
  (bind _returnvalue_x_2 (`KismetMathLibrary.BreakVector` (`self.K2_GetActorLocation` _playerref)))
  ;[1 1 1] Facing Player
  (`/Engine/EditorBlueprintResources/StandardMacros.IsValid` _playerref
    (:`Is Valid`
      (if (`self.isDeath`)
        _
        (elif (< _returnvalue_x_2 _returnvalue_x)
          (`self.K2_SetActorRotation` (struct :`Yaw` 180.0))
          (else
            (`self.K2_SetActorRotation` (struct))))))))

(event `self.ReceiveBeginPlay`
  ;[1 1 1] Default
  (bind _asplayer_sword_bp (cast `/Game/Blueprints/Player/PlayerSword_BP` (`GameplayStatics.GetPlayerCharacter` 0)))
  (set `self.PlayerRef` _asplayer_sword_bp)
  (`KismetSystemLibrary.K2_SetTimerDelegate` (delegate `FacingPlayer`) 0.5 true))

(event `self.BoxColliderIN.OnComponentBeginOverlap`
  (params (OverlappedComponent :type "PrimitiveComponent Object Reference") (OtherActor :type "Actor Object Reference") (OtherComp :type "PrimitiveComponent Object Reference") (OtherBodyIndex :type Integer) (bFromSweep :type Boolean) (SweepResult :type "HitResult Structure (by ref)"))
  ;[1 1 1] Start Talk (Block Player)
  (if (`self.isActive`)
    (cast `/Game/Blueprints/Player/PlayerSword_BP` OtherActor)
    (set `self.isActive` false)
    (set `/Game/Blueprints/Player/PlayerSword_BP.InputDisabled` true (`self.PlayerRef`))
    (set `/Game/Blueprints/Player/PlayerSword_BP.isTalking` true (`self.PlayerRef`))
    (bind _returnvalue (`|CreateWidget` "/Game/Widgets/DialogWoundedHero_HUD.DialogWoundedHero_HUD_C"))
    (`UserWidget.AddToViewport` _returnvalue 0)
    (set `self.WidgetRef` _returnvalue)
    (`self.ScrollingText` (`/Game/Widgets/DialogWoundedHero_HUD.MultiLineEditableTextBox_72` (`self.WidgetRef`)) (select `int` (`self.StageIndex`) :`0` (`self.DialogArray_0`) :`1` (`self.DialogArray_1`)) (`self.TextSpeed`))))

(event `self.ReceiveTick`
  (params (DeltaSeconds :type "Float (single-precision)"))
  (bind _playerref (`self.PlayerRef`))
  ;[1 1 1] Waiting for Input to free player
  (if (`self.isWaitingForPlayer`)
    (if (`PlayerController.WasInputKeyJustPressed` (`GameplayStatics.GetPlayerController` 0) "AnyKey")
      (set `self.isWaitingForPlayer` false)
      (set `/Game/Blueprints/Player/PlayerSword_BP.isTalking` false _playerref)
      (bind _foundwidgets (`WidgetBlueprintLibrary.GetAllWidgetsOfClass` "/Game/Widgets/DialogWoundedHero_HUD.DialogWoundedHero_HUD_C"))
      (`Widget.RemoveFromParent` _foundwidgets)
      (if (`self.isDeath`)
        (set `/Game/Blueprints/Player/PlayerSword_BP.InputDisabled` false _playerref)
        (else
          (`GameplayStatics.PlaySound2D` "/Game/Sound/SFXs/sfx_WoundedHeroDeath_Cue.sfx_WoundedHeroDeath_Cue" 1.0 1.0 0.0 null null)
          (`PaperFlipbookComponent.SetFlipbook` (`self.PaperFlipbook`) "/Game/Sprites/NPCs/WoundedHero/WoundedHeroDeath.WoundedHeroDeath")
          (`KismetSystemLibrary.Delay` 1.3)
          (set `self.isDeath` true)
          (set `/Game/Blueprints/Player/PlayerSword_BP.InputDisabled` false _playerref)
          (`PaperFlipbookComponent.Stop` (`self.PaperFlipbook`)))))))

(event `self.BoxColliderOut.OnComponentEndOverlap`
  (params (OverlappedComponent :type "PrimitiveComponent Object Reference") (OtherActor :type "Actor Object Reference") (OtherComp :type "PrimitiveComponent Object Reference") (OtherBodyIndex :type Integer))
  ;[1 1 1] Reactivate NPC
  (cast `/Game/Blueprints/Player/PlayerSword_BP` OtherActor)
  (set `self.isActive` true))

(fn `UserConstructionScript`)