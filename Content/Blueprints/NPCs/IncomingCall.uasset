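; IncomingCall is a trigger actor that starts a phone-call dialogue when the player overlaps its box, optionally removing itself after the boss phase.
; Tick polls for an accept key, then pauses the game and music and opens the Call_HUD chat.
; A recursive-loop ScrollingText macro types up to five dialogue stages letter by letter with sound and skipping, waiting for key presses between stages before restoring player control.
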(event `self.ReceiveBeginPlay`
  (bind _asplayer_bp (cast `/Game/Blueprints/Player/Player_BP` (`GameplayStatics.GetPlayerCharacter` 0)))
  (set `self.PlayerRef` _asplayer_bp)
  (bind _outactors (`GameplayStatics.GetAllActorsOfClass` "/Game/Blueprints/MusicController.MusicController_C"))
  (set `self.MusicControllerRef` (`|GetArrayItem` _outactors))
  (`KismetSystemLibrary.Delay` 0.05)
  (if (`/Game/Blueprints/Player/Player_BP.PreBoss?` (`self.PlayerRef`))
    _
    (elif (`self.CallAfterKilledByBoss`)
      (`self.K2_DestroyActor`))))

(event `self.BoxCollider.OnComponentBeginOverlap`
  (params (OverlappedComponent :type "PrimitiveComponent Object Reference") (OtherActor :type "Actor Object Reference") (OtherComp :type "PrimitiveComponent Object Reference") (OtherBodyIndex :type Integer) (bFromSweep :type Boolean) (SweepResult :type "HitResult Structure (by ref)"))
  (cast `/Game/Blueprints/Player/Player_BP` OtherActor)
  (`/Engine/EditorBlueprintResources/StandardMacros.DoOnce` false :!label _label
    (:`Completed`
      (if (`self.Calling`)
        _
        (elif (not (`self.CallAlreadyDone`))
          (set `self.Calling` true)
          (bind _outactors (`GameplayStatics.GetAllActorsOfClass` "/Game/Blueprints/MenuController.MenuController_C"))
          (set `/Game/Blueprints/MenuController.isCalling` true (`|GetArrayItem` _outactors))
          (bind _returnvalue (`|CreateWidget` "/Game/Widgets/NPCs/IncomingCall_HUD.IncomingCall_HUD_C"))
          (`UserWidget.AddToViewport` _returnvalue 0)
          (`KismetSystemLibrary.Delay` 12.0)
          (goto _label :!via `Reset`))))))

(event `self.ReceiveTick`
  (params (DeltaSeconds :type "Float (single-precision)"))
  (if (`/Game/Blueprints/Player/Player_BP.isMenuOn?` (`self.PlayerRef`))
    _
    (elif (`self.Calling`)
      (if (`self.CallAlreadyDone`)
        (`self.FreePlayer`)
        (`self.SkipTextListener`)
        (elif (`PlayerController.WasInputKeyJustPressed` (`GameplayStatics.GetPlayerController` 0) "Enter")
          (bind _foundwidgets (`WidgetBlueprintLibrary.GetAllWidgetsOfClass` "/Game/Widgets/NPCs/IncomingCall_HUD.IncomingCall_HUD_C" :!label _label_2))
          (`Widget.RemoveFromParent` _foundwidgets)
          (set `self.CallAlreadyDone` true)
          (`self.StartTalk`)
          (`GameplayStatics.PlaySound2D` "/Game/Sound/SFXs/sfx_CallAccepted_Cue.sfx_CallAccepted_Cue" 1.0 1.0 0.0 null null)
          (`GameplayStatics.SetGamePaused` true)
          (`/Game/Blueprints/MusicController.PauseVolume` (`self.MusicControllerRef`))
          (elif (`PlayerController.WasInputKeyJustPressed` (`GameplayStatics.GetPlayerController` 0) "Gamepad_Special_Right")
            (goto _label_2)))))))

(event `StartTalk`
  ;[1 0 0.401] Chat
  (set `/Game/Blueprints/Player/Player_BP.isTalkingPaused` true (`self.PlayerRef`))
  (`self.DialogsNumberCalculator`)
  (set `self.ChatIsRunning` true)
  (set `/Game/Blueprints/Player/Player_BP.isSkipText` false (`self.PlayerRef`))
  (bind _returnvalue (`|CreateWidget` "/Game/Widgets/NPCs/Call_HUD.Call_HUD_C"))
  (`UserWidget.AddToViewport` _returnvalue 0)
  (set `self.WidgetRef` _returnvalue)
  (`self.ScrollingText` (`/Game/Widgets/NPCs/Call_HUD.DialogText` (`self.WidgetRef`)) (select `int` (`self.StageIndex`) :`0` (`self.DialogArray_0`) :`1` (`self.DialogArray_1`) :`2` (`self.DialogArray_2`) :`3` (`self.DialogArray_3`) :`4` (`self.DialogArray_4`)) (`self.TextSpeed`)))

(event `PressAnyKey`
  (bind _pressanykey (`/Game/Widgets/NPCs/Call_HUD.PressAnyKey` (`self.WidgetRef`)))
  ;[1 0 0.401] Chat
  ;;[1 0 0.5463] EnterKey
  (`/Engine/EditorBlueprintResources/StandardMacros.DoOnce` false :!label _label_3
    (:`Completed`
      (if (`self.isWaitingForPlayer`)
        (`/Engine/EditorBlueprintResources/StandardMacros.FlipFlop`
          (:`A`
            (`Widget.SetVisibility` _pressanykey "Visible"))
          (:`B`
            (`Widget.SetVisibility` _pressanykey "Hidden")))
        (`KismetSystemLibrary.Delay` 0.5)
        (goto _label_3 :!via `Reset`)))))

(event `FreePlayer`
  (bind _playerref (`self.PlayerRef`))
  ;[1 0 0.401] Chat
  ;;[1 0 0.6276] Waiting for Input to free player
  (if (`self.isWaitingForPlayer`)
    (`self.PressAnyKey`)
    (if (`PlayerController.WasInputKeyJustPressed` (`GameplayStatics.GetPlayerController` 0) "Enter")
      (`Widget.SetVisibility` (`/Game/Widgets/NPCs/Call_HUD.PressAnyKey` (`self.WidgetRef`)) "Hidden" :!label _label_4)
      (if (< (`self.StageIndex`) (`self.DialogsNumber`))
        (`KismetSystemLibrary.Delay` 0.05)
        (set `self.isWaitingForPlayer` false)
        (set `/Game/Blueprints/Player/Player_BP.isSkipText` false (`self.PlayerRef`))
        (`self.ScrollingText` (`/Game/Widgets/NPCs/Call_HUD.DialogText` (`self.WidgetRef`)) (select `int` (`self.StageIndex`) :`0` (`self.DialogArray_0`) :`1` (`self.DialogArray_1`) :`2` (`self.DialogArray_2`) :`3` (`self.DialogArray_3`) :`4` (`self.DialogArray_4`)) (`self.TextSpeed`))
        (else
          ;;;[1 1 1] Free Player
          (`self.EnableInput` (`self.PlayerRef`) (`GameplayStatics.GetPlayerController` 0))
          (set `/Game/Blueprints/Player/Player_BP.isTalkingPaused` false _playerref)
          (set `/Game/Blueprints/Player/Player_BP.InputDisabled` false _playerref)
          (if (`PlayerController.IsInputKeyDown` (`GameplayStatics.GetPlayerController` 0) "RightControl")
            (`/Game/Blueprints/Player/Player_BP.ContinueShooting` (`self.PlayerRef`) :!label _label_5)
            (elif (`PlayerController.IsInputKeyDown` (`GameplayStatics.GetPlayerController` 0) "Gamepad_FaceButton_Left")
              (goto _label_5)
              (else
                _)))
          ;;;[1 1 1] Chat End
          (set `/Game/Blueprints/Player/Player_BP.InputDisabled` false (`self.PlayerRef`))
          (set `self.isWaitingForPlayer` false)
          (bind _foundwidgets (`WidgetBlueprintLibrary.GetAllWidgetsOfClass` "/Game/Widgets/NPCs/Call_HUD.Call_HUD_C"))
          (`Widget.RemoveFromParent` _foundwidgets)
          (set `self.ChatIsRunning` false)
          (set `/Game/Blueprints/Player/Player_BP.isSkipText` false (`self.PlayerRef`))
          (`GameplayStatics.SetGamePaused` false)
          (`/Game/Blueprints/MusicController.inGameVolume` (`self.MusicControllerRef`))))
      (elif (`PlayerController.WasInputKeyJustPressed` (`GameplayStatics.GetPlayerController` 0) "SpaceBar")
        (goto _label_4)
        (elif (`PlayerController.WasInputKeyJustPressed` (`GameplayStatics.GetPlayerController` 0) "RightControl")
          (goto _label_4)
          (elif (`PlayerController.WasInputKeyJustPressed` (`GameplayStatics.GetPlayerController` 0) "Gamepad_FaceButton_Right")
            (goto _label_4)
            (elif (`PlayerController.WasInputKeyJustPressed` (`GameplayStatics.GetPlayerController` 0) "Gamepad_FaceButton_Left")
              (goto _label_4)
              (elif (`PlayerController.WasInputKeyJustPressed` (`GameplayStatics.GetPlayerController` 0) "Gamepad_FaceButton_Bottom")
                (goto _label_4)))))))))

(event `SkipTextListener`
  ;[1 0 0.401] Chat
  ;;[1 0 0.6276] Waiting for Input to free player
  ;;;[1 1 1] Skip Text Listener
  (if (`self.isTalking`)
    (if (`PlayerController.WasInputKeyJustPressed` (`GameplayStatics.GetPlayerController` 0) "Enter")
      (set `/Game/Blueprints/Player/Player_BP.isSkipText` true (`self.PlayerRef`) :!label _label_6)
      (elif (`PlayerController.WasInputKeyJustPressed` (`GameplayStatics.GetPlayerController` 0) "SpaceBar")
        (goto _label_6)
        (elif (`PlayerController.WasInputKeyJustPressed` (`GameplayStatics.GetPlayerController` 0) "RightControl")
          (goto _label_6)
          (elif (`PlayerController.WasInputKeyJustPressed` (`GameplayStatics.GetPlayerController` 0) "Gamepad_FaceButton_Right")
            (goto _label_6)
            (elif (`PlayerController.WasInputKeyJustPressed` (`GameplayStatics.GetPlayerController` 0) "Gamepad_FaceButton_Left")
              (goto _label_6)
              (elif (`PlayerController.WasInputKeyJustPressed` (`GameplayStatics.GetPlayerController` 0) "Gamepad_FaceButton_Bottom")
                (goto _label_6)))))))))

(event `DialogsNumberCalculator`
  ;[1 0 0.401] Chat
  ;;[1 1 1] Dialog Number Calculator
  (if (`KismetStringLibrary.NotEqual_StrStr` (`|GetArrayItem` (`KismetStringLibrary.GetCharacterArrayFromString` (`|GetArrayItem` (`self.DialogArray_0`)))))
    (set `self.DialogsNumber` (+ (`self.DialogsNumber`) 1))
    (if (`KismetStringLibrary.NotEqual_StrStr` (`|GetArrayItem` (`KismetStringLibrary.GetCharacterArrayFromString` (`|GetArrayItem` (`self.DialogArray_1`)))))
      (set `self.DialogsNumber` (+ (`self.DialogsNumber`) 1))
      (if (`KismetStringLibrary.NotEqual_StrStr` (`|GetArrayItem` (`KismetStringLibrary.GetCharacterArrayFromString` (`|GetArrayItem` (`self.DialogArray_2`)))))
        (set `self.DialogsNumber` (+ (`self.DialogsNumber`) 1))
        (if (`KismetStringLibrary.NotEqual_StrStr` (`|GetArrayItem` (`KismetStringLibrary.GetCharacterArrayFromString` (`|GetArrayItem` (`self.DialogArray_3`)))))
          (set `self.DialogsNumber` (+ (`self.DialogsNumber`) 1))
          (if (`KismetStringLibrary.NotEqual_StrStr` (`|GetArrayItem` (`KismetStringLibrary.GetCharacterArrayFromString` (`|GetArrayItem` (`self.DialogArray_4`)))))
            (set `self.DialogsNumber` (+ (`self.DialogsNumber`) 1))))))))

(fn `UserConstructionScript`)