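; NPC that faces the player on a looping timer and opens a dialogue widget when the player enters its inner box.
; Talking pauses the game and blocks input while ScrollingText types the stage's lines letter by letter with sound, or instantly when skipped.
; Afterwards the stage is set to 1, and any key press on Tick closes widgets and frees the player.
; Leaving the outer box re-arms the NPC.
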(event `FacingPlayer`
  (bind _returnvalue_x (`KismetMathLibrary.BreakVector` (`self.K2_GetActorLocation`)))
  (bind _playerref (`self.PlayerRef`))
  (bind _returnvalue_x_2 (`KismetMathLibrary.BreakVector` (`self.K2_GetActorLocation` _playerref)))
  ;[1 1 1] Facing Player
  (`/Engine/EditorBlueprintResources/StandardMacros.IsValid` _playerref
    (:`Is Valid`
      (if (< _returnvalue_x_2 _returnvalue_x)
        (`self.K2_SetActorRotation` (struct :`Yaw` 180.0))
        (else
          (`self.K2_SetActorRotation` (struct)))))))

(event `self.ReceiveBeginPlay`
  ;[1 1 1] Default
  (bind _asplayer_bp (cast `/Game/Blueprints/Player/Player_BP` (`GameplayStatics.GetPlayerCharacter` 0)))
  (set `self.PlayerRef` _asplayer_bp)
  (`KismetSystemLibrary.K2_SetTimerDelegate` (delegate `FacingPlayer`) 0.5 true))

(event `self.BoxColliderIN.OnComponentBeginOverlap`
  (params (OverlappedComponent :type "PrimitiveComponent Object Reference") (OtherActor :type "Actor Object Reference") (OtherComp :type "PrimitiveComponent Object Reference") (OtherBodyIndex :type Integer) (bFromSweep :type Boolean) (SweepResult :type "HitResult Structure (by ref)"))
  ;[1 1 1] Start Talk (Block Player)
  (if (`self.isActive`)
    (bind _asplayer_bp (cast `/Game/Blueprints/Player/Player_BP` OtherActor))
    (set `self.isRunning` true)
    (`GameplayStatics.SetGamePaused` true)
    (set `/Game/Blueprints/Player/Player_BP.InputDisabled` true _asplayer_bp)
    (set `self.isActive` false)
    (bind _returnvalue (`|CreateWidget` null))
    (`UserWidget.AddToViewport` _returnvalue 0)
    (set `self.WidgetRef` _returnvalue)
    (`self.ScrollingText` (`/Game/Blueprints/NPCs/Talker.DialogText` (`self.WidgetRef`)) (select `int` (`self.StageIndex`) :`0` (`self.DialogArray_0`) :`1` (`self.DialogArray_1`) :`2` (`self.DialogArray_2`) :`3` (`self.DialogArray_3`) :`4` (`self.DialogArray_4`)) (`self.TextSpeed`))))

(event `self.BoxColliderOUT.OnComponentEndOverlap`
  (params (OverlappedComponent :type "PrimitiveComponent Object Reference") (OtherActor :type "Actor Object Reference") (OtherComp :type "PrimitiveComponent Object Reference") (OtherBodyIndex :type Integer))
  ;[1 1 1] Reactivate NPC
  (cast `/Game/Blueprints/Player/Player_BP` OtherActor)
  (set `self.isActive` true))

(event `self.ReceiveTick`
  (params (DeltaSeconds :type "Float (single-precision)"))
  ;[1 1 1] Waiting for Input to free player
  (if (`self.isWaitingForPlayer`)
    (if (`PlayerController.WasInputKeyJustPressed` (`GameplayStatics.GetPlayerController` 0) "AnyKey")
      (`GameplayStatics.PlaySound2D` "/Game/Sound/SFXs/sfx_StepBlock1_Cue.sfx_StepBlock1_Cue" 1.0 1.0 0.0 null null)
      (`GameplayStatics.SetGamePaused` false)
      (set `self.isWaitingForPlayer` false)
      (set `/Game/Blueprints/Player/Player_BP.InputDisabled` false (`self.PlayerRef`))
      (bind _foundwidgets (`WidgetBlueprintLibrary.GetAllWidgetsOfClass` null))
      (`Widget.RemoveFromParent` _foundwidgets)
      (set `self.isRunning` false)
      (set `/Game/Blueprints/Player/Player_BP.isSkipText` false (`self.PlayerRef`)))))

(fn `UserConstructionScript`)