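; DesignTip is a Paper2D tip marker actor that swaps between two sprites according to its Closer flag, refreshed every tick.
; It follows FollowActor at a Z offset, or without one starts a Floating timeline once that adds to its current Z.
; BeginPlay picks a random Y that every move reuses, and prints an error for a missing WidgetRef when Closer is false.
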(event `self.ReceiveBeginPlay`
  (bind (_returnvalue_x _returnvalue_y _returnvalue_z) (`KismetMathLibrary.BreakVector` (`self.K2_GetActorLocation`)))
  (set `self.RandomY` (`KismetMathLibrary.RandomFloatInRange` 5.0 10.0))
  (`self.K2_SetActorLocation` (`KismetMathLibrary.MakeVector` _returnvalue_x (`self.RandomY`) _returnvalue_z))
  (if (not (`self.Closer`))
    (`SceneComponent.SetVisibility` (`self.PaperSprite`) false false)
    (`SceneComponent.SetVisibility` (`self.PaperSprite1`) true false)
    (if (not (`KismetSystemLibrary.IsValidClass` (`self.WidgetRef`)))
      (`KismetSystemLibrary.PrintString` (`KismetStringLibrary.Concat_StrStr` "ERROR: " (`KismetSystemLibrary.GetDisplayName` self) " has no WidgetRef value") true true (struct :`R` 1.0 :`G` 0.028078 :`A` 1.0) 20.0))))

(event `self.ReceiveTick`
  (params (DeltaSeconds :type "Float (single-precision)"))
  (bind (_returnvalue_x _returnvalue_y _returnvalue_z) (`KismetMathLibrary.BreakVector` (`self.K2_GetActorLocation`)))
  (bind _followactor (`self.FollowActor`))
  (bind (_returnvalue_x_2 _returnvalue_y_2 _returnvalue_z_2) (`KismetMathLibrary.BreakVector` (`self.K2_GetActorLocation` _followactor)))
  (`self.CloserOrNot`)
  (`/Engine/EditorBlueprintResources/StandardMacros.IsValid` _followactor
    (:`Is Valid`
      (`self.K2_SetActorLocation` (`KismetMathLibrary.MakeVector` _returnvalue_x_2 (`self.RandomY`) (+ _returnvalue_z_2 (`self.Offset`)))))
    (:`Is Not Valid`
      (`/Engine/EditorBlueprintResources/StandardMacros.DoOnce` false
        (:`Completed`
          (bind (_direction _floatingz) (`Timeline|Floating` :!via `PlayFromStart`)
            (:`Update`
              (`self.K2_SetActorLocation` (`KismetMathLibrary.MakeVector` _returnvalue_x (`self.RandomY`) (+ _floatingz _returnvalue_z))))))))))

(event `CloserOrNot`
  (if (`self.Closer`)
    (`SceneComponent.SetVisibility` (`self.PaperSprite`) true false)
    (`SceneComponent.SetVisibility` (`self.PaperSprite1`) false false)
    (else
      (`SceneComponent.SetVisibility` (`self.PaperSprite`) false false)
      (`SceneComponent.SetVisibility` (`self.PaperSprite1`) true false))))

(fn `UserConstructionScript`)