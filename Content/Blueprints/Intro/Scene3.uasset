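; Scene3 is an intro scene Blueprint that loops a small shaking animation on two hand components, HandL and HandR.
; BeginPlay starts HandShacking, which nudges the hands along X in opposite directions, then back, with short Delays between steps.
; A HandIndex counter groups the shakes into bursts of three, each followed by a longer pause, repeating indefinitely through a looped exec wire.
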(event `HandShacking`
  (bind _handl (`self.HandL`))
  (bind _handl_2 (`self.HandL`))
  (bind _handr (`self.HandR`))
  (bind _handr_2 (`self.HandR`))
  (bind (_relativelocation_x _relativelocation_y _relativelocation_z) (`KismetMathLibrary.BreakVector` (`SceneComponent.RelativeLocation` _handl)))
  (bind (_relativelocation_x_2 _relativelocation_y_2 _relativelocation_z_2) (`KismetMathLibrary.BreakVector` (`SceneComponent.RelativeLocation` _handl_2)))
  (bind (_relativelocation_x_3 _relativelocation_y_3 _relativelocation_z_3) (`KismetMathLibrary.BreakVector` (`SceneComponent.RelativeLocation` _handr)))
  (bind (_relativelocation_x_4 _relativelocation_y_4 _relativelocation_z_4) (`KismetMathLibrary.BreakVector` (`SceneComponent.RelativeLocation` _handr_2)))
  (`SceneComponent.K2_SetRelativeLocation` _handl (`KismetMathLibrary.MakeVector` (+ _relativelocation_x 1.0) _relativelocation_y _relativelocation_z) false false :!label _label)
  (`SceneComponent.K2_SetRelativeLocation` _handr_2 (`KismetMathLibrary.MakeVector` (+ _relativelocation_x_4 -1.0) _relativelocation_y_4 _relativelocation_z_4) false false)
  (`KismetSystemLibrary.Delay` 0.08)
  (`SceneComponent.K2_SetRelativeLocation` _handl_2 (`KismetMathLibrary.MakeVector` (+ _relativelocation_x_2 -1.0) _relativelocation_y_2 _relativelocation_z_2) false false)
  (`SceneComponent.K2_SetRelativeLocation` _handr (`KismetMathLibrary.MakeVector` (+ _relativelocation_x_3 1.0) _relativelocation_y_3 _relativelocation_z_3) false false)
  (`KismetSystemLibrary.Delay` 0.08)
  (if (< (`self.HandIndex`) 2)
    (set `self.HandIndex` (+ (`self.HandIndex`) 1))
    (goto _label)
    (else
      (set `self.HandIndex` 0)
      (`KismetSystemLibrary.Delay` 0.7)
      (goto _label))))

(event `self.ReceiveBeginPlay`
  (`self.HandShacking`))

(fn `UserConstructionScript`)