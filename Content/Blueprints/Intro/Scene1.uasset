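; Intro scene actor that animates the 2D Paper2D characters and props of the first intro scene with endless randomized loops.
; BeginPlay starts four independent Delay-based loops, one each for the Arm, Mati, Bella and Hand.
; Arm flip-flops between two sprites at random intervals, and Hand returns to a base sprite before randomly showing one of two others.
; Mati and Bella hold one flipbook for a random time, then play a second for its full length.
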(event `ArmAnimation`
  (bind _arm (`self.Arm`))
  (`/Engine/EditorBlueprintResources/StandardMacros.FlipFlop` :!label _label
    (:`A`
      (`PaperSpriteComponent.SetSprite` _arm "/Game/Sprites/Intro/Scene1/Scene1Sprites_Sprite_1.Scene1Sprites_Sprite_1"))
    (:`B`
      (`PaperSpriteComponent.SetSprite` _arm "/Game/Sprites/Intro/Scene1/Scene1Sprites_Sprite_6.Scene1Sprites_Sprite_6")))
  (`KismetSystemLibrary.Delay` (`KismetMathLibrary.RandomFloatInRange` 0.3 1.2))
  (goto _label))

(event `self.ReceiveBeginPlay`
  (`self.ArmAnimation`)
  (`self.MatiAnimation`)
  (`self.BellaAnimation`)
  (`self.HandAnimation`))

(event `MatiAnimation`
  (bind _mati (`self.Mati`))
  (`PaperFlipbookComponent.SetFlipbook` (`self.Mati`) "/Game/Sprites/Intro/Scene1/Mati0.Mati0" :!label _label_2)
  (`KismetSystemLibrary.Delay` (`KismetMathLibrary.RandomFloatInRange` 0.2 1.5))
  (`PaperFlipbookComponent.SetFlipbook` _mati "/Game/Sprites/Intro/Scene1/Mati1.Mati1")
  (`KismetSystemLibrary.Delay` (`PaperFlipbookComponent.GetFlipbookLength` _mati))
  (goto _label_2))

(event `BellaAnimation`
  (bind _bella (`self.Bella`))
  (`PaperFlipbookComponent.SetFlipbook` (`self.Bella`) "/Game/Sprites/Intro/Scene1/Bella0.Bella0" :!label _label_3)
  (`KismetSystemLibrary.Delay` (`KismetMathLibrary.RandomFloatInRange` 0.8 1.5))
  (`PaperFlipbookComponent.SetFlipbook` _bella "/Game/Sprites/Intro/Scene1/Bella1.Bella1")
  (`KismetSystemLibrary.Delay` (`PaperFlipbookComponent.GetFlipbookLength` _bella))
  (goto _label_3))

(event `HandAnimation`
  (bind _hand (`self.Hand`))
  (`PaperSpriteComponent.SetSprite` _hand "/Game/Sprites/Intro/Scene1/Scene1Sprites_Sprite_3.Scene1Sprites_Sprite_3" :!label _label_4)
  (`KismetSystemLibrary.Delay` 0.1)
  (if (`KismetMathLibrary.RandomBool`)
    (`PaperSpriteComponent.SetSprite` _hand "/Game/Sprites/Intro/Scene1/Scene1Sprites_Sprite_2.Scene1Sprites_Sprite_2")
    (else
      (`PaperSpriteComponent.SetSprite` _hand "/Game/Sprites/Intro/Scene1/Scene1Sprites_Sprite_4.Scene1Sprites_Sprite_4")))
  (`KismetSystemLibrary.Delay` 0.2)
  (goto _label_4))

(fn `UserConstructionScript`)