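; Scene2 is an intro scene Blueprint that animates two characters, Mati and Bella, a pair of hands and a screen.
; BeginPlay starts four independent endless loops built from Delays and jumps back.
; HandShacking jitters both hands in opposite X directions in short bursts separated by pauses.
; The character and screen loops swap flipbooks after random waits, with random glitch variants and occasional extra plays timed by flipbook length.
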(event `HandShacking`
  (bind _handl (`self.HandL`))
  (bind _handl_2 (`self.HandL`))
  (bind _handr (`self.HandR`))
  (bind _handr_2 (`self.HandR`))
  (bind (_relativelocation_x _relativelocation_y _relativelocation_z) (`KismetMathLibrary.BreakVector` (`SceneComponent.RelativeLocation` _handl)))
  (bind (_relativelocation_x_2 _relativelocation_y_2 _relativelocation_z_2) (`KismetMathLibrary.BreakVector` (`SceneComponent.RelativeLocation` _handl_2)))
  (bind (_relativelocation_x_3 _relativelocation_y_3 _relativelocation_z_3) (`KismetMathLibrary.BreakVector` (`SceneComponent.RelativeLocation` _handr)))
  (bind (_relativelocation_x_4 _relativelocation_y_4 _relativelocation_z_4) (`KismetMathLibrary.BreakVector` (`SceneComponent.RelativeLocation` _handr_2)))
  (`SceneComponent.K2_SetRelativeLocation` _handl (`KismetMathLibrary.MakeVector` (+ _relativelocation_x 1.0) _relativelocation_y _relativelocation_z) false false :!label _label)
  (`SceneComponent.K2_SetRelativeLocation` _handr_2 (`KismetMathLibrary.MakeVector` (+ _relativelocation_x_4 -1.0) _relativelocation_y_4 _relativelocation_z_4) false false)
  (`KismetSystemLibrary.Delay` 0.08)
  (`SceneComponent.K2_SetRelativeLocation` _handl_2 (`KismetMathLibrary.MakeVector` (+ _relativelocation_x_2 -1.0) _relativelocation_y_2 _relativelocation_z_2) false false)
  (`SceneComponent.K2_SetRelativeLocation` _handr (`KismetMathLibrary.MakeVector` (+ _relativelocation_x_3 1.0) _relativelocation_y_3 _relativelocation_z_3) false false)
  (`KismetSystemLibrary.Delay` 0.08)
  (if (< (`self.HandIndex`) 2)
    (set `self.HandIndex` (+ (`self.HandIndex`) 1))
    (goto _label)
    (else
      (set `self.HandIndex` 0)
      (`KismetSystemLibrary.Delay` 0.7)
      (goto _label))))

(event `Mati`
  (bind _s2mati (`self.s2Mati`))
  (bind _s2mati_2 (`self.s2Mati`))
  (`PaperFlipbookComponent.SetFlipbook` (`self.s2Mati`) "/Game/Sprites/Intro/Scene2/s2Mati0.s2Mati0" :!label _label_2)
  (`KismetSystemLibrary.Delay` (`KismetMathLibrary.RandomFloatInRange` 1.0 2.0))
  (`PaperFlipbookComponent.SetFlipbook` _s2mati "/Game/Sprites/Intro/Scene2/s2Mati1.s2Mati1")
  (`KismetSystemLibrary.Delay` (`PaperFlipbookComponent.GetFlipbookLength` _s2mati))
  (if (< (`KismetMathLibrary.RandomFloatInRange` 0.0 100.0) 75.0)
    (goto _label_2)
    (else
      (`PaperFlipbookComponent.SetFlipbook` _s2mati_2 "/Game/Sprites/Intro/Scene2/s2Mati1.s2Mati1")
      (`KismetSystemLibrary.Delay` (`PaperFlipbookComponent.GetFlipbookLength` _s2mati_2))
      (goto _label_2))))

(event `self.ReceiveBeginPlay`
  (`self.HandShacking`)
  (`self.Mati`)
  (`self.Bella`)
  (`self.ScreenAnimation`))

(event `Bella`
  (bind _s2bella (`self.s2Bella`))
  (bind _s2bella_2 (`self.s2Bella`))
  (`PaperFlipbookComponent.SetFlipbook` (`self.s2Bella`) "/Game/Sprites/Intro/Scene2/s2Bella0.s2Bella0" :!label _label_3)
  (`KismetSystemLibrary.Delay` (`KismetMathLibrary.RandomFloatInRange` 1.0 2.0))
  (`PaperFlipbookComponent.SetFlipbook` _s2bella_2 "/Game/Sprites/Intro/Scene2/s2Bella1.s2Bella1")
  (`KismetSystemLibrary.Delay` (`PaperFlipbookComponent.GetFlipbookLength` _s2bella_2))
  (if (< (`KismetMathLibrary.RandomFloatInRange` 0.0 100.0) 75.0)
    (goto _label_3)
    (else
      (`PaperFlipbookComponent.SetFlipbook` _s2bella "/Game/Sprites/Intro/Scene2/s2Bella1.s2Bella1")
      (`KismetSystemLibrary.Delay` (`PaperFlipbookComponent.GetFlipbookLength` _s2bella))
      (goto _label_3))))

(event `ScreenAnimation`
  (bind _screen (`self.Screen`))
  (bind _screen_2 (`self.Screen`))
  (bind _screen_3 (`self.Screen`))
  (bind _screen_4 (`self.Screen`))
  (`PaperFlipbookComponent.SetFlipbook` (`self.Screen`) "/Game/Sprites/Intro/Scene2/Screen.Screen" :!label _label_4)
  (`KismetSystemLibrary.Delay` (`KismetMathLibrary.RandomFloatInRange` 0.5 1.5))
  (`/Engine/EditorBlueprintResources/StandardMacros.CompareInt` (`KismetMathLibrary.RandomIntegerInRange` 0 2) 1
    (:`>`
      (`PaperFlipbookComponent.SetFlipbook` _screen_4 "/Game/Sprites/Intro/Scene2/ScreenGlitch1.ScreenGlitch1")
      (`KismetSystemLibrary.Delay` (`PaperFlipbookComponent.GetFlipbookLength` _screen_4)))
    (:`==`
      (`PaperFlipbookComponent.SetFlipbook` _screen_3 "/Game/Sprites/Intro/Scene2/ScreenGlitch2.ScreenGlitch2")
      (`KismetSystemLibrary.Delay` (`PaperFlipbookComponent.GetFlipbookLength` _screen_3)))
    (:`<`
      (`PaperFlipbookComponent.SetFlipbook` _screen "/Game/Sprites/Intro/Scene2/ScreenGlitch3.ScreenGlitch3")
      (`KismetSystemLibrary.Delay` (`PaperFlipbookComponent.GetFlipbookLength` _screen))))
  (if (< (`KismetMathLibrary.RandomFloatInRange` 0.0 100.0) 85.0)
    (goto _label_4)
    (else
      (`PaperFlipbookComponent.SetFlipbook` _screen_2 "/Game/Sprites/Intro/Scene2/ScreenGlitch4.ScreenGlitch4")
      (`KismetSystemLibrary.Delay` (`PaperFlipbookComponent.GetFlipbookLength` _screen_2))
      (goto _label_4))))

(fn `UserConstructionScript`)