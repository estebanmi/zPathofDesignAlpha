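; Intro scene 5 actor that animates the player falling amid spawned particle actors.
; BeginPlay starts a one-shot timeline moving the player along Z, plus a connector Z timeline that replays after a delay.
; Three endless delay loops spawn small, mid and big particles at random X at fixed low heights.
; Small and mid spawns leave a central gap, while big ones span the width at a different Y depth.
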(event `ConnectorAnim`
  (bind _connector (`self.Connector`))
  (bind (_relativelocation_x _relativelocation_y) (`KismetMathLibrary.BreakVector` (`SceneComponent.RelativeLocation` _connector)))
  (`KismetSystemLibrary.Delay` 1.5 :!label _label)
  (bind (_direction _z) (`Timeline|ConnectorZAnim` :!via `PlayFromStart`)
    (:`Update`
      (`SceneComponent.K2_SetRelativeLocation` _connector (`KismetMathLibrary.MakeVector` _relativelocation_x _relativelocation_y _z) false false))
    (:`Finished`
      (goto _label))))

(event `self.ReceiveBeginPlay`
  (`self.ConnectorAnim`)
  (`self.SmallParticles`)
  (`self.BiggParticles`)
  (`self.MiddParticles`)
  (`self.PlayerFalls`))

(event `SmallParticles`
  (`KismetSystemLibrary.Delay` 0.1 :!label _label_2)
  (`|SpawnActorFromClass` "/Game/Blueprints/Intro/IntroS5Small.IntroS5Small_C" (`KismetMathLibrary.MakeTransform` (`KismetMathLibrary.MakeVector` (select `bool` (`KismetMathLibrary.RandomBool`) :`false` (`KismetMathLibrary.Conv_IntToDouble` (`KismetMathLibrary.RandomIntegerInRange` -62 -16)) :`true` (`KismetMathLibrary.Conv_IntToDouble` (`KismetMathLibrary.RandomIntegerInRange` 17 63))) 0.2 -55.0)) "AlwaysSpawn" "OverrideRootScale" null null)
  (goto _label_2))

(event `PlayerFalls`
  (bind _s5player (`self.s5Player`))
  (bind (_relativelocation_x _relativelocation_y) (`KismetMathLibrary.BreakVector` (`SceneComponent.RelativeLocation` _s5player)))
  (bind (_direction _z) (`Timeline|PlayerFalling` :!via `PlayFromStart`)
    (:`Update`
      (`SceneComponent.K2_SetRelativeLocation` _s5player (`KismetMathLibrary.MakeVector` _relativelocation_x _relativelocation_y _z) false false))))

(event `MiddParticles`
  (`KismetSystemLibrary.Delay` 0.2 :!label _label_3)
  (`|SpawnActorFromClass` "/Game/Blueprints/Intro/IntroS5Mid.IntroS5Mid_C" (`KismetMathLibrary.MakeTransform` (`KismetMathLibrary.MakeVector` (select `bool` (`KismetMathLibrary.RandomBool`) :`false` (`KismetMathLibrary.Conv_IntToDouble` (`KismetMathLibrary.RandomIntegerInRange` -61 -17)) :`true` (`KismetMathLibrary.Conv_IntToDouble` (`KismetMathLibrary.RandomIntegerInRange` 18 62))) 0.2 -65.0)) "AlwaysSpawn" "OverrideRootScale" null null)
  (goto _label_3))

(event `BiggParticles`
  (`KismetSystemLibrary.Delay` 0.4 :!label _label_4)
  (`|SpawnActorFromClass` "/Game/Blueprints/Intro/IntroS5Big.IntroS5Big_C" (`KismetMathLibrary.MakeTransform` (`KismetMathLibrary.MakeVector` (`KismetMathLibrary.Conv_IntToDouble` (`KismetMathLibrary.RandomIntegerInRange` -58 60)) 3.0 -65.0)) "AlwaysSpawn" "OverrideRootScale" null null)
  (goto _label_4))

(fn `UserConstructionScript`)