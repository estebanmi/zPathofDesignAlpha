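; Intro cutscene controller that plays dialogue over five sequentially spawned scene actors, then opens IntroLevel.
; StartScene swaps the scene actor and creates an IntroText widget, counting its non-empty dialog arrays.
; The ScrollingText macro types each string letter by letter with sound, dropping the delay when PlayerIntro's skip flag is set.
; Tick polls for keyboard or gamepad confirmation, blinking a prompt while waiting, to advance dialogue or scene.
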(event `self.ReceiveBeginPlay`
  (bind _asplayer_intro (cast `/Game/Blueprints/TitleScreen/PlayerIntro` (`GameplayStatics.GetPlayerPawn` 0)))
  (set `self.PlayerIntroRef` _asplayer_intro)
  (bind _outactors (`GameplayStatics.GetAllActorsOfClass` "/Game/Blueprints/MusicController.MusicController_C"))
  (set `self.MusicControllerRef` (`|GetArrayItem` _outactors))
  (`KismetSystemLibrary.Delay` 1.0)
  (`self.Start Scene`))

(event `Start Scene`
  (bind _sceneindex (`self.SceneIndex`))
  (`self.StartTalk`)
  (set `self.SceneIndex` (+ _sceneindex 1))
  (switch `int` _sceneindex
    (:`1`
      (`|SpawnActorFromClass` "/Game/Blueprints/Intro/Scene1.Scene1_C" (`KismetMathLibrary.MakeTransform` (0.0 0.0 0.0)) "Undefined" "OverrideRootScale" null null))
    (:`2`
      (bind _outactors (`GameplayStatics.GetAllActorsOfClass` "/Game/Blueprints/Intro/Scene1.Scene1_C"))
      (`self.K2_DestroyActor` (`|GetArrayItem` _outactors))
      (`KismetSystemLibrary.Delay` 0.2)
      (`|SpawnActorFromClass` "/Game/Blueprints/Intro/Scene2.Scene2_C" (`KismetMathLibrary.MakeTransform` (0.0 0.0 0.0)) "Undefined" "OverrideRootScale" null null))
    (:`3`
      (bind _outactors_2 (`GameplayStatics.GetAllActorsOfClass` "/Game/Blueprints/Intro/Scene2.Scene2_C"))
      (`self.K2_DestroyActor` (`|GetArrayItem` _outactors_2))
      (`KismetSystemLibrary.Delay` 0.2)
      (`|SpawnActorFromClass` "/Game/Blueprints/Intro/Scene3.Scene3_C" (`KismetMathLibrary.MakeTransform` (0.0 0.0 0.0)) "Undefined" "OverrideRootScale" null null))
    (:`4`
      (bind _outactors_3 (`GameplayStatics.GetAllActorsOfClass` "/Game/Blueprints/Intro/Scene3.Scene3_C"))
      (`self.K2_DestroyActor` (`|GetArrayItem` _outactors_3))
      (`KismetSystemLibrary.Delay` 0.2)
      (`|SpawnActorFromClass` "/Game/Blueprints/Intro/Scene4.Scene4_C" (`KismetMathLibrary.MakeTransform` (0.0 0.0 0.0)) "Undefined" "OverrideRootScale" null null))
    (:`5`
      (bind _outactors_4 (`GameplayStatics.GetAllActorsOfClass` "/Game/Blueprints/Intro/Scene4.Scene4_C"))
      (`self.K2_DestroyActor` (`|GetArrayItem` _outactors_4))
      (`KismetSystemLibrary.Delay` 0.2)
      (`|SpawnActorFromClass` "/Game/Blueprints/Intro/Scene5.Scene5_C" (`KismetMathLibrary.MakeTransform` (0.0 0.0 0.0)) "Undefined" "OverrideRootScale" null null))))

(event `self.ReceiveTick`
  (params (DeltaSeconds :type "Float (single-precision)"))
  (`self.FreePlayer`))

(event `StartTalk`
  ;[1 0 0.401] Chat
  (`KismetSystemLibrary.Delay` 1.0)
  (`self.DialogsNumberCalculator`)
  (set `/Game/Blueprints/TitleScreen/PlayerIntro.IsSkipText` false (`self.PlayerIntroRef`))
  (bind _returnvalue (`|CreateWidget` "/Game/Widgets/NPCs/IntroText.IntroText_C"))
  (`UserWidget.AddToViewport` _returnvalue 0)
  (set `self.WidgetReff` _returnvalue)
  (`self.ScrollingText` (`/Game/Widgets/NPCs/IntroText.DialogText` (`self.WidgetReff`)) (select `int` (`self.StageIndex`) :`0` (`self.DialogArray_0`) :`1` (`self.DialogArray_1`) :`2` (`self.DialogArray_2`) :`3` (`self.DialogArray_3`) :`4` (`self.DialogArray_4`)) (`self.TextSpeed`)))

(event `PressAnyKey`
  (bind _pressanykey (`/Game/Widgets/NPCs/IntroText.PressAnyKey` (`self.WidgetReff`)))
  ;[1 0 0.401] Chat
  ;;[1 0 0.5463] EnterKey
  (`/Engine/EditorBlueprintResources/StandardMacros.DoOnce` false :!label _label
    (:`Completed`
      (if (`self.isWaitingForPlayer`)
        (`/Engine/EditorBlueprintResources/StandardMacros.FlipFlop`
          (:`A`
            (`Widget.SetVisibility` _pressanykey "Visible"))
          (:`B`
            (`Widget.SetVisibility` _pressanykey "Hidden")))
        (`KismetSystemLibrary.Delay` 0.5)
        (goto _label :!via `Reset`)))))

(event `FreePlayer`
  ;[1 0 0.401] Chat
  ;;[1 0 0.6276] Waiting for Input to free player
  (if (`self.isWaitingForPlayer`)
    (`self.PressAnyKey`)
    (if (`PlayerController.WasInputKeyJustPressed` (`GameplayStatics.GetPlayerController` 0) "Enter")
      (`Widget.SetVisibility` (`/Game/Widgets/NPCs/IntroText.PressAnyKey` (`self.WidgetReff`)) "Hidden" :!label _label_2)
      (if (< (`self.StageIndex`) (`self.DialogsNumber`))
        (`KismetSystemLibrary.Delay` 0.05)
        (set `self.isWaitingForPlayer` false)
        (set `/Game/Blueprints/TitleScreen/PlayerIntro.IsSkipText` false (`self.PlayerIntroRef`))
        (`self.ScrollingText` (`/Game/Widgets/NPCs/IntroText.DialogText` (`self.WidgetReff`)) (select `int` (`self.StageIndex`) :`0` (`self.DialogArray_0`) :`1` (`self.DialogArray_1`) :`2` (`self.DialogArray_2`) :`3` (`self.DialogArray_3`) :`4` (`self.DialogArray_4`)) (`self.TextSpeed`))
        (else
          ;;;[1 1 1] End Scene
          (`self.EnableInput` (`self.PlayerIntroRef`) (`GameplayStatics.GetPlayerController` 0))
          (set `self.isWaitingForPlayer` false)
          (bind _foundwidgets (`WidgetBlueprintLibrary.GetAllWidgetsOfClass` "/Game/Widgets/NPCs/IntroText.IntroText_C"))
          (`Widget.RemoveFromParent` _foundwidgets)
          (set `/Game/Blueprints/TitleScreen/PlayerIntro.IsSkipText` false (`self.PlayerIntroRef`))
          (if (< (`self.SceneIndex`) 5)
            (set `self.StageIndex` 0)
            (`self.Start Scene`)
            (set `self.DialogsNumber` 0)
            (else
              (`KismetSystemLibrary.Delay` 1.0)
              (`GameplayStatics.OpenLevel` "IntroLevel")))))
      (elif (`PlayerController.WasInputKeyJustPressed` (`GameplayStatics.GetPlayerController` 0) "SpaceBar")
        (goto _label_2)
        (elif (`PlayerController.WasInputKeyJustPressed` (`GameplayStatics.GetPlayerController` 0) "RightControl")
          (goto _label_2)
          (elif (`PlayerController.WasInputKeyJustPressed` (`GameplayStatics.GetPlayerController` 0) "Gamepad_FaceButton_Right")
            (goto _label_2)
            (elif (`PlayerController.WasInputKeyJustPressed` (`GameplayStatics.GetPlayerController` 0) "Gamepad_FaceButton_Left")
              (goto _label_2)
              (elif (`PlayerController.WasInputKeyJustPressed` (`GameplayStatics.GetPlayerController` 0) "Gamepad_FaceButton_Bottom")
                (goto _label_2)))))))))

(event `SkipTextListener`
  ;[1 0 0.401] Chat
  ;;[1 0 0.6276] Waiting for Input to free player
  ;;;[1 1 1] Skip Text Listener
  (if (`self.isTalking`)
    (if (`PlayerController.WasInputKeyJustPressed` (`GameplayStatics.GetPlayerController` 0) "Enter")
      (set `/Game/Blueprints/TitleScreen/PlayerIntro.IsSkipText` true (`self.PlayerIntroRef`) :!label _label_3)
      (elif (`PlayerController.WasInputKeyJustPressed` (`GameplayStatics.GetPlayerController` 0) "SpaceBar")
        (goto _label_3)
        (elif (`PlayerController.WasInputKeyJustPressed` (`GameplayStatics.GetPlayerController` 0) "RightControl")
          (goto _label_3)
          (elif (`PlayerController.WasInputKeyJustPressed` (`GameplayStatics.GetPlayerController` 0) "Gamepad_FaceButton_Right")
            (goto _label_3)
            (elif (`PlayerController.WasInputKeyJustPressed` (`GameplayStatics.GetPlayerController` 0) "Gamepad_FaceButton_Left")
              (goto _label_3)
              (elif (`PlayerController.WasInputKeyJustPressed` (`GameplayStatics.GetPlayerController` 0) "Gamepad_FaceButton_Bottom")
                (goto _label_3)))))))))

(event `DialogsNumberCalculator`
  ;[1 0 0.401] Chat
  ;;[1 1 1] Dialog Number Calculator
  (if (`KismetStringLibrary.NotEqual_StrStr` (`|GetArrayItem` (`KismetStringLibrary.GetCharacterArrayFromString` (`|GetArrayItem` (`self.DialogArray_0`)))))
    (set `self.DialogsNumber` (+ (`self.DialogsNumber`) 1))
    (if (`KismetStringLibrary.NotEqual_StrStr` (`|GetArrayItem` (`KismetStringLibrary.GetCharacterArrayFromString` (`|GetArrayItem` (`self.DialogArray_1`)))))
      (set `self.DialogsNumber` (+ (`self.DialogsNumber`) 1))
      (if (`KismetStringLibrary.NotEqual_StrStr` (`|GetArrayItem` (`KismetStringLibrary.GetCharacterArrayFromString` (`|GetArrayItem` (`self.DialogArray_2`)))))
        (set `self.DialogsNumber` (+ (`self.DialogsNumber`) 1))
        (if (`KismetStringLibrary.NotEqual_StrStr` (`|GetArrayItem` (`KismetStringLibrary.GetCharacterArrayFromString` (`|GetArrayItem` (`self.DialogArray_3`)))))
          (set `self.DialogsNumber` (+ (`self.DialogsNumber`) 1))
          (if (`KismetStringLibrary.NotEqual_StrStr` (`|GetArrayItem` (`KismetStringLibrary.GetCharacterArrayFromString` (`|GetArrayItem` (`self.DialogArray_4`)))))
            (set `self.DialogsNumber` (+ (`self.DialogsNumber`) 1))))))))

(fn `UserConstructionScript`)