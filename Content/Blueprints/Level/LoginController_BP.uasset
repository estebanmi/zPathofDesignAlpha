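; Level controller for a login-themed puzzle that opens the first ArmoredDoor_BP found once every Passterisk in the level is collected.
; On BeginPlay it counts the Passterisks and spawns a row of evenly spaced low-bar placeholders at PassteriskPosition.
; Each PassteriskCollected event fills the next slot with a login asterisk and plays a pickup or completion sound.
; Tick compares collected to total, then opens the door and swaps the login button sprite.
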(event `self.ReceiveBeginPlay`
  (bind (_returnvalue_x _returnvalue_y _returnvalue_z) (`KismetMathLibrary.BreakVector` (`SceneComponent.K2_GetComponentLocation` (`self.PassteriskPosition`))))
  (bind _outactors (`GameplayStatics.GetAllActorsOfClass` "/Game/Blueprints/Level/ArmoredDoor_BP.ArmoredDoor_BP_C"))
  (set `self.ArmoredDoorRef` (`|GetArrayItem` _outactors))
  (bind _outactors_2 (`GameplayStatics.GetAllActorsOfClass` "/Game/Blueprints/Collectibles/Passterisk.Passterisk_C"))
  (set `self.PassteriksTotal` (`KismetArrayLibrary.Array_Length` _outactors_2))
  (if (< (`self.Index`) (`self.PassteriksTotal`)) :!label _label
    (`|SpawnActorFromClass` "/Game/Blueprints/Level/LoginLowBar.LoginLowBar_C" (`KismetMathLibrary.MakeTransform` (`KismetMathLibrary.MakeVector` (+ (* (`KismetMathLibrary.Conv_IntToDouble` (`self.Index`)) 7.0) _returnvalue_x) (- _returnvalue_y 1.0) _returnvalue_z)) "Undefined" "OverrideRootScale" null null)
    (set `self.Index` (+ (`self.Index`) 1))
    (goto _label)))

(event `self.ReceiveTick`
  (params (DeltaSeconds :type "Float (single-precision)"))
  (if (== (`self.PassteriksCollected`) (`self.PassteriksTotal`))
    (set `/Game/Blueprints/Level/ArmoredDoor_BP.isOpen` true (`self.ArmoredDoorRef`))
    (`/Engine/EditorBlueprintResources/StandardMacros.DoOnce` false
      (:`Completed`
        (`PaperSpriteComponent.SetSprite` (`self.LoginSprite`) "/Game/Sprites/Login/LoginButton_Sprite_1.LoginButton_Sprite_1")))))

(event `Passterisk Collected`
  (bind (_returnvalue_x _returnvalue_y _returnvalue_z) (`KismetMathLibrary.BreakVector` (`SceneComponent.K2_GetComponentLocation` (`self.PassteriskPosition`))))
  (set `self.PassteriksCollected` (+ (`self.PassteriksCollected`) 1))
  (`|SpawnActorFromClass` "/Game/Blueprints/Level/LoginPassterisk.LoginPassterisk_C" (`KismetMathLibrary.MakeTransform` (`KismetMathLibrary.MakeVector` (+ (* (`KismetMathLibrary.Conv_IntToDouble` (- (`self.PassteriksCollected`) 1)) 7.0) _returnvalue_x) _returnvalue_y _returnvalue_z)) "Undefined" "OverrideRootScale" null null)
  (if (== (`self.PassteriksCollected`) (`self.PassteriksTotal`))
    (`GameplayStatics.PlaySound2D` "/Game/Sound/SFXs/sfx_AllPassterisksCollected_Cue.sfx_AllPassterisksCollected_Cue" 1.0 1.0 0.0 null null)
    (else
      (`GameplayStatics.PlaySound2D` "/Game/Sound/SFXs/sfx_PassteriskCollected_Cue.sfx_PassteriskCollected_Cue" 1.0 1.0 0.0 null null))))

(fn `UserConstructionScript`)