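; FadingPlatform_BP is a one-way Paper2D platform that fades away and returns, either when the player hits it or on a repeating timer, depending on FadeOnHit.
; A delay-driven sequence sets IsFading and IsFaded, moving from solid through fading to faded and back.
; Tick picks the matching flipbook and enables box collision only when the platform is not faded and the player is above it.
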(event `self.ReceiveBeginPlay`
  (bind _asplayer_sword_bp (cast `/Game/Blueprints/Player/PlayerSword_BP` (`GameplayStatics.GetPlayerCharacter` 0)))
  (set `self.PlayerRef` _asplayer_sword_bp)
  (if (not (`self.FadeOnHit?`))
    (`KismetSystemLibrary.Delay` (`self.SolidTime`))
    (`self.FadeOnHitOff`)))

(event `Control Animations`
  (if (`self.isFading`)
    (`PaperFlipbookComponent.SetFlipbook` (`self.PaperFlipbook`) "/Game/Sprites/Level/FadePlatform/FadePlatform1.FadePlatform1")
    (elif (`self.isFaded`)
      (`PaperFlipbookComponent.SetFlipbook` (`self.PaperFlipbook`) "/Game/Sprites/Level/FadePlatform/FadePlatform0G.FadePlatform0G")
      (else
        (`PaperFlipbookComponent.SetFlipbook` (`self.PaperFlipbook`) "/Game/Sprites/Level/FadePlatform/FadePlatform2.FadePlatform2")))))

(event `self.ReceiveTick`
  (params (DeltaSeconds :type "Float (single-precision)"))
  (bind (_returnvalue_x _returnvalue_y _returnvalue_z) (`KismetMathLibrary.BreakVector` (`self.K2_GetActorLocation`)))
  (bind _boxcolldier (`self.BoxColldier`))
  (bind (_returnvalue_x_2 _returnvalue_y_2 _returnvalue_z_2) (`KismetMathLibrary.BreakVector` (`self.K2_GetActorLocation` (`self.PlayerRef`))))
  (`self.Control Animations`)
  (`/Engine/EditorBlueprintResources/StandardMacros.IsValid` (`self.PlayerRef`)
    (:`Is Valid`
      (if (< (- _returnvalue_z_2 9.0) (+ _returnvalue_z 4.0))
        (`PrimitiveComponent.SetCollisionEnabled` _boxcolldier "NoCollision" :!label _label)
        (elif (`self.isFaded`)
          (goto _label)
          (else
            (`PrimitiveComponent.SetCollisionEnabled` _boxcolldier "QueryAndPhysics")))))))

(event `FadeOnHitOff`
  (if (`self.isFading`) :!label _label_2
    _
    (elif (not (`self.isFaded`))
      (set `self.isFading` true)
      (`KismetSystemLibrary.Delay` 3.2)
      (set `self.isFading` false)
      (set `self.isFaded` true)
      (`KismetSystemLibrary.Delay` (- (`self.FadedTime`) 0.1))
      (set `self.isFading` false)
      (set `self.isFaded` false)
      (if (not (`self.FadeOnHit?`))
        (`KismetSystemLibrary.Delay` (`self.SolidTime`))
        (`self.FadeOnHitOff`)))))

(event `self.BoxColldier.OnComponentHit`
  (params (HitComponent :type "PrimitiveComponent Object Reference") (OtherActor :type "Actor Object Reference") (OtherComp :type "PrimitiveComponent Object Reference") (NormalImpulse :type "Vector Structure") (Hit :type "HitResult Structure (by ref)"))
  (if (`self.FadeOnHit?`)
    (cast `/Game/Blueprints/Player/PlayerSword_BP` OtherActor)
    (goto _label_2)))

(fn `UserConstructionScript`)