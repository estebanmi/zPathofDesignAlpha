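; Armored level-exit door with flipbook door and screen visuals that lets the player travel to another level when unlocked.
; Entering its box opens the door once if IsOpen is set, otherwise flashes a blocked alert with sound on a cooldown.
; Pressing Up in range disables player input, movement and collision, then loads LevelToOpen, or plays the blocked sound if closed.
; Tick drives the screen flipbook from the opening and alert flags.
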(event `InputAction|UpAction`
  (params (Key :type "Key Structure"))
  (bind _leveltoopen (`self.LevelToOpen`))
  (bind _playerref (`self.PlayerRef`))
  (bind _playerref_2 (`self.PlayerRef`))
  ;[1 0.4966 0] Enter Door
  (:`Pressed`
    (if (`/Game/Blueprints/Player/Player_BP.InputDisabled` _playerref)
      _
      (elif (`/Game/Blueprints/Player/Player_BP.isDead` _playerref)
        _
        (elif (`/Game/Blueprints/Player/Player_BP.isOnAir` _playerref)
          _
          (elif (`self.inRange`)
            (if (`self.isOpen`)
              (set `/Game/Blueprints/Player/Player_BP.InputDisabled` true _playerref_2)
              (`MovementComponent.StopMovementImmediately` (`Character.CharacterMovement` _playerref_2))
              (`PrimitiveComponent.SetCollisionEnabled` (`Character.CapsuleComponent` _playerref_2) "NoCollision")
              (`/Game/Blueprints/Player/Player_BP.BinaryBumper` _playerref_2)
              (`KismetSystemLibrary.Delay` 0.3)
              (if (!= _leveltoopen "None")
                (`GameplayStatics.OpenLevel` _leveltoopen))
              (else
                (`/Engine/EditorBlueprintResources/StandardMacros.DoOnce` false :!label _label
                  (:`Completed`
                    (`GameplayStatics.PlaySound2D` "/Game/Sound/SFXs/sfx_DoorBlocked_Cue.sfx_DoorBlocked_Cue" 1.0 1.0 0.0 null null)
                    (`KismetSystemLibrary.Delay` 1.0)
                    (goto _label :!via `Reset`)))))))))))

(event `Control Animations`
  ;[1 0 0.5456] Control Animations
  (if (`self.isOpening`)
    (`PaperFlipbookComponent.SetFlipbook` (`self.ScreenFlipbook`) "/Game/Sprites/Level/ArmoredDoor/ScreenOpening.ScreenOpening")
    (`KismetSystemLibrary.Delay` 0.8)
    (`PaperFlipbookComponent.Stop` (`self.ScreenFlipbook`))
    (elif (`self.ClosedAlert`)
      (`PaperFlipbookComponent.SetFlipbook` (`self.ScreenFlipbook`) "/Game/Sprites/Level/ArmoredDoor/Screen_ClosedAlert.Screen_ClosedAlert")
      (else
        (`PaperFlipbookComponent.SetFlipbook` (`self.ScreenFlipbook`) "/Game/Sprites/Level/ArmoredDoor/Screen_Closed.Screen_Closed")))))

(event `self.ReceiveBeginPlay`
  ;[1 0 0] Default
  (bind _asplayer_bp (cast `/Game/Blueprints/Player/Player_BP` (`GameplayStatics.GetPlayerCharacter` 0)))
  (set `self.PlayerRef` _asplayer_bp))

(event `self.ReceiveTick`
  (params (DeltaSeconds :type "Float (single-precision)"))
  ;[1 0 0] Default
  (`self.Control Animations`))

(event `self.BoxColldier.OnComponentBeginOverlap`
  (params (OverlappedComponent :type "PrimitiveComponent Object Reference") (OtherActor :type "Actor Object Reference") (OtherComp :type "PrimitiveComponent Object Reference") (OtherBodyIndex :type Integer) (bFromSweep :type Boolean) (SweepResult :type "HitResult Structure (by ref)"))
  ;[1 1 1] Overlaping the Door
  (cast `/Game/Blueprints/Player/Player_BP` OtherActor)
  (set `self.inRange` true)
  (if (`self.isOpen`)
    (`self.DoorOpening`)
    (else
      (`self.DoorClosed`))))

(event `self.BoxColldier.OnComponentEndOverlap`
  (params (OverlappedComponent :type "PrimitiveComponent Object Reference") (OtherActor :type "Actor Object Reference") (OtherComp :type "PrimitiveComponent Object Reference") (OtherBodyIndex :type Integer))
  ;[1 1 1] Overlaping the Door
  (cast `/Game/Blueprints/Player/Player_BP` OtherActor)
  (set `self.inRange` false))

(event `DoorClosed`
  ;[1 1 1] Door Closed Alert
  (`/Engine/EditorBlueprintResources/StandardMacros.DoOnce` false :!label _label_2
    (:`Completed`
      (set `self.ClosedAlert` true)
      (`GameplayStatics.PlaySound2D` "/Game/Sound/SFXs/sfx_DoorBlocked_Cue.sfx_DoorBlocked_Cue" 1.0 1.0 0.0 null null)
      (`KismetSystemLibrary.Delay` 0.7)
      (set `self.ClosedAlert` false)
      (`KismetSystemLibrary.Delay` 2.0)
      (goto _label_2 :!via `Reset`))))

(event `DoorOpening`
  ;[1 0 0.5677] Door Opening
  (`/Engine/EditorBlueprintResources/StandardMacros.DoOnce` false
    (:`Completed`
      (set `self.isOpening` true)
      (`GameplayStatics.PlaySound2D` "/Game/Sound/SFXs/sfx_DoorOpening_Cue.sfx_DoorOpening_Cue" 1.0 1.0 0.0 null null)
      (`PaperFlipbookComponent.SetFlipbook` (`self.DoorFlipbook`) "/Game/Sprites/Level/ArmoredDoor/NewFolder/ArmoredDoorOpening.ArmoredDoorOpening")
      (`KismetSystemLibrary.Delay` 0.8)
      (set `self.isOpened` true)
      (`KismetSystemLibrary.Delay` 0.2)
      (`PaperFlipbookComponent.SetFlipbook` (`self.DoorFlipbook`) "/Game/Sprites/Level/ArmoredDoor/NewFolder/ArmoredDoorOpened.ArmoredDoorOpened"))))

(fn `UserConstructionScript`)