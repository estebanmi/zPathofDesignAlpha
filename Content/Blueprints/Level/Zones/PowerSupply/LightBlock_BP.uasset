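; Power-supply zone block that lights up while anything overlaps its trigger, or starts lit if the player's PowerSupplyON is set.
; With power off, an overlap counter drives the on and off transition flipbooks, using a Delay to settle on lit and a Tick timer to settle on dark.
; At BeginPlay, if VideoCardON, it tints the sprite from the ColorController's scheme row, picking Level or Interacts color by power state.
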(event `ColorControl`
  (bind _paperflipbook (`self.PaperFlipbook`))
  ;[0 1 1] Color Control
  (bind _asplayer_bp (cast `/Game/Blueprints/Player/Player_BP` (`GameplayStatics.GetPlayerCharacter` 0)))
  (if (`/Game/Blueprints/Player/Player_BP.VideoCardON` _asplayer_bp)
    (bind _outactors (`GameplayStatics.GetAllActorsOfClass` "/Game/Blueprints/Art/ColorController.ColorController_C"))
    (bind _returnvalue (`|GetDataTableRow` "/Game/Blueprints/Art/ColorSchemeTable.ColorSchemeTable" (`/Game/Blueprints/Art/ColorController.ColorScheme` (`|GetArrayItem` _outactors)))
      (:`then`
        (if (`/Game/Blueprints/Player/Player_BP.PowerSupplyON` (`self.PlayerRef`))
          (`PaperFlipbookComponent.SetSpriteColor` _paperflipbook (`.Level_31_53E2F58345BAE2A33F5ED5BE59653F21` (break `/Game/Blueprints/Art/ColorScheme` _returnvalue)))
          (else
            (`PaperFlipbookComponent.SetSpriteColor` _paperflipbook (`.Interacts_30_7CD79F4D4E2B0C70BB0AEE8CDEB583F1` (break `/Game/Blueprints/Art/ColorScheme` _returnvalue)))))))))

(event `self.ReceiveBeginPlay`
  (bind _paperflipbook (`self.PaperFlipbook`))
  (bind _asplayer_bp (cast `/Game/Blueprints/Player/Player_BP` (`GameplayStatics.GetPlayerCharacter` 0)))
  (bind _output_get (set `self.PlayerRef` _asplayer_bp))
  (if (`/Game/Blueprints/Player/Player_BP.PowerSupplyON` _output_get)
    (`PaperFlipbookComponent.SetFlipbook` _paperflipbook "/Game/Sprites/Level/Zones/PowerSupply/Light_BlockONN.Light_BlockONN")
    (else
      (`PaperFlipbookComponent.SetFlipbook` _paperflipbook "/Game/Sprites/Level/Zones/PowerSupply/Light_BlockOFF.Light_BlockOFF")))
  (`self.ColorControl`))

(event `self.ReceiveTick`
  (params (DeltaSeconds :type "Float (single-precision)"))
  (if (`/Game/Blueprints/Player/Player_BP.PowerSupplyON` (`self.PlayerRef`))
    _
    (elif (`self.FadeToBlack`)
      (bind _output_get (set `self.Timer` (+ (`self.Timer`) DeltaSeconds)))
      (if (> _output_get (`self.MaxFTB`))
        (set `self.FadeToBlack` false)
        (if (not (`self.Contact`))
          (`PaperFlipbookComponent.SetFlipbook` (`self.PaperFlipbook`) "/Game/Sprites/Level/Zones/PowerSupply/Light_BlockOFF.Light_BlockOFF"))))))

(event `self.Trigger.OnComponentBeginOverlap`
  (params (OverlappedComponent :type "PrimitiveComponent Object Reference") (OtherActor :type "Actor Object Reference") (OtherComp :type "PrimitiveComponent Object Reference") (OtherBodyIndex :type Integer) (bFromSweep :type Boolean) (SweepResult :type "HitResult Structure (by ref)"))
  (bind _paperflipbook (`self.PaperFlipbook`))
  (if (not (`/Game/Blueprints/Player/Player_BP.PowerSupplyON` (`self.PlayerRef`)))
    (set `self.ThingsOver` (+ (`self.ThingsOver`) 1))
    (set `self.Contact` true)
    (if (== (`self.ThingsOver`) 1)
      (`PaperFlipbookComponent.SetFlipbook` _paperflipbook "/Game/Sprites/Level/Zones/PowerSupply/Light_BlockToON.Light_BlockToON")
      (`KismetSystemLibrary.Delay` (`PaperFlipbookComponent.GetFlipbookLength` _paperflipbook))
      (if (> (`self.ThingsOver`) 0)
        (`PaperFlipbookComponent.SetFlipbook` (`self.PaperFlipbook`) "/Game/Sprites/Level/Zones/PowerSupply/Light_BlockONN.Light_BlockONN")))))

(event `self.Trigger.OnComponentEndOverlap`
  (params (OverlappedComponent :type "PrimitiveComponent Object Reference") (OtherActor :type "Actor Object Reference") (OtherComp :type "PrimitiveComponent Object Reference") (OtherBodyIndex :type Integer))
  (bind _paperflipbook (`self.PaperFlipbook`))
  (if (not (`/Game/Blueprints/Player/Player_BP.PowerSupplyON` (`self.PlayerRef`)))
    (set `self.ThingsOver` (- (`self.ThingsOver`) 1))
    (if (== (`self.ThingsOver`) 0)
      (set `self.Contact` false)
      (set `self.FadeToBlack` true)
      (set `self.Timer` 0.0)
      (`PaperFlipbookComponent.SetFlipbook` _paperflipbook "/Game/Sprites/Level/Zones/PowerSupply/Light_BlockToOFF.Light_BlockToOFF")
      (`PaperFlipbookComponent.PlayFromStart` _paperflipbook)
      (set `self.MaxFTB` (- (`PaperFlipbookComponent.GetFlipbookLength` _paperflipbook) 0.04)))))

(fn `UserConstructionScript`)