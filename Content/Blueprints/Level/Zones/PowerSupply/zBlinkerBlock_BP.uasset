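; Blinking block for the Power Supply zone that animates its Paper2D sprite until the player has the power supply on.
; At BeginPlay it checks the player's PowerSupplyON: if on, it shows one static sprite, otherwise it loops three Timer-delayed sprite steps, the middle one depending on VideoCardON.
; With VideoCardON, it is also tinted once from the ColorController's scheme row, using Level color when powered and Interacts color otherwise.
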(event `ColorControl`
  (bind _papersprite (`self.PaperSprite`))
  ;[0 1 1] Color Control
  (bind _asplayer_bp (cast `/Game/Blueprints/Player/Player_BP` (`GameplayStatics.GetPlayerCharacter` 0)))
  (if (`/Game/Blueprints/Player/Player_BP.VideoCardON` _asplayer_bp)
    (bind _outactors (`GameplayStatics.GetAllActorsOfClass` "/Game/Blueprints/Art/ColorController.ColorController_C"))
    (bind _returnvalue (`|GetDataTableRow` "/Game/Blueprints/Art/ColorSchemeTable.ColorSchemeTable" (`/Game/Blueprints/Art/ColorController.ColorScheme` (`|GetArrayItem` _outactors)))
      (:`then`
        (if (`/Game/Blueprints/Player/Player_BP.PowerSupplyON` (`self.PlayerRef`))
          (`PaperSpriteComponent.SetSpriteColor` _papersprite (`.Level_31_53E2F58345BAE2A33F5ED5BE59653F21` (break `/Game/Blueprints/Art/ColorScheme` _returnvalue)))
          (else
            (`PaperSpriteComponent.SetSpriteColor` _papersprite (`.Interacts_30_7CD79F4D4E2B0C70BB0AEE8CDEB583F1` (break `/Game/Blueprints/Art/ColorScheme` _returnvalue)))))))))

(event `self.ReceiveBeginPlay`
  (bind _papersprite (`self.PaperSprite`))
  (bind _asplayer_bp (cast `/Game/Blueprints/Player/Player_BP` (`GameplayStatics.GetPlayerCharacter` 0)))
  (bind _output_get (set `self.PlayerRef` _asplayer_bp))
  (`self.ColorControl`)
  (if (`/Game/Blueprints/Player/Player_BP.PowerSupplyON` _output_get)
    (`PaperSpriteComponent.SetSprite` _papersprite "/Game/Sprites/Level/Zones/PowerSupply/BlinkerBlock_Sprite_6.BlinkerBlock_Sprite_6")
    (else
      (`PaperSpriteComponent.SetSprite` _papersprite "/Game/Sprites/Level/Zones/PowerSupply/BlinkerBlock_Sprite_3.BlinkerBlock_Sprite_3" :!label _label)
      (`KismetSystemLibrary.Delay` (`self.Timer`))
      (if (`/Game/Blueprints/Player/Player_BP.VideoCardON` (`self.PlayerRef`))
        (`PaperSpriteComponent.SetSprite` _papersprite "/Game/Sprites/Level/Zones/PowerSupply/BlinkerBlock_Sprite_4.BlinkerBlock_Sprite_4")
        (else
          (`PaperSpriteComponent.SetSprite` _papersprite "/Game/Sprites/Level/Zones/PowerSupply/BlinkerBlock_Sprite_5.BlinkerBlock_Sprite_5")))
      (`KismetSystemLibrary.Delay` (`self.Timer`))
      (`PaperSpriteComponent.SetSprite` _papersprite "/Game/Sprites/Level/Zones/PowerSupply/BlinkerBlock_Sprite_6.BlinkerBlock_Sprite_6")
      (`KismetSystemLibrary.Delay` (`self.Timer`))
      (goto _label))))

(event `self.ReceiveTick`
  (params (DeltaSeconds :type "Float (single-precision)")))

(fn `UserConstructionScript`)