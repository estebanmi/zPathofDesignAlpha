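; MemoryBlock_BP is an HDD zone block that periodically appears as a solid obstacle, then vanishes.
; BeginPlay starts it off without collision, waits a configurable Delay, then runs a looping timer at a configurable Time interval.
; Each cycle plays an LED warning flipbook for twice its length, then a stomp sound, enables Box collision with the code-block flipbook, and turns off after two seconds.
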(event `Appears`
  (bind _paperflipbook (`self.PaperFlipbook`))
  (`PaperFlipbookComponent.SetFlipbook` _paperflipbook "/Game/Sprites/Level/Zones/PowerSupply/LedBlockON.LedBlockON")
  (`KismetSystemLibrary.Delay` (* (`PaperFlipbookComponent.GetFlipbookLength` _paperflipbook) 2.0))
  (`GameplayStatics.PlaySound2D` "/Game/Sound/SFXs/sfx_BlopBossStomp1_Cue.sfx_BlopBossStomp1_Cue" 1.0 1.0 0.0 null null)
  (`PrimitiveComponent.SetCollisionEnabled` (`self.Box`) "QueryAndPhysics")
  (`PaperFlipbookComponent.SetFlipbook` (`self.PaperFlipbook`) "/Game/Sprites/Collectibles/CodeBlock/CodeBlock1.CodeBlock1")
  (`KismetSystemLibrary.Delay` 2.0)
  (`PaperFlipbookComponent.SetFlipbook` (`self.PaperFlipbook`) "/Game/Sprites/Level/Zones/PowerSupply/LedBlockOFF.LedBlockOFF")
  (`PrimitiveComponent.SetCollisionEnabled` (`self.Box`) "NoCollision"))

(event `self.ReceiveBeginPlay`
  (`PaperFlipbookComponent.SetFlipbook` (`self.PaperFlipbook`) "/Game/Sprites/Level/Zones/PowerSupply/LedBlockOFF.LedBlockOFF")
  (`PrimitiveComponent.SetCollisionEnabled` (`self.Box`) "NoCollision")
  (`KismetSystemLibrary.Delay` (`self.Delay`))
  (`KismetSystemLibrary.K2_SetTimerDelegate` (delegate `Appears`) (`self.Time`) true))

(event `self.ReceiveTick`
  (params (DeltaSeconds :type "Float (single-precision)")))

(fn `UserConstructionScript`)