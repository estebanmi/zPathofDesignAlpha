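; SaveBlock_BP is a checkpoint block that saves the game when the player enters its trigger, provided the HDD is enabled.
; A DoOnce gates saving, which records the checkpoint and PreBoss flag, re-arms save blocks, and plays sounds and a scale pop.
; A state refreshed on Tick selects the flipbook, starting as Saved if the player spawns on it.
; Sprite color follows the color scheme table, and bullet hits play a bounce sound.
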(event `ColorControl`
  (bind _paperflipbook (`self.PaperFlipbook`))
  ;[0 1 1] Color Control
  (if (`/Game/Blueprints/Player/Player_BP.VideoCardON` (`self.PlayerRef`))
    (bind _outactors (`GameplayStatics.GetAllActorsOfClass` "/Game/Blueprints/Art/ColorController.ColorController_C"))
    (bind _returnvalue (`|GetDataTableRow` "/Game/Blueprints/Art/ColorSchemeTable.ColorSchemeTable" (`/Game/Blueprints/Art/ColorController.ColorScheme` (`|GetArrayItem` _outactors)))
      (:`then`
        (if (`/Game/Blueprints/Player/Player_BP.HDDON` (`self.PlayerRef`))
          (`PaperFlipbookComponent.SetSpriteColor` _paperflipbook (`.Interacts_30_7CD79F4D4E2B0C70BB0AEE8CDEB583F1` (break `/Game/Blueprints/Art/ColorScheme` _returnvalue)))
          (else
            (`PaperFlipbookComponent.SetSpriteColor` _paperflipbook (`.Level_31_53E2F58345BAE2A33F5ED5BE59653F21` (break `/Game/Blueprints/Art/ColorScheme` _returnvalue)))))))))

(event `UpdateAnimation`
  (bind _paperflipbook (`self.PaperFlipbook`))
  ;[1 0 0.7035] Update Animation
  (switch `/Game/Blueprints/Level/Zones/HDD/SaveBlockStates` (`self.SaveBlockState`)
    (:`NewEnumerator0`
      (`PaperFlipbookComponent.SetFlipbook` _paperflipbook "/Game/Sprites/Level/Zones/HDD/SaveBlockOFF.SaveBlockOFF"))
    (:`NewEnumerator1`
      (`PaperFlipbookComponent.SetFlipbook` _paperflipbook "/Game/Sprites/Level/Zones/HDD/SaveBlockError.SaveBlockError"))
    (:`NewEnumerator2`
      (`PaperFlipbookComponent.SetFlipbook` _paperflipbook "/Game/Sprites/Level/Zones/HDD/SaveBlockON.SaveBlockON"))
    (:`NewEnumerator3`
      (`PaperFlipbookComponent.SetFlipbook` _paperflipbook "/Game/Sprites/Level/Zones/HDD/SaveBlockSaving.SaveBlockSaving"))
    (:`NewEnumerator4`
      (`PaperFlipbookComponent.SetFlipbook` _paperflipbook "/Game/Sprites/Level/Zones/HDD/SaveBlockSaved.SaveBlockSaved"))))

(event `self.ReceiveBeginPlay`
  ;[1 0.4842 0] DEFAULT
  (`KismetSystemLibrary.Delay` 0.1)
  (bind _asplayer_bp (cast `/Game/Blueprints/Player/Player_BP` (`GameplayStatics.GetPlayerCharacter` 0)))
  (bind _output_get (set `self.PlayerRef` _asplayer_bp))
  (`self.ColorControl`)
  (if (`/Game/Blueprints/Player/Player_BP.HDDON` _output_get)
    (if (> (`self.GetDistanceTo` _output_get) 20.0)
      (set `self.SaveBlockState` "NewEnumerator2")
      (else
        (set `self.SaveBlockState` "NewEnumerator4")
        (set `self.StartClosed?` true)))
    (else
      (set `self.SaveBlockState` "NewEnumerator0"))))

(event `self.ReceiveTick`
  (params (DeltaSeconds :type "Float (single-precision)"))
  ;[1 0.4842 0] DEFAULT
  (`self.UpdateAnimation`))

(event `Reset SaveBlock`
  (bind _returnvalue_x (`KismetMathLibrary.BreakVector` (`self.K2_GetActorLocation`)))
  (bind _playerref (`self.PlayerRef`))
  (bind (_returnvalue_x_2 _returnvalue_y _returnvalue_z) (`KismetMathLibrary.BreakVector` (`self.K2_GetActorLocation` _playerref)))
  ;[1 1 1] Step In
  (set `self.SaveBlockState` "NewEnumerator2")
  (goto _label :!via `Reset`))

(event `self.Trigger.OnComponentBeginOverlap`
  (params (OverlappedComponent :type "PrimitiveComponent Object Reference") (OtherActor :type "Actor Object Reference") (OtherComp :type "PrimitiveComponent Object Reference") (OtherBodyIndex :type Integer) (bFromSweep :type Boolean) (SweepResult :type "HitResult Structure (by ref)"))
  (bind _returnvalue_x (`KismetMathLibrary.BreakVector` (`self.K2_GetActorLocation`)))
  (bind _playerref (`self.PlayerRef`))
  (bind (_returnvalue_x_2 _returnvalue_y _returnvalue_z) (`KismetMathLibrary.BreakVector` (`self.K2_GetActorLocation` _playerref)))
  ;[1 1 1] Step In
  (bind _asplayer_bp (cast `/Game/Blueprints/Player/Player_BP` OtherActor))
  (set `self.PlayerRef` _asplayer_bp)
  (if (`|EnumEquality` (`self.SaveBlockState`) "NewEnumerator2")
    (if (`/Game/Blueprints/Player/Player_BP.HDDON` _asplayer_bp)
      (`/Engine/EditorBlueprintResources/StandardMacros.DoOnce` (`self.StartClosed?`) :!label _label
        (:`Completed`
          (set `/Game/Blueprints/Player/Player_BP.LastCheckPoint` (`KismetMathLibrary.MakeVector` _returnvalue_x _returnvalue_y _returnvalue_z) _playerref)
          (set `/Game/Blueprints/Player/Player_BP.PreBoss?` (select `bool` (`self.PreBoss?`) :`true` true) _playerref)
          (`/Game/Blueprints/Player/Player_BP.SaveGame` _playerref)
          (`self.Reset Other SaveBlocks`)
          (`GameplayStatics.PlaySound2D` "/Game/Sound/SFXs/DesignMap/sfx_DMLockerOpen_Cue.sfx_DMLockerOpen_Cue" 1.0 1.0 0.0 null null)
          (set `self.SaveBlockState` "NewEnumerator3")
          (`KismetSystemLibrary.Delay` 0.6)
          (`GameplayStatics.PlaySound2D` "/Game/Sound/SFXs/DesignMap/sfx_EnterPOI_Cue.sfx_EnterPOI_Cue" 1.0 1.0 0.0 null null)
          (set `self.SaveBlockState` "NewEnumerator4")
          (`SceneComponent.SetRelativeScale3D` (`self.PaperFlipbook`) (1.1 1.0 1.1))
          (`KismetSystemLibrary.Delay` 0.1)
          (`SceneComponent.SetRelativeScale3D` (`self.PaperFlipbook`) (1.0 1.0 1.0))))
      (else
        (`KismetSystemLibrary.PrintString` "You need to disinfect HDD in order to use Save Points" true true (struct :`R` 1.0 :`G` 0.017682 :`A` 1.0) 6.0)))))

(event `Reset Other SaveBlocks`
  ;[1 1 1] Step In
  (set `self.Index` 0)
  (bind _outactors (`GameplayStatics.GetAllActorsOfClass` "SaveBlock_BP_C"))
  (bind _output (`|GetArrayItem` _outactors (`self.Index`)))
  (if (!= _output (`|GetArrayItem` (`PrimitiveComponent.GetOverlappingActors` (`self.Trigger`) null))) :!label _label_2
    (`self.Reset SaveBlock` _output)
    (if (< (`self.Index`) (- (`KismetArrayLibrary.Array_Length` _outactors) 1))
      (set `self.Index` (+ (`self.Index`) 1))
      (goto _label_2))))

(event `self.Box.OnComponentHit`
  (params (HitComponent :type "PrimitiveComponent Object Reference") (OtherActor :type "Actor Object Reference") (OtherComp :type "PrimitiveComponent Object Reference") (NormalImpulse :type "Vector Structure") (Hit :type "HitResult Structure (by ref)"))
  ;[1 1 1] Bullet Bounce
  (cast `/Game/Blueprints/Player/ActionPlayer/PlayerBullet2_BP` OtherActor)
  (`GameplayStatics.PlaySound2D` "/Game/Sound/SFXs/sfx_BulletBounce_Cue.sfx_BulletBounce_Cue" (`KismetMathLibrary.RandomFloatInRange` 0.5 0.7) (`KismetMathLibrary.RandomFloatInRange` 0.9 1.1) 0.0 null null))

(fn `UserConstructionScript`)