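; HDD zone block that tints its sprite from the active color scheme according to the player's hardware state.
; Shortly after BeginPlay it caches the player and runs ColorControl, which reads the scheme row named by the level's ColorController.
; With the video card on, the sprite takes the Level color if the HDD is on, otherwise the Interacts color.
; A flipbook swap and collision-disable sequence is present but unconnected.
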(event `ColorControl`
  (bind _papersprite (`self.PaperSprite`))
  ;[0 1 1] Color Control
  (if (`/Game/Blueprints/Player/Player_BP.VideoCardON` (`self.PlayerRef`))
    (bind _outactors (`GameplayStatics.GetAllActorsOfClass` "/Game/Blueprints/Art/ColorController.ColorController_C"))
    (bind _returnvalue (`|GetDataTableRow` "/Game/Blueprints/Art/ColorSchemeTable.ColorSchemeTable" (`/Game/Blueprints/Art/ColorController.ColorScheme` (`|GetArrayItem` _outactors)))
      (:`then`
        (if (`/Game/Blueprints/Player/Player_BP.HDDON` (`self.PlayerRef`))
          (`PaperSpriteComponent.SetSpriteColor` _papersprite (`.Level_31_53E2F58345BAE2A33F5ED5BE59653F21` (break `/Game/Blueprints/Art/ColorScheme` _returnvalue)))
          (else
            (`PaperSpriteComponent.SetSpriteColor` _papersprite (`.Interacts_30_7CD79F4D4E2B0C70BB0AEE8CDEB583F1` (break `/Game/Blueprints/Art/ColorScheme` _returnvalue)))))))))

(event `self.ReceiveBeginPlay`
  (`KismetSystemLibrary.Delay` 0.1)
  (bind _asplayer_bp (cast `/Game/Blueprints/Player/Player_BP` (`GameplayStatics.GetPlayerCharacter` 0)))
  (set `self.PlayerRef` _asplayer_bp)
  (`self.ColorControl`))

(event `self.ReceiveTick`
  (params (DeltaSeconds :type "Float (single-precision)")))

(fn `UserConstructionScript`)