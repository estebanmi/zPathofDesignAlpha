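; HDD zone bomb block that disguises or reveals itself by sprite swaps and explodes on contact while the player's HDDON flag is off.
; The outer Trigger toggles sprites through a brief in-between frame; Trigger2 plays a sound, spawns Explosion_BP and destroys the actor.
; With HDDON set at BeginPlay, both triggers are removed, leaving an inert block.
; When VideoCardON is set, block and explosion take colors from the active ColorSchemeTable row.
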(event `ColorControl`
  (bind _papersprite (`self.PaperSprite`))
  ;[0 1 1] Color Control
  (if (`/Game/Blueprints/Player/Player_BP.VideoCardON` (`self.PlayerRef`))
    (bind _outactors (`GameplayStatics.GetAllActorsOfClass` "/Game/Blueprints/Art/ColorController.ColorController_C"))
    (bind _returnvalue (`|GetDataTableRow` "/Game/Blueprints/Art/ColorSchemeTable.ColorSchemeTable" (`/Game/Blueprints/Art/ColorController.ColorScheme` (`|GetArrayItem` _outactors)))
      (:`then`
        (if (`/Game/Blueprints/Player/Player_BP.HDDON` (`self.PlayerRef`))
          (`PaperSpriteComponent.SetSpriteColor` _papersprite (`.Level_31_53E2F58345BAE2A33F5ED5BE59653F21` (break `/Game/Blueprints/Art/ColorScheme` _returnvalue)))
          (else
            (`PaperSpriteComponent.SetSpriteColor` _papersprite (`.Interacts_30_7CD79F4D4E2B0C70BB0AEE8CDEB583F1` (break `/Game/Blueprints/Art/ColorScheme` _returnvalue)))))))))

(event `self.ReceiveBeginPlay`
  (bind _asplayer_bp (cast `/Game/Blueprints/Player/Player_BP` (`GameplayStatics.GetPlayerCharacter` 0)))
  (bind _output_get (set `self.PlayerRef` _asplayer_bp))
  (`self.ColorControl`)
  (if (`/Game/Blueprints/Player/Player_BP.HDDON` _output_get)
    (`PaperSpriteComponent.SetSprite` (`self.PaperSprite`) "/Game/Sprites/Level/Zones/HDD/HDDBlock_Sprite_0.HDDBlock_Sprite_0")
    (`ActorComponent.K2_DestroyComponent` (`self.Trigger`))
    (`ActorComponent.K2_DestroyComponent` (`self.Trigger2`))))

(event `self.Trigger.OnComponentBeginOverlap`
  (params (OverlappedComponent :type "PrimitiveComponent Object Reference") (OtherActor :type "Actor Object Reference") (OtherComp :type "PrimitiveComponent Object Reference") (OtherBodyIndex :type Integer) (bFromSweep :type Boolean) (SweepResult :type "HitResult Structure (by ref)"))
  (bind _asplayer_bp (cast `/Game/Blueprints/Player/Player_BP` OtherActor))
  (if (not (`/Game/Blueprints/Player/Player_BP.HDDON` _asplayer_bp))
    (`PaperSpriteComponent.SetSprite` (`self.PaperSprite`) "/Game/Sprites/Level/Zones/HDD/HDDBlock_Sprite_2.HDDBlock_Sprite_2")
    (`KismetSystemLibrary.Delay` 0.05)
    (`PaperSpriteComponent.SetSprite` (`self.PaperSprite`) "/Game/Sprites/Level/Zones/HDD/HDDBlock_Sprite_0.HDDBlock_Sprite_0")))

(event `self.Trigger.OnComponentEndOverlap`
  (params (OverlappedComponent :type "PrimitiveComponent Object Reference") (OtherActor :type "Actor Object Reference") (OtherComp :type "PrimitiveComponent Object Reference") (OtherBodyIndex :type Integer))
  (bind _asplayer_bp (cast `/Game/Blueprints/Player/Player_BP` OtherActor))
  (if (not (`/Game/Blueprints/Player/Player_BP.HDDON` _asplayer_bp))
    (`PaperSpriteComponent.SetSprite` (`self.PaperSprite`) "/Game/Sprites/Level/Zones/HDD/HDDBlock_Sprite_2.HDDBlock_Sprite_2")
    (`KismetSystemLibrary.Delay` 0.05)
    (`PaperSpriteComponent.SetSprite` (`self.PaperSprite`) "/Game/Sprites/Level/Zones/HDD/HDDBlock_Sprite_1.HDDBlock_Sprite_1")))

(event `self.Trigger2.OnComponentBeginOverlap`
  (params (OverlappedComponent :type "PrimitiveComponent Object Reference") (OtherActor :type "Actor Object Reference") (OtherComp :type "PrimitiveComponent Object Reference") (OtherBodyIndex :type Integer) (bFromSweep :type Boolean) (SweepResult :type "HitResult Structure (by ref)"))
  (bind _asplayer_bp (cast `/Game/Blueprints/Player/Player_BP` OtherActor))
  (if (not (`/Game/Blueprints/Player/Player_BP.HDDON` _asplayer_bp))
    (`GameplayStatics.PlaySound2D` "/Game/Sound/SFXs/sfx_StepDoorClose_Cue.sfx_StepDoorClose_Cue" 1.0 1.0 0.0 null null)
    (`PaperSpriteComponent.SetSprite` (`self.PaperSprite`) "/Game/Sprites/Level/Zones/HDD/HDDBlock_Sprite_2.HDDBlock_Sprite_2")
    (`KismetSystemLibrary.Delay` 0.05)
    (`PaperSpriteComponent.SetSprite` (`self.PaperSprite`) "/Game/Sprites/Level/Zones/HDD/HDDBlock_Sprite_1.HDDBlock_Sprite_1")
    (`KismetSystemLibrary.Delay` 0.05)
    (bind _returnvalue (`|SpawnActorFromClass` "/Game/Blueprints/Enemies/SoundBomb/Explosion_BP.Explosion_BP_C" (`KismetMathLibrary.MakeTransform` (`self.K2_GetActorLocation`)) "Undefined" "OverrideRootScale" null null))
    (if (`/Game/Blueprints/Player/Player_BP.VideoCardON` (`self.PlayerRef`))
      (`PaperFlipbookComponent.SetSpriteColor` (`/Game/Blueprints/Enemies/SoundBomb/Explosion_BP.PaperFlipbook` _returnvalue) (`.Explosion_34_AFEABEF2445912176FAE47AD02015058` (break `/Game/Blueprints/Art/ColorScheme` (stale `ColorControl` _returnvalue)))))
    (`KismetSystemLibrary.Delay` 0.01)
    (`self.K2_DestroyActor`)))

(fn `UserConstructionScript`)