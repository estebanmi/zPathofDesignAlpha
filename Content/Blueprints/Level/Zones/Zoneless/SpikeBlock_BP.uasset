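; SpikeBlock_BP is a spike block level hazard that damages the player while they touch it.
; On BeginPlay it caches the player reference and sets its Paper2D sprite from the SpikeBlockSprite variant, with names suggesting numpad-style spike directions.
; Trigger overlap events toggle a Contact flag for Player_BP, and Tick applies fixed damage every frame while it is set, with no cooldown or delta-time scaling.
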(event `self.ReceiveBeginPlay`
  (bind _papersprite (`self.PaperSprite`))
  (bind _asplayer_bp (cast `/Game/Blueprints/Player/Player_BP` (`GameplayStatics.GetPlayerCharacter` 0)))
  (set `self.PlayerRef` _asplayer_bp)
  (switch `/Game/Blueprints/Level/Zones/Zoneless/SpikeBlockSprite` (`self.SpikeBlockSprite`)
    (:`NewEnumerator0`
      (`PaperSpriteComponent.SetSprite` _papersprite "/Game/Sprites/Level/Zones/ZoneLess/SpikeBlock5.SpikeBlock5"))
    (:`NewEnumerator6`
      (`PaperSpriteComponent.SetSprite` _papersprite "/Game/Sprites/Level/Zones/ZoneLess/SpikeBlock4.SpikeBlock4"))
    (:`NewEnumerator7`
      (`PaperSpriteComponent.SetSprite` _papersprite "/Game/Sprites/Level/Zones/ZoneLess/SpikeBlock8.SpikeBlock8"))
    (:`NewEnumerator8`
      (`PaperSpriteComponent.SetSprite` _papersprite "/Game/Sprites/Level/Zones/ZoneLess/SpikeBlock6.SpikeBlock6"))
    (:`NewEnumerator9`
      (`PaperSpriteComponent.SetSprite` _papersprite "/Game/Sprites/Level/Zones/ZoneLess/SpikeBlock2.SpikeBlock2"))
    (:`NewEnumerator3`
      (`PaperSpriteComponent.SetSprite` _papersprite "/Game/Sprites/Level/Zones/ZoneLess/SpikeBlock4-8.SpikeBlock4-8"))
    (:`NewEnumerator1`
      (`PaperSpriteComponent.SetSprite` _papersprite "/Game/Sprites/Level/Zones/ZoneLess/SpikeBlock4-6.SpikeBlock4-6"))
    (:`NewEnumerator2`
      (`PaperSpriteComponent.SetSprite` _papersprite "/Game/Sprites/Level/Zones/ZoneLess/SpikeBlock4-2.SpikeBlock4-2"))
    (:`NewEnumerator4`
      (`PaperSpriteComponent.SetSprite` _papersprite "/Game/Sprites/Level/Zones/ZoneLess/SpikeBlock8-2.SpikeBlock8-2"))
    (:`NewEnumerator5`
      (`PaperSpriteComponent.SetSprite` _papersprite "/Game/Sprites/Level/Zones/ZoneLess/SpikeBlock8-6.SpikeBlock8-6"))
    (:`NewEnumerator10`
      (`PaperSpriteComponent.SetSprite` _papersprite "/Game/Sprites/Level/Zones/ZoneLess/SpikeBlock4826.SpikeBlock4826"))))

(event `self.ReceiveTick`
  (params (DeltaSeconds :type "Float (single-precision)"))
  (if (`self.Contact`)
    (`GameplayStatics.ApplyDamage` (`self.PlayerRef`) 20.0 null self)))

(event `self.Trigger.OnComponentBeginOverlap`
  (params (OverlappedComponent :type "PrimitiveComponent Object Reference") (OtherActor :type "Actor Object Reference") (OtherComp :type "PrimitiveComponent Object Reference") (OtherBodyIndex :type Integer) (bFromSweep :type Boolean) (SweepResult :type "HitResult Structure (by ref)"))
  (cast `/Game/Blueprints/Player/Player_BP` OtherActor)
  (set `self.Contact` true))

(event `self.Trigger.OnComponentEndOverlap`
  (params (OverlappedComponent :type "PrimitiveComponent Object Reference") (OtherActor :type "Actor Object Reference") (OtherComp :type "PrimitiveComponent Object Reference") (OtherBodyIndex :type Integer))
  (cast `/Game/Blueprints/Player/Player_BP` OtherActor)
  (set `self.Contact` false))

(fn `UserConstructionScript`)