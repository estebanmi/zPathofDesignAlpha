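; NeedleBlock is a hazard block that turns angry when the player comes near and damages them on contact, then falls asleep and stops reacting.
; Two overlap volumes drive a state enum: AngryArea toggles Idle and Angry, while Trigger deals damage and moves through Attack to Happy after a delay.
; Tick maps the state to a flipbook.
; At BeginPlay, the sprite is tinted from the ColorController's scheme if the player's VideoCardON is set.
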(event `self.ReceiveTick`
  (params (DeltaSeconds :type "Float (single-precision)"))
  (bind _paperflipbook (`self.PaperFlipbook`))
  (switch `/Game/Blueprints/Level/Zones/Zoneless/NeedleBlock/NeedleBlockStates` (`self.NeedleBlockStates`)
    (:`NewEnumerator0`
      (`PaperFlipbookComponent.SetFlipbook` _paperflipbook "/Game/Sprites/Traps/NeedleBlock/NeedleBlockIdle.NeedleBlockIdle"))
    (:`NewEnumerator1`
      (`PaperFlipbookComponent.SetFlipbook` _paperflipbook "/Game/Sprites/Traps/NeedleBlock/NeedleBlockAngry.NeedleBlockAngry"))
    (:`NewEnumerator2`
      (`PaperFlipbookComponent.SetFlipbook` _paperflipbook "/Game/Sprites/Traps/NeedleBlock/NeedleBlockAttack.NeedleBlockAttack"))
    (:`NewEnumerator3`
      (`PaperFlipbookComponent.SetFlipbook` _paperflipbook "/Game/Sprites/Traps/NeedleBlock/NeedleBlockSleep.NeedleBlockSleep"))))

(event `self.ReceiveBeginPlay`
  (bind _asplayer_bp (cast `/Game/Blueprints/Player/Player_BP` (`GameplayStatics.GetPlayerCharacter` 0)))
  (set `self.PlayerRef` _asplayer_bp)
  (`self.ColorControl`))

(event `self.Trigger.OnComponentBeginOverlap`
  (params (OverlappedComponent :type "PrimitiveComponent Object Reference") (OtherActor :type "Actor Object Reference") (OtherComp :type "PrimitiveComponent Object Reference") (OtherBodyIndex :type Integer) (bFromSweep :type Boolean) (SweepResult :type "HitResult Structure (by ref)"))
  (bind _asplayer_bp (cast `/Game/Blueprints/Player/Player_BP` OtherActor))
  (if (`|EnumInequality` (`self.NeedleBlockStates`) "NewEnumerator3")
    (`GameplayStatics.PlaySound2D` "/Game/Sound/SFXs/sfx_Sword_Cue.sfx_Sword_Cue" 1.0 1.0 0.0 null null)
    (`GameplayStatics.ApplyDamage` _asplayer_bp (`self.Damage`) null self)
    (set `self.NeedleBlockStates` "NewEnumerator2")
    (`KismetSystemLibrary.Delay` 0.8)
    (set `self.NeedleBlockStates` "NewEnumerator3")))

(event `self.AngryArea.OnComponentBeginOverlap`
  (params (OverlappedComponent :type "PrimitiveComponent Object Reference") (OtherActor :type "Actor Object Reference") (OtherComp :type "PrimitiveComponent Object Reference") (OtherBodyIndex :type Integer) (bFromSweep :type Boolean) (SweepResult :type "HitResult Structure (by ref)"))
  (cast `/Game/Blueprints/Player/Player_BP` OtherActor)
  (if (`|EnumInequality` (`self.NeedleBlockStates`) "NewEnumerator3")
    (set `self.NeedleBlockStates` "NewEnumerator1")))

(event `ColorControl`
  ;[0 1 1] Color Control
  (if (`/Game/Blueprints/Player/Player_BP.VideoCardON` (`self.PlayerRef`))
    (bind _outactors (`GameplayStatics.GetAllActorsOfClass` "/Game/Blueprints/Art/ColorController.ColorController_C"))
    (bind _returnvalue (`|GetDataTableRow` "/Game/Blueprints/Art/ColorSchemeTable.ColorSchemeTable" (`/Game/Blueprints/Art/ColorController.ColorScheme` (`|GetArrayItem` _outactors)))
      (:`then`
        (`PaperFlipbookComponent.SetSpriteColor` (`self.PaperFlipbook`) (`.Interacts_30_7CD79F4D4E2B0C70BB0AEE8CDEB583F1` (break `/Game/Blueprints/Art/ColorScheme` _returnvalue)))))))

(event `self.AngryArea.OnComponentEndOverlap`
  (params (OverlappedComponent :type "PrimitiveComponent Object Reference") (OtherActor :type "Actor Object Reference") (OtherComp :type "PrimitiveComponent Object Reference") (OtherBodyIndex :type Integer))
  (cast `/Game/Blueprints/Player/Player_BP` OtherActor)
  (if (`|EnumInequality` (`self.NeedleBlockStates`) "NewEnumerator3")
    (set `self.NeedleBlockStates` "NewEnumerator0")))

(fn `UserConstructionScript`)