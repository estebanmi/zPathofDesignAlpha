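; ArrowBlockDOWN_BP is a one-shot arrow block that moves downward when the player touches its trigger.
; The first Player_BP overlap swaps the sprite, plays a step sound and runs a timeline that lowers the actor from its captured location, restoring the sprite when finished.
; At BeginPlay, if the player's VideoCardON is set, it tints the sprite with the Interacts color from the ColorController's scheme row in ColorSchemeTable.
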(event `ColorControl`
  ;[0 1 1] Color Control
  (if (`/Game/Blueprints/Player/Player_BP.VideoCardON` (`self.PlayerRef`))
    (bind _outactors (`GameplayStatics.GetAllActorsOfClass` "/Game/Blueprints/Art/ColorController.ColorController_C"))
    (bind _returnvalue (`|GetDataTableRow` "/Game/Blueprints/Art/ColorSchemeTable.ColorSchemeTable" (`/Game/Blueprints/Art/ColorController.ColorScheme` (`|GetArrayItem` _outactors)))
      (:`then`
        (`PaperSpriteComponent.SetSpriteColor` (`self.PaperSprite`) (`.Interacts_30_7CD79F4D4E2B0C70BB0AEE8CDEB583F1` (break `/Game/Blueprints/Art/ColorScheme` _returnvalue)))))))

(event `self.ReceiveBeginPlay`
  (bind _asplayer_bp (cast `/Game/Blueprints/Player/Player_BP` (`GameplayStatics.GetPlayerCharacter` 0)))
  (set `self.PlayerRef` _asplayer_bp)
  (`self.ColorControl`))

(event `self.ReceiveTick`
  (params (DeltaSeconds :type "Float (single-precision)")))

(event `self.Trigger.OnComponentBeginOverlap`
  (params (OverlappedComponent :type "PrimitiveComponent Object Reference") (OtherActor :type "Actor Object Reference") (OtherComp :type "PrimitiveComponent Object Reference") (OtherBodyIndex :type Integer) (bFromSweep :type Boolean) (SweepResult :type "HitResult Structure (by ref)"))
  (bind (_location_x _location_y _location_z) (`KismetMathLibrary.BreakVector` (`self.Location`)))
  (cast `/Game/Blueprints/Player/Player_BP` OtherActor)
  (`/Engine/EditorBlueprintResources/StandardMacros.DoOnce` false
    (:`Completed`
      (`PaperSpriteComponent.SetSprite` (`self.PaperSprite`) "/Game/Sprites/Level/Zones/ZoneLess/ArrowBlock_Sprite_1.ArrowBlock_Sprite_1")
      (`GameplayStatics.PlaySound2D` "/Game/Sound/SFXs/sfx_StepBlock1_Cue.sfx_StepBlock1_Cue" 1.0 1.0 0.0 null null)
      (set `self.Location` (`self.K2_GetActorLocation`))
      (bind (_direction _newtrack_0) (`Timeline|Timeline_0` :!via `PlayFromStart`)
        (:`Update`
          (`self.K2_SetActorLocation` (`KismetMathLibrary.MakeVector` _location_x _location_y (+ _location_z (* _newtrack_0 -1.0)))))
        (:`Finished`
          (`PaperSpriteComponent.SetSprite` (`self.PaperSprite`) "/Game/Sprites/Level/Zones/ZoneLess/ArrowBlock_Sprite_0.ArrowBlock_Sprite_0"))))))

(fn `UserConstructionScript`)