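; HiddenBlock_BP is a destroyable Paper2D block that spawns a configurable actor (BlockSpawned) when shot down.
; On BeginPlay it tints its flipbook from the level ColorController's data table scheme if the player's VideoCardON is set.
; Damage lowers HP and plays a horizontal shake timeline.
; At zero HP it disables collision, optionally spawns fragment pieces, plays an explosion flipbook, spawns BlockSpawned, then destroys itself.
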(event `ColorControl`
  ;[0 1 1] Color Control
  (if (`/Game/Blueprints/Player/Player_BP.VideoCardON` (`self.PlayerRef`))
    (bind _outactors (`GameplayStatics.GetAllActorsOfClass` "/Game/Blueprints/Art/ColorController.ColorController_C"))
    (bind _returnvalue (`|GetDataTableRow` "/Game/Blueprints/Art/ColorSchemeTable.ColorSchemeTable" (`/Game/Blueprints/Art/ColorController.ColorScheme` (`|GetArrayItem` _outactors)))
      (:`then`
        (`PaperFlipbookComponent.SetSpriteColor` (`self.PaperFlipbook`) (`.Interacts_30_7CD79F4D4E2B0C70BB0AEE8CDEB583F1` (break `/Game/Blueprints/Art/ColorScheme` _returnvalue)))))
    (else
      (`PaperFlipbookComponent.SetSpriteColor` (`self.PaperFlipbook`) (struct :`R` 1.0 :`G` 1.0 :`B` 1.0 :`A` 1.0)))))

(event `self.ReceiveBeginPlay`
  (`KismetSystemLibrary.Delay` 0.1)
  (bind _asplayer_bp (cast `/Game/Blueprints/Player/Player_BP` (`GameplayStatics.GetPlayerCharacter` 0)))
  (set `self.PlayerRef` _asplayer_bp)
  (`self.ColorControl`))

(event `self.ReceiveAnyDamage`
  (params (Damage :type "Float (single-precision)") (DamageType :type "DamageType Object Reference") (InstigatedBy :type "Controller Object Reference") (DamageCauser :type "Actor Object Reference"))
  (bind (_returnvalue_x _returnvalue_y _returnvalue_z) (`KismetMathLibrary.BreakVector` (`self.K2_GetActorLocation`)))
  (bind _paperflipbook (`self.PaperFlipbook`))
  (bind _paperflipbook_2 (`self.PaperFlipbook`))
  (bind (_relativelocation_x _relativelocation_y _relativelocation_z) (`KismetMathLibrary.BreakVector` (`SceneComponent.RelativeLocation` _paperflipbook)))
  ;[1 1 1] Receive Damage
  (set `self.HP` (- (`self.HP`) Damage))
  (`GameplayStatics.PlaySound2D` "/Game/Sound/SFXs/sfx_BulletHit_Cue.sfx_BulletHit_Cue" 1.0 1.0 0.0 null null)
  (if (> (`self.HP`) 0.0)
    (bind (_direction _horizontalshake) (`Timeline|Timeline_0` :!via `PlayFromStart`)
      (:`Update`
        (`SceneComponent.K2_SetRelativeLocation` _paperflipbook (`KismetMathLibrary.MakeVector` _horizontalshake _relativelocation_y _relativelocation_z) false false)))
    (else
      (`/Engine/EditorBlueprintResources/StandardMacros.DoOnce` false
        (:`Completed`
          (`PrimitiveComponent.SetCollisionEnabled` (`self.BoxCollider`) "NoCollision")
          (`GameplayStatics.PlaySound2D` "/Game/Sound/SFXs/sfx_CodeBlockExplosion_Cue.sfx_CodeBlockExplosion_Cue" 1.0 1.0 0.0 null null)
          (if (`self.Fragments?`)
            (`self.Fragments`))
          (`PaperFlipbookComponent.SetFlipbook` (`self.PaperFlipbook`) "/Game/Sprites/Level/Zones/ZoneLess/DestroyableBlocks/DestroyableBlock2.DestroyableBlock2")
          (if (`/Game/Blueprints/Player/Player_BP.VideoCardON` (`self.PlayerRef`))
            (`PaperFlipbookComponent.SetSpriteColor` _paperflipbook_2 (`.Explosion_34_AFEABEF2445912176FAE47AD02015058` (break `/Game/Blueprints/Art/ColorScheme` (stale `ColorControl` _returnvalue)))))
          (`SceneComponent.K2_SetRelativeLocation` _paperflipbook_2 (0.0 6.0 0.0) false false)
          (`|SpawnActorFromClass` (`self.BlockSpawned`) (`KismetMathLibrary.MakeTransform` (`KismetMathLibrary.MakeVector` _returnvalue_x (- _returnvalue_y 1.0) _returnvalue_z)) "AlwaysSpawn" "OverrideRootScale" null null)
          (`KismetSystemLibrary.Delay` (`PaperFlipbookComponent.GetFlipbookLength` (`self.PaperFlipbook`)))
          (`self.K2_DestroyActor`))))))

(event `Fragments`
  (bind (_returnvalue_x _returnvalue_y _returnvalue_z) (`KismetMathLibrary.BreakVector` (`self.K2_GetActorLocation`)))
  ;[1 1 1] Fragments
  (`KismetSystemLibrary.Delay` 0.18)
  (bind _returnvalue (`|SpawnActorFromClass` "/Game/Blueprints/Level/Zones/Zoneless/DestroyableBlock/DestroyableBlockPiece_BP.DestroyableBlockPiece_BP_C" (`KismetMathLibrary.MakeTransform` (`KismetMathLibrary.MakeVector` _returnvalue_x 0.0 _returnvalue_z)) "Undefined" "OverrideRootScale" null null :!label _label))
  (if (`/Game/Blueprints/Player/Player_BP.VideoCardON` (`self.PlayerRef`))
    (`PaperSpriteComponent.SetSpriteColor` (`/Game/Blueprints/Level/Zones/Zoneless/DestroyableBlock/DestroyableBlockPiece_BP.PaperSprite` _returnvalue) (`.Interacts_30_7CD79F4D4E2B0C70BB0AEE8CDEB583F1` (break `/Game/Blueprints/Art/ColorScheme` (stale `ColorControl` _returnvalue)))))
  (if (< (`self.Index`) 10)
    (set `self.Index` (+ (`self.Index`) 1))
    (goto _label)))

(fn `UserConstructionScript`)