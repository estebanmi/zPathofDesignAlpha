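; Debris piece for a destroyable block: a short-lived Paper2D fragment that scatters on spawn.
; On BeginPlay it picks one of two sprites at random, slightly jitters its location, and applies a random sideways and upward impulse to its Sphere component in the XZ plane.
; It destroys itself after a random delay of a few seconds.
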(event `self.ReceiveBeginPlay`
  (bind (_returnvalue_x _returnvalue_y _returnvalue_z) (`KismetMathLibrary.BreakVector` (`self.K2_GetActorLocation`)))
  (`PaperSpriteComponent.SetSprite` (`self.PaperSprite`) (select `bool` (`KismetMathLibrary.RandomBool`) :`false` "/Game/Sprites/Level/Zones/ZoneLess/DestroyableBlocks/DestroyableBlock_Sprite_8.DestroyableBlock_Sprite_8" :`true` "/Game/Sprites/Level/Zones/ZoneLess/DestroyableBlocks/DestroyableBlock_Sprite_9.DestroyableBlock_Sprite_9" :!type "PaperSprite Object Reference"))
  (`self.K2_SetActorLocation` (`KismetMathLibrary.MakeVector` (+ _returnvalue_x (`KismetMathLibrary.RandomFloatInRange` -3.0 3.0)) (+ _returnvalue_y (`KismetMathLibrary.RandomFloatInRange` -1.0 2.0)) (+ _returnvalue_z (`KismetMathLibrary.RandomFloatInRange` -3.0 3.0))))
  (`PrimitiveComponent.AddImpulse` (`self.Sphere`) (`KismetMathLibrary.MakeVector` (`KismetMathLibrary.RandomFloatInRange` -40.0 40.0) 0.0 (`KismetMathLibrary.RandomFloatInRange` 0.0 70.0)) "None" false)
  (`KismetSystemLibrary.Delay` (`KismetMathLibrary.RandomFloatInRange` 1.0 3.0))
  (`self.K2_DestroyActor`))

(fn `UserConstructionScript`)