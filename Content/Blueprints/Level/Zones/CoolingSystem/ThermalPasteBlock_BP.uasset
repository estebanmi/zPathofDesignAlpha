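; Thermal paste block in the cooling system zone that halves the player's walk speed on contact.
; Overlap events on its trigger swap sprites and apply the slowdown, restoring the cached original speed only when the player overlaps no other paste block.
; CheckCoolingSystem, also run at BeginPlay, turns the block happy and harmless and restores speed when the player's CoolingSystemON flag is set.
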(event `Check Cooling System`
  (if (`/Game/Blueprints/Player/Player_BP.CoolingSystemON` (`self.PlayerRef`)) :!label _label
    (set `self.Happy` true)
    (`PaperSpriteComponent.SetSprite` (`self.PaperSprite`) "/Game/Sprites/Level/Zones/CoolingSystem/Thermal_Paste_Block_Happy.Thermal_Paste_Block_Happy")
    (set `CharacterMovementComponent.MaxWalkSpeed` (`self.OriginalSpeed`) (`Character.CharacterMovement` (`self.PlayerRef`)))
    (else
      (set `self.Happy` false))))

(event `self.ReceiveBeginPlay`
  (bind _asplayer_bp (cast `/Game/Blueprints/Player/Player_BP` (`GameplayStatics.GetPlayerCharacter` 0)))
  (set `self.PlayerRef` _asplayer_bp)
  (set `self.OriginalSpeed` (`CharacterMovementComponent.MaxWalkSpeed` (`Character.CharacterMovement` (`self.PlayerRef`))))
  (goto _label))

(event `self.ReceiveTick`
  (params (DeltaSeconds :type "Float (single-precision)")))

(event `self.Trigger.OnComponentBeginOverlap`
  (params (OverlappedComponent :type "PrimitiveComponent Object Reference") (OtherActor :type "Actor Object Reference") (OtherComp :type "PrimitiveComponent Object Reference") (OtherBodyIndex :type Integer) (bFromSweep :type Boolean) (SweepResult :type "HitResult Structure (by ref)"))
  (cast `/Game/Blueprints/Player/Player_BP` OtherActor)
  (if (not (`self.Happy`))
    (set `self.Contact` true)
    (`PaperSpriteComponent.SetSprite` (`self.PaperSprite`) "/Game/Sprites/Level/Zones/CoolingSystem/Thermal_Paste_Block_Over.Thermal_Paste_Block_Over")
    (set `CharacterMovementComponent.MaxWalkSpeed` (/ (`self.OriginalSpeed`) 2.0) (`Character.CharacterMovement` (`self.PlayerRef`)))))

(event `self.Trigger.OnComponentEndOverlap`
  (params (OverlappedComponent :type "PrimitiveComponent Object Reference") (OtherActor :type "Actor Object Reference") (OtherComp :type "PrimitiveComponent Object Reference") (OtherBodyIndex :type Integer))
  (cast `/Game/Blueprints/Player/Player_BP` OtherActor)
  (if (not (`self.Happy`))
    (set `self.Contact` false)
    (`PaperSpriteComponent.SetSprite` (`self.PaperSprite`) "/Game/Sprites/Level/Zones/CoolingSystem/Thermal_Paste_Block_Idle.Thermal_Paste_Block_Idle")
    (if (== (`KismetArrayLibrary.Array_Length` (`PrimitiveComponent.GetOverlappingActors` (`Character.CapsuleComponent` (`self.PlayerRef`)) "ThermalPasteBlock_BP_C")) 0)
      (set `CharacterMovementComponent.MaxWalkSpeed` (`self.OriginalSpeed`) (`Character.CharacterMovement` (`self.PlayerRef`))))))

(fn `UserConstructionScript`)