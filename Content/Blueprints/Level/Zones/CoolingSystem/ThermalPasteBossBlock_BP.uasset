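; Thermal paste block for the cooling system zone that slows the player and HostageMass actors overlapping its trigger.
; Overlaps adjust each actor's slow counter and a local occupancy count, which swaps idle and over sprites.
; CheckCoolingSystem sets a happy, non-slowing state when cooling is on.
; Sprite tint follows the ColorController's scheme when the video card is on, and player bullet hits play a randomized sound.
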(event `ColorControl`
  ;[0 1 1] Color Control
  (if (`/Game/Blueprints/Player/Player_BP.VideoCardON` (`self.PlayerRef`))
    (bind _outactors (`GameplayStatics.GetAllActorsOfClass` "/Game/Blueprints/Art/ColorController.ColorController_C"))
    (bind _returnvalue (`|GetDataTableRow` "/Game/Blueprints/Art/ColorSchemeTable.ColorSchemeTable" (`/Game/Blueprints/Art/ColorController.ColorScheme` (`|GetArrayItem` _outactors)))
      (:`then`
        (if (`/Game/Blueprints/Player/Player_BP.CoolingSystemON` (`self.PlayerRef`))
          (`PaperSpriteComponent.SetSpriteColor` (`self.PaperSprite`) (`.Level_31_53E2F58345BAE2A33F5ED5BE59653F21` (break `/Game/Blueprints/Art/ColorScheme` _returnvalue)))
          (else
            (`PaperSpriteComponent.SetSpriteColor` (`self.PaperSprite`) (`.Interacts_30_7CD79F4D4E2B0C70BB0AEE8CDEB583F1` (break `/Game/Blueprints/Art/ColorScheme` _returnvalue)))))))))

(event `Check Cooling System`
  (if (`/Game/Blueprints/Player/Player_BP.CoolingSystemON` (`self.PlayerRef`)) :!label _label
    (set `self.Happy` true)
    (`PaperSpriteComponent.SetSprite` (`self.PaperSprite`) "/Game/Sprites/Level/Zones/CoolingSystem/Thermal_Paste_Block_Happy.Thermal_Paste_Block_Happy")
    (else
      (set `self.Happy` false))))

(event `self.ReceiveBeginPlay`
  (`KismetSystemLibrary.Delay` 0.1)
  (bind _asplayer_bp (cast `/Game/Blueprints/Player/Player_BP` (`GameplayStatics.GetPlayerCharacter` 0))
    (:`then`
      (set `self.PlayerRef` _asplayer_bp)
      (`self.ColorControl`)
      (goto _label))
    (:`CastFailed`
      (`KismetSystemLibrary.PrintString` "ThermalPasteBlock: Player_BP missing")
      (goto _label))))

(event `self.ReceiveTick`
  (params (DeltaSeconds :type "Float (single-precision)")))

(event `self.Trigger.OnComponentBeginOverlap`
  (params (OverlappedComponent :type "PrimitiveComponent Object Reference") (OtherActor :type "Actor Object Reference") (OtherComp :type "PrimitiveComponent Object Reference") (OtherBodyIndex :type Integer) (bFromSweep :type Boolean) (SweepResult :type "HitResult Structure (by ref)"))
  (bind _thingsover (`self.ThingsOver`))
  (if (not (`self.Happy`))
    (bind _asplayer_bp (cast `/Game/Blueprints/Player/Player_BP` OtherActor)
      (:`then`
        (set `/Game/Blueprints/Player/Player_BP.isPlayerSlowed` (+ (`/Game/Blueprints/Player/Player_BP.isPlayerSlowed` _asplayer_bp) 1) _asplayer_bp)
        (`/Game/Blueprints/Player/Player_BP.SlowCheck` _asplayer_bp))
      (:`CastFailed`
        (bind _ashostage_mass_bp (cast `/Game/Blueprints/Enemies/Hostage/HostageMass_BP` OtherActor)
          (:`then`
            (set `/Game/Blueprints/Enemies/Hostage/HostageMass_BP.IsSlowed` (+ (`/Game/Blueprints/Enemies/Hostage/HostageMass_BP.IsSlowed` _ashostage_mass_bp) 1) _ashostage_mass_bp)
            (`/Game/Blueprints/Enemies/Hostage/HostageMass_BP.SlowCheck` _ashostage_mass_bp))
          (:`CastFailed`
            _))))
    (set `self.ThingsOver` (+ _thingsover 1))
    (if (> _thingsover 0)
      (`PaperSpriteComponent.SetSprite` (`self.PaperSprite`) "/Game/Sprites/Level/Zones/CoolingSystem/Thermal_Paste_Block_Over.Thermal_Paste_Block_Over"))))

(event `self.Trigger.OnComponentEndOverlap`
  (params (OverlappedComponent :type "PrimitiveComponent Object Reference") (OtherActor :type "Actor Object Reference") (OtherComp :type "PrimitiveComponent Object Reference") (OtherBodyIndex :type Integer))
  (bind _thingsover (`self.ThingsOver`))
  (if (not (`self.Happy`))
    (bind _asplayer_bp (cast `/Game/Blueprints/Player/Player_BP` OtherActor)
      (:`then`
        (set `/Game/Blueprints/Player/Player_BP.isPlayerSlowed` (- (`/Game/Blueprints/Player/Player_BP.isPlayerSlowed` _asplayer_bp) 1) _asplayer_bp)
        (`/Game/Blueprints/Player/Player_BP.SlowCheck` _asplayer_bp))
      (:`CastFailed`
        (bind _ashostage_mass_bp (cast `/Game/Blueprints/Enemies/Hostage/HostageMass_BP` OtherActor)
          (:`then`
            (set `/Game/Blueprints/Enemies/Hostage/HostageMass_BP.IsSlowed` (- (`/Game/Blueprints/Enemies/Hostage/HostageMass_BP.IsSlowed` _ashostage_mass_bp) 1) _ashostage_mass_bp)
            (`/Game/Blueprints/Enemies/Hostage/HostageMass_BP.SlowCheck` _ashostage_mass_bp))
          (:`CastFailed`
            _))))
    (set `self.ThingsOver` (- _thingsover 1))
    (if (== _thingsover 0)
      (`PaperSpriteComponent.SetSprite` (`self.PaperSprite`) "/Game/Sprites/Level/Zones/CoolingSystem/Thermal_Paste_Block_Idle.Thermal_Paste_Block_Idle"))))

(event `self.Box.OnComponentHit`
  (params (HitComponent :type "PrimitiveComponent Object Reference") (OtherActor :type "Actor Object Reference") (OtherComp :type "PrimitiveComponent Object Reference") (NormalImpulse :type "Vector Structure") (Hit :type "HitResult Structure (by ref)"))
  ;[1 1 1] Bullet Bounce
  (cast `/Game/Blueprints/Player/ActionPlayer/PlayerBullet2_BP` OtherActor)
  (`GameplayStatics.PlaySound2D` "/Game/Sound/SFXs/sfx_BulletHitTileMap_Cue.sfx_BulletHitTileMap_Cue" (`KismetMathLibrary.RandomFloatInRange` 0.5 0.7) (`KismetMathLibrary.RandomFloatInRange` 0.9 1.1) 0.0 null null))

(fn `UserConstructionScript`)