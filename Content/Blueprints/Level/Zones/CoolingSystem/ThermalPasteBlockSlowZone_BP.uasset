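; Thermal paste block slow zone that slows the player and EnemyRunnerMass enemies while they overlap its box.
; BeginPlay sizes the box width from the Blocks count, caches the player and checks the player's CoolingSystemON flag.
; If cooling is on, the block turns Happy, swaps to its happy sprite and stops affecting overlaps.
; Otherwise, begin and end overlap toggle each actor's slowed flag and call its SlowCheck.
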(event `Check Cooling System`
  (if (`/Game/Blueprints/Player/Player_BP.CoolingSystemON` (`self.PlayerRef`)) :!label _label
    (set `self.Happy` true)
    (`PaperSpriteComponent.SetSprite` (`self.PaperSprite`) "/Game/Sprites/Level/Zones/CoolingSystem/Thermal_Paste_Block_Happy.Thermal_Paste_Block_Happy")
    (else
      (set `self.Happy` false))))

(event `self.ReceiveBeginPlay`
  (`BoxComponent.SetBoxExtent` (`self.Box`) (`KismetMathLibrary.MakeVector` (* (`self.Blocks`) 8.0) 6.0 8.0) true)
  (bind _asplayer_bp (cast `/Game/Blueprints/Player/Player_BP` (`GameplayStatics.GetPlayerCharacter` 0))
    (:`then`
      (set `self.PlayerRef` _asplayer_bp)
      (goto _label))
    (:`CastFailed`
      (`KismetSystemLibrary.PrintString` "ThermalPasteBlock: Player_BP missing")
      (goto _label))))

(event `self.ReceiveTick`
  (params (DeltaSeconds :type "Float (single-precision)")))

(event `self.Box.OnComponentBeginOverlap`
  (params (OverlappedComponent :type "PrimitiveComponent Object Reference") (OtherActor :type "Actor Object Reference") (OtherComp :type "PrimitiveComponent Object Reference") (OtherBodyIndex :type Integer) (bFromSweep :type Boolean) (SweepResult :type "HitResult Structure (by ref)"))
  (if (not (`self.Happy`))
    (bind _asplayer_bp (cast `/Game/Blueprints/Player/Player_BP` OtherActor)
      (:`then`
        (set `/Game/Blueprints/Player/Player_BP.isPlayerSlowed` true _asplayer_bp)
        (`/Game/Blueprints/Player/Player_BP.SlowCheck` _asplayer_bp))
      (:`CastFailed`
        (bind _asenemy_runner_mass_bp (cast `/Game/Blueprints/Enemies/Runner/EnemyRunnerMass_BP` OtherActor))
        (set `/Game/Blueprints/Enemies/Runner/EnemyRunnerMass_BP.IsSlowed` true _asenemy_runner_mass_bp)
        (`/Game/Blueprints/Enemies/Runner/EnemyRunnerMass_BP.SlowCheck` _asenemy_runner_mass_bp)))))

(event `self.Box.OnComponentEndOverlap`
  (params (OverlappedComponent :type "PrimitiveComponent Object Reference") (OtherActor :type "Actor Object Reference") (OtherComp :type "PrimitiveComponent Object Reference") (OtherBodyIndex :type Integer))
  (if (not (`self.Happy`))
    (bind _asplayer_bp (cast `/Game/Blueprints/Player/Player_BP` OtherActor)
      (:`then`
        (set `/Game/Blueprints/Player/Player_BP.isPlayerSlowed` false _asplayer_bp)
        (`/Game/Blueprints/Player/Player_BP.SlowCheck` _asplayer_bp))
      (:`CastFailed`
        (bind _asenemy_runner_mass_bp (cast `/Game/Blueprints/Enemies/Runner/EnemyRunnerMass_BP` OtherActor))
        (set `/Game/Blueprints/Enemies/Runner/EnemyRunnerMass_BP.IsSlowed` false _asenemy_runner_mass_bp)
        (`/Game/Blueprints/Enemies/Runner/EnemyRunnerMass_BP.SlowCheck` _asenemy_runner_mass_bp)))))

(fn `UserConstructionScript`)