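; Sound-card zone block that changes game speed when a living player without the SoundCard touches it.
; Its SoundBlockType sets the sprite, global time dilation and MusicController pitch, while player and existing bullets get counter-scaled CustomTimeDilation.
; Contact restarts the player's ManipulatedTime; repeat contact with the same state only does that, always flashing the 05 sprite.
; At BeginPlay, SoundCard ownership shows the off sprite, and VideoCard enables color-scheme tinting.
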(event `ColorControl`
  ;[0 1 1] Color Control
  (if (`/Game/Blueprints/Player/Player_BP.VideoCardON` (`self.PlayerRef`))
    (bind _outactors (`GameplayStatics.GetAllActorsOfClass` "/Game/Blueprints/Art/ColorController.ColorController_C"))
    (bind _returnvalue (`|GetDataTableRow` "/Game/Blueprints/Art/ColorSchemeTable.ColorSchemeTable" (`/Game/Blueprints/Art/ColorController.ColorScheme` (`|GetArrayItem` _outactors)))
      (:`then`
        (if (`/Game/Blueprints/Player/Player_BP.SoundCardON` (`self.PlayerRef`))
          (`PaperSpriteComponent.SetSpriteColor` (`self.PaperSprite`) (`.Level_31_53E2F58345BAE2A33F5ED5BE59653F21` (break `/Game/Blueprints/Art/ColorScheme` _returnvalue)))
          (else
            (`PaperSpriteComponent.SetSpriteColor` (`self.PaperSprite`) (`.Interacts_30_7CD79F4D4E2B0C70BB0AEE8CDEB583F1` (break `/Game/Blueprints/Art/ColorScheme` _returnvalue)))))))))

(event `self.ReceiveBeginPlay`
  (bind _papersprite (`self.PaperSprite`))
  (bind _asplayer_bp (cast `/Game/Blueprints/Player/Player_BP` (`GameplayStatics.GetPlayerCharacter` 0)))
  (bind _output_get (set `self.PlayerRef` _asplayer_bp))
  (`self.ColorControl`)
  (if (`/Game/Blueprints/Player/Player_BP.SoundCardON` _output_get)
    (`PaperSpriteComponent.SetSprite` _papersprite "/Game/Sprites/Level/Zones/SoundCard/SoundBlock/SoundBlockOff_B.SoundBlockOff_B")
    (else
      (switch `/Game/Blueprints/Level/Zones/SoundCard/SoundBlocks` (`self.SoundBlockType`)
        (:`NewEnumerator0`
          (`PaperSpriteComponent.SetSprite` _papersprite "/Game/Sprites/Level/Zones/SoundCard/SoundBlock/SoundBlock_05.SoundBlock_05"))
        (:`NewEnumerator1`
          (`PaperSpriteComponent.SetSprite` _papersprite "/Game/Sprites/Level/Zones/SoundCard/SoundBlock/SoundBlock_1.SoundBlock_1"))
        (:`NewEnumerator2`
          (`PaperSpriteComponent.SetSprite` _papersprite "/Game/Sprites/Level/Zones/SoundCard/SoundBlock/SoundBlock_15.SoundBlock_15"))
        (:`NewEnumerator3`
          (`PaperSpriteComponent.SetSprite` _papersprite "/Game/Sprites/Level/Zones/SoundCard/SoundBlock/SoundBlock_2.SoundBlock_2"))))))

(event `self.ReceiveTick`
  (params (DeltaSeconds :type "Float (single-precision)")))

(event `self.Trigger.OnComponentBeginOverlap`
  (params (OverlappedComponent :type "PrimitiveComponent Object Reference") (OtherActor :type "Actor Object Reference") (OtherComp :type "PrimitiveComponent Object Reference") (OtherBodyIndex :type Integer) (bFromSweep :type Boolean) (SweepResult :type "HitResult Structure (by ref)"))
  (bind _playerref (`self.PlayerRef`))
  (bind _playerref_2 (`self.PlayerRef`))
  (bind _playerref_3 (`self.PlayerRef`))
  (bind _playerref_4 (`self.PlayerRef`))
  (bind _soundblocktype (`self.SoundBlockType`))
  (bind _asplayer_bp (cast `/Game/Blueprints/Player/Player_BP` OtherActor))
  (if (> (`/Game/Blueprints/Player/Player_BP.HPCurrent` _asplayer_bp) 0.0)
    (if (`/Game/Blueprints/Player/Player_BP.SoundCardON` _asplayer_bp)
      _
      (elif (`|EnumInequality` _soundblocktype (`/Game/Blueprints/Player/Player_BP.SoundState` _asplayer_bp))
        (bind _output_get (set `/Game/Blueprints/Player/Player_BP.SoundState` _soundblocktype _asplayer_bp))
        (switch `/Game/Blueprints/Level/Zones/SoundCard/SoundBlocks` _output_get
          (:`NewEnumerator0`
            (`PaperSpriteComponent.SetSprite` (`self.PaperSprite`) "/Game/Sprites/Level/Zones/SoundCard/SoundBlock/SoundBlock_05B.SoundBlock_05B")
            (`GameplayStatics.PlaySound2D` "/Game/Sound/SFXs/sfx_DoorBlocked_Cue.sfx_DoorBlocked_Cue" 1.0 1.0 0.0 null null)
            (`KismetSystemLibrary.Delay` 0.2)
            (`PaperSpriteComponent.SetSprite` (`self.PaperSprite`) "/Game/Sprites/Level/Zones/SoundCard/SoundBlock/SoundBlock_05.SoundBlock_05")
            (`GameplayStatics.SetGlobalTimeDilation` 0.5)
            (bind _outactors (`GameplayStatics.GetAllActorsOfClass` "/Game/Blueprints/MusicController.MusicController_C"))
            (bind _output (`|GetArrayItem` _outactors))
            (`/Game/Blueprints/MusicController.SetPitch` _output 0.5)
            (`/Game/Blueprints/MusicController.ResetPitch` _output)
            (set `Actor.CustomTimeDilation` 2.0 _playerref_2)
            (set `/Game/Blueprints/Player/Player_BP.ManipulatedTime` 0.0 _playerref_2)
            (set `/Game/Blueprints/Player/Player_BP.ManipulatedTimeCounting` true _playerref_2)
            (set `/Game/Blueprints/Player/Player_BP.SoundState` "NewEnumerator0" _playerref_2))
          (:`NewEnumerator1`
            (`PaperSpriteComponent.SetSprite` (`self.PaperSprite`) "/Game/Sprites/Level/Zones/SoundCard/SoundBlock/SoundBlock_1B.SoundBlock_1B")
            (`GameplayStatics.PlaySound2D` "/Game/Sound/SFXs/sfx_DoorBlocked_Cue.sfx_DoorBlocked_Cue" 1.0 1.0 0.0 null null)
            (`KismetSystemLibrary.Delay` 0.2)
            (`PaperSpriteComponent.SetSprite` (`self.PaperSprite`) "/Game/Sprites/Level/Zones/SoundCard/SoundBlock/SoundBlock_1.SoundBlock_1")
            (`GameplayStatics.SetGlobalTimeDilation` 1.0)
            (bind _outactors_2 (`GameplayStatics.GetAllActorsOfClass` "/Game/Blueprints/MusicController.MusicController_C"))
            (bind _output_2 (`|GetArrayItem` _outactors_2))
            (`/Game/Blueprints/MusicController.SetPitch` _output_2 1.0)
            (`/Game/Blueprints/MusicController.ResetPitch` _output_2)
            (set `Actor.CustomTimeDilation` 1.0 _playerref_3)
            (set `/Game/Blueprints/Player/Player_BP.ManipulatedTime` 0.0 _playerref_3)
            (set `/Game/Blueprints/Player/Player_BP.ManipulatedTimeCounting` true _playerref_3)
            (set `/Game/Blueprints/Player/Player_BP.SoundState` "NewEnumerator1" _playerref_3))
          (:`NewEnumerator2`
            (`PaperSpriteComponent.SetSprite` (`self.PaperSprite`) "/Game/Sprites/Level/Zones/SoundCard/SoundBlock/SoundBlock_15B.SoundBlock_15B")
            (`GameplayStatics.PlaySound2D` "/Game/Sound/SFXs/sfx_DoorBlocked_Cue.sfx_DoorBlocked_Cue" 1.0 1.0 0.0 null null)
            (`KismetSystemLibrary.Delay` 0.2)
            (`PaperSpriteComponent.SetSprite` (`self.PaperSprite`) "/Game/Sprites/Level/Zones/SoundCard/SoundBlock/SoundBlock_15.SoundBlock_15")
            (`GameplayStatics.SetGlobalTimeDilation` 1.5)
            (bind _outactors_3 (`GameplayStatics.GetAllActorsOfClass` "/Game/Blueprints/MusicController.MusicController_C"))
            (bind _output_3 (`|GetArrayItem` _outactors_3))
            (`/Game/Blueprints/MusicController.SetPitch` _output_3 1.5)
            (`/Game/Blueprints/MusicController.ResetPitch` _output_3)
            (set `Actor.CustomTimeDilation` 0.75 _playerref_4)
            (set `/Game/Blueprints/Player/Player_BP.ManipulatedTime` 0.0 _playerref_4)
            (set `/Game/Blueprints/Player/Player_BP.ManipulatedTimeCounting` true _playerref_4)
            (set `/Game/Blueprints/Player/Player_BP.SoundState` "NewEnumerator2" _playerref_4))
          (:`NewEnumerator3`
            (`PaperSpriteComponent.SetSprite` (`self.PaperSprite`) "/Game/Sprites/Level/Zones/SoundCard/SoundBlock/SoundBlock_2B.SoundBlock_2B")
            (`GameplayStatics.PlaySound2D` "/Game/Sound/SFXs/sfx_DoorBlocked_Cue.sfx_DoorBlocked_Cue" 1.0 1.0 0.0 null null)
            (`KismetSystemLibrary.Delay` 0.2)
            (`PaperSpriteComponent.SetSprite` (`self.PaperSprite`) "/Game/Sprites/Level/Zones/SoundCard/SoundBlock/SoundBlock_2.SoundBlock_2")
            (`GameplayStatics.SetGlobalTimeDilation` 2.0)
            (bind _outactors_4 (`GameplayStatics.GetAllActorsOfClass` "/Game/Blueprints/MusicController.MusicController_C"))
            (bind _output_4 (`|GetArrayItem` _outactors_4))
            (`/Game/Blueprints/MusicController.SetPitch` _output_4 2.0)
            (`/Game/Blueprints/MusicController.ResetPitch` _output_4)
            (set `Actor.CustomTimeDilation` 0.5 _playerref)
            (set `/Game/Blueprints/Player/Player_BP.ManipulatedTime` 0.0 _playerref)
            (set `/Game/Blueprints/Player/Player_BP.ManipulatedTimeCounting` true _playerref)
            (set `/Game/Blueprints/Player/Player_BP.SoundState` "NewEnumerator3" _playerref)))
        (set `self.Index` 0)
        (bind _outactors_5 (`GameplayStatics.GetAllActorsOfClass` "/Game/Blueprints/Player/ActionPlayer/PlayerBullet2_BP.PlayerBullet2_BP_C"))
        (bind _output_5 (`|GetArrayItem` _outactors_5 (`self.Index`)))
        (`/Engine/EditorBlueprintResources/StandardMacros.IsValid` _output_5
          (:`Is Valid`
            (set `Actor.CustomTimeDilation` (select `/Game/Blueprints/Level/Zones/SoundCard/SoundBlocks` (`self.SoundBlockType`) :`NewEnumerator0` 2.0 :`NewEnumerator1` 1.0 :`NewEnumerator2` 0.75 :`NewEnumerator3` 0.5 :!type "Float (single-precision)") _output_5 :!label _label)
            (if (< (`self.Index`) (- (`KismetArrayLibrary.Array_Length` _outactors_5) 1)) :!label _label_2
              (set `self.Index` (+ (`self.Index`) 1))
              (goto _label)))
          (:`Is Not Valid`
            (goto _label_2)))
        (else
          (`PaperSpriteComponent.SetSprite` (`self.PaperSprite`) "/Game/Sprites/Level/Zones/SoundCard/SoundBlock/SoundBlock_05B.SoundBlock_05B")
          (`GameplayStatics.PlaySound2D` "/Game/Sound/SFXs/sfx_DoorBlocked_Cue.sfx_DoorBlocked_Cue" 1.0 1.0 0.0 null null)
          (`KismetSystemLibrary.Delay` 0.2)
          (`PaperSpriteComponent.SetSprite` (`self.PaperSprite`) "/Game/Sprites/Level/Zones/SoundCard/SoundBlock/SoundBlock_05.SoundBlock_05")
          (set `/Game/Blueprints/Player/Player_BP.ManipulatedTime` 0.0 (`self.PlayerRef`)))))))

(fn `UserConstructionScript`)