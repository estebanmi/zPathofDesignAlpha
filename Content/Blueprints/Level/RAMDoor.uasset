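; RAM-world level door that opens with animation and sound when the player overlaps with BitCoinsMax above BitcoinsRequired, otherwise flashing a blocked alert.
; EnterDoor, when in range and IsOpen, freezes the player, marks UnlocksRAMLevel in WorldRAM, saves and loads RAMWorld.
; Opening sets IsOpened, a different variable from the IsOpen that EnterDoor checks.
; Tick drives screen flipbooks; BeginPlay tints the door from the color scheme table if VideoCardON.
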(event `Update Unlocks`
  (bind _unlocksramlevel_ (`self.UnlocksRAMLevel:`))
  (set `/Game/Blueprints/Player/Player_BP.CurrentWorldLevel` 0 (`self.PlayerRef`))
  (set `/Game/Blueprints/Player/Player_BP.CurrentWorldType` "NewEnumerator6" (`self.PlayerRef`))
  (bind _output_get (set `self.CurrentWorld` (`/Game/Blueprints/Player/Player_BP.WorldRAM` (`self.PlayerRef`))))
  (bind _output_get_2 (set `self.CurrentWorld` (`|MakeArray` (select `bool` (== _unlocksramlevel_ 0) :`false` (`|GetArrayItem` _output_get) :`true` true) (select `bool` (== _unlocksramlevel_ 1) :`false` (`|GetArrayItem` _output_get 1) :`true` true) (select `bool` (== _unlocksramlevel_ 2) :`false` (`|GetArrayItem` _output_get 2) :`true` true) (select `bool` (== _unlocksramlevel_ 3) :`false` (`|GetArrayItem` _output_get 3) :`true` true) (select `bool` (== _unlocksramlevel_ 4) :`false` (`|GetArrayItem` _output_get 4) :`true` true) (select `bool` (== _unlocksramlevel_ 5) :`false` (`|GetArrayItem` _output_get 5) :`true` true) (select `bool` (== _unlocksramlevel_ 6) :`false` (`|GetArrayItem` _output_get 6) :`true` true) (select `bool` (== _unlocksramlevel_ 7) :`false` (`|GetArrayItem` _output_get 7) :`true` true))))
  (set `/Game/Blueprints/Player/Player_BP.WorldRAM` _output_get_2 (`self.PlayerRef`))
  (`/Game/Blueprints/Player/Player_BP.SaveGame` (`self.PlayerRef`)))

(event `ColorControl`
  ;[0 1 1] Color Control
  (if (`/Game/Blueprints/Player/Player_BP.VideoCardON` (`self.PlayerRef`))
    (bind _outactors (`GameplayStatics.GetAllActorsOfClass` "/Game/Blueprints/Art/ColorController.ColorController_C"))
    (bind _returnvalue (`|GetDataTableRow` "/Game/Blueprints/Art/ColorSchemeTable.ColorSchemeTable" (`/Game/Blueprints/Art/ColorController.ColorScheme` (`|GetArrayItem` _outactors)))
      (:`then`
        (`PaperFlipbookComponent.SetSpriteColor` (`self.DoorFlipbook`) (`.Level_31_53E2F58345BAE2A33F5ED5BE59653F21` (break `/Game/Blueprints/Art/ColorScheme` _returnvalue)))))))

(event `EnterDoor`
  (bind _playerref (`self.PlayerRef`))
  ;[1 0.4966 0] Enter Door
  (if (`self.inRange`)
    (if (`self.isOpen`)
      (set `/Game/Blueprints/Player/Player_BP.InputDisabled` true _playerref)
      (`MovementComponent.StopMovementImmediately` (`Character.CharacterMovement` _playerref))
      (`PrimitiveComponent.SetCollisionEnabled` (`Character.CapsuleComponent` _playerref) "NoCollision")
      (`/Game/Blueprints/Player/Player_BP.BinaryBumper` _playerref)
      (`KismetSystemLibrary.Delay` 0.15)
      (`self.Update Unlocks`)
      (`KismetSystemLibrary.Delay` 0.15)
      (`GameplayStatics.OpenLevel` "RAMWorld")
      (else
        (`/Engine/EditorBlueprintResources/StandardMacros.DoOnce` false :!label _label
          (:`Completed`
            (`GameplayStatics.PlaySound2D` "/Game/Sound/SFXs/sfx_DoorBlocked_Cue.sfx_DoorBlocked_Cue" 1.0 1.0 0.0 null null)
            (`KismetSystemLibrary.Delay` 1.0)
            (goto _label :!via `Reset`)))))))

(event `Control Animations`
  ;[1 0 0.5456] Control Animations
  (if (`self.isOpening`)
    (`PaperFlipbookComponent.SetFlipbook` (`self.ScreenFlipbook`) "/Game/Sprites/Level/ArmoredDoor/ScreenOpening.ScreenOpening")
    (`KismetSystemLibrary.Delay` 0.8)
    (`PaperFlipbookComponent.Stop` (`self.ScreenFlipbook`))
    (elif (`self.ClosedAlert`)
      (`PaperFlipbookComponent.SetFlipbook` (`self.ScreenFlipbook`) "/Game/Sprites/Level/ArmoredDoor/Screen_ClosedAlert.Screen_ClosedAlert")
      (else
        (`PaperFlipbookComponent.SetFlipbook` (`self.ScreenFlipbook`) "/Game/Sprites/Level/ArmoredDoor/Screen_Closed.Screen_Closed")))))

(event `self.ReceiveBeginPlay`
  ;[1 0.4617 0] Default
  (`KismetSystemLibrary.Delay` 0.1)
  (bind _asplayer_bp (cast `/Game/Blueprints/Player/Player_BP` (`GameplayStatics.GetPlayerCharacter` 0)))
  (set `self.PlayerRef` _asplayer_bp)
  (`self.ColorControl`))

(event `self.ReceiveTick`
  (params (DeltaSeconds :type "Float (single-precision)"))
  ;[1 0.4617 0] Default
  (`self.Control Animations`))

(event `self.BoxColldier.OnComponentBeginOverlap`
  (params (OverlappedComponent :type "PrimitiveComponent Object Reference") (OtherActor :type "Actor Object Reference") (OtherComp :type "PrimitiveComponent Object Reference") (OtherBodyIndex :type Integer) (bFromSweep :type Boolean) (SweepResult :type "HitResult Structure (by ref)"))
  ;[1 1 1] Overlaping the Door
  (cast `/Game/Blueprints/Player/Player_BP` OtherActor)
  (set `self.inRange` true)
  (if (> (`/Game/Blueprints/Player/Player_BP.BitCoinsMax` (`self.PlayerRef`)) (`self.BitcoinsRequired`))
    (`self.DoorOpening`)
    (else
      (`self.DoorClosed`))))

(event `self.BoxColldier.OnComponentEndOverlap`
  (params (OverlappedComponent :type "PrimitiveComponent Object Reference") (OtherActor :type "Actor Object Reference") (OtherComp :type "PrimitiveComponent Object Reference") (OtherBodyIndex :type Integer))
  ;[1 1 1] Overlaping the Door
  (cast `/Game/Blueprints/Player/Player_BP` OtherActor)
  (set `self.inRange` false))

(event `DoorClosed`
  ;[1 1 1] Door Closed Alert
  (`/Engine/EditorBlueprintResources/StandardMacros.DoOnce` false :!label _label_2
    (:`Completed`
      (set `self.ClosedAlert` true)
      (`GameplayStatics.PlaySound2D` "/Game/Sound/SFXs/sfx_DoorBlocked_Cue.sfx_DoorBlocked_Cue" 1.0 1.0 0.0 null null)
      (`KismetSystemLibrary.Delay` 0.7)
      (set `self.ClosedAlert` false)
      (`KismetSystemLibrary.Delay` 2.0)
      (goto _label_2 :!via `Reset`))))

(event `DoorOpening`
  ;[1 0 0.5677] Door Opening
  (`/Engine/EditorBlueprintResources/StandardMacros.DoOnce` false
    (:`Completed`
      (set `self.isOpening` true)
      (`GameplayStatics.PlaySound2D` "/Game/Sound/SFXs/sfx_DoorOpening_Cue.sfx_DoorOpening_Cue" 1.0 1.0 0.0 null null)
      (`PaperFlipbookComponent.SetFlipbook` (`self.DoorFlipbook`) "/Game/Sprites/Level/ArmoredDoor/NewFolder/ArmoredDoorOpening.ArmoredDoorOpening")
      (`KismetSystemLibrary.Delay` 0.8)
      (set `self.isOpened` true)
      (`KismetSystemLibrary.Delay` 0.2)
      (`PaperFlipbookComponent.SetFlipbook` (`self.DoorFlipbook`) "/Game/Sprites/Level/ArmoredDoor/NewFolder/ArmoredDoorOpened.ArmoredDoorOpened"))))

(fn `UserConstructionScript`)