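; BinaryBumperController Blueprint that builds and clears a string of random binary digits in Text0101.
; Adding01 appends random 1s and 0s in fixed-size batches, looping back with a short Delay between batches until a batch counter reaches its limit.
; Remove01 empties the string and resets both counters.
; BeginPlay, Tick and the construction script are empty, and nothing in this Blueprint calls either event or displays the text.
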(event `Remove01`
  (set `self.Text0101` "")
  (set `self.Index` 0)
  (set `self.Index2` 0))

(event `self.ReceiveBeginPlay`)

(event `Adding01`
  (if (< (`self.Index`) 50) :!label _label
    (if (`KismetMathLibrary.RandomBool`)
      (set `self.Text0101` (`KismetStringLibrary.Concat_StrStr` (`self.Text0101`) "1"))
      (else
        (set `self.Text0101` (`KismetStringLibrary.Concat_StrStr` (`self.Text0101`) "0"))))
    (set `self.Index` (+ (`self.Index`) 1))
    (goto _label)
    (elif (< (`self.Index2`) 20)
      (set `self.Text0101` (`KismetStringLibrary.Concat_StrStr` (`self.Text0101`) " "))
      (set `self.Index2` (+ (`self.Index2`) 1))
      (set `self.Index` 0)
      (`KismetSystemLibrary.Delay` 0.01)
      (goto _label))))

(event `self.ReceiveTick`
  (params (DeltaSeconds :type "Float (single-precision)")))

(fn `UserConstructionScript`)