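; HorrorDoorBack is a Paper2D level door with a screen, acting as an entrance that animates shut or an exit to another level, depending on IsExit.
; An Open event plays sounds and an opening flipbook, then marks the door open.
; Pressing Up within its overlap box, while grounded and alive, either saves and loads LevelToOpen or, if the exit is closed, flashes a blocked alert guarded by a DoOnce.
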(event `Starting Flipbooks`
  (bind _paperflipbookdoor (`self.PaperFlipbookDoor`))
  (if (`self.isExit`)
    (if (`self.isOpen`)
      (`PaperFlipbookComponent.SetFlipbook` (`self.PaperFlipbookDoor`) "/Game/Sprites/Level/HorrorDoor/HorrorDoorOpen.HorrorDoorOpen"))
    (else
      (`PaperFlipbookComponent.SetFlipbook` (`self.PaperFlipbookDoor`) "/Game/Sprites/Level/HorrorDoor/HorrorDoorOpen.HorrorDoorOpen")
      (`PaperFlipbookComponent.SetFlipbook` (`self.PaperFlipbookScreen`) "/Game/Sprites/Level/ArmoredDoor/Screen_Closed.Screen_Closed")
      (`KismetSystemLibrary.Delay` 0.5)
      (`PaperFlipbookComponent.SetFlipbook` _paperflipbookdoor "/Game/Sprites/Level/HorrorDoor/HorrorDoorClosing.HorrorDoorClosing")
      (`KismetSystemLibrary.Delay` (`PaperFlipbookComponent.GetFlipbookLength` _paperflipbookdoor))
      (`PaperFlipbookComponent.SetFlipbook` (`self.PaperFlipbookDoor`) "/Game/Sprites/Level/HorrorDoor/HorrorDoorClosed1.HorrorDoorClosed1"))))

(event `self.ReceiveBeginPlay`
  (bind _asplayer_bp (cast `/Game/Blueprints/Player/Player_BP` (`GameplayStatics.GetPlayerCharacter` 0)))
  (set `self.PlayerRef` _asplayer_bp)
  (`self.Starting Flipbooks`))

(event `Open`
  (bind _paperflipbookscreen (`self.PaperFlipbookScreen`))
  (`GameplayStatics.PlaySound2D` null 1.0 1.0 0.0 null null)
  (`KismetSystemLibrary.Delay` 1.0)
  (`PaperFlipbookComponent.SetFlipbook` _paperflipbookscreen "/Game/Sprites/Level/HorrorDoor/HorrorDoorOpening.HorrorDoorOpening")
  (`GameplayStatics.PlaySound2D` null 1.0 1.0 0.0 null null)
  (`KismetSystemLibrary.Delay` (`PaperFlipbookComponent.GetFlipbookLength` _paperflipbookscreen))
  (`PaperFlipbookComponent.SetFlipbook` (`self.PaperFlipbookScreen`) "/Game/Sprites/Level/HorrorDoor/HorrorDoorOpening.HorrorDoorOpening")
  (set `self.isOpen` true))

(event `self.Box.OnComponentBeginOverlap`
  (params (OverlappedComponent :type "PrimitiveComponent Object Reference") (OtherActor :type "Actor Object Reference") (OtherComp :type "PrimitiveComponent Object Reference") (OtherBodyIndex :type Integer) (bFromSweep :type Boolean) (SweepResult :type "HitResult Structure (by ref)"))
  (cast `/Game/Blueprints/Player/Player_BP` OtherActor)
  (set `self.inRange` true))

(event `self.Box.OnComponentEndOverlap`
  (params (OverlappedComponent :type "PrimitiveComponent Object Reference") (OtherActor :type "Actor Object Reference") (OtherComp :type "PrimitiveComponent Object Reference") (OtherBodyIndex :type Integer))
  (cast `/Game/Blueprints/Player/Player_BP` OtherActor)
  (set `self.inRange` false))

(event `InputAction|UpAction`
  (params (Key :type "Key Structure"))
  (bind _playerref (`self.PlayerRef`))
  (bind _playerref_2 (`self.PlayerRef`))
  (:`Pressed`
    (if (`/Game/Blueprints/Player/Player_BP.InputDisabled` _playerref)
      _
      (elif (`/Game/Blueprints/Player/Player_BP.isDead` _playerref)
        _
        (elif (`/Game/Blueprints/Player/Player_BP.isOnAir` _playerref)
          _
          (elif (`self.inRange`)
            (if (`self.isExit`)
              (if (`self.isOpen`)
                (set `/Game/Blueprints/Player/Player_BP.InputDisabled` false _playerref_2)
                (`MovementComponent.StopMovementImmediately` (`Character.CharacterMovement` _playerref_2))
                (`PrimitiveComponent.SetCollisionEnabled` (`Character.CapsuleComponent` _playerref_2) "NoCollision")
                (`KismetSystemLibrary.Delay` 0.5)
                (`/Game/Blueprints/Player/Player_BP.SaveGame` _playerref_2)
                (`/Game/Blueprints/Player/Player_BP.BinaryBumper` _playerref_2)
                (`KismetSystemLibrary.Delay` 0.3)
                (`GameplayStatics.OpenLevel` (`self.LevelToOpen`))
                (else
                  (`/Engine/EditorBlueprintResources/StandardMacros.DoOnce` false :!label _label
                    (:`Completed`
                      (`PaperFlipbookComponent.SetFlipbook` (`self.PaperFlipbookScreen`) "/Game/Sprites/Level/ArmoredDoor/Screen_ClosedAlert.Screen_ClosedAlert")
                      (`GameplayStatics.PlaySound2D` "/Game/Sound/SFXs/sfx_DoorBlocked_Cue.sfx_DoorBlocked_Cue" 1.0 1.0 0.0 null null)
                      (`KismetSystemLibrary.Delay` 0.7)
                      (`PaperFlipbookComponent.SetFlipbook` (`self.PaperFlipbookScreen`) "/Game/Sprites/Level/HorrorDoor/ExitScreen1.ExitScreen1")
                      (`KismetSystemLibrary.Delay` 2.0)
                      (goto _label :!via `Reset`))))))))))))

(fn `UserConstructionScript`)