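; A falling dead zone for the level that kills the player or destroys any other actor hitting its box collider.
; A player hit hides the character, flags it dead, zeroes HP and plays a death sound.
; After a delay, it shows the BinaryBumper HUD, calls Adding01 on the level's BinaryBumper controller, then reloads into DemoMap.
; Other actors are destroyed immediately with a quieter blop death sound.
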(event `self.Box Collider.OnComponentHit`
  (params (HitComponent :type "PrimitiveComponent Object Reference") (OtherActor :type "Actor Object Reference") (OtherComp :type "PrimitiveComponent Object Reference") (NormalImpulse :type "Vector Structure") (Hit :type "HitResult Structure (by ref)"))
  (bind _asplayer_bp (cast `/Game/Blueprints/Player/Player_BP` OtherActor)
    (:`then`
      (`self.SetActorHiddenInGame` _asplayer_bp true)
      (set `/Game/Blueprints/Player/Player_BP.isDead` true _asplayer_bp)
      (set `/Game/Blueprints/Player/Player_BP.InputDisabled` false _asplayer_bp)
      (set `/Game/Blueprints/Player/Player_BP.HPCurrent` 0.0 _asplayer_bp)
      (`GameplayStatics.PlaySound2D` "/Game/Sound/SFXs/sfx_PlayerDeath_Cue.sfx_PlayerDeath_Cue" 1.0 1.0 0.0 null null)
      (`KismetSystemLibrary.Delay` 2.0)
      (bind _returnvalue (`|CreateWidget` "/Game/Widgets/BinaryBumper_HUD.BinaryBumper_HUD_C"))
      (`UserWidget.AddToViewport` _returnvalue 0)
      (bind _outactors (`GameplayStatics.GetAllActorsOfClass` "/Game/Blueprints/Level/BinaryBumperController_BP.BinaryBumperController_BP_C"))
      (`/Game/Blueprints/Level/BinaryBumperController_BP.Adding01` (`|GetArrayItem` _outactors))
      (`KismetSystemLibrary.Delay` 0.3)
      (`GameplayStatics.OpenLevel` "DemoMap"))
    (:`CastFailed`
      (`self.K2_DestroyActor` OtherActor)
      (`GameplayStatics.PlaySound2D` "/Game/Sound/SFXs/sfx_BlopDeath_Cue.sfx_BlopDeath_Cue" 0.3 1.0 0.0 null null))))

(fn `UserConstructionScript`)