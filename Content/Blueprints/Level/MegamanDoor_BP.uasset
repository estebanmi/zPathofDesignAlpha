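; Mega Man-style shutter door that moves the player rightward into a boss room or corridor.
; Entering BoxTrigger from the left clears calls and enemies, locks input and blends to that area's fixed camera.
; Twelve sprites hide then reappear sequentially with sound while Tick auto-walks the player through, ending in boss dialogue or restored control.
; Also handles color-scheme tinting, bullet-bounce sounds and an EndLevel exit to DesignMap.
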(event `ColorControl`
  ;[0 1 1] Color Control
  (if (`/Game/Blueprints/Player/Player_BP.VideoCardON` (`self.PlayerRef`))
    (bind _outactors (`GameplayStatics.GetAllActorsOfClass` "/Game/Blueprints/Art/ColorController.ColorController_C"))
    (bind _returnvalue (`|GetDataTableRow` "/Game/Blueprints/Art/ColorSchemeTable.ColorSchemeTable" (`/Game/Blueprints/Art/ColorController.ColorScheme` (`|GetArrayItem` _outactors)))
      (:`then`
        (`PaperSpriteComponent.SetSpriteColor` (`self.PaperSprite`) (`.Interacts_30_7CD79F4D4E2B0C70BB0AEE8CDEB583F1` (break `/Game/Blueprints/Art/ColorScheme` _returnvalue)))
        (`PaperSpriteComponent.SetSpriteColor` (`self.PaperSprite1`) (`.Interacts_30_7CD79F4D4E2B0C70BB0AEE8CDEB583F1` (break `/Game/Blueprints/Art/ColorScheme` _returnvalue)))
        (`PaperSpriteComponent.SetSpriteColor` (`self.PaperSprite2`) (`.Interacts_30_7CD79F4D4E2B0C70BB0AEE8CDEB583F1` (break `/Game/Blueprints/Art/ColorScheme` _returnvalue)))
        (`PaperSpriteComponent.SetSpriteColor` (`self.PaperSprite3`) (`.Interacts_30_7CD79F4D4E2B0C70BB0AEE8CDEB583F1` (break `/Game/Blueprints/Art/ColorScheme` _returnvalue)))
        (`PaperSpriteComponent.SetSpriteColor` (`self.PaperSprite4`) (`.Interacts_30_7CD79F4D4E2B0C70BB0AEE8CDEB583F1` (break `/Game/Blueprints/Art/ColorScheme` _returnvalue)))
        (`PaperSpriteComponent.SetSpriteColor` (`self.PaperSprite5`) (`.Interacts_30_7CD79F4D4E2B0C70BB0AEE8CDEB583F1` (break `/Game/Blueprints/Art/ColorScheme` _returnvalue)))
        (`PaperSpriteComponent.SetSpriteColor` (`self.PaperSprite6`) (`.Interacts_30_7CD79F4D4E2B0C70BB0AEE8CDEB583F1` (break `/Game/Blueprints/Art/ColorScheme` _returnvalue)))
        (`PaperSpriteComponent.SetSpriteColor` (`self.PaperSprite7`) (`.Interacts_30_7CD79F4D4E2B0C70BB0AEE8CDEB583F1` (break `/Game/Blueprints/Art/ColorScheme` _returnvalue)))
        (`PaperSpriteComponent.SetSpriteColor` (`self.PaperSprite8`) (`.Interacts_30_7CD79F4D4E2B0C70BB0AEE8CDEB583F1` (break `/Game/Blueprints/Art/ColorScheme` _returnvalue)))
        (`PaperSpriteComponent.SetSpriteColor` (`self.PaperSprite9`) (`.Interacts_30_7CD79F4D4E2B0C70BB0AEE8CDEB583F1` (break `/Game/Blueprints/Art/ColorScheme` _returnvalue)))
        (`PaperSpriteComponent.SetSpriteColor` (`self.PaperSprite10`) (`.Interacts_30_7CD79F4D4E2B0C70BB0AEE8CDEB583F1` (break `/Game/Blueprints/Art/ColorScheme` _returnvalue)))
        (`PaperSpriteComponent.SetSpriteColor` (`self.PaperSprite11`) (`.Interacts_30_7CD79F4D4E2B0C70BB0AEE8CDEB583F1` (break `/Game/Blueprints/Art/ColorScheme` _returnvalue)))))))

(event `CameraBoss`
  (bind _outactors (`GameplayStatics.GetAllActorsOfClass` "/Game/Blueprints/CameraBoss_BP.CameraBoss_BP_C"))
  (bind _output (`|GetArrayItem` _outactors))
  (`PlayerController.SetViewTargetWithBlend` (`GameplayStatics.GetPlayerController` 0) _output 2.5 "VTBlend_Linear" 0.0 false)
  (bind _outactors_2 (`GameplayStatics.GetAllActorsOfClass` "/Game/Blueprints/Level/ScreenCollider_BP.ScreenCollider_BP_C"))
  (`/Game/Blueprints/Level/ScreenCollider_BP.ToFixedCam` (`|GetArrayItem` _outactors_2) (`self.K2_GetActorLocation` _output)))

(event `CameraCorridor`
  (bind _outactors (`GameplayStatics.GetAllActorsOfClass` "/Game/Blueprints/CameraCorridor_BP.CameraCorridor_BP_C"))
  (bind _output (`|GetArrayItem` _outactors))
  (`PlayerController.SetViewTargetWithBlend` (`GameplayStatics.GetPlayerController` 0) _output 2.5 "VTBlend_Linear" 0.0 false)
  (bind _outactors_2 (`GameplayStatics.GetAllActorsOfClass` "/Game/Blueprints/Level/ScreenCollider_BP.ScreenCollider_BP_C"))
  (`/Game/Blueprints/Level/ScreenCollider_BP.ToFixedCam` (`|GetArrayItem` _outactors_2) (`self.K2_GetActorLocation` _output)))

(event `OpenDoor`
  (`/Engine/EditorBlueprintResources/StandardMacros.DoOnce` false
    (:`Completed`
      (`GameplayStatics.PlaySound2D` "/Game/Sound/SFXs/sfx_MegamanDoor_Cue.sfx_MegamanDoor_Cue" 1.0 1.0 0.0 null null)
      (`SceneComponent.SetVisibility` (`self.PaperSprite`) false false)
      (`KismetSystemLibrary.Delay` (`self.DoorSpeed`))
      (`GameplayStatics.PlaySound2D` "/Game/Sound/SFXs/sfx_MegamanDoor_Cue.sfx_MegamanDoor_Cue" 1.0 1.0 0.0 null null)
      (`SceneComponent.SetVisibility` (`self.PaperSprite1`) false false)
      (`KismetSystemLibrary.Delay` (`self.DoorSpeed`))
      (`GameplayStatics.PlaySound2D` "/Game/Sound/SFXs/sfx_MegamanDoor_Cue.sfx_MegamanDoor_Cue" 1.0 1.0 0.0 null null)
      (`SceneComponent.SetVisibility` (`self.PaperSprite2`) false false)
      (`KismetSystemLibrary.Delay` (`self.DoorSpeed`))
      (`GameplayStatics.PlaySound2D` "/Game/Sound/SFXs/sfx_MegamanDoor_Cue.sfx_MegamanDoor_Cue" 1.0 1.0 0.0 null null)
      (`SceneComponent.SetVisibility` (`self.PaperSprite3`) false false)
      (`KismetSystemLibrary.Delay` (`self.DoorSpeed`))
      (`GameplayStatics.PlaySound2D` "/Game/Sound/SFXs/sfx_MegamanDoor_Cue.sfx_MegamanDoor_Cue" 1.0 1.0 0.0 null null)
      (`SceneComponent.SetVisibility` (`self.PaperSprite4`) false false)
      (`KismetSystemLibrary.Delay` (`self.DoorSpeed`))
      (`GameplayStatics.PlaySound2D` "/Game/Sound/SFXs/sfx_MegamanDoor_Cue.sfx_MegamanDoor_Cue" 1.0 1.0 0.0 null null)
      (`SceneComponent.SetVisibility` (`self.PaperSprite5`) false false)
      (`KismetSystemLibrary.Delay` (`self.DoorSpeed`))
      (`GameplayStatics.PlaySound2D` "/Game/Sound/SFXs/sfx_MegamanDoor_Cue.sfx_MegamanDoor_Cue" 1.0 1.0 0.0 null null)
      (`SceneComponent.SetVisibility` (`self.PaperSprite6`) false false)
      (`KismetSystemLibrary.Delay` (`self.DoorSpeed`))
      (`GameplayStatics.PlaySound2D` "/Game/Sound/SFXs/sfx_MegamanDoor_Cue.sfx_MegamanDoor_Cue" 1.0 1.0 0.0 null null)
      (`SceneComponent.SetVisibility` (`self.PaperSprite7`) false false)
      (`KismetSystemLibrary.Delay` (`self.DoorSpeed`))
      (`GameplayStatics.PlaySound2D` "/Game/Sound/SFXs/sfx_MegamanDoor_Cue.sfx_MegamanDoor_Cue" 1.0 1.0 0.0 null null)
      (`SceneComponent.SetVisibility` (`self.PaperSprite8`) false false)
      (`KismetSystemLibrary.Delay` (`self.DoorSpeed`))
      (`GameplayStatics.PlaySound2D` "/Game/Sound/SFXs/sfx_MegamanDoor_Cue.sfx_MegamanDoor_Cue" 1.0 1.0 0.0 null null)
      (`SceneComponent.SetVisibility` (`self.PaperSprite9`) false false)
      (`KismetSystemLibrary.Delay` (`self.DoorSpeed`))
      (`GameplayStatics.PlaySound2D` "/Game/Sound/SFXs/sfx_MegamanDoor_Cue.sfx_MegamanDoor_Cue" 1.0 1.0 0.0 null null)
      (`SceneComponent.SetVisibility` (`self.PaperSprite10`) false false)
      (`KismetSystemLibrary.Delay` (`self.DoorSpeed`))
      (`GameplayStatics.PlaySound2D` "/Game/Sound/SFXs/sfx_MegamanDoor_Cue.sfx_MegamanDoor_Cue" 1.0 1.0 0.0 null null)
      (`SceneComponent.SetVisibility` (`self.PaperSprite11`) false false)
      (`KismetSystemLibrary.Delay` (`self.DoorSpeed`))
      (`PrimitiveComponent.SetCollisionEnabled` (`self.BoxDoor`) "NoCollision")
      (`self.MovingPlayer`))))

(event `CloseDoor`
  (`/Engine/EditorBlueprintResources/StandardMacros.DoOnce` false
    (:`Completed`
      (`GameplayStatics.PlaySound2D` "/Game/Sound/SFXs/sfx_MegamanDoor_Cue.sfx_MegamanDoor_Cue" 1.0 1.0 0.0 null null)
      (`SceneComponent.SetVisibility` (`self.PaperSprite11`) true false)
      (`KismetSystemLibrary.Delay` (`self.DoorSpeed`))
      (`GameplayStatics.PlaySound2D` "/Game/Sound/SFXs/sfx_MegamanDoor_Cue.sfx_MegamanDoor_Cue" 1.0 1.0 0.0 null null)
      (`SceneComponent.SetVisibility` (`self.PaperSprite10`) true false)
      (`KismetSystemLibrary.Delay` (`self.DoorSpeed`))
      (`GameplayStatics.PlaySound2D` "/Game/Sound/SFXs/sfx_MegamanDoor_Cue.sfx_MegamanDoor_Cue" 1.0 1.0 0.0 null null)
      (`SceneComponent.SetVisibility` (`self.PaperSprite9`) true false)
      (`KismetSystemLibrary.Delay` (`self.DoorSpeed`))
      (`GameplayStatics.PlaySound2D` "/Game/Sound/SFXs/sfx_MegamanDoor_Cue.sfx_MegamanDoor_Cue" 1.0 1.0 0.0 null null)
      (`SceneComponent.SetVisibility` (`self.PaperSprite8`) true false)
      (`KismetSystemLibrary.Delay` (`self.DoorSpeed`))
      (`GameplayStatics.PlaySound2D` "/Game/Sound/SFXs/sfx_MegamanDoor_Cue.sfx_MegamanDoor_Cue" 1.0 1.0 0.0 null null)
      (`SceneComponent.SetVisibility` (`self.PaperSprite7`) true false)
      (`KismetSystemLibrary.Delay` (`self.DoorSpeed`))
      (`GameplayStatics.PlaySound2D` "/Game/Sound/SFXs/sfx_MegamanDoor_Cue.sfx_MegamanDoor_Cue" 1.0 1.0 0.0 null null)
      (`SceneComponent.SetVisibility` (`self.PaperSprite6`) true false)
      (`KismetSystemLibrary.Delay` (`self.DoorSpeed`))
      (`GameplayStatics.PlaySound2D` "/Game/Sound/SFXs/sfx_MegamanDoor_Cue.sfx_MegamanDoor_Cue" 1.0 1.0 0.0 null null)
      (`SceneComponent.SetVisibility` (`self.PaperSprite5`) true false)
      (`KismetSystemLibrary.Delay` (`self.DoorSpeed`))
      (`GameplayStatics.PlaySound2D` "/Game/Sound/SFXs/sfx_MegamanDoor_Cue.sfx_MegamanDoor_Cue" 1.0 1.0 0.0 null null)
      (`SceneComponent.SetVisibility` (`self.PaperSprite4`) true false)
      (`KismetSystemLibrary.Delay` (`self.DoorSpeed`))
      (`GameplayStatics.PlaySound2D` "/Game/Sound/SFXs/sfx_MegamanDoor_Cue.sfx_MegamanDoor_Cue" 1.0 1.0 0.0 null null)
      (`SceneComponent.SetVisibility` (`self.PaperSprite3`) true false)
      (`KismetSystemLibrary.Delay` (`self.DoorSpeed`))
      (`GameplayStatics.PlaySound2D` "/Game/Sound/SFXs/sfx_MegamanDoor_Cue.sfx_MegamanDoor_Cue" 1.0 1.0 0.0 null null)
      (`SceneComponent.SetVisibility` (`self.PaperSprite2`) true false)
      (`KismetSystemLibrary.Delay` (`self.DoorSpeed`))
      (`GameplayStatics.PlaySound2D` "/Game/Sound/SFXs/sfx_MegamanDoor_Cue.sfx_MegamanDoor_Cue" 1.0 1.0 0.0 null null)
      (`SceneComponent.SetVisibility` (`self.PaperSprite1`) true false)
      (`KismetSystemLibrary.Delay` (`self.DoorSpeed`))
      (`GameplayStatics.PlaySound2D` "/Game/Sound/SFXs/sfx_MegamanDoor_Cue.sfx_MegamanDoor_Cue" 1.0 1.0 0.0 null null)
      (`SceneComponent.SetVisibility` (`self.PaperSprite`) true false)
      (`KismetSystemLibrary.Delay` (`self.DoorSpeed`))
      (if (`self.DoorBeforeBoss?`)
        (`KismetSystemLibrary.Delay` 1.0)
        ;[1 1 1] Boss Chat
        (bind _outactors (`GameplayStatics.GetAllActorsOfClass` "/Game/Blueprints/Bosses/BossNew/BossNew.BossNew_C"))
        (`/Game/Blueprints/Bosses/BossNew/BossNew.BossTalk` (`|GetArrayItem` _outactors))
        (else
          (`self.FreePlayer`))))))

(event `self.BoxTrigger.OnComponentBeginOverlap`
  (params (OverlappedComponent :type "PrimitiveComponent Object Reference") (OtherActor :type "Actor Object Reference") (OtherComp :type "PrimitiveComponent Object Reference") (OtherBodyIndex :type Integer) (bFromSweep :type Boolean) (SweepResult :type "HitResult Structure (by ref)"))
  (bind _returnvalue_x (`KismetMathLibrary.BreakVector` (`self.K2_GetActorLocation`)))
  (bind _asplayer_bp (cast `/Game/Blueprints/Player/Player_BP` OtherActor))
  (`self.Remove Calls`)
  (bind _returnvalue_x_2 (`KismetMathLibrary.BreakVector` (`self.K2_GetActorLocation` _asplayer_bp)))
  (if (< _returnvalue_x_2 _returnvalue_x)
    (`/Engine/EditorBlueprintResources/StandardMacros.DoOnce` false
      (:`Completed`
        (`self.DisableInput` _asplayer_bp (`GameplayStatics.GetPlayerController` 0))
        (set `/Game/Blueprints/Player/Player_BP.InputDisabled` true _asplayer_bp)
        (set `/Game/Blueprints/Player/Player_BP.ShootButtonDown` false _asplayer_bp)
        (`KismetSystemLibrary.Delay` 0.5)
        (`self.OpenDoor`)
        (`self.DeleteEnemies`)
        (if (`self.DoorBeforeBoss?`)
          (`self.CameraBoss`)
          (else
            (`self.CameraCorridor`)))))))

(event `FreePlayer`
  (`self.EnableInput` (`self.PlayerRef`) (`GameplayStatics.GetPlayerController` 0))
  (set `/Game/Blueprints/Player/Player_BP.InputDisabled` false (`self.PlayerRef`))
  (if (`PlayerController.IsInputKeyDown` (`GameplayStatics.GetPlayerController` 0) "RightControl")
    (`/Game/Blueprints/Player/Player_BP.ContinueShooting` (`self.PlayerRef`) :!label _label)
    (elif (`PlayerController.IsInputKeyDown` (`GameplayStatics.GetPlayerController` 0) "Gamepad_FaceButton_Left")
      (goto _label))))

(event `self.ReceiveBeginPlay`
  (`KismetSystemLibrary.Delay` 0.1)
  (bind _asplayer_bp (cast `/Game/Blueprints/Player/Player_BP` (`GameplayStatics.GetPlayerCharacter` 0)))
  (set `self.PlayerRef` _asplayer_bp)
  (`self.ColorControl`))

(event `EndLevel`
  (set `self.AutoMovePlayer` true)
  (`GameplayStatics.PlaySound2D` "/Game/Sound/Music/sm_ActionLevelEnd_Cue.sm_ActionLevelEnd_Cue" 1.0 1.0 0.0 null null)
  (`KismetSystemLibrary.Delay` 1.5)
  (set `self.AutoMovePlayer` false)
  (`KismetSystemLibrary.Delay` 1.5)
  (`/Game/Blueprints/Player/Player_BP.BinaryBumper` (`self.PlayerRef`))
  (`KismetSystemLibrary.Delay` 0.3)
  (`GameplayStatics.OpenLevel` "DesignMap"))

(event `MovingPlayer`
  ;[1 1 1] Moving Player
  (set `self.AutoMovePlayer` true)
  (set `/Game/Blueprints/Player/Player_BP.isMovingRight` true (`self.PlayerRef`))
  (`KismetSystemLibrary.Delay` 0.3)
  (`PrimitiveComponent.SetCollisionEnabled` (`self.BoxDoor`) "QueryAndPhysics")
  (`self.CloseDoor`)
  (if (`self.DoorBeforeBoss?`)
    (`KismetSystemLibrary.Delay` 0.5))
  (set `self.AutoMovePlayer` false))

(event `self.ReceiveTick`
  (params (DeltaSeconds :type "Float (single-precision)"))
  ;[1 1 1] Moving Player
  (if (`self.AutoMovePlayer`)
    (`Pawn.AddMovementInput` (`self.PlayerRef`) (100.0 0.0 0.0) 1.0 false)))

(event `DeleteEnemies`
  (set `self.Index` 0)
  (bind _outactors (`GameplayStatics.GetAllActorsWithTag` "Enemy"))
  (bind _output (`|GetArrayItem` _outactors (`self.Index`)))
  (`/Engine/EditorBlueprintResources/StandardMacros.IsValid` _output
    (:`Is Valid`
      (`self.K2_DestroyActor` _output :!label _label_2)
      (if (< (`self.Index`) (- (`KismetArrayLibrary.Array_Length` _outactors) 1))
        (set `self.Index` (+ (`self.Index`) 1))
        (goto _label_2)))))

(event `Remove Calls`
  ;[1 1 1] Remove Calls
  (bind _outactors (`GameplayStatics.GetAllActorsOfClass` "/Game/Blueprints/NPCs/IncomingCall.IncomingCall_C"))
  (bind _output (`|GetArrayItem` _outactors (`self.Index2`)))
  (if (`/Game/Blueprints/NPCs/IncomingCall.Calling` _output) :!label _label_3
    (set `/Game/Blueprints/NPCs/IncomingCall.Calling` false _output)
    (set `/Game/Blueprints/NPCs/IncomingCall.CallAlreadyDone` true _output))
  (if (< (`self.Index2`) (- (`KismetArrayLibrary.Array_Length` _outactors) 1))
    (set `self.Index2` (+ (`self.Index2`) 1))
    (goto _label_3)
    (else
      (bind _foundwidgets (`WidgetBlueprintLibrary.GetAllWidgetsOfClass` "/Game/Widgets/NPCs/IncomingCall_HUD.IncomingCall_HUD_C"))
      (`Widget.RemoveFromParent` _foundwidgets))))

(event `self.BoxDoor.OnComponentHit`
  (params (HitComponent :type "PrimitiveComponent Object Reference") (OtherActor :type "Actor Object Reference") (OtherComp :type "PrimitiveComponent Object Reference") (NormalImpulse :type "Vector Structure") (Hit :type "HitResult Structure (by ref)"))
  ;[1 1 1] Bullet Bounce
  (cast `/Game/Blueprints/Player/ActionPlayer/PlayerBullet2_BP` OtherActor)
  (`GameplayStatics.PlaySound2D` "/Game/Sound/SFXs/sfx_BulletBounce_Cue.sfx_BulletBounce_Cue" (`KismetMathLibrary.RandomFloatInRange` 0.5 0.7) (`KismetMathLibrary.RandomFloatInRange` 0.9 1.1) 0.0 null null))

(fn `UserConstructionScript`)