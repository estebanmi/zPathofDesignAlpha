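; HorrorDoor is a level door with door and screen flipbooks, serving as either an exit or a door that closes shortly after play begins.
; Open plays sounds, switches the screen flipbook to the opening animation and marks the door open.
; An open exit stops the overlapping player, disables their collision, calls BinaryBumper and loads DesignMap.
; A closed exit flashes a blocked alert with sound, throttled by a resetting DoOnce.
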(event `self.ReceiveBeginPlay`
  (bind _paperflipbookdoor (`self.PaperFlipbookDoor`))
  (if (`self.isExit`)
    (if (`self.isOpen`)
      (`PaperFlipbookComponent.SetFlipbook` (`self.PaperFlipbookDoor`) "/Game/Sprites/Level/HorrorDoor/HorrorDoorOpen.HorrorDoorOpen"))
    (else
      (`PaperFlipbookComponent.SetFlipbook` (`self.PaperFlipbookDoor`) "/Game/Sprites/Level/HorrorDoor/HorrorDoorOpen.HorrorDoorOpen")
      (`PaperFlipbookComponent.SetFlipbook` (`self.PaperFlipbookScreen`) "/Game/Sprites/Level/ArmoredDoor/Screen_Closed.Screen_Closed")
      (`KismetSystemLibrary.Delay` 0.5)
      (`PaperFlipbookComponent.SetFlipbook` _paperflipbookdoor "/Game/Sprites/Level/HorrorDoor/HorrorDoorClosing.HorrorDoorClosing")
      (`KismetSystemLibrary.Delay` (`PaperFlipbookComponent.GetFlipbookLength` _paperflipbookdoor))
      (`PaperFlipbookComponent.SetFlipbook` (`self.PaperFlipbookDoor`) "/Game/Sprites/Level/HorrorDoor/HorrorDoorClosed1.HorrorDoorClosed1"))))

(event `Open`
  (bind _paperflipbookscreen (`self.PaperFlipbookScreen`))
  (`GameplayStatics.PlaySound2D` null 1.0 1.0 0.0 null null)
  (`KismetSystemLibrary.Delay` 1.0)
  (`PaperFlipbookComponent.SetFlipbook` _paperflipbookscreen "/Game/Sprites/Level/HorrorDoor/HorrorDoorOpening.HorrorDoorOpening")
  (`GameplayStatics.PlaySound2D` null 1.0 1.0 0.0 null null)
  (`KismetSystemLibrary.Delay` (`PaperFlipbookComponent.GetFlipbookLength` _paperflipbookscreen))
  (`PaperFlipbookComponent.SetFlipbook` (`self.PaperFlipbookScreen`) "/Game/Sprites/Level/HorrorDoor/HorrorDoorOpening.HorrorDoorOpening")
  (set `self.isOpen` true))

(event `self.Box.OnComponentBeginOverlap`
  (params (OverlappedComponent :type "PrimitiveComponent Object Reference") (OtherActor :type "Actor Object Reference") (OtherComp :type "PrimitiveComponent Object Reference") (OtherBodyIndex :type Integer) (bFromSweep :type Boolean) (SweepResult :type "HitResult Structure (by ref)"))
  (if (`self.isExit`)
    (if (`self.isOpen`)
      (bind _asplayer_bp (cast `/Game/Blueprints/Player/Player_BP` OtherActor))
      (set `/Game/Blueprints/Player/Player_BP.InputDisabled` false _asplayer_bp)
      (`MovementComponent.StopMovementImmediately` (`Character.CharacterMovement` _asplayer_bp))
      (`PrimitiveComponent.SetCollisionEnabled` (`Character.CapsuleComponent` _asplayer_bp) "NoCollision")
      (`KismetSystemLibrary.Delay` 0.5)
      (`/Game/Blueprints/Player/Player_BP.BinaryBumper` _asplayer_bp)
      (`KismetSystemLibrary.Delay` 0.3)
      (`GameplayStatics.OpenLevel` "DesignMap")
      (else
        (`/Engine/EditorBlueprintResources/StandardMacros.DoOnce` false :!label _label
          (:`Completed`
            (`PaperFlipbookComponent.SetFlipbook` (`self.PaperFlipbookScreen`) "/Game/Sprites/Level/ArmoredDoor/Screen_ClosedAlert.Screen_ClosedAlert")
            (`GameplayStatics.PlaySound2D` "/Game/Sound/SFXs/sfx_DoorBlocked_Cue.sfx_DoorBlocked_Cue" 1.0 1.0 0.0 null null)
            (`KismetSystemLibrary.Delay` 0.7)
            (`PaperFlipbookComponent.SetFlipbook` (`self.PaperFlipbookScreen`) "/Game/Sprites/Level/HorrorDoor/ExitScreen1.ExitScreen1")
            (`KismetSystemLibrary.Delay` 2.0)
            (goto _label :!via `Reset`)))))))

(fn `UserConstructionScript`)