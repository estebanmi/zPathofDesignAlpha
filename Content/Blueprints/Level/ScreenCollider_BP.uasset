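; ScreenCollider_BP is a collision box actor that follows the level's adventure or action camera.
; BeginPlay finds CameraAdventure_BP, falling back to CameraAction_BP, then sets the box extent after a short delay.
; Tick copies the camera's location unless InFixedCam is set.
; ToFixedCam and ToDynamicCam use timelines to lerp toward a given point or actor location, with the latter re-enabling following from its first update.
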(event `self.ReceiveBeginPlay`
  (bind _outactors (`GameplayStatics.GetAllActorsOfClass` "/Game/Blueprints/CameraAdventure_BP.CameraAdventure_BP_C"))
  (bind _output (`|GetArrayItem` _outactors))
  (`/Engine/EditorBlueprintResources/StandardMacros.IsValid` _output
    (:`Is Valid`
      (set `self.CameraAdvRef` _output))
    (:`Is Not Valid`
      (bind _outactors_2 (`GameplayStatics.GetAllActorsOfClass` "/Game/Blueprints/CameraAction_BP.CameraAction_BP_C"))
      (bind _output_2 (`|GetArrayItem` _outactors_2))
      (`/Engine/EditorBlueprintResources/StandardMacros.IsValid` _output_2
        (:`Is Valid`
          (set `self.CameraActionRef` _output_2)))))
  (`KismetSystemLibrary.Delay` 0.2)
  (`BoxComponent.SetBoxExtent` (`self.ScreenCollider`) (200.0 6.0 100.0) true))

(event `self.ReceiveTick`
  (params (DeltaSeconds :type "Float (single-precision)"))
  (if (not (`self.InFixedCam`))
    (`/Engine/EditorBlueprintResources/StandardMacros.IsValid` (`self.CameraAdvRef`)
      (:`Is Valid`
        (`self.K2_SetActorLocation` (`self.K2_GetActorLocation` (`self.CameraAdvRef`))))
      (:`Is Not Valid`
        (`/Engine/EditorBlueprintResources/StandardMacros.IsValid` (`self.CameraActionRef`)
          (:`Is Valid`
            (`self.K2_SetActorLocation` (`self.K2_GetActorLocation` (`self.CameraActionRef`)))))))))

(event `ToFixedCam`
  (params (NewLocation :type "Vector Structure"))
  ;[1 1 1] Move to FixedCam
  (set `self.InFixedCam` true)
  (set `self.FixedLocation` NewLocation)
  (bind (_direction _alpha) (`Timeline|CameraTransition` :!via `PlayFromStart`)
    (:`Update`
      (`self.K2_SetActorLocation` (`KismetMathLibrary.VLerp` (`self.K2_GetActorLocation`) (`self.FixedLocation`) _alpha)))))

(event `ToDynamicCam`
  (params (NewActor :type "Actor Object Reference"))
  ;[1 1 1] Move to FixedCam
  (set `self.DynamicLocation` (`self.K2_GetActorLocation` NewActor))
  (bind (_direction _alpha) (`Timeline|Timeline_0` :!via `PlayFromStart`)
    (:`Update`
      (`self.K2_SetActorLocation` (`KismetMathLibrary.VLerp` (`self.K2_GetActorLocation`) (`self.DynamicLocation`) _alpha))
      (set `self.InFixedCam` false))))

(fn `UserConstructionScript`)