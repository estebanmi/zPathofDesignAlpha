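; Armored level-exit door that opens when the player overlaps it with a BitCoinsMax above the required amount, otherwise flashing a blocked alert.
; EnterDoor, if in range and open, saves up to two unlocks into the player's current world array, then loads the target level or RAMWorld.
; Tick drives the screen flipbook from door state flags.
; With VideoCardON, the door is tinted from the level's color scheme table.
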(event `Update Unlocks`
  (bind _playerref (`self.PlayerRef`))
  (bind _playerref_2 (`self.PlayerRef`))
  (bind _unlockslevel_ (`self.UnlocksLevel:`))
  (bind _output_get (set `self.CurrentWorld` (select `/Game/Blueprints/WorldMap/CurrentWorld` (`/Game/Blueprints/Player/Player_BP.CurrentWorldType` (`self.PlayerRef`)) :`NewEnumerator0` (`/Game/Blueprints/Player/Player_BP.WorldMother` _playerref) :`NewEnumerator1` (`/Game/Blueprints/Player/Player_BP.WorldHDD` _playerref) :`NewEnumerator2` (`/Game/Blueprints/Player/Player_BP.WorldVideo` _playerref) :`NewEnumerator3` (`/Game/Blueprints/Player/Player_BP.WorldSound` _playerref) :`NewEnumerator4` (`/Game/Blueprints/Player/Player_BP.WorldPower` _playerref) :`NewEnumerator5` (`/Game/Blueprints/Player/Player_BP.WorldCooling` _playerref) :`NewEnumerator6` (`/Game/Blueprints/Player/Player_BP.WorldRAM` _playerref) :`NewEnumerator7` (`/Game/Blueprints/Player/Player_BP.WorldCPU` _playerref))))
  (bind _output_get_2 (set `self.CurrentWorld` (`|MakeArray` (select `bool` (== _unlockslevel_ 0) :`false` (`|GetArrayItem` _output_get) :`true` true) (select `bool` (== _unlockslevel_ 1) :`false` (`|GetArrayItem` _output_get 1) :`true` true) (select `bool` (== _unlockslevel_ 2) :`false` (`|GetArrayItem` _output_get 2) :`true` true) (select `bool` (== _unlockslevel_ 3) :`false` (`|GetArrayItem` _output_get 3) :`true` true) (select `bool` (== _unlockslevel_ 4) :`false` (`|GetArrayItem` _output_get 4) :`true` true) (select `bool` (== _unlockslevel_ 5) :`false` (`|GetArrayItem` _output_get 5) :`true` true) (select `bool` (== _unlockslevel_ 6) :`false` (`|GetArrayItem` _output_get 6) :`true` true) (select `bool` (== _unlockslevel_ 7) :`false` (`|GetArrayItem` _output_get 7) :`true` true))))
  (switch `/Game/Blueprints/WorldMap/CurrentWorld` (`/Game/Blueprints/Player/Player_BP.CurrentWorldType` (`self.PlayerRef`))
    (:`NewEnumerator0`
      (set `/Game/Blueprints/Player/Player_BP.WorldMother` _output_get_2 _playerref_2))
    (:`NewEnumerator1`
      (set `/Game/Blueprints/Player/Player_BP.WorldHDD` _output_get_2 _playerref_2))
    (:`NewEnumerator2`
      (set `/Game/Blueprints/Player/Player_BP.WorldVideo` _output_get_2 _playerref_2))
    (:`NewEnumerator3`
      (set `/Game/Blueprints/Player/Player_BP.WorldSound` _output_get_2 _playerref_2))
    (:`NewEnumerator4`
      (set `/Game/Blueprints/Player/Player_BP.WorldPower` _output_get_2 _playerref_2))
    (:`NewEnumerator5`
      (set `/Game/Blueprints/Player/Player_BP.WorldCooling` _output_get_2 _playerref_2))
    (:`NewEnumerator6`
      (set `/Game/Blueprints/Player/Player_BP.WorldRAM` _output_get_2 _playerref_2))
    (:`NewEnumerator7`
      (set `/Game/Blueprints/Player/Player_BP.WorldCPU` _output_get_2 _playerref_2)))
  (`/Game/Blueprints/Player/Player_BP.SaveGame` (`self.PlayerRef`)))

(event `ColorControl`
  ;[0 1 1] Color Control
  (if (`/Game/Blueprints/Player/Player_BP.VideoCardON` (`self.PlayerRef`))
    (bind _outactors (`GameplayStatics.GetAllActorsOfClass` "/Game/Blueprints/Art/ColorController.ColorController_C"))
    (bind _returnvalue (`|GetDataTableRow` "/Game/Blueprints/Art/ColorSchemeTable.ColorSchemeTable" (`/Game/Blueprints/Art/ColorController.ColorScheme` (`|GetArrayItem` _outactors)))
      (:`then`
        (`PaperFlipbookComponent.SetSpriteColor` (`self.DoorFlipbook`) (`.Level_31_53E2F58345BAE2A33F5ED5BE59653F21` (break `/Game/Blueprints/Art/ColorScheme` _returnvalue)))))))

(event `EnterDoor`
  (bind _playerref (`self.PlayerRef`))
  ;[1 0.4966 0] Enter Door
  (if (`self.inRange`)
    (if (`self.isOpen`)
      (set `/Game/Blueprints/Player/Player_BP.InputDisabled` true _playerref)
      (`MovementComponent.StopMovementImmediately` (`Character.CharacterMovement` _playerref))
      (`PrimitiveComponent.SetCollisionEnabled` (`Character.CapsuleComponent` _playerref) "NoCollision")
      ;[1 1 1] PlayerAnimation
      (`/Game/Blueprints/Player/Player_BP.BinaryBumper` _playerref)
      (`self.Update Unlocks`)
      (if (not (== (`self.Unlocks2Level:`) 0))
        (set `self.UnlocksLevel:` (`self.Unlocks2Level:`))
        (`self.Update Unlocks`))
      (`KismetSystemLibrary.Delay` 0.3)
      (if (`/Game/Blueprints/Player/Player_BP.RAM?` (`self.PlayerRef`))
        (`GameplayStatics.PlaySound2D` "/Game/Sound/SFXs/Sfx_Boss_RAMOpen_Cue.Sfx_Boss_RAMOpen_Cue" 1.0 1.0 0.0 null null)
        (`KismetSystemLibrary.Delay` 4.0)
        (`GameplayStatics.OpenLevel` "RAMWorld")
        (else
          (`GameplayStatics.OpenLevel` (`self.LevelToOpen`))))
      (else
        (`/Engine/EditorBlueprintResources/StandardMacros.DoOnce` false :!label _label
          (:`Completed`
            (`GameplayStatics.PlaySound2D` "/Game/Sound/SFXs/sfx_DoorBlocked_Cue.sfx_DoorBlocked_Cue" 1.0 1.0 0.0 null null)
            (`KismetSystemLibrary.Delay` 1.0)
            (goto _label :!via `Reset`)))))))

(event `Control Animations`
  ;[1 0 0.5456] Control Animations
  (if (`self.isOpening`)
    (`PaperFlipbookComponent.SetFlipbook` (`self.ScreenFlipbook`) "/Game/Sprites/Level/ArmoredDoor/ScreenOpening.ScreenOpening")
    (`KismetSystemLibrary.Delay` 0.8)
    (`PaperFlipbookComponent.Stop` (`self.ScreenFlipbook`))
    (elif (`self.ClosedAlert`)
      (`PaperFlipbookComponent.SetFlipbook` (`self.ScreenFlipbook`) "/Game/Sprites/Level/ArmoredDoor/Screen_ClosedAlert.Screen_ClosedAlert")
      (else
        (`PaperFlipbookComponent.SetFlipbook` (`self.ScreenFlipbook`) "/Game/Sprites/Level/ArmoredDoor/Screen_Closed.Screen_Closed")))))

(event `self.ReceiveBeginPlay`
  ;[1 0.4617 0] Default
  (`KismetSystemLibrary.Delay` 0.1)
  (bind _asplayer_bp (cast `/Game/Blueprints/Player/Player_BP` (`GameplayStatics.GetPlayerCharacter` 0)))
  (set `self.PlayerRef` _asplayer_bp)
  (`self.ColorControl`))

(event `self.ReceiveTick`
  (params (DeltaSeconds :type "Float (single-precision)"))
  ;[1 0.4617 0] Default
  (`self.Control Animations`))

(event `self.BoxColldier.OnComponentBeginOverlap`
  (params (OverlappedComponent :type "PrimitiveComponent Object Reference") (OtherActor :type "Actor Object Reference") (OtherComp :type "PrimitiveComponent Object Reference") (OtherBodyIndex :type Integer) (bFromSweep :type Boolean) (SweepResult :type "HitResult Structure (by ref)"))
  ;[1 1 1] Overlaping the Door
  (cast `/Game/Blueprints/Player/Player_BP` OtherActor)
  (set `self.inRange` true)
  (if (> (`/Game/Blueprints/Player/Player_BP.BitCoinsMax` (`self.PlayerRef`)) (`self.BitcoinsRequired`))
    (`self.DoorOpening`)
    (else
      (`self.DoorClosed`))))

(event `self.BoxColldier.OnComponentEndOverlap`
  (params (OverlappedComponent :type "PrimitiveComponent Object Reference") (OtherActor :type "Actor Object Reference") (OtherComp :type "PrimitiveComponent Object Reference") (OtherBodyIndex :type Integer))
  ;[1 1 1] Overlaping the Door
  (cast `/Game/Blueprints/Player/Player_BP` OtherActor)
  (set `self.inRange` false))

(event `DoorClosed`
  ;[1 1 1] Door Closed Alert
  (`/Engine/EditorBlueprintResources/StandardMacros.DoOnce` false :!label _label_2
    (:`Completed`
      (set `self.ClosedAlert` true)
      (`GameplayStatics.PlaySound2D` "/Game/Sound/SFXs/sfx_DoorBlocked_Cue.sfx_DoorBlocked_Cue" 1.0 1.0 0.0 null null)
      (`KismetSystemLibrary.Delay` 0.7)
      (set `self.ClosedAlert` false)
      (`KismetSystemLibrary.Delay` 2.0)
      (goto _label_2 :!via `Reset`))))

(event `DoorOpening`
  ;[1 0 0.5677] Door Opening
  (`/Engine/EditorBlueprintResources/StandardMacros.DoOnce` false
    (:`Completed`
      (set `self.isOpening` true)
      (`GameplayStatics.PlaySound2D` "/Game/Sound/SFXs/sfx_DoorOpening_Cue.sfx_DoorOpening_Cue" 1.0 1.0 0.0 null null)
      (`PaperFlipbookComponent.SetFlipbook` (`self.DoorFlipbook`) "/Game/Sprites/Level/ArmoredDoor/NewFolder/ArmoredDoorOpening.ArmoredDoorOpening")
      (`KismetSystemLibrary.Delay` 0.8)
      (set `self.isOpened` true)
      (`KismetSystemLibrary.Delay` 0.2)
      (`PaperFlipbookComponent.SetFlipbook` (`self.DoorFlipbook`) "/Game/Sprites/Level/ArmoredDoor/NewFolder/ArmoredDoorOpened.ArmoredDoorOpened"))))

(fn `UserConstructionScript`)