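; WhiteBG_BP is a white background sprite actor that follows the level camera in a 2D side-view setup.
; On BeginPlay it scales its Paper2D sprite up and caches the first CameraAdventure_BP, falling back to CameraAction_BP if none exists.
; Each Tick it moves to the cached camera's X and Z at a fixed Y depth, keeping the backdrop aligned with the camera.
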(event `self.ReceiveBeginPlay`
  (`SceneComponent.SetRelativeScale3D` (`self.PaperSprite`) (250.0 1.0 150.0))
  (bind _outactors (`GameplayStatics.GetAllActorsOfClass` "/Game/Blueprints/CameraAdventure_BP.CameraAdventure_BP_C"))
  (bind _output (`|GetArrayItem` _outactors))
  (`/Engine/EditorBlueprintResources/StandardMacros.IsValid` _output
    (:`Is Valid`
      (set `self.CameraAdvRef` _output))
    (:`Is Not Valid`
      (bind _outactors_2 (`GameplayStatics.GetAllActorsOfClass` "/Game/Blueprints/CameraAction_BP.CameraAction_BP_C"))
      (bind _output_2 (`|GetArrayItem` _outactors_2))
      (`/Engine/EditorBlueprintResources/StandardMacros.IsValid` _output_2
        (:`Is Valid`
          (set `self.CameraActionRef` _output_2))))))

(event `self.ReceiveTick`
  (params (DeltaSeconds :type "Float (single-precision)"))
  (bind (_returnvalue_x _returnvalue_y _returnvalue_z) (`KismetMathLibrary.BreakVector` (`self.K2_GetActorLocation` (`self.CameraActionRef`))))
  (bind (_returnvalue_x_2 _returnvalue_y_2 _returnvalue_z_2) (`KismetMathLibrary.BreakVector` (`self.K2_GetActorLocation` (`self.CameraAdvRef`))))
  (`/Engine/EditorBlueprintResources/StandardMacros.IsValid` (`self.CameraAdvRef`)
    (:`Is Valid`
      (`self.K2_SetActorLocation` (`KismetMathLibrary.MakeVector` _returnvalue_x_2 -20.0 _returnvalue_z_2)))
    (:`Is Not Valid`
      (`/Engine/EditorBlueprintResources/StandardMacros.IsValid` (`self.CameraActionRef`)
        (:`Is Valid`
          (`self.K2_SetActorLocation` (`KismetMathLibrary.MakeVector` _returnvalue_x -20.0 _returnvalue_z)))))))

(fn `UserConstructionScript`)