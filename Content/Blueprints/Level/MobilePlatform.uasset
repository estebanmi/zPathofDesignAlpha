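; Moving one-way platform actor that travels horizontally or vertically, optionally reversed, from its starting position.
; A timeline adds vector offsets to the stored location, triggered either after a start delay on BeginPlay or when the player hits its box collider.
; Each tick it compares player and platform heights, disabling the box collision while the player is below so the platform only blocks from above.
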(event `StartOnContact`
  (set `self.PlatformLocation` (`self.K2_GetActorLocation`) :!label _label)
  (bind (_direction _horizontalvector _reversehorizontalvector _verticalvector _reverseverticalvector) (`Timeline|Timeline_0`)
    (:`Update`
      (if (`self.isHorizontal`)
        (if (`self.Reverse`)
          (`self.K2_SetActorLocation` (+ (`self.PlatformLocation`) _reversehorizontalvector))
          (else
            (`self.K2_SetActorLocation` (+ (`self.PlatformLocation`) _horizontalvector))))
        (elif (`self.Reverse`)
          (`self.K2_SetActorLocation` (+ (`self.PlatformLocation`) _reverseverticalvector))
          (else
            (`self.K2_SetActorLocation` (+ (`self.PlatformLocation`) _verticalvector))))))))

(event `self.ReceiveBeginPlay`
  (bind _asplayer_bp (cast `/Game/Blueprints/Player/Player_BP` (`GameplayStatics.GetPlayerCharacter` 0)))
  (set `self.PlayerRef` _asplayer_bp)
  (if (`self.itMoves`)
    (if (not (`self.StartOnContact?`))
      (`KismetSystemLibrary.Delay` (`self.DelayStart`))
      (goto _label))))

(event `self.ReceiveTick`
  (params (DeltaSeconds :type "Float (single-precision)"))
  (bind (_returnvalue_x _returnvalue_y _returnvalue_z) (`KismetMathLibrary.BreakVector` (`self.K2_GetActorLocation`)))
  (bind _boxcollider (`self.BoxCollider`))
  (bind (_returnvalue_x_2 _returnvalue_y_2 _returnvalue_z_2) (`KismetMathLibrary.BreakVector` (`self.K2_GetActorLocation` (`self.PlayerRef`))))
  (`/Engine/EditorBlueprintResources/StandardMacros.IsValid` (`self.PlayerRef`)
    (:`Is Valid`
      (if (< (- _returnvalue_z_2 9.0) (+ _returnvalue_z 4.0))
        (`PrimitiveComponent.SetCollisionEnabled` _boxcollider "NoCollision")
        (else
          (`PrimitiveComponent.SetCollisionEnabled` _boxcollider "QueryAndPhysics"))))))

(event `self.BoxCollider.OnComponentHit`
  (params (HitComponent :type "PrimitiveComponent Object Reference") (OtherActor :type "Actor Object Reference") (OtherComp :type "PrimitiveComponent Object Reference") (NormalImpulse :type "Vector Structure") (Hit :type "HitResult Structure (by ref)"))
  (cast `/Game/Blueprints/Player/Player_BP` OtherActor)
  (if (`self.StartOnContact?`)
    (`self.StartOnContact`)))

(fn `UserConstructionScript`)