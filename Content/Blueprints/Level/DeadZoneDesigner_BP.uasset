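; DeadZoneDesigner_BP is a level kill zone that respawns the player and destroys anything else that hits its box collider.
; On BeginPlay it caches the player and records their starting X and Y, with a fixed Z, as the respawn point.
; A player hit plays a death sound, disables input, then after a short delay teleports them back facing right with input restored.
; Other actors are destroyed with a quieter death sound.
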(event `self.ReceiveBeginPlay`
  (bind _asplayer_bp (cast `/Game/Blueprints/Player/Player_BP` (`GameplayStatics.GetPlayerCharacter` 0)))
  (set `self.PlayerRef` _asplayer_bp)
  (bind (_returnvalue_x _returnvalue_y) (`KismetMathLibrary.BreakVector` (`self.K2_GetActorLocation` _asplayer_bp)))
  (set `self.StartingPosition` (`KismetMathLibrary.MakeVector` _returnvalue_x _returnvalue_y -78.0)))

(event `self.Box Collider.OnComponentHit`
  (params (HitComponent :type "PrimitiveComponent Object Reference") (OtherActor :type "Actor Object Reference") (OtherComp :type "PrimitiveComponent Object Reference") (NormalImpulse :type "Vector Structure") (Hit :type "HitResult Structure (by ref)"))
  (bind _playerref (`self.PlayerRef`))
  (cast `/Game/Blueprints/Player/Player_BP` OtherActor
    (:`then`
      (`GameplayStatics.PlaySound2D` "/Game/Sound/SFXs/sfx_PlayerDeath_Cue.sfx_PlayerDeath_Cue" 1.0 1.0 0.0 null null)
      (set `/Game/Blueprints/Player/Player_BP.InputDisabled` true (`self.PlayerRef`))
      (`KismetSystemLibrary.Delay` 1.5)
      (`GameplayStatics.PlaySound2D` "/Game/Sound/SFXs/sfx_PassteriskCollected_Cue.sfx_PassteriskCollected_Cue" 1.0 1.0 0.0 null null)
      (`self.K2_SetActorLocation` (`self.PlayerRef`) (`self.StartingPosition`) false false)
      (set `/Game/Blueprints/Player/Player_BP.InputDisabled` false _playerref)
      (set `/Game/Blueprints/Player/Player_BP.isMovingRight` true _playerref))
    (:`CastFailed`
      (`self.K2_DestroyActor` OtherActor)
      (`GameplayStatics.PlaySound2D` "/Game/Sound/SFXs/sfx_BlopDeath_Cue.sfx_BlopDeath_Cue" 0.3 1.0 0.0 null null))))

(fn `UserConstructionScript`)