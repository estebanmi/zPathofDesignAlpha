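; Blop boss enemy with Paper2D flipbooks that turns toward the visible player, crouches, then leaps, re-arming its attack on each landing with a camera shake.
; Tick derives a state from flags, which selects the active collider, flipbook and contact-damage check.
; Depleting HP first triggers a timeline-driven enrage that refills health, repositions and enlarges the boss, shortens attack delays and makes landings damage grounded players.
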(event `StompDamage`
  (bind _playerref (`self.PlayerRef`))
  ;[1 1 1] Stomp Damage
  (if (not (`/Game/Blueprints/Player/Player_BP.isOnAir` _playerref))
    (`GameplayStatics.ApplyDamage` _playerref (`self.DamageContact`) null self)))

(event `OverlappingDamage`
  (bind _output (`|GetArrayItem` (`PrimitiveComponent.GetOverlappingActors` (`self.BossCollisionIDLE`) "/Game/Blueprints/Player/Player_BP.Player_BP_C")))
  (bind _output_2 (`|GetArrayItem` (`PrimitiveComponent.GetOverlappingActors` (`self.BossCollisionJUMP`) "/Game/Blueprints/Player/Player_BP.Player_BP_C")))
  (bind _output_3 (`|GetArrayItem` (`PrimitiveComponent.GetOverlappingActors` (`self.BossCollisionCROUCH`) "/Game/Blueprints/Player/Player_BP.Player_BP_C")))
  ;[1 1 1] Overlapping Damage
  (switch `/Game/Blueprints/Enemies/Blop/EnemyBlopStates` (`self.BlopStates`)
    (:`NewEnumerator0`
      (`/Engine/EditorBlueprintResources/StandardMacros.IsValid` _output :!label _label
        (:`Is Valid`
          (`GameplayStatics.ApplyDamage` _output (`self.DamageContact`) null self))))
    (:`NewEnumerator1`
      (goto _label))
    (:`NewEnumerator2`
      (`/Engine/EditorBlueprintResources/StandardMacros.IsValid` _output_3
        (:`Is Valid`
          (`GameplayStatics.ApplyDamage` _output_3 (`self.DamageContact`) null self))))
    (:`NewEnumerator3`
      (`/Engine/EditorBlueprintResources/StandardMacros.IsValid` _output_2
        (:`Is Valid`
          (`GameplayStatics.ApplyDamage` _output_2 (`self.DamageContact`) null self))))))

(event `self.ReceiveAnyDamage`
  (params (Damage :type "Float (single-precision)") (DamageType :type "DamageType Object Reference") (InstigatedBy :type "Controller Object Reference") (DamageCauser :type "Actor Object Reference"))
  (bind _sprite (`self.Sprite`))
  (bind (_relativelocation_x _relativelocation_y _relativelocation_z) (`KismetMathLibrary.BreakVector` (`SceneComponent.RelativeLocation` _sprite)))
  ;[1 0.1155 0] ReceiveDamage
  (bind _output_get (set `self.HP` (- (`self.HP`) Damage)))
  (`GameplayStatics.PlaySound2D` "/Game/Sound/SFXs/sfx_BlopHit_Cue.sfx_BlopHit_Cue" 1.0 1.0 0.0 null null)
  (if (<= (`self.HP`) 0.0)
    (if (not (`self.Furious`))
      (`self.GetFurious`)
      (set `self.HP` 200.0))
    (else
      (bind (_direction _horizontalshake) (`Timeline|HitShaking` :!via `PlayFromStart`)
        (:`Update`
          (`SceneComponent.K2_SetRelativeLocation` _sprite (`KismetMathLibrary.MakeVector` _horizontalshake _relativelocation_y _relativelocation_z) false false))
        (:`Finished`
          (if (<= (`self.HP`) 0.0)
            (set `self.isDead` true)
            (`/Engine/EditorBlueprintResources/StandardMacros.DoOnce` false
              (:`Completed`
                (`KismetSystemLibrary.Delay` 0.3)
                (`GameplayStatics.PlaySound2D` "/Game/Sound/SFXs/sfx_BlopDeath_Cue.sfx_BlopDeath_Cue" 1.0 1.0 0.0 null null)
                (`KismetSystemLibrary.Delay` 0.15)
                (`self.DropLoot`)
                (`KismetSystemLibrary.Delay` 0.55)
                (`/Game/Blueprints/Player/Player_BP.EmenyKilled` (`self.PlayerRef`))
                (`self.K2_DestroyActor`)))))))))

(event `DropLoot`
  ;[1 1 1] Drop Loot
)

(event `DeadZone`
  (params (OtherActor :type "Actor Object Reference"))
  ;[1 0.1155 0] ReceiveDamage
  ;;[1 1 1] Dead Zone
  (cast `/Game/Blueprints/Level/DeadZoneFalling_BP` OtherActor)
  (`GameplayStatics.PlaySound2D` "/Game/Sound/SFXs/sfx_BlopDeath_Cue.sfx_BlopDeath_Cue" 0.3 1.0 0.0 null null)
  (`self.K2_DestroyActor`))

(event `self.BossCollisionIDLE.OnComponentBeginOverlap`
  (params (OverlappedComponent :type "PrimitiveComponent Object Reference") (OtherActor :type "Actor Object Reference") (OtherComp :type "PrimitiveComponent Object Reference") (OtherBodyIndex :type Integer) (bFromSweep :type Boolean) (SweepResult :type "HitResult Structure (by ref)"))
  ;[1 0.9688 0.9688] Apply Damage
  (bind _asplayer_bp (cast `/Game/Blueprints/Player/Player_BP` OtherActor)
    (:`then`
      (`GameplayStatics.ApplyDamage` _asplayer_bp (`self.DamageContact`) null self))
    (:`CastFailed`
      (`self.DeadZone` OtherActor))))

(event `self.BossCollisionCROUCH.OnComponentBeginOverlap`
  (params (OverlappedComponent :type "PrimitiveComponent Object Reference") (OtherActor :type "Actor Object Reference") (OtherComp :type "PrimitiveComponent Object Reference") (OtherBodyIndex :type Integer) (bFromSweep :type Boolean) (SweepResult :type "HitResult Structure (by ref)"))
  ;[1 0.9688 0.9688] Apply Damage
  (bind _asplayer_bp (cast `/Game/Blueprints/Player/Player_BP` OtherActor)
    (:`then`
      (`GameplayStatics.ApplyDamage` _asplayer_bp (`self.DamageContact`) null self))
    (:`CastFailed`
      (`self.DeadZone` OtherActor))))

(event `Attack`
  ;[1 0 0] Attack Jump
  (if (not (`self.GettingFurious`))
    (set `CharacterMovementComponent.MaxAcceleration` (`KismetMathLibrary.RandomFloatInRange` 10000.0 15000.0) (`self.CharacterMovement`))
    (`self.TurnToPlayer`)
    (if (not (`self.isDead`))
      (set `self.isCrouching` true)
      (`KismetSystemLibrary.Delay` 1.0)
      (if (`self.isDead`)
        _
        (elif (`self.GettingFurious`)
          _
          (elif (`self.isCrouching`)
            (set `self.isCrouching` false)
            (if (not (`self.isHit`))
              (set `self.IsJumping` true)
              (if (`self.isFacingLeft`)
                (`self.AddMovementInput` (-1.0 0.0 0.0))
                (else
                  (`self.AddMovementInput` (1.0 0.0 0.0))))
              (`self.Jump`)
              (`GameplayStatics.PlaySound2D` "/Game/Sound/SFXs/sfx_BlopJump_Cue.sfx_BlopJump_Cue" 1.0 1.0 0.0 null null)
              (set `self.IsJumping` true))))))))

(event `ResetAttack`
  ;[1 0 0] Attack Jump
  (if (`self.Furious`) :!label _label_2
    (`KismetSystemLibrary.Delay` (`KismetMathLibrary.RandomFloatInRange` 1.0 2.0))
    (else
      (`KismetSystemLibrary.Delay` (`KismetMathLibrary.RandomFloatInRange` 1.5 3.0))))
  (if (`self.isDead`)
    _
    (elif (not (`self.GettingFurious`))
      (`self.Attack`))))

(event `ToAttack`
  ;[1 0 0] Attack Jump
  (goto _label_2))

(event `self.BossCollisionJUMP.OnComponentBeginOverlap`
  (params (OverlappedComponent :type "PrimitiveComponent Object Reference") (OtherActor :type "Actor Object Reference") (OtherComp :type "PrimitiveComponent Object Reference") (OtherBodyIndex :type Integer) (bFromSweep :type Boolean) (SweepResult :type "HitResult Structure (by ref)"))
  ;[1 0.9688 0.9688] Apply Damage
  (bind _asplayer_bp (cast `/Game/Blueprints/Player/Player_BP` OtherActor)
    (:`then`
      (`GameplayStatics.ApplyDamage` _asplayer_bp (`self.DamageContact`) null self))
    (:`CastFailed`
      (`self.DeadZone` OtherActor))))

(event `ControlAnimation`
  ;[0.0133 0.4271 0] Control Animation
  (if (`self.isDead`)
    (set `self.BlopStates` "NewEnumerator4")
    (`/Engine/EditorBlueprintResources/StandardMacros.DoOnce` false
      (:`Completed`
        (`KismetSystemLibrary.Delay` 0.6)
        (`PaperFlipbookComponent.Stop` (`self.Sprite`))))
    (elif (`self.isHit`)
      (set `self.BlopStates` "NewEnumerator0")
      (elif (`self.isCrouching`)
        (set `self.BlopStates` "NewEnumerator2")
        (elif (`self.IsJumping`)
          (set `self.BlopStates` "NewEnumerator3" :!label _label_3)
          (elif (`NavMovementComponent.IsFalling` (`self.CharacterMovement`))
            (goto _label_3)
            (else
              (set `self.BlopStates` "NewEnumerator1"))))))))

(event `ColliderSelect`
  (switch `/Game/Blueprints/Enemies/Blop/EnemyBlopStates` (`self.BlopStates`)
    (:`NewEnumerator0`
      (`PrimitiveComponent.SetCollisionEnabled` (`self.BossCollisionIDLE`) "QueryAndPhysics" :!label _label_4)
      (`PrimitiveComponent.SetCollisionEnabled` (`self.BossCollisionCROUCH`) "NoCollision")
      (`PrimitiveComponent.SetCollisionEnabled` (`self.BossCollisionJUMP`) "NoCollision"))
    (:`NewEnumerator1`
      (goto _label_4))
    (:`NewEnumerator2`
      (`PrimitiveComponent.SetCollisionEnabled` (`self.BossCollisionIDLE`) "NoCollision")
      (`PrimitiveComponent.SetCollisionEnabled` (`self.BossCollisionCROUCH`) "QueryAndPhysics")
      (`PrimitiveComponent.SetCollisionEnabled` (`self.BossCollisionJUMP`) "NoCollision"))
    (:`NewEnumerator3`
      (`PrimitiveComponent.SetCollisionEnabled` (`self.BossCollisionIDLE`) "NoCollision")
      (`PrimitiveComponent.SetCollisionEnabled` (`self.BossCollisionCROUCH`) "NoCollision")
      (`PrimitiveComponent.SetCollisionEnabled` (`self.BossCollisionJUMP`) "QueryAndPhysics"))
    (:`NewEnumerator4`
      (`PrimitiveComponent.SetCollisionEnabled` (`self.BossCollisionIDLE`) "NoCollision")
      (`PrimitiveComponent.SetCollisionEnabled` (`self.BossCollisionCROUCH`) "NoCollision")
      (`PrimitiveComponent.SetCollisionEnabled` (`self.BossCollisionJUMP`) "NoCollision"))))

(event `TurnToPlayer`
  (bind _returnvalue_x (`KismetMathLibrary.BreakVector` (`KismetMathLibrary.GetDirectionUnitVector` (`self.K2_GetActorLocation`) (`self.K2_GetActorLocation` (`self.PlayerRef`)))))
  ;[0 0.218 1] Turn To Player
  (if (`KismetSystemLibrary.IsValid` (`self.PlayerRef`))
    (if (> _returnvalue_x 0.0)
      (if (`self.isFacingLeft`)
        (if (not (`/Game/Blueprints/Player/Player_BP.isInvisible` (`self.PlayerRef`)))
          (`self.DirectionChange`)))
      (elif (`self.isFacingLeft`)
        _
        (elif (not (`/Game/Blueprints/Player/Player_BP.isInvisible` (`self.PlayerRef`)))
          (`self.DirectionChange`))))))

(event `self.OnLanded`
  (params (Hit :type "HitResult Structure (by ref)"))
  ;[0.0133 0.4271 0] Control Animation
  ;;[1 1 1] OnLanded
  (`self.ResetAttack`)
  (if (`self.Furious`)
    (`self.StompDamage`))
  (`GameplayStatics.PlaySound2D` "/Game/Sound/SFXs/sfx_BlopBossStomp_Cue.sfx_BlopBossStomp_Cue" 1.0 1.0 0.0 null null)
  (`self.CameraShake`)
  (set `self.IsJumping` false)
  (set `self.isCrouching` true)
  (`KismetSystemLibrary.Delay` 0.5)
  (set `self.isCrouching` false))

(event `CameraShake`
  (bind _cameraadvref (`self.CameraAdvRef`))
  (bind (_returnvalue_x _returnvalue_y _returnvalue_z) (`KismetMathLibrary.BreakVector` (`self.K2_GetActorLocation` _cameraadvref)))
  ;[1 1 1] Camera Shake
  (bind _outactors (`GameplayStatics.GetAllActorsOfClass` "/Game/Blueprints/CameraAdventure_BP.CameraAdventure_BP_C"))
  (bind _output (`|GetArrayItem` _outactors))
  (`/Engine/EditorBlueprintResources/StandardMacros.IsValid` _output
    (:`Is Valid`
      (set `self.CameraAdvRef` _output)
      (if (`self.Furious`)
        (bind (_direction _newtrack_0) (`Timeline|CamShakeHigh` :!via `PlayFromStart`)
          (:`Update`
            (`self.K2_SetActorRelativeLocation` _cameraadvref (`KismetMathLibrary.MakeVector` _returnvalue_x _returnvalue_y (+ (.z _newtrack_0) _returnvalue_z)) false false)))
        (else
          (bind (_direction_2 _newtrack_0_2) (`Timeline|CameShakeLow` :!via `PlayFromStart`)
            (:`Update`
              (`self.K2_SetActorRelativeLocation` _cameraadvref (`KismetMathLibrary.MakeVector` _returnvalue_x _returnvalue_y (+ (.z _newtrack_0_2) _returnvalue_z)) false false))))))))

(event `UpdateAnimations`
  ;[0.07908 0.1965 1] UpdateAnimations
  (if (`self.GettingFurious`)
    _
    (elif (`self.Furious`)
      (switch `/Game/Blueprints/Enemies/Blop/EnemyBlopStates` (`self.BlopStates`)
        (:`NewEnumerator0`
          (`PaperFlipbookComponent.SetFlipbook` (`self.Sprite`) "/Game/Sprites/Bosses/BlopBoss/BossBlopFuriousHit.BossBlopFuriousHit"))
        (:`NewEnumerator1`
          (`PaperFlipbookComponent.SetFlipbook` (`self.Sprite`) "/Game/Sprites/Bosses/BlopBoss/BossBlopFuriousIdle.BossBlopFuriousIdle"))
        (:`NewEnumerator2`
          (`PaperFlipbookComponent.SetFlipbook` (`self.Sprite`) "/Game/Sprites/Bosses/BlopBoss/BossBlopFuriousCrouch.BossBlopFuriousCrouch"))
        (:`NewEnumerator3`
          (`PaperFlipbookComponent.SetFlipbook` (`self.Sprite`) "/Game/Sprites/Bosses/BlopBoss/BossBlopFuriousJump.BossBlopFuriousJump"))
        (:`NewEnumerator4`
          (`PaperFlipbookComponent.SetFlipbook` (`self.Sprite`) "/Game/Sprites/Enemies/Blop/EnemyBlopDeath1.EnemyBlopDeath1")))
      (else
        (switch `/Game/Blueprints/Enemies/Blop/EnemyBlopStates` (`self.BlopStates`)
          (:`NewEnumerator0`
            (`PaperFlipbookComponent.SetFlipbook` (`self.Sprite`) "/Game/Sprites/Enemies/Blop/EnemyBlopHIT.EnemyBlopHIT"))
          (:`NewEnumerator1`
            (`PaperFlipbookComponent.SetFlipbook` (`self.Sprite`) "/Game/Sprites/Enemies/Blop/EnemyBlopIDLE.EnemyBlopIDLE"))
          (:`NewEnumerator2`
            (`PaperFlipbookComponent.SetFlipbook` (`self.Sprite`) "/Game/Sprites/Enemies/Blop/EnemyBlopTOJUMP.EnemyBlopTOJUMP"))
          (:`NewEnumerator3`
            (`PaperFlipbookComponent.SetFlipbook` (`self.Sprite`) "/Game/Sprites/Enemies/Blop/EnemyBlopJUMP.EnemyBlopJUMP"))
          (:`NewEnumerator4`
            (`PaperFlipbookComponent.SetFlipbook` (`self.Sprite`) "/Game/Sprites/Enemies/Blop/EnemyBlopHIT.EnemyBlopHIT")))))))

(event `DirectionStart`
  ;[0.1362 0.1893 1] Facing Control
  (if (`self.isFacingLeft`)
    (`SceneComponent.K2_SetWorldRotation` :`self` (`self.CapsuleComponent`))
    (else
      (`SceneComponent.K2_SetWorldRotation` (`self.CapsuleComponent`) (struct :`Yaw` 180.0) false false))))

(event `RevealCollider`)

(event `DirectionChange`
  ;[0.1362 0.1893 1] Facing Control
  (if (`self.isFacingLeft`)
    (`SceneComponent.K2_SetWorldRotation` (`self.CapsuleComponent`) (struct :`Yaw` 180.0) false false)
    (set `self.isFacingLeft` false)
    (else
      (`SceneComponent.K2_SetWorldRotation` :`self` (`self.CapsuleComponent`))
      (set `self.isFacingLeft` true))))

(event `self.ReceiveBeginPlay`
  ;[0.9624 1 0.9789] DEFAULT
  (`self.DirectionStart`)
  (`self.ToAttack`)
  (`self.CastPlayerRef`))

(event `self.ReceiveTick`
  (params (DeltaSeconds :type "Float (single-precision)"))
  ;[0.9624 1 0.9789] DEFAULT
  (`self.ColliderSelect`)
  (`self.ControlAnimation`)
  (`self.UpdateAnimations`)
  (`self.OverlappingDamage`)
  (`self.RevealCollider`))

(event `CastPlayerRef`
  ;[0.9624 1 0.9789] DEFAULT
  ;;[1 1 1] CastPlayer
  (bind _asplayer_bp (cast `/Game/Blueprints/Player/Player_BP` (`GameplayStatics.GetPlayerCharacter` 0)))
  (set `self.PlayerRef` _asplayer_bp))

(event `GetFurious`
  (bind (_returnvalue_x _returnvalue_y _returnvalue_z) (`KismetMathLibrary.BreakVector` (`self.K2_GetActorLocation`)))
  (bind _charactermovement (`self.CharacterMovement`))
  (bind _sprite (`self.Sprite`))
  (bind (_relativelocation_x _relativelocation_y _relativelocation_z) (`KismetMathLibrary.BreakVector` (`SceneComponent.RelativeLocation` _sprite)))
  ;[1 0 0.007289] ENRAGE
  (`self.TurnToPlayer`)
  (set `self.isDead` true)
  (set `self.GettingFurious` true)
  (`PaperFlipbookComponent.SetFlipbook` (`self.Sprite`) "/Game/Sprites/Enemies/Blop/EnemyBlopHIT.EnemyBlopHIT")
  (set `CharacterMovementComponent.GravityScale` 0.0 _charactermovement)
  (`MovementComponent.StopMovementImmediately` _charactermovement)
  (bind (_direction _furiousshaking) (`Timeline|FuriousShaking` :!via `PlayFromStart`)
    (:`Update`
      (`SceneComponent.K2_SetRelativeLocation` _sprite (`KismetMathLibrary.MakeVector` _furiousshaking _relativelocation_y _relativelocation_z) false false))
    (:`Finished`
      (set `self.isDead` false)
      (`PaperFlipbookComponent.SetFlipbook` (`self.Sprite`) "/Game/Sprites/Bosses/BlopBoss/BossBlopFuriousJump.BossBlopFuriousJump")
      (bind (_direction_2 _furiousalpha) (`Timeline|AlphaZ` :!via `PlayFromStart`)
        (:`Update`
          (bind _returnvalue_x_2 (`KismetMathLibrary.BreakVector` (`KismetMathLibrary.VLerp` (`KismetMathLibrary.MakeVector` _returnvalue_x) (-225.0 0.0 0.0) (.x _furiousalpha))))
          (bind (_returnvalue_x_3 _returnvalue_y_2 _returnvalue_z_2) (`KismetMathLibrary.BreakVector` (`KismetMathLibrary.VLerp` (`KismetMathLibrary.MakeVector` 0.0 0.0 _returnvalue_z) (0.0 0.0 820.0) (.z _furiousalpha))))
          (`self.K2_SetActorLocation` (`KismetMathLibrary.MakeVector` _returnvalue_x_2 _returnvalue_y _returnvalue_z_2)))
        (:`Finished`
          (set `self.Furious` true)
          (`PaperFlipbookComponent.SetFlipbook` (`self.Sprite`) "/Game/Sprites/Bosses/BlopBoss/BossBlopFuriousIdle.BossBlopFuriousIdle")
          (`KismetSystemLibrary.Delay` 0.4)
          (`self.SizeChange`))))))

(event `SizeChange`
  (bind _bosscollisionidle (`self.BossCollisionIDLE`))
  (bind _bosscollisioncrouch (`self.BossCollisionCROUCH`))
  (bind _bosscollisionjump (`self.BossCollisionJUMP`))
  ;[1 0 0.007289] ENRAGE
  ;;[1 0 0.01326] SizeChange
  (`SceneComponent.SetRelativeScale3D` (`self.Sprite`) (8.0 8.0 8.0))
  (`KismetSystemLibrary.Delay` 0.1)
  (`SceneComponent.SetRelativeScale3D` (`self.Sprite`) (4.0 4.0 4.0))
  (`KismetSystemLibrary.Delay` 0.1)
  (`SceneComponent.SetRelativeScale3D` (`self.Sprite`) (8.0 8.0 8.0))
  (`KismetSystemLibrary.Delay` 0.1)
  (`SceneComponent.SetRelativeScale3D` (`self.Sprite`) (4.0 4.0 4.0))
  (`KismetSystemLibrary.Delay` 0.1)
  (`SceneComponent.SetRelativeScale3D` (`self.Sprite`) (8.0 8.0 8.0))
  (`KismetSystemLibrary.Delay` 0.1)
  (`SceneComponent.SetRelativeScale3D` (`self.Sprite`) (4.0 4.0 4.0))
  (`KismetSystemLibrary.Delay` 0.1)
  (`SceneComponent.SetRelativeScale3D` (`self.Sprite`) (8.0 8.0 8.0))
  (`SceneComponent.SetRelativeScale3D` (`self.Sprite`) (8.0 8.0 8.0))
  (`SceneComponent.SetRelativeScale3D` _bosscollisionidle (2.0 0.0 2.0))
  (`SceneComponent.K2_SetRelativeLocation` _bosscollisionidle (4.0 0.0 12.0) false false)
  (`SceneComponent.SetRelativeScale3D` _bosscollisioncrouch (2.0 2.0 2.0))
  (`SceneComponent.K2_SetRelativeLocation` _bosscollisioncrouch (4.0 0.0 9.0) false false)
  (`SceneComponent.SetRelativeScale3D` _bosscollisionjump (2.0 2.0 2.0))
  (`SceneComponent.K2_SetRelativeLocation` _bosscollisionjump (8.0 0.0 32.0) false false)
  (`KismetSystemLibrary.Delay` 0.5)
  (set `CharacterMovementComponent.GravityScale` 1.5 (`self.CharacterMovement`))
  (set `self.GettingFurious` false))

(fn `UserConstructionScript`)