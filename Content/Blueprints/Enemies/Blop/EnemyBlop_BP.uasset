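; Blop enemy for a 2D flipbook game that periodically hops toward the player and deals contact damage.
; A looping timer, with its interval randomized at start, triggers Attack, which randomizes acceleration, turns to the player, crouches, then jumps.
; Hits freeze movement and shake the sprite via timeline, leading to delayed destruction at zero HP; dead zones kill immediately.
; Tick derives an animation state from status flags and selects the flipbook.
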(event `self.ReceiveAnyDamage`
  (params (Damage :type "Float (single-precision)") (DamageType :type "DamageType Object Reference") (InstigatedBy :type "Controller Object Reference") (DamageCauser :type "Actor Object Reference"))
  (bind _sprite (`self.Sprite`))
  (bind (_relativelocation_x _relativelocation_y _relativelocation_z) (`KismetMathLibrary.BreakVector` (`SceneComponent.RelativeLocation` _sprite)))
  ;[1 0.1155 0] ReceiveDamage
  (bind _output_get (set `self.HP` (- (`self.HP`) Damage)))
  (if (<= _output_get 0.0)
    (`PrimitiveComponent.SetCollisionEnabled` (`self.CapsuleComponent`) "NoCollision"))
  (set `self.isHit` true)
  (`GameplayStatics.PlaySound2D` "/Game/Sound/SFXs/sfx_BlopHit_Cue.sfx_BlopHit_Cue" 1.0 1.0 0.0 null null)
  (set `CharacterMovementComponent.GravityScale` 0.0 (`self.CharacterMovement`))
  (`MovementComponent.StopMovementImmediately` (`self.CharacterMovement`))
  (bind (_direction _horizontalshake) (`Timeline|Timeline_0` :!via `PlayFromStart`)
    (:`Update`
      (`SceneComponent.K2_SetRelativeLocation` _sprite (`KismetMathLibrary.MakeVector` _horizontalshake _relativelocation_y _relativelocation_z) false false))
    (:`Finished`
      (if (<= (`self.HP`) 0.0)
        (set `self.isDead` true)
        (`/Engine/EditorBlueprintResources/StandardMacros.DoOnce` false
          (:`Completed`
            (`KismetSystemLibrary.Delay` 0.3)
            (`GameplayStatics.PlaySound2D` "/Game/Sound/SFXs/sfx_BlopDeath_Cue.sfx_BlopDeath_Cue" 1.0 1.0 0.0 null null)
            (`KismetSystemLibrary.Delay` 0.7)
            (`self.K2_DestroyActor`)))
        (else
          (set `CharacterMovementComponent.GravityScale` 2.0 (`self.CharacterMovement`))
          (set `self.isHit` false))))))

(event `self.CapsuleComponent.OnComponentBeginOverlap`
  (params (OverlappedComponent :type "PrimitiveComponent Object Reference") (OtherActor :type "Actor Object Reference") (OtherComp :type "PrimitiveComponent Object Reference") (OtherBodyIndex :type Integer) (bFromSweep :type Boolean) (SweepResult :type "HitResult Structure (by ref)"))
  ;[1 0.1155 0] ReceiveDamage
  ;;[1 1 1] Dead Zone
  (cast `/Game/Blueprints/Level/DeadZoneFalling_BP` OtherActor)
  (`GameplayStatics.PlaySound2D` "/Game/Sound/SFXs/sfx_BlopDeath_Cue.sfx_BlopDeath_Cue" 0.3 1.0 0.0 null null)
  (`self.K2_DestroyActor`))

(event `Attack`
  ;[1 0 0] Attack Jump
  (set `CharacterMovementComponent.MaxAcceleration` (`KismetMathLibrary.RandomFloatInRange` 0.0 20000.0) (`self.CharacterMovement`))
  (`self.TurnToPlayer`)
  (if (not (`self.isDead`))
    (set `self.isCrouching` true)
    (`KismetSystemLibrary.Delay` 1.0)
    (if (`self.isCrouching`)
      (set `self.isCrouching` false)
      (if (not (`self.isHit`))
        (set `self.IsJumping` true)
        (if (`self.isFacingLeft`)
          (`self.AddMovementInput` (-1.0 0.0 0.0))
          (else
            (`self.AddMovementInput` (1.0 0.0 0.0))))
        (`self.Jump`)
        (`GameplayStatics.PlaySound2D` "/Game/Sound/SFXs/sfx_BlopJump_Cue.sfx_BlopJump_Cue" 1.0 1.0 0.0 null null)
        (set `self.IsJumping` true)))))

(event `self.CapsuleComponent.OnComponentHit`
  (params (HitComponent :type "PrimitiveComponent Object Reference") (OtherActor :type "Actor Object Reference") (OtherComp :type "PrimitiveComponent Object Reference") (NormalImpulse :type "Vector Structure") (Hit :type "HitResult Structure (by ref)"))
  ;[1 0 0] Attack Jump
  ;;[1 0.9688 0.9688] Apply Damage
  (bind _asplayer_bp (cast `/Game/Blueprints/Player/Player_BP` OtherActor))
  (`GameplayStatics.ApplyDamage` _asplayer_bp (`self.DamageContact`) null self))

(event `ToAttack`
  ;[1 0 0] Attack Jump
  (`KismetSystemLibrary.K2_SetTimerDelegate` (delegate `Attack`) (`KismetMathLibrary.RandomFloatInRange` 2.0 4.0) true))

(event `ControlAnimation`
  ;[0.0133 0.4271 0] Control Animation
  (if (`self.isDead`)
    (set `self.BlopStates` "NewEnumerator4")
    (`/Engine/EditorBlueprintResources/StandardMacros.DoOnce` false
      (:`Completed`
        (`KismetSystemLibrary.Delay` 0.6)
        (`PaperFlipbookComponent.Stop` (`self.Sprite`))))
    (elif (`self.isHit`)
      (set `self.BlopStates` "NewEnumerator0")
      (elif (`self.isCrouching`)
        (set `self.BlopStates` "NewEnumerator2")
        (elif (`self.IsJumping`)
          (set `self.BlopStates` "NewEnumerator3" :!label _label)
          (elif (`NavMovementComponent.IsFalling` (`self.CharacterMovement`))
            (goto _label)
            (else
              (set `self.BlopStates` "NewEnumerator1"))))))))

(event `TurnToPlayer`
  (bind _returnvalue_x (`KismetMathLibrary.BreakVector` (`KismetMathLibrary.GetDirectionUnitVector` (`self.K2_GetActorLocation`) (`self.K2_GetActorLocation` (`self.PlayerRef`)))))
  ;[0 0.218 1] Turn To Player
  (if (`KismetSystemLibrary.IsValid` (`self.PlayerRef`))
    (if (> _returnvalue_x 0.0)
      (if (`self.isFacingLeft`)
        (`self.DirectionChange`))
      (elif (not (`self.isFacingLeft`))
        (`self.DirectionChange`)))))

(event `self.OnLanded`
  (params (Hit :type "HitResult Structure (by ref)"))
  ;[0.0133 0.4271 0] Control Animation
  ;;[1 1 1] OnLanded
  (if (> (`self.HP`) 0.0)
    (set `self.IsJumping` false)
    (set `self.isCrouching` true)
    (`KismetSystemLibrary.Delay` 0.5)
    (set `self.isCrouching` false)))

(event `self.ReceiveBeginPlay`
  ;[0.9624 1 0.9789] DEFAULT
  (`self.DirectionStart`)
  (`self.ToAttack`)
  (`self.CastPlayerRef`))

(event `DirectionStart`
  ;[0.1362 0.1893 1] Facing Control
  (if (`self.isFacingLeft`)
    (`SceneComponent.K2_SetWorldRotation` :`self` (`self.CapsuleComponent`))
    (set `self.isFacingLeft` false)
    (else
      (`SceneComponent.K2_SetWorldRotation` (`self.CapsuleComponent`) (struct :`Yaw` 180.0) false false)
      (set `self.isFacingLeft` true))))

(event `self.ReceiveTick`
  (params (DeltaSeconds :type "Float (single-precision)"))
  ;[0.9624 1 0.9789] DEFAULT
  (`self.ControlAnimation`)
  (`self.UpdateAnimations`))

(event `UpdateAnimations`
  ;[0.07908 0.1965 1] UpdateAnimations
  (switch `/Game/Blueprints/Enemies/Blop/EnemyBlopStates` (`self.BlopStates`)
    (:`NewEnumerator0`
      (`PaperFlipbookComponent.SetFlipbook` (`self.Sprite`) "/Game/Sprites/Enemies/Blop/EnemyBlopHIT.EnemyBlopHIT"))
    (:`NewEnumerator1`
      (`PaperFlipbookComponent.SetFlipbook` (`self.Sprite`) "/Game/Sprites/Enemies/Blop/EnemyBlopIDLE.EnemyBlopIDLE"))
    (:`NewEnumerator2`
      (`PaperFlipbookComponent.SetFlipbook` (`self.Sprite`) "/Game/Sprites/Enemies/Blop/EnemyBlopTOJUMP.EnemyBlopTOJUMP"))
    (:`NewEnumerator3`
      (`PaperFlipbookComponent.SetFlipbook` (`self.Sprite`) "/Game/Sprites/Enemies/Blop/EnemyBlopJUMP.EnemyBlopJUMP"))
    (:`NewEnumerator4`
      (`PaperFlipbookComponent.SetFlipbook` (`self.Sprite`) "/Game/Sprites/Enemies/Blop/EnemyBlopDeath1.EnemyBlopDeath1"))))

(event `CastPlayerRef`
  ;[0.9624 1 0.9789] DEFAULT
  ;;[1 1 1] CastPlayer
  (bind _asplayer_bp (cast `/Game/Blueprints/Player/Player_BP` (`GameplayStatics.GetPlayerCharacter` 0)))
  (set `self.PlayerRef` _asplayer_bp))

(event `DirectionChange`
  ;[0.1362 0.1893 1] Facing Control
  (if (`self.isFacingLeft`)
    (`SceneComponent.K2_SetWorldRotation` (`self.CapsuleComponent`) (struct :`Yaw` 180.0) false false)
    (set `self.isFacingLeft` false)
    (else
      (`SceneComponent.K2_SetWorldRotation` :`self` (`self.CapsuleComponent`))
      (set `self.isFacingLeft` true))))

(fn `UserConstructionScript`)