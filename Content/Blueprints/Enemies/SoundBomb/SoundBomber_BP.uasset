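; SoundBomber_BP is an enemy trigger that rains SoundBomb_BP actors around the player.
; When the player overlaps its Box, it plays an alarm if their SoundCardON is set, then calls Bombard after a short delay.
; Bombard samples the player's position once, then spawns bombs overhead in a line stepping along world -X.
; A delay loop staggers the drops at random intervals, with BombsNumber controlling the count.
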(event `self.ReceiveBeginPlay`
  (bind _asplayer_bp (cast `/Game/Blueprints/Player/Player_BP` (`GameplayStatics.GetPlayerCharacter` 0)))
  (set `self.PlayerRef` _asplayer_bp))

(event `self.Box.OnComponentBeginOverlap`
  (params (OverlappedComponent :type "PrimitiveComponent Object Reference") (OtherActor :type "Actor Object Reference") (OtherComp :type "PrimitiveComponent Object Reference") (OtherBodyIndex :type Integer) (bFromSweep :type Boolean) (SweepResult :type "HitResult Structure (by ref)"))
  (bind _asplayer_bp (cast `/Game/Blueprints/Player/Player_BP` OtherActor))
  (if (`/Game/Blueprints/Player/Player_BP.SoundCardON` _asplayer_bp)
    (`GameplayStatics.PlaySound2D` "/Game/Sound/SFXs/sfx_LowHPAlarm_Cue.sfx_LowHPAlarm_Cue" 1.0 1.0 0.0 null null))
  (`KismetSystemLibrary.Delay` 1.0)
  (`self.Bombard`))

(event `Bombard`
  (bind (_spawnlocation_x _spawnlocation_y _spawnlocation_z) (`KismetMathLibrary.BreakVector` (`self.SpawnLocation`)))
  (bind (_returnvalue_x _returnvalue_y _returnvalue_z) (`KismetMathLibrary.BreakVector` (`self.K2_GetActorLocation` (`self.PlayerRef`))))
  (set `self.BombsIndex` 0)
  (bind _output_get (set `self.SpawnLocation` (`KismetMathLibrary.MakeVector` (+ _returnvalue_x 80.0) (- _returnvalue_y 1.0) (+ _returnvalue_z 100.0))))
  (`|SpawnActorFromClass` "/Game/Blueprints/Enemies/SoundBomb/SoundBomb_BP.SoundBomb_BP_C" (`KismetMathLibrary.MakeTransform` _output_get) "Undefined" "OverrideRootScale" null null :!label _label)
  (`KismetSystemLibrary.Delay` (`KismetMathLibrary.RandomFloatInRange` 0.1 0.3))
  (set `self.SpawnLocation` (`KismetMathLibrary.MakeVector` (- _spawnlocation_x 16.0) _spawnlocation_y _spawnlocation_z))
  (if (< (`self.BombsIndex`) (`self.BombsNumber`))
    (set `self.BombsIndex` (+ (`self.BombsIndex`) 1))
    (goto _label)))

(fn `UserConstructionScript`)