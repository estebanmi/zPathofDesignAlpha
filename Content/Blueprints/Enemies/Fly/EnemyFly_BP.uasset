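; Flying enemy that tracks the player's height, then locks its facing and charges horizontally once level, dealing contact damage.
; Timers update direction until detection, while Tick drives movement, overlap damage and flipbook states.
; Hits pause it with a timeline shake; death spawns bitcoin loot before destruction.
; Sprite tint follows the color scheme when VideoCardON, and a gate destroys it after a delay off-screen.
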(event `self.ReceiveAnyDamage`
  (params (Damage :type "Float (single-precision)") (DamageType :type "DamageType Object Reference") (InstigatedBy :type "Controller Object Reference") (DamageCauser :type "Actor Object Reference"))
  (bind _sprite (`self.Sprite`))
  (bind (_relativelocation_x _relativelocation_y _relativelocation_z) (`KismetMathLibrary.BreakVector` (`SceneComponent.RelativeLocation` _sprite)))
  ;[1 0.1155 0] ReceiveDamage
  (bind _output_get (set `self.HP` (- (`self.HP`) Damage)))
  (if (<= _output_get 0.0)
    (`PrimitiveComponent.SetCollisionEnabled` (`self.CapsuleComponent`) "NoCollision"))
  (set `self.isHit` true)
  (`GameplayStatics.PlaySound2D` "/Game/Sound/SFXs/sfx_BlopHit_Cue.sfx_BlopHit_Cue" 1.0 1.0 0.0 null null)
  (`MovementComponent.StopMovementImmediately` (`self.CharacterMovement`))
  (bind (_direction _horizontalshake) (`Timeline|Timeline_0` :!via `PlayFromStart`)
    (:`Update`
      (`SceneComponent.K2_SetRelativeLocation` _sprite (`KismetMathLibrary.MakeVector` _horizontalshake _relativelocation_y _relativelocation_z) false false))
    (:`Finished`
      (if (<= (`self.HP`) 0.0)
        (set `self.isDead` true)
        (`/Engine/EditorBlueprintResources/StandardMacros.DoOnce` false
          (:`Completed`
            (`KismetSystemLibrary.Delay` 0.2)
            (`GameplayStatics.PlaySound2D` "/Game/Sound/SFXs/sfx_BlopDeath_Cue.sfx_BlopDeath_Cue" 1.0 1.0 0.0 null null)
            (`self.DropLoot`)
            (`KismetSystemLibrary.Delay` 0.2)
            (`self.K2_DestroyActor`)))
        (else
          (set `self.isHit` false))))))

(event `OverlappingDamage`
  (bind _output (`|GetArrayItem` (`PrimitiveComponent.GetOverlappingActors` (`self.CapsuleComponent`) "/Game/Blueprints/Player/Player_BP.Player_BP_C")))
  ;[1 0.1155 0] ReceiveDamage
  ;;[1 0 0] Overlapping Damage
  (`/Engine/EditorBlueprintResources/StandardMacros.IsValid` _output
    (:`Is Valid`
      (`GameplayStatics.ApplyDamage` _output (`self.DamageContact`) null self))))

(event `PlayerDetection`
  (bind (_returnvalue_x _returnvalue_y _returnvalue_z) (`KismetMathLibrary.BreakVector` (`self.K2_GetActorLocation`)))
  (bind (_returnvalue_x_2 _returnvalue_y_2 _returnvalue_z_2) (`KismetMathLibrary.BreakVector` (`self.K2_GetActorLocation` (`self.PlayerRef`))))
  ;[1 1 1] Attack (Player Detection)
  (if (`self.PlayerDetected`)
    _
    (elif (> (+ _returnvalue_z_2 1.0) _returnvalue_z)
      (if (< (- _returnvalue_z_2 1.0) _returnvalue_z)
        (set `self.PlayerDetected` true)))))

(event `DropLoot`
  (bind (_returnvalue_x _returnvalue_y _returnvalue_z) (`KismetMathLibrary.BreakVector` (`self.K2_GetActorLocation`)))
  ;[1 1 1] Drop Loot
  (`|SpawnActorFromClass` "/Game/Blueprints/Collectibles/Loot/BitCoinLoot_BP.BitCoinLoot_BP_C" (`KismetMathLibrary.MakeTransform` (`KismetMathLibrary.MakeVector` _returnvalue_x 1.0 _returnvalue_z)) "Undefined" "OverrideRootScale" null null))

(event `ColorControl`
  (bind _returnvalue (`KismetMathLibrary.RandomFloatInRange` 0.6 1.0))
  ;[0 0.9169 1] Color Control
  (if (`/Game/Blueprints/Player/Player_BP.VideoCardON` (`self.PlayerRef`))
    (bind _outactors (`GameplayStatics.GetAllActorsOfClass` "/Game/Blueprints/Art/ColorController.ColorController_C"))
    (bind _returnvalue_2 (`|GetDataTableRow` "/Game/Blueprints/Art/ColorSchemeTable.ColorSchemeTable" (`/Game/Blueprints/Art/ColorController.ColorScheme` (`|GetArrayItem` _outactors)))
      (:`then`
        (`PaperFlipbookComponent.SetSpriteColor` (`self.Sprite`) (* (`.Enemies_33_D3933F8042CE8CB253100FB32ECD27F6` (break `/Game/Blueprints/Art/ColorScheme` _returnvalue_2)) (make `LinearColor` _returnvalue _returnvalue _returnvalue 1.0)))))
    (else
      (`PaperFlipbookComponent.SetSpriteColor` :`self` (`self.Sprite`)))))

(event `ControlAnimation`
  ;[0.0133 0.4271 0] Control Animation
  (if (`self.isDead`)
    (set `self.FlyStates` "NewEnumerator4")
    (`/Engine/EditorBlueprintResources/StandardMacros.DoOnce` false
      (:`Completed`
        (`KismetSystemLibrary.Delay` 1.0)
        (`PaperFlipbookComponent.Stop` (`self.Sprite`))))
    (elif (`self.isHit`)
      (set `self.FlyStates` "NewEnumerator0")
      (else
        (set `self.FlyStates` "NewEnumerator1")))))

(event `VerticalDirection`
  (bind (_returnvalue_x _returnvalue_y _returnvalue_z) (`KismetMathLibrary.BreakVector` (`self.K2_GetActorLocation`)))
  (bind (_returnvalue_x_2 _returnvalue_y_2 _returnvalue_z_2) (`KismetMathLibrary.BreakVector` (`self.K2_GetActorLocation` (`self.PlayerRef`))))
  ;[1 1 1] Vertical Direction Control
  (if (`self.PlayerDetected`)
    _
    (elif (< _returnvalue_z_2 _returnvalue_z)
      (set `self.IsOverPlayer` true)
      (else
        (set `self.IsOverPlayer` false)))))

(event `DirectionControl`
  (bind _returnvalue_x (`KismetMathLibrary.BreakVector` (`self.K2_GetActorLocation`)))
  (bind _returnvalue_x_2 (`KismetMathLibrary.BreakVector` (`self.K2_GetActorLocation` (`self.PlayerRef`))))
  ;[0.1362 0.1893 1] Facing Control
  (if (`self.PlayerDetected`)
    _
    (elif (< _returnvalue_x_2 _returnvalue_x)
      (`SceneComponent.K2_SetWorldRotation` :`self` (`self.CapsuleComponent`))
      (set `self.isFacingLeft` true)
      (else
        (`SceneComponent.K2_SetWorldRotation` (`self.CapsuleComponent`) (struct :`Yaw` 180.0) false false)
        (set `self.isFacingLeft` false)))))

(event `self.ReceiveBeginPlay`
  ;[0.9624 1 0.9789] DEFAULT
  (bind _asplayer_bp (cast `/Game/Blueprints/Player/Player_BP` (`GameplayStatics.GetPlayerCharacter` 0)))
  (set `self.PlayerRef` _asplayer_bp)
  (`self.ColorControl`)
  (`self.DirectionControl`)
  (`KismetSystemLibrary.K2_SetTimerDelegate` (delegate `VerticalDirection`) 0.1 true)
  (`KismetSystemLibrary.K2_SetTimerDelegate` (delegate `DirectionControl`) 0.5 true))

(event `self.ReceiveTick`
  (params (DeltaSeconds :type "Float (single-precision)"))
  ;[0.9624 1 0.9789] DEFAULT
  (`self.OverlappingDamage`)
  (`self.PlayerDetection`)
  (`self.ControlAnimation`)
  (`self.UpdateAnimations`)
  (if (`self.isDead`)
    _
    (elif (`self.PlayerDetected`)
      (`self.HorizontalFly`)
      (else
        (`self.VerticalFly`)))))

(event `UpdateAnimations`
  ;[0.07908 0.1965 1] UpdateAnimations
  (switch `/Game/Blueprints/Enemies/Fly/EnemyFlyStates` (`self.FlyStates`)
    (:`NewEnumerator0`
      (`PaperFlipbookComponent.SetFlipbook` (`self.Sprite`) "/Game/Sprites/Enemies/Fly/EnemyFlyHit.EnemyFlyHit"))
    (:`NewEnumerator1`
      (`PaperFlipbookComponent.SetFlipbook` (`self.Sprite`) "/Game/Sprites/Enemies/Fly/EnemyFlyFlying.EnemyFlyFlying"))
    (:`NewEnumerator4`
      (`PaperFlipbookComponent.SetFlipbook` (`self.Sprite`) "/Game/Sprites/FXs/explsoion3Skull1.explsoion3Skull1"))))

(event `self.CapsuleComponent.OnComponentBeginOverlap`
  (params (OverlappedComponent :type "PrimitiveComponent Object Reference") (OtherActor :type "Actor Object Reference") (OtherComp :type "PrimitiveComponent Object Reference") (OtherBodyIndex :type Integer) (bFromSweep :type Boolean) (SweepResult :type "HitResult Structure (by ref)"))
  ;[0 0 0] OnScreen or Not
  (cast `/Game/Blueprints/Level/ScreenCollider_BP` OtherActor)
  (goto _label :!via `Close`))

(event `CloseGate`
  ;[0 0 0] OnScreen or Not
  (goto _label :!via `Open`))

(event `HorizontalFly`
  ;[1 1 1] Vertical & Horizontal Flight
  (if (`self.isHit`)
    _
    (elif (`self.isFacingLeft`)
      (`self.AddMovementInput` (250.0 0.0 0.0) -1.0)
      (else
        (`self.AddMovementInput` (250.0 0.0 0.0))))))

(event `VerticalFly`
  ;[1 1 1] Vertical & Horizontal Flight
  (if (`self.isHit`)
    _
    (elif (`self.IsOverPlayer`)
      (`self.K2_AddActorWorldOffset` (0.0 0.0 -0.5))
      (else
        (`self.K2_AddActorWorldOffset` (0.0 0.0 0.5))))))

(event `self.CapsuleComponent.OnComponentEndOverlap`
  (params (OverlappedComponent :type "PrimitiveComponent Object Reference") (OtherActor :type "Actor Object Reference") (OtherComp :type "PrimitiveComponent Object Reference") (OtherBodyIndex :type Integer))
  ;[0 0 0] OnScreen or Not
  (cast `/Game/Blueprints/Level/ScreenCollider_BP` OtherActor)
  (`self.CloseGate`)
  (`KismetSystemLibrary.Delay` 1.0)
  (`/Engine/EditorBlueprintResources/StandardMacros.Gate` true :!label _label
    (:`Exit`
      (`self.K2_DestroyActor`))))

(fn `UserConstructionScript`)