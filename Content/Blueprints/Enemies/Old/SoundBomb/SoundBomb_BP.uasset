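; SoundBomb_BP is an enemy bomb projectile that drops straight down, damages the player and explodes.
; BeginPlay caches the player and drives the physics Box downward at BulletSpeed.
; Player contact applies Damage, detected by both begin-overlap and a per-Tick overlap poll that catches existing overlaps.
; Both player contact and any Box hit spawn BigExplosion_BP and destroy the bomb; the hit path applies no damage itself.
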(event `OverlappingDamage`
  (bind _output (`|GetArrayItem` (`PrimitiveComponent.GetOverlappingActors` (`self.Box`) "/Game/Blueprints/Player/Player_BP.Player_BP_C")))
  ;[1 1 1] Overlapping Damage
  (`/Engine/EditorBlueprintResources/StandardMacros.IsValid` _output
    (:`Is Valid`
      (`GameplayStatics.ApplyDamage` _output (`self.Damage`) null self)
      (`|SpawnActorFromClass` "/Game/Blueprints/FX/BigExplosion_BP.BigExplosion_BP_C" (`KismetMathLibrary.MakeTransform` (`self.K2_GetActorLocation`)) "Undefined" "OverrideRootScale" null null)
      (`self.K2_DestroyActor`))))

(event `self.ReceiveTick`
  (params (DeltaSeconds :type "Float (single-precision)"))
  (`self.OverlappingDamage`))

(event `self.ReceiveBeginPlay`
  (bind _asplayer_bp (cast `/Game/Blueprints/Player/Player_BP` (`GameplayStatics.GetPlayerCharacter` 0)))
  (set `self.PlayerRef` _asplayer_bp)
  (`PrimitiveComponent.SetPhysicsLinearVelocity` (`self.Box`) (`KismetMathLibrary.MakeVector` 0.0 0.0 (* (`self.BulletSpeed`) -1.0)) false "None"))

(event `self.Box.OnComponentHit`
  (params (HitComponent :type "PrimitiveComponent Object Reference") (OtherActor :type "Actor Object Reference") (OtherComp :type "PrimitiveComponent Object Reference") (NormalImpulse :type "Vector Structure") (Hit :type "HitResult Structure (by ref)"))
  (`|SpawnActorFromClass` "/Game/Blueprints/FX/BigExplosion_BP.BigExplosion_BP_C" (`KismetMathLibrary.MakeTransform` (`self.K2_GetActorLocation`)) "Undefined" "OverrideRootScale" null null)
  (`self.K2_DestroyActor`))

(event `self.Box.OnComponentBeginOverlap`
  (params (OverlappedComponent :type "PrimitiveComponent Object Reference") (OtherActor :type "Actor Object Reference") (OtherComp :type "PrimitiveComponent Object Reference") (OtherBodyIndex :type Integer) (bFromSweep :type Boolean) (SweepResult :type "HitResult Structure (by ref)"))
  (bind _asplayer_bp (cast `/Game/Blueprints/Player/Player_BP` OtherActor))
  (`GameplayStatics.ApplyDamage` _asplayer_bp (`self.Damage`) null self)
  (`|SpawnActorFromClass` "/Game/Blueprints/FX/BigExplosion_BP.BigExplosion_BP_C" (`KismetMathLibrary.MakeTransform` (`self.K2_GetActorLocation`)) "Undefined" "OverrideRootScale" null null)
  (`self.K2_DestroyActor`))

(fn `UserConstructionScript`)