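; Enemy spawner that releases a mass of EnemyRunnerMass_BP runners when its BoxCollider overlaps a ScreenCollider_BP.
; An index-driven loop with a short random Delay staggers the 21 spawns over time.
; Each runner appears at the spawner's X and Z with slight random X jitter, adjusting for collisions but always spawning.
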(event `self.ReceiveBeginPlay`)

(event `self.BoxCollider.OnComponentBeginOverlap`
  (params (OverlappedComponent :type "PrimitiveComponent Object Reference") (OtherActor :type "Actor Object Reference") (OtherComp :type "PrimitiveComponent Object Reference") (OtherBodyIndex :type Integer) (bFromSweep :type Boolean) (SweepResult :type "HitResult Structure (by ref)"))
  (bind (_returnvalue_x _returnvalue_y _returnvalue_z) (`KismetMathLibrary.BreakVector` (`self.K2_GetActorLocation`)))
  (cast `/Game/Blueprints/Level/ScreenCollider_BP` OtherActor)
  (set `self.Index` 0)
  (`|SpawnActorFromClass` "/Game/Blueprints/Enemies/Runner/EnemyRunnerMass_BP.EnemyRunnerMass_BP_C" (`KismetMathLibrary.MakeTransform` (`KismetMathLibrary.MakeVector` (+ _returnvalue_x (`KismetMathLibrary.RandomFloatInRange` -2.0 2.0)) 0.0 _returnvalue_z)) "AdjustIfPossibleButAlwaysSpawn" "OverrideRootScale" null null :!label _label)
  (`KismetSystemLibrary.Delay` (`KismetMathLibrary.RandomFloatInRange` 0.0 0.1))
  (if (< (`self.Index`) 20)
    (set `self.Index` (+ (`self.Index`) 1))
    (goto _label)))

(fn `UserConstructionScript`)