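; Paper2D enemy turret that opens while the player is in its activation box, fires a burst of bullets, then closes and repeats.
; Tick derives a state from boolean flags and sets the matching flipbook; DoOnce-gated delays timed to flipbook length advance opening, shooting and closing.
; It takes damage only when open, shakes via a timeline, and on death drops a coin before being destroyed.
; It also destroys itself on leaving the screen collider.
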(event `self.ReceiveAnyDamage`
  (params (Damage :type "Float (single-precision)") (DamageType :type "DamageType Object Reference") (InstigatedBy :type "Controller Object Reference") (DamageCauser :type "Actor Object Reference"))
  (bind _paperflipbook (`self.PaperFlipbook`))
  (bind (_relativelocation_x _relativelocation_y _relativelocation_z) (`KismetMathLibrary.BreakVector` (`SceneComponent.RelativeLocation` _paperflipbook)))
  ;[1 0.1155 0] ReceiveDamage
  (if (`self.IsOpened`)
    (bind _output_get (set `self.HP` (- (`self.HP`) Damage)))
    (if (<= _output_get 0.0)
      (`PrimitiveComponent.SetCollisionEnabled` (`self.BoxCollider`) "NoCollision"))
    (set `self.isHit` true)
    (`GameplayStatics.PlaySound2D` "/Game/Sound/SFXs/sfx_BlopHit_Cue.sfx_BlopHit_Cue" 1.0 1.0 0.0 null null)
    (bind (_direction _horizontalshake) (`Timeline|Timeline_0` :!via `PlayFromStart`)
      (:`Update`
        (`SceneComponent.K2_SetRelativeLocation` _paperflipbook (`KismetMathLibrary.MakeVector` _horizontalshake _relativelocation_y _relativelocation_z) false false))
      (:`Finished`
        (if (<= (`self.HP`) 0.0)
          (set `self.isDead` true)
          (`/Engine/EditorBlueprintResources/StandardMacros.DoOnce` false
            (:`Completed`
              (`KismetSystemLibrary.Delay` 0.3)
              (`GameplayStatics.PlaySound2D` "/Game/Sound/SFXs/sfx_BlopDeath_Cue.sfx_BlopDeath_Cue" 1.0 1.0 0.0 null null)
              (`KismetSystemLibrary.Delay` 0.15)
              (`self.DropLoot`)
              (`self.K2_DestroyActor`)))
          (else
            (set `self.isHit` false)))))))

(event `TurretActive`
  ;[1 0 0] Open / Fire
  (if (not (`self.IsOpened`))
    (`KismetSystemLibrary.Delay` (`KismetMathLibrary.RandomFloatInRange` 2.0 3.0))
    (if (`self.IsActive`)
      (set `self.isOpening` true))))

(event `DropLoot`
  (bind (_returnvalue_x _returnvalue_y _returnvalue_z) (`KismetMathLibrary.BreakVector` (`self.K2_GetActorLocation`)))
  ;[1 1 1] Drop Loot
  (`|SpawnActorFromClass` "/Game/Blueprints/Collectibles/BinaryCoinLoot.BinaryCoinLoot_C" (`KismetMathLibrary.MakeTransform` (`KismetMathLibrary.MakeVector` _returnvalue_x 1.0 _returnvalue_z)) "Undefined" "OverrideRootScale" null null))

(event `Shoot`
  (bind (_returnvalue_x _returnvalue_y _returnvalue_z) (`KismetMathLibrary.BreakVector` (`self.K2_GetActorLocation`)))
  ;[1 0 0] Open / Fire
  (set `self.IndexShots` 1)
  (`|SpawnActorFromClass` "/Game/Blueprints/Enemies/Turret/TurretBullet_BP.TurretBullet_BP_C" (`KismetMathLibrary.MakeTransform` (`KismetMathLibrary.MakeVector` _returnvalue_x 1.0 _returnvalue_z)) "Undefined" "OverrideRootScale" null null :!label _label)
  (if (< (`self.IndexShots`) (`self.NumberOfShots`))
    (set `self.IndexShots` (+ (`self.IndexShots`) 1))
    (`KismetSystemLibrary.Delay` 0.3)
    (goto _label)
    (else
      (`KismetSystemLibrary.Delay` 0.5)
      (set `self.IsOpened` false)
      (set `self.isClosing` true)
      (`self.ResetShoot`))))

(event `ControlAnimation`
  ;[0.0133 0.4271 0] Control Animation
  (if (`self.isDead`)
    (set `self.TurretStates` "NewEnumerator6")
    (`/Engine/EditorBlueprintResources/StandardMacros.DoOnce` false
      (:`Completed`
        (`KismetSystemLibrary.Delay` 0.6)
        (`PaperFlipbookComponent.Stop` (`self.PaperFlipbook`))))
    (elif (`self.isHit`)
      (set `self.TurretStates` "NewEnumerator5")
      (elif (`self.isOpening`)
        (set `self.TurretStates` "NewEnumerator1")
        (elif (`self.isClosing`)
          (set `self.TurretStates` "NewEnumerator3")
          (elif (`self.IsOpened`)
            (set `self.TurretStates` "NewEnumerator4")
            (else
              (set `self.TurretStates` "NewEnumerator0"))))))))

(event `UpdateAnimations`
  (bind _paperflipbook (`self.PaperFlipbook`))
  (bind _paperflipbook_2 (`self.PaperFlipbook`))
  ;[0.07908 0.1965 1] UpdateAnimations
  (switch `/Game/Blueprints/Enemies/Turret/EnemyTurretStates` (`self.TurretStates`)
    (:`NewEnumerator0`
      (`PaperFlipbookComponent.SetFlipbook` (`self.PaperFlipbook`) "/Game/Sprites/Enemies/Turret/TurretClosed1.TurretClosed1"))
    (:`NewEnumerator1`
      (`PaperFlipbookComponent.SetFlipbook` _paperflipbook_2 "/Game/Sprites/Enemies/Turret/TurretOpening1.TurretOpening1")
      (`/Engine/EditorBlueprintResources/StandardMacros.DoOnce` false :!label _label_2
        (:`Completed`
          (`KismetSystemLibrary.Delay` (`PaperFlipbookComponent.GetFlipbookLength` _paperflipbook_2))
          (set `self.isOpening` false)
          (set `self.IsOpened` true)
          (goto _label_2 :!via `Reset`))))
    (:`NewEnumerator3`
      (`PaperFlipbookComponent.SetFlipbook` _paperflipbook "/Game/Sprites/Enemies/Turret/TurretClosing1.TurretClosing1")
      (`/Engine/EditorBlueprintResources/StandardMacros.DoOnce` false :!label _label_3
        (:`Completed`
          (`KismetSystemLibrary.Delay` (`PaperFlipbookComponent.GetFlipbookLength` _paperflipbook))
          (set `self.isClosing` false)
          (set `self.IsOpened` false)
          (`self.TurretActive`)
          (goto _label_3 :!via `Reset`))))
    (:`NewEnumerator4`
      (`PaperFlipbookComponent.SetFlipbook` (`self.PaperFlipbook`) "/Game/Sprites/Enemies/Turret/TurretOpened1.TurretOpened1")
      (`/Engine/EditorBlueprintResources/StandardMacros.DoOnce` false :!label _label_4
        (:`Completed`
          (`KismetSystemLibrary.Delay` 0.2)
          (`self.Shoot`))))
    (:`NewEnumerator5`
      (`PaperFlipbookComponent.SetFlipbook` (`self.PaperFlipbook`) "/Game/Sprites/Enemies/Turret/TurretHit1.TurretHit1"))
    (:`NewEnumerator6`
      (`PaperFlipbookComponent.SetFlipbook` (`self.PaperFlipbook`) "/Game/Sprites/Collectibles/CodeBlock/FlashExplosion/CodeBlockExplosion3.CodeBlockExplosion3"))))

(event `ResetShoot`
  ;[0.07908 0.1965 1] UpdateAnimations
  (goto _label_4 :!via `Reset`))

(event `self.BoxColldierActive.OnComponentBeginOverlap`
  (params (OverlappedComponent :type "PrimitiveComponent Object Reference") (OtherActor :type "Actor Object Reference") (OtherComp :type "PrimitiveComponent Object Reference") (OtherBodyIndex :type Integer) (bFromSweep :type Boolean) (SweepResult :type "HitResult Structure (by ref)"))
  ;[1 1 1] Overlap Active
  (cast `/Game/Blueprints/Player/Player_BP` OtherActor)
  (set `self.IsActive` true)
  (`self.TurretActive`))

(event `self.ReceiveBeginPlay`
  ;[0.9624 1 0.9789] DEFAULT
  (bind _asplayer_bp (cast `/Game/Blueprints/Player/Player_BP` (`GameplayStatics.GetPlayerCharacter` 0)))
  (set `self.PlayerRef` _asplayer_bp))

(event `self.ReceiveTick`
  (params (DeltaSeconds :type "Float (single-precision)"))
  ;[0.9624 1 0.9789] DEFAULT
  (`self.ControlAnimation`)
  (`self.UpdateAnimations`))

(event `self.BoxColldierActive.OnComponentEndOverlap`
  (params (OverlappedComponent :type "PrimitiveComponent Object Reference") (OtherActor :type "Actor Object Reference") (OtherComp :type "PrimitiveComponent Object Reference") (OtherBodyIndex :type Integer))
  ;[1 1 1] Overlap Active
  (cast `/Game/Blueprints/Player/Player_BP` OtherActor)
  (set `self.IsActive` false))

(event `self.BoxCollider.OnComponentEndOverlap`
  (params (OverlappedComponent :type "PrimitiveComponent Object Reference") (OtherActor :type "Actor Object Reference") (OtherComp :type "PrimitiveComponent Object Reference") (OtherBodyIndex :type Integer))
  ;[1 1 1] Out Of Screen
  (cast `/Game/Blueprints/Level/ScreenCollider_BP` OtherActor)
  (`self.K2_DestroyActor`))

(fn `UserConstructionScript`)