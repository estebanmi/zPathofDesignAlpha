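; Paper2D ghost enemy that stays hidden until the player turns invisible, then flickers via a FlipFlop on a fast timer.
; A looping timer with a randomized period triggers walking; Tick picks idle or walk flipbooks, nudging it forward after each walk animation.
; Probability-based turn-to-player logic exists but is never called here.
; Player contact only prints a message, and dead-zone destruction is marked as not working.
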(event `self.CapsuleComponent.OnComponentBeginOverlap`
  (params (OverlappedComponent :type "PrimitiveComponent Object Reference") (OtherActor :type "Actor Object Reference") (OtherComp :type "PrimitiveComponent Object Reference") (OtherBodyIndex :type Integer) (bFromSweep :type Boolean) (SweepResult :type "HitResult Structure (by ref)"))
  ;[1 0.9688 0.9688] Apply Damage
  (cast `/Game/Blueprints/Player/Player_BP` OtherActor)
  (`KismetSystemLibrary.PrintString` "CONTACT" true true (struct :`R` 0.212642 :`B` 1.0 :`A` 1.0)))

(event `DeadZone`
  (params (OtherActor :type "Actor Object Reference"))
  ;[1 1 1] DeadZone (Does not works)
  (cast `/Game/Blueprints/Level/DeadZoneFalling_BP` OtherActor)
  (`self.K2_DestroyActor`)
  (`KismetSystemLibrary.PrintString` (`KismetStringLibrary.Concat_StrStr` (`KismetSystemLibrary.GetObjectName` self) " Destroyed") true true (struct :`R` 1.0 :`A` 1.0) 3.0))

(event `TurnToPlayer`
  (bind _returnvalue_x (`KismetMathLibrary.BreakVector` (`KismetMathLibrary.GetDirectionUnitVector` (`self.K2_GetActorLocation`) (`self.K2_GetActorLocation` (`self.PlayerRef`)))))
  ;[0 0.218 1] Turn To Player
  (if (`KismetSystemLibrary.IsValid` (`self.PlayerRef`))
    (if (`/Game/Blueprints/Player/Player_BP.isInvisible` (`self.PlayerRef`))
      _
      (elif (> _returnvalue_x 0.0)
        (if (`self.isFacingLeft`)
          (`self.DirectionChange`))
        (elif (not (`self.isFacingLeft`))
          (`self.DirectionChange`))))))

(event `ControlAnimation`
  ;[0.0133 0.4271 0] Control Animation
  (if (`self.isWalking`)
    (set `self.GhostStates` "NewEnumerator3")
    (else
      (set `self.GhostStates` "NewEnumerator1"))))

(event `DirectionStart`
  ;[0.1362 0.1893 1] Facing Control
  (if (`self.isFacingLeft`)
    (`SceneComponent.K2_SetWorldRotation` :`self` (`self.CapsuleComponent`))
    (else
      (`SceneComponent.K2_SetWorldRotation` (`self.CapsuleComponent`) (struct :`Yaw` 180.0) false false))))

(event `UpdateAnimations`
  (bind (_returnvalue_x _returnvalue_y _returnvalue_z) (`KismetMathLibrary.BreakVector` (`self.K2_GetActorLocation`)))
  (bind _sprite (`self.Sprite`))
  ;[0.07908 0.1965 1] UpdateAnimations
  (switch `/Game/Blueprints/Enemies/Ghost/EnemyGhostStates` (`self.GhostStates`)
    (:`NewEnumerator1`
      (`PaperFlipbookComponent.SetFlipbook` (`self.Sprite`) "/Game/Sprites/Enemies/Ghost/EnemyGhostIdle1.EnemyGhostIdle1"))
    (:`NewEnumerator3`
      (`PaperFlipbookComponent.SetFlipbook` _sprite "/Game/Sprites/Enemies/Ghost/EnemyGhostWalk1.EnemyGhostWalk1")
      (`KismetSystemLibrary.Delay` (`PaperFlipbookComponent.GetFlipbookLength` _sprite))
      (if (`self.isFacingLeft`)
        (`self.K2_SetActorLocation` (`KismetMathLibrary.MakeVector` (- _returnvalue_x 3.0) _returnvalue_y _returnvalue_z))
        (else
          (`self.K2_SetActorLocation` (`KismetMathLibrary.MakeVector` (+ _returnvalue_x 3.0) _returnvalue_y _returnvalue_z))))
      (set `self.isWalking` false))))

(event `self.ReceiveBeginPlay`
  ;[1 0.3304 0] DEFAULT
  (`self.CastPlayerRef`)
  (`self.DirectionStart`)
  (`KismetSystemLibrary.K2_SetTimerDelegate` (delegate `Walk`) (`KismetMathLibrary.RandomFloatInRange` 1.0 3.0) true)
  (`KismetSystemLibrary.K2_SetTimerDelegate` (delegate `UpdateVisibility`) 0.04 true))

(event `self.ReceiveTick`
  (params (DeltaSeconds :type "Float (single-precision)"))
  ;[1 0.3304 0] DEFAULT
  (`self.ControlAnimation`)
  (`self.UpdateAnimations`))

(event `DirectionChange`
  ;[0.1362 0.1893 1] Facing Control
  (if (`self.isFacingLeft`)
    (`SceneComponent.K2_SetWorldRotation` (`self.CapsuleComponent`) (struct :`Yaw` 180.0) false false)
    (set `self.isFacingLeft` false)
    (else
      (`SceneComponent.K2_SetWorldRotation` :`self` (`self.CapsuleComponent`))
      (set `self.isFacingLeft` true))))

(event `CastPlayerRef`
  ;[1 0.3304 0] DEFAULT
  ;;[1 1 1] CastPlayer
  (bind _asplayer_bp (cast `/Game/Blueprints/Player/Player_BP` (`GameplayStatics.GetPlayerCharacter` 0)))
  (set `self.PlayerRef` _asplayer_bp))

(event `Walk`
  ;[1 0.3304 0] DEFAULT
  ;;[1 0.7887 0] Walk
  (set `self.isWalking` true))

(event `CheckPlayerLocation`
  ;[1 1 1] TurnToPlayer Prob
  (if (`self.isDead`)
    _
    (elif (`self.IsJumping`)
      _
      (elif (< (`KismetMathLibrary.RandomFloatInRange` 0.0 100.0) (`self.TurnToPlayerProb`))
        (`self.TurnToPlayer`)))))

(event `UpdateVisibility`
  (bind _sprite (`self.Sprite`))
  ;[1 1 1] UpdateVisibility
  (if (`/Game/Blueprints/Player/Player_BP.isInvisible` (`self.PlayerRef`))
    (`/Engine/EditorBlueprintResources/StandardMacros.FlipFlop`
      (:`A`
        (`SceneComponent.SetVisibility` _sprite true false))
      (:`B`
        (`SceneComponent.SetVisibility` _sprite false false)))
    (else
      (`SceneComponent.SetVisibility` (`self.Sprite`) false false))))

(fn `UserConstructionScript`)