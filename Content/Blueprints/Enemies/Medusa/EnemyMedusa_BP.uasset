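; Medusa flying enemy for a 2D side-scroller that damages the player on contact and drops a BitCoin when killed.
; A timeline drives vertical flight while Tick applies horizontal movement, repeats overlap damage and picks flipbooks from hit and death flags.
; Damage triggers a shake, or a death sequence that stops movement, notifies the player and destroys the actor.
; It faces the player on spawn, and a looping timer destroys it when far from the screen collider.
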(event `self.ReceiveAnyDamage`
  (params (Damage :type "Float (single-precision)") (DamageType :type "DamageType Object Reference") (InstigatedBy :type "Controller Object Reference") (DamageCauser :type "Actor Object Reference"))
  (bind _sprite (`self.Sprite`))
  (bind (_relativelocation_x _relativelocation_y _relativelocation_z) (`KismetMathLibrary.BreakVector` (`SceneComponent.RelativeLocation` _sprite)))
  ;[1 0.1155 0] ReceiveDamage
  (bind _output_get (set `self.HP` (- (`self.HP`) Damage)))
  (if (<= _output_get 0.0)
    (`PrimitiveComponent.SetCollisionEnabled` (`self.CapsuleComponent`) "NoCollision")
    (set `self.isDead` true)
    (`/Engine/EditorBlueprintResources/StandardMacros.DoOnce` false
      (:`Completed`
        (`self.StopZ`)
        (set `CharacterMovementComponent.MaxWalkSpeed` 0.0 (`self.CharacterMovement`))
        (`MovementComponent.StopMovementImmediately` (`self.CharacterMovement`))
        (`KismetSystemLibrary.Delay` (`PaperFlipbookComponent.GetFlipbookLength` (`self.Sprite`)))
        (`GameplayStatics.PlaySound2D` "/Game/Sound/SFXs/sfx_BlopDeath_Cue.sfx_BlopDeath_Cue" 1.0 1.0 0.0 null null)
        (`self.DropLoot`)
        (`/Game/Blueprints/Player/Player_BP.EmenyKilled` (`self.PlayerRef`))
        (`self.K2_DestroyActor`)))
    (else
      (set `self.isHit` true)
      (`GameplayStatics.PlaySound2D` "/Game/Sound/SFXs/sfx_BlopHit_Cue.sfx_BlopHit_Cue" 1.0 1.0 0.0 null null)
      (`MovementComponent.StopMovementImmediately` (`self.CharacterMovement`))
      (bind (_direction _horizontalshake) (`Timeline|HitShaking` :!via `PlayFromStart`)
        (:`Update`
          (`SceneComponent.K2_SetRelativeLocation` _sprite (`KismetMathLibrary.MakeVector` _horizontalshake _relativelocation_y _relativelocation_z) false false))
        (:`Finished`
          (set `self.isHit` false))))))

(event `OverlappingDamage`
  (bind _output (`|GetArrayItem` (`PrimitiveComponent.GetOverlappingActors` (`self.CapsuleComponent`) "/Game/Blueprints/Player/Player_BP.Player_BP_C")))
  ;[1 0.1155 0] ReceiveDamage
  ;;[1 1 1] Overlapping Damage
  (`/Engine/EditorBlueprintResources/StandardMacros.IsValid` _output
    (:`Is Valid`
      (`GameplayStatics.ApplyDamage` _output (`self.DamageContact`) null self))))

(event `self.CapsuleComponent.OnComponentBeginOverlap`
  (params (OverlappedComponent :type "PrimitiveComponent Object Reference") (OtherActor :type "Actor Object Reference") (OtherComp :type "PrimitiveComponent Object Reference") (OtherBodyIndex :type Integer) (bFromSweep :type Boolean) (SweepResult :type "HitResult Structure (by ref)"))
  ;[1 0.9688 0.9688] Apply Damage
  (bind _asplayer_bp (cast `/Game/Blueprints/Player/Player_BP` OtherActor))
  (`GameplayStatics.ApplyDamage` _asplayer_bp (`self.DamageContact`) null self))

(event `DropLoot`
  (bind (_returnvalue_x _returnvalue_y _returnvalue_z) (`KismetMathLibrary.BreakVector` (`self.K2_GetActorLocation`)))
  ;[1 1 1] Drop Loot
  (`|SpawnActorFromClass` "/Game/Blueprints/Collectibles/Loot/BitCoinLoot_BP.BitCoinLoot_BP_C" (`KismetMathLibrary.MakeTransform` (`KismetMathLibrary.MakeVector` _returnvalue_x 1.0 _returnvalue_z)) "Undefined" "OverrideRootScale" null null))

(event `ControlAnimation`
  ;[0.0133 0.4271 0] Control Animation
  (if (`self.isDead`)
    (set `self.FlyStates` "NewEnumerator4")
    (`/Engine/EditorBlueprintResources/StandardMacros.DoOnce` false
      (:`Completed`
        (`KismetSystemLibrary.Delay` (`PaperFlipbookComponent.GetFlipbookLength` (`self.Sprite`)))))
    (elif (`self.isHit`)
      (set `self.FlyStates` "NewEnumerator0")
      (else
        (set `self.FlyStates` "NewEnumerator1")))))

(event `DirectionStart`
  (bind _returnvalue_x (`KismetMathLibrary.BreakVector` (`self.K2_GetActorLocation`)))
  (bind _returnvalue_x_2 (`KismetMathLibrary.BreakVector` (`self.K2_GetActorLocation` (`self.PlayerRef`))))
  ;[0.1362 0.1893 1] Facing Control
  (if (< _returnvalue_x_2 _returnvalue_x)
    (`SceneComponent.K2_SetWorldRotation` :`self` (`self.CapsuleComponent`))
    (else
      (`SceneComponent.K2_SetWorldRotation` (`self.CapsuleComponent`) (struct :`Yaw` 180.0) false false))))

(event `self.ReceiveBeginPlay`
  ;[0.9624 1 0.9789] DEFAULT
  (bind _asplayer_bp (cast `/Game/Blueprints/Player/Player_BP` (`GameplayStatics.GetPlayerCharacter` 0)))
  (set `self.PlayerRef` _asplayer_bp)
  (`self.DirectionStart`)
  (`KismetSystemLibrary.K2_SetTimerDelegate` (delegate `CheckOutOfScreen`) 0.5 true)
  (`self.VerticalFly`))

(event `self.ReceiveTick`
  (params (DeltaSeconds :type "Float (single-precision)"))
  ;[0.9624 1 0.9789] DEFAULT
  (`self.OverlappingDamage`)
  (`self.ControlAnimation`)
  (`self.UpdateAnimations`)
  (`self.HorizontalFly`))

(event `UpdateAnimations`
  ;[0.07908 0.1965 1] UpdateAnimations
  (switch `/Game/Blueprints/Enemies/Fly/EnemyFlyStates` (`self.FlyStates`)
    (:`NewEnumerator0`
      (`PaperFlipbookComponent.SetFlipbook` (`self.Sprite`) "/Game/Sprites/Enemies/Medusa/Medusa1.Medusa1"))
    (:`NewEnumerator1`
      (`PaperFlipbookComponent.SetFlipbook` (`self.Sprite`) "/Game/Sprites/Enemies/Medusa/Medusa1.Medusa1"))
    (:`NewEnumerator4`
      (`PaperFlipbookComponent.SetFlipbook` (`self.Sprite`) "/Game/Sprites/Enemies/Medusa/MedusaDeath.MedusaDeath"))))

(event `CheckOutOfScreen`
  (bind _returnvalue_x (`KismetMathLibrary.BreakVector` (`self.K2_GetActorLocation`)))
  ;[1 1 1] Destroy if Out of Screen
  (bind _outactors (`GameplayStatics.GetAllActorsOfClass` "/Game/Blueprints/Level/ScreenCollider_BP.ScreenCollider_BP_C"))
  (bind _returnvalue_x_2 (`KismetMathLibrary.BreakVector` (`self.K2_GetActorLocation` (`|GetArrayItem` _outactors))))
  (if (> (- _returnvalue_x_2 200.0) _returnvalue_x)
    (`self.K2_DestroyActor` :!label _label)
    (elif (<= (+ _returnvalue_x_2 200.0) _returnvalue_x)
      (goto _label))))

(event `VerticalFly`
  (bind (_returnvalue_x _returnvalue_y _returnvalue_z) (`KismetMathLibrary.BreakVector` (`self.K2_GetActorLocation`)))
  ;[1 1 1] Vertical & Horizontal Flight
  (bind (_direction _newtrack_0) (`Timeline|Vertical Flight` :!via `PlayFromStart` :!label _label_2)
    (:`Update`
      (`self.K2_SetActorLocation` (`KismetMathLibrary.MakeVector` _returnvalue_x _returnvalue_y (+ _newtrack_0 _returnvalue_z))))))

(event `HorizontalFly`
  ;[1 1 1] Vertical & Horizontal Flight
  (if (not (`self.isDead`))
    (`self.AddMovementInput` (`KismetMathLibrary.SelectVector` (-1.0 0.0 0.0) (1.0 0.0 0.0) (`self.isFacingLeft`)))))

(event `StopZ`
  ;[1 1 1] Vertical & Horizontal Flight
  (goto _label_2 :!via `Stop`))

(fn `UserConstructionScript`)