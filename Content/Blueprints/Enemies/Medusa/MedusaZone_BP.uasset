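; Trigger zone that spawns EnemyMedusa_BP enemies at either side of the player while the player is inside its box.
; A looping timer checks zone occupancy and caps the world-wide medusa count, then spawns after a short random delay.
; Spawns use a fixed horizontal offset from the player and a height relative to the zone.
; SpawnFrom selects right, left or alternating sides via FlipFlop, with left-side spawns set to face right.
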(event `Cast Medusa`
  (bind (_returnvalue_x _returnvalue_y _returnvalue_z) (`KismetMathLibrary.BreakVector` (`self.K2_GetActorLocation`)))
  (bind (_returnvalue_x_2 _returnvalue_y_2 _returnvalue_z_2) (`KismetMathLibrary.BreakVector` (`self.K2_GetActorLocation`)))
  (bind (_returnvalue_x_3 _returnvalue_y_3) (`KismetMathLibrary.BreakVector` (`self.K2_GetActorLocation` (`self.PlayerRef`))))
  (bind (_returnvalue_x_4 _returnvalue_y_4) (`KismetMathLibrary.BreakVector` (`self.K2_GetActorLocation` (`self.PlayerRef`))))
  (if (`self.InZone`)
    (bind _outactors (`GameplayStatics.GetAllActorsOfClass` "/Game/Blueprints/Enemies/Medusa/EnemyMedusa_BP.EnemyMedusa_BP_C"))
    (if (< (`KismetArrayLibrary.Array_Length` _outactors) (`self.MaxMedusas`))
      (`KismetSystemLibrary.Delay` (`KismetMathLibrary.RandomFloatInRange` 0.0 0.5))
      (switch `/Game/Blueprints/Enemies/Medusa/MedusaZoneSelect` (`self.SpawnFrom`)
        (:`NewEnumerator0`
          (`|SpawnActorFromClass` "/Game/Blueprints/Enemies/Medusa/EnemyMedusa_BP.EnemyMedusa_BP_C" (`KismetMathLibrary.MakeTransform` (`KismetMathLibrary.MakeVector` (+ _returnvalue_x_4 220.0) (- _returnvalue_y_4 1.0) (+ _returnvalue_z_2 (`self.Z-Spawn`)))) "Undefined" "OverrideRootScale" null null :!label _label))
        (:`NewEnumerator1`
          (bind _returnvalue (`|SpawnActorFromClass` "/Game/Blueprints/Enemies/Medusa/EnemyMedusa_BP.EnemyMedusa_BP_C" (`KismetMathLibrary.MakeTransform` (`KismetMathLibrary.MakeVector` (+ _returnvalue_x_3 -220.0) (- _returnvalue_y_3 1.0) (+ _returnvalue_z (`self.Z-Spawn`)))) "Undefined" "OverrideRootScale" null null :!label _label_2))
          (set `/Game/Blueprints/Enemies/Medusa/EnemyMedusa_BP.isFacingLeft` false _returnvalue))
        (:`NewEnumerator2`
          (`/Engine/EditorBlueprintResources/StandardMacros.FlipFlop`
            (:`A`
              (goto _label))
            (:`B`
              (goto _label_2))))))))

(event `self.ReceiveBeginPlay`
  (bind _asplayer_bp (cast `/Game/Blueprints/Player/Player_BP` (`GameplayStatics.GetPlayerCharacter` 0)))
  (set `self.PlayerRef` _asplayer_bp)
  (`KismetSystemLibrary.K2_SetTimerDelegate` (delegate `Cast Medusa`) (`self.SpawnEach`) true))

(event `self.Box.OnComponentBeginOverlap`
  (params (OverlappedComponent :type "PrimitiveComponent Object Reference") (OtherActor :type "Actor Object Reference") (OtherComp :type "PrimitiveComponent Object Reference") (OtherBodyIndex :type Integer) (bFromSweep :type Boolean) (SweepResult :type "HitResult Structure (by ref)"))
  (cast `/Game/Blueprints/Player/Player_BP` OtherActor)
  (set `self.InZone` true)
  (`KismetSystemLibrary.PrintString` "Medusa Zone ON"))

(event `self.Box.OnComponentEndOverlap`
  (params (OverlappedComponent :type "PrimitiveComponent Object Reference") (OtherActor :type "Actor Object Reference") (OtherComp :type "PrimitiveComponent Object Reference") (OtherBodyIndex :type Integer))
  (cast `/Game/Blueprints/Player/Player_BP` OtherActor)
  (set `self.InZone` false)
  (`KismetSystemLibrary.PrintString` "Medusa Zone OFF"))

(fn `UserConstructionScript`)