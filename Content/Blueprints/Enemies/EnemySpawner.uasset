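; EnemySpawner is a one-shot trigger actor that spawns its configured Enemy class when its BoxCollider overlaps a ScreenCollider.
; The enemy spawns at the spawner's location with adjusted-but-guaranteed placement, or a warning prints if no class is set.
; The spawner destroys itself after either outcome.
; BeginPlay derives a TurnDirection rotation from the TurnLeft flag, but the spawn call does not use it.
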(event `self.ReceiveBeginPlay`
  (if (`self.TurnLeft`)
    (set `self.TurnDirection` (struct))
    (else
      (set `self.TurnDirection` (struct :`Yaw` 180.0)))))

(event `self.BoxCollider.OnComponentBeginOverlap`
  (params (OverlappedComponent :type "PrimitiveComponent Object Reference") (OtherActor :type "Actor Object Reference") (OtherComp :type "PrimitiveComponent Object Reference") (OtherBodyIndex :type Integer) (bFromSweep :type Boolean) (SweepResult :type "HitResult Structure (by ref)"))
  (cast `/Game/Blueprints/Level/ScreenCollider` OtherActor)
  (if (!= (`self.Enemy`) null)
    (`|SpawnActorFromClass` (`self.Enemy`) (`KismetMathLibrary.MakeTransform` (`self.K2_GetActorLocation`)) "AdjustIfPossibleButAlwaysSpawn" "OverrideRootScale" null null)
    (else
      (`KismetSystemLibrary.PrintString` "Enemy Spawner Invalid")))
  (`self.K2_DestroyActor`))

(fn `UserConstructionScript`)