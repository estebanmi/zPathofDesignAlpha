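; Flipbook-based 2D ghost enemy that steps along platforms, damages the player on contact and flickers by toggling sprite visibility.
; A one-second timer line-traces for walls and ledges, then either patrols a set step count or randomly turns toward the player.
; Walk and turn flags pick the animation state each tick, with movement and flips applied after flipbook delays.
; A gate destroys it if it stays outside the screen collider for a second.
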(event `TurnToPlayer`
  (bind _returnvalue_x (`KismetMathLibrary.BreakVector` (`KismetMathLibrary.GetDirectionUnitVector` (`self.K2_GetActorLocation`) (`self.K2_GetActorLocation` (`self.PlayerRef`)))))
  ;[0 0.218 1] Turn To Player
  (if (`KismetSystemLibrary.IsValid` (`self.PlayerRef`))
    (if (`/Game/Blueprints/Player/Player_BP.isInvisible` (`self.PlayerRef`))
      _
      (elif (> _returnvalue_x 0.0)
        (if (`self.isFacingLeft`)
          (`self.DirectionChange`))
        (elif (not (`self.isFacingLeft`))
          (`self.DirectionChange`))))))

(event `OverlappingDamage`
  (bind _output (`|GetArrayItem` (`PrimitiveComponent.GetOverlappingActors` (`self.CapsuleComponent`) "/Game/Blueprints/Player/Player_BP.Player_BP_C")))
  ;[1 0 0] Apply Damage
  (`/Engine/EditorBlueprintResources/StandardMacros.IsValid` _output
    (:`Is Valid`
      (`GameplayStatics.ApplyDamage` _output (`self.DamageContact`) null self))))

(event `ControlAnimation`
  ;[0.0133 0.4271 0] Control Animation
  (if (`self.isWalking`)
    (set `self.GhostStates` "NewEnumerator3")
    (elif (`self.isTurning`)
      (set `self.GhostStates` "NewEnumerator6")
      (else
        (set `self.GhostStates` "NewEnumerator1")))))

(event `DirectionStart`
  ;[0.1362 0.1893 1] Facing Control
  (if (`self.isFacingLeft`)
    (`SceneComponent.K2_SetWorldRotation` :`self` (`self.CapsuleComponent`))
    (else
      (`SceneComponent.K2_SetWorldRotation` (`self.CapsuleComponent`) (struct :`Yaw` 180.0) false false))))

(event `UpdateAnimations`
  (bind (_returnvalue_x _returnvalue_y _returnvalue_z) (`KismetMathLibrary.BreakVector` (`self.K2_GetActorLocation`)))
  (bind _sprite (`self.Sprite`))
  (bind _sprite_2 (`self.Sprite`))
  ;[0.07908 0.1965 1] UpdateAnimations
  (switch `/Game/Blueprints/Enemies/RAM/Ghost/EnemyGhostStates` (`self.GhostStates`)
    (:`NewEnumerator1`
      (`PaperFlipbookComponent.SetFlipbook` (`self.Sprite`) "/Game/Sprites/Enemies/Ghost/EnemyGhostIdle1.EnemyGhostIdle1"))
    (:`NewEnumerator3`
      (`PaperFlipbookComponent.SetFlipbook` _sprite "/Game/Sprites/Enemies/Ghost/EnemyGhostWalk1.EnemyGhostWalk1")
      (`KismetSystemLibrary.Delay` (`PaperFlipbookComponent.GetFlipbookLength` _sprite))
      (if (`self.isFacingLeft`)
        (`self.K2_SetActorLocation` (`KismetMathLibrary.MakeVector` (- _returnvalue_x 3.0) _returnvalue_y _returnvalue_z))
        (else
          (`self.K2_SetActorLocation` (`KismetMathLibrary.MakeVector` (+ _returnvalue_x 3.0) _returnvalue_y _returnvalue_z))))
      (set `self.isWalking` false))
    (:`NewEnumerator6`
      (`PaperFlipbookComponent.SetFlipbook` _sprite_2 "/Game/Sprites/Enemies/Ghost/EnemyGhostTurn1.EnemyGhostTurn1")
      (`KismetSystemLibrary.Delay` (`PaperFlipbookComponent.GetFlipbookLength` _sprite_2))
      (set `self.isTurning` false)
      (`self.DirectionChange`))))

(event `self.ReceiveBeginPlay`
  ;[1 0.3304 0] DEFAULT
  (`self.CastPlayerRef`)
  (`self.DirectionStart`)
  (`KismetSystemLibrary.K2_SetTimerDelegate` (delegate `Walk`) 1.0 true)
  (`KismetSystemLibrary.K2_SetTimerDelegate` (delegate `UpdateVisibility`) 0.2 true))

(event `self.ReceiveTick`
  (params (DeltaSeconds :type "Float (single-precision)"))
  ;[1 0.3304 0] DEFAULT
  (`self.ControlAnimation`)
  (`self.UpdateAnimations`)
  ;;[1 1 1] ojo+
  (`self.OverlappingDamage`)
  (`self.UpdateVisibility`))

(event `DirectionChange`
  ;[0.1362 0.1893 1] Facing Control
  (if (`self.isFacingLeft`)
    (`SceneComponent.K2_SetWorldRotation` (`self.CapsuleComponent`) (struct :`Yaw` 180.0) false false)
    (set `self.isFacingLeft` false)
    (else
      (`SceneComponent.K2_SetWorldRotation` :`self` (`self.CapsuleComponent`))
      (set `self.isFacingLeft` true))))

(event `CastPlayerRef`
  ;[1 0.3304 0] DEFAULT
  ;;[1 1 1] CastPlayer
  (bind _asplayer_bp (cast `/Game/Blueprints/Player/Player_BP` (`GameplayStatics.GetPlayerCharacter` 0)))
  (set `self.PlayerRef` _asplayer_bp))

(event `UpdateVisibility`
  (bind _sprite (`self.Sprite`))
  ;[1 1 1] UpdateVisibility
  (if (`/Game/Blueprints/Player/Player_BP.isInvisible` (`self.PlayerRef`))
    _
    (else
      _))
  (`/Engine/EditorBlueprintResources/StandardMacros.FlipFlop`
    (:`A`
      (`SceneComponent.SetVisibility` _sprite true false))
    (:`B`
      (`SceneComponent.SetVisibility` _sprite false false))))

(event `Walk`
  ;[1 0 0.8246] Walk
  (if (not (`self.KilledPlayer`))
    (`self.CheckFront`)
    (`self.CheckFall`)
    (if (`self.isPatrol`)
      (set `self.Steps` (+ (`self.Steps`) 1))
      (if (== (`self.Steps`) (`self.StepsToTurn`))
        (set `self.isTurning` true)
        (set `self.Steps` 0)
        (elif (`self.isBlocked`)
          (if (`self.isPatrol`)
            (set `self.isTurning` true)
            (set `self.isBlocked` false)
            (else
              (set `self.isBlocked` false)))
          (else
            (set `self.isWalking` true))))
      (else
        (`self.CheckTurning`)))))

(event `self.CapsuleComponent.OnComponentBeginOverlap`
  (params (OverlappedComponent :type "PrimitiveComponent Object Reference") (OtherActor :type "Actor Object Reference") (OtherComp :type "PrimitiveComponent Object Reference") (OtherBodyIndex :type Integer) (bFromSweep :type Boolean) (SweepResult :type "HitResult Structure (by ref)"))
  ;[0 0 0] OnScreen or Not
  (cast `/Game/Blueprints/Level/ScreenCollider_BP` OtherActor)
  (goto _label :!via `Close`))

(event `CloseGate`
  ;[0 0 0] OnScreen or Not
  (goto _label :!via `Open`))

(event `CheckTurning`
  (bind _returnvalue_x (`KismetMathLibrary.BreakVector` (`self.K2_GetActorLocation`)))
  (bind _returnvalue_x_2 (`KismetMathLibrary.BreakVector` (`self.K2_GetActorLocation` (`self.PlayerRef`))))
  ;[1 0 0.5945] TurnToPlayer Prob
  (if (`self.isDead`)
    _
    (elif (< (`KismetMathLibrary.RandomFloatInRange` 0.0 100.0) (`self.TurnToPlayerProb`))
      (if (< _returnvalue_x _returnvalue_x_2)
        (if (`self.isFacingLeft`)
          (set `self.isTurning` true)
          (elif (`self.isBlocked`)
            (set `self.isBlocked` false)
            (else
              (set `self.isWalking` true))))
        (elif (`self.isFacingLeft`)
          (if (`self.isBlocked`)
            (set `self.isBlocked` false)
            (else
              (set `self.isWalking` true)))
          (else
            (set `self.isTurning` true))))
      (elif (`self.isBlocked`)
        (set `self.isBlocked` false)
        (else
          (set `self.isWalking` true))))))

(event `self.CapsuleComponent.OnComponentEndOverlap`
  (params (OverlappedComponent :type "PrimitiveComponent Object Reference") (OtherActor :type "Actor Object Reference") (OtherComp :type "PrimitiveComponent Object Reference") (OtherBodyIndex :type Integer))
  ;[0 0 0] OnScreen or Not
  (cast `/Game/Blueprints/Level/ScreenCollider_BP` OtherActor)
  (`self.CloseGate`)
  (`KismetSystemLibrary.Delay` 1.0)
  (`/Engine/EditorBlueprintResources/StandardMacros.Gate` true :!label _label
    (:`Exit`
      (`self.K2_DestroyActor`))))

(event `ColorControl`
  (bind _returnvalue (`KismetMathLibrary.RandomFloatInRange` 0.6 1.0))
  ;[0 1 1] Color Control
  (bind _asplayer_bp (cast `/Game/Blueprints/Player/Player_BP` (`GameplayStatics.GetPlayerCharacter` 0)))
  (if (`/Game/Blueprints/Player/Player_BP.VideoCardON` _asplayer_bp)
    (bind _outactors (`GameplayStatics.GetAllActorsOfClass` "/Game/Blueprints/Art/ColorController.ColorController_C"))
    (bind _returnvalue_2 (`|GetDataTableRow` "/Game/Blueprints/Art/ColorSchemeTable.ColorSchemeTable" (`/Game/Blueprints/Art/ColorController.ColorScheme` (`|GetArrayItem` _outactors)))
      (:`then`
        (`PaperFlipbookComponent.SetSpriteColor` (`self.Sprite`) (* (`.Enemies_33_D3933F8042CE8CB253100FB32ECD27F6` (break `/Game/Blueprints/Art/ColorScheme` _returnvalue_2)) (make `LinearColor` _returnvalue _returnvalue _returnvalue 1.0)))))))

(event `CheckFront`
  (bind _returnvalue (`self.K2_GetActorLocation`))
  ;[1 0 0.7959] Check Front & Fall
  (bind _outactors (`GameplayStatics.GetAllActorsWithTag` "Enemy"))
  (bind _outhit (`KismetSystemLibrary.LineTraceSingle` (`self.K2_GetActorLocation`) (select `bool` (`self.isFacingLeft`) :`false` (+ _returnvalue (10.0 0.0 0.0)) :`true` (+ _returnvalue (-10.0 0.0 0.0))) "TraceTypeQuery1" false _outactors "None" true (struct :`R` 1.0 :`A` 1.0) (struct :`G` 1.0 :`A` 1.0) 1.0))
  (`/Engine/EditorBlueprintResources/StandardMacros.IsValid` (`.HitActor` (`GameplayStatics.BreakHitResult` _outhit))
    (:`Is Valid`
      (if (!= (`.HitActor` (`GameplayStatics.BreakHitResult` _outhit)) "/Game/Blueprints/Player/Player_BP.Player_BP")
        (set `self.isBlocked` true)))))

(event `CheckFall`
  (bind _returnvalue (`self.K2_GetActorLocation`))
  ;[1 0 0.7959] Check Front & Fall
  (bind _outactors (`GameplayStatics.GetAllActorsWithTag` "Enemy"))
  (bind _outhit (`KismetSystemLibrary.LineTraceSingle` (`self.K2_GetActorLocation`) (select `bool` (`self.isFacingLeft`) :`false` (+ _returnvalue (10.0 0.0 -15.0)) :`true` (+ _returnvalue (-10.0 0.0 -15.0))) "TraceTypeQuery1" false _outactors "None" true (struct :`R` 1.0 :`A` 1.0) (struct :`G` 1.0 :`A` 1.0) 1.0))
  (`/Engine/EditorBlueprintResources/StandardMacros.IsValid` (`.HitActor` (`GameplayStatics.BreakHitResult` _outhit))
    (:`Is Not Valid`
      (if (!= (`.HitActor` (`GameplayStatics.BreakHitResult` _outhit)) "/Game/Blueprints/Player/Player_BP.Player_BP")
        (set `self.isBlocked` true)
        (set `self.Steps` 0)))))

(fn `UserConstructionScript`)