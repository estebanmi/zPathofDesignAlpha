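; Goblin enemy for a 2D side-scroller that patrols around its spawn point, chases the player and deals contact damage.
; Looping timers drive AI checks: sight-box detection, spreading alerts to nearby goblins, losing invisible players, and jumping when stuck or at ledges.
; Tick moves it and derives an animation state from boolean flags to pick the flipbook.
; Hits play a timeline shake; death drops BitCoin loot.
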(event `self.ReceiveAnyDamage`
  (params (Damage :type "Float (single-precision)") (DamageType :type "DamageType Object Reference") (InstigatedBy :type "Controller Object Reference") (DamageCauser :type "Actor Object Reference"))
  (bind _sprite (`self.Sprite`))
  (bind (_relativelocation_x _relativelocation_y _relativelocation_z) (`KismetMathLibrary.BreakVector` (`SceneComponent.RelativeLocation` _sprite)))
  ;[1 0.1155 0] ReceiveDamage
  (bind _output_get (set `self.HP` (- (`self.HP`) Damage)))
  (if (<= _output_get 0.0)
    (`PrimitiveComponent.SetCollisionEnabled` (`self.CapsuleComponent`) "NoCollision"))
  (set `self.isAlert` true)
  (`GameplayStatics.PlaySound2D` "/Game/Sound/SFXs/sfx_BlopHit_Cue.sfx_BlopHit_Cue" 1.0 1.0 0.0 null null)
  (set `CharacterMovementComponent.GravityScale` 0.0 (`self.CharacterMovement`))
  (`MovementComponent.StopMovementImmediately` (`self.CharacterMovement`))
  (bind (_direction _horizontalshake) (`Timeline|Timeline_0` :!via `PlayFromStart`)
    (:`Update`
      (`SceneComponent.K2_SetRelativeLocation` _sprite (`KismetMathLibrary.MakeVector` _horizontalshake _relativelocation_y _relativelocation_z) false false))
    (:`Finished`
      (if (<= (`self.HP`) 0.0)
        (set `self.isChase` true)
        (`/Engine/EditorBlueprintResources/StandardMacros.DoOnce` false
          (:`Completed`
            (`KismetSystemLibrary.Delay` 0.3)
            (`GameplayStatics.PlaySound2D` "/Game/Sound/SFXs/sfx_BlopDeath_Cue.sfx_BlopDeath_Cue" 1.0 1.0 0.0 null null)
            (`KismetSystemLibrary.Delay` 0.3)
            (`self.DropLoot`)
            (`KismetSystemLibrary.Delay` 0.4)
            (`self.K2_DestroyActor`)))
        (else
          (set `CharacterMovementComponent.GravityScale` 2.0 (`self.CharacterMovement`))
          (set `self.isAlert` false))))))

(event `DeadZone`
  (params (OtherActor :type "Actor Object Reference"))
  ;[1 0.1155 0] ReceiveDamage
  ;;[1 1 1] DeadZone
  (cast `/Game/Blueprints/Level/DeadZoneFalling_BP` OtherActor)
  (`GameplayStatics.PlaySound2D` "/Game/Sound/SFXs/sfx_BlopDeath_Cue.sfx_BlopDeath_Cue" 0.3 1.0 0.0 null null)
  (`self.K2_DestroyActor`))

(event `DropLoot`
  (bind (_returnvalue_x _returnvalue_y _returnvalue_z) (`KismetMathLibrary.BreakVector` (`self.K2_GetActorLocation`)))
  ;[1 1 1] Drop Loot
  (`|SpawnActorFromClass` "/Game/Blueprints/Collectibles/BitCoinLoot.BitCoinLoot_C" (`KismetMathLibrary.MakeTransform` (`KismetMathLibrary.MakeVector` _returnvalue_x 1.0 _returnvalue_z)) "Undefined" "OverrideRootScale" null null))

(event `Attack`
  ;[1 0 0] Attack Jump
  (set `CharacterMovementComponent.MaxAcceleration` (`KismetMathLibrary.RandomFloatInRange` 0.0 20000.0) (`self.CharacterMovement`))
  (`self.TurnToPlayer`)
  (if (not (`self.isChase`))
    (`KismetSystemLibrary.Delay` 1.0)
    (if (not (`self.isAlert`))
      (set `self.IsJumping` true)
      (if (`self.isFacingLeft`)
        (`self.AddMovementInput` (-1.0 0.0 0.0))
        (else
          (`self.AddMovementInput` (1.0 0.0 0.0))))
      (`self.Jump`)
      (`GameplayStatics.PlaySound2D` "/Game/Sound/SFXs/sfx_BlopJump_Cue.sfx_BlopJump_Cue" 1.0 1.0 0.0 null null)
      (set `self.IsJumping` true))))

(event `self.CapsuleComponent.OnComponentBeginOverlap`
  (params (OverlappedComponent :type "PrimitiveComponent Object Reference") (OtherActor :type "Actor Object Reference") (OtherComp :type "PrimitiveComponent Object Reference") (OtherBodyIndex :type Integer) (bFromSweep :type Boolean) (SweepResult :type "HitResult Structure (by ref)"))
  ;[1 0 0] Attack Jump
  ;;[1 0.9688 0.9688] Apply Damage
  (bind _asplayer_bp (cast `/Game/Blueprints/Player/Player_BP` OtherActor))
  (`GameplayStatics.ApplyDamage` _asplayer_bp (`self.DamageContact`) null self))

(event `ToAttack`
  ;[1 0 0] Attack Jump
  (`KismetSystemLibrary.K2_SetTimerDelegate` (delegate `Attack`) (`KismetMathLibrary.RandomFloatInRange` 2.0 4.0) true))

(event `ControlAnimation`
  (bind _returnvalue_x (`KismetMathLibrary.BreakVector` (`self.GetVelocity`)))
  ;[0.0133 0.4271 0] Control Animation
  (if (`self.isChase`)
    (set `self.GoblinStates` "NewEnumerator5")
    (elif (`self.isAlert`)
      (set `self.GoblinStates` "NewEnumerator6")
      (elif (`self.isLost`)
        (set `self.GoblinStates` "NewEnumerator0")
        (elif (`self.IsJumping`)
          (set `self.GoblinStates` "NewEnumerator3" :!label _label)
          (elif (`NavMovementComponent.IsFalling` (`self.CharacterMovement`))
            (goto _label)
            (elif (!= _returnvalue_x 0.0)
              (set `self.GoblinStates` "NewEnumerator1")
              (else
                (set `self.GoblinStates` "NewEnumerator7")))))))))

(event `TurnToPlayer`
  (bind _returnvalue_x (`KismetMathLibrary.BreakVector` (`KismetMathLibrary.GetDirectionUnitVector` (`self.K2_GetActorLocation`) (`self.K2_GetActorLocation` (`self.PlayerRef`)))))
  ;[0 0.218 1] Turn To Player
  (if (`KismetSystemLibrary.IsValid` (`self.PlayerRef`))
    (if (`/Game/Blueprints/Player/Player_BP.isInvisible` (`self.PlayerRef`))
      _
      (elif (> _returnvalue_x 0.0)
        (if (`self.isFacingLeft`)
          (`self.DirectionChange`))
        (elif (not (`self.isFacingLeft`))
          (`self.DirectionChange`))))))

(event `TurnToStartX`
  (bind _returnvalue_x (`KismetMathLibrary.BreakVector` (`KismetMathLibrary.GetDirectionUnitVector` (`self.K2_GetActorLocation`) (`KismetMathLibrary.MakeVector` (`self.StartingLocation`)))))
  ;[0 0.2437 1] Turn To Start X
  (if (> _returnvalue_x 0.0)
    (if (`self.isFacingLeft`)
      (`self.DirectionChange`))
    (elif (not (`self.isFacingLeft`))
      (`self.DirectionChange`))))

(event `RandomXY`
  (bind (_returnvalue_x _returnvalue_y _returnvalue_z) (`KismetMathLibrary.BreakVector` (`self.K2_GetActorLocation`)))
  (bind _returnvalue_x_2 (`KismetMathLibrary.BreakVector` (`self.K2_GetActorLocation`)))
  (bind (_returnvalue_x_3 _returnvalue_y_2 _returnvalue_z_2) (`KismetMathLibrary.BreakVector` (`self.K2_GetActorLocation`)))
  ;[1 1 1] Random Start Pos
  (`self.K2_SetActorLocation` (`KismetMathLibrary.MakeVector` (+ _returnvalue_x (`KismetMathLibrary.RandomFloatInRange` -3.0 3.0)) _returnvalue_y _returnvalue_z))
  (`self.K2_SetActorLocation` (`KismetMathLibrary.MakeVector` _returnvalue_x_3 (- _returnvalue_y_2 (`KismetMathLibrary.RandomFloatInRange` 0.0 1.0)) _returnvalue_z_2))
  (set `self.StartingLocation` _returnvalue_x_2))

(event `self.OnLanded`
  (params (Hit :type "HitResult Structure (by ref)"))
  ;[0.0133 0.4271 0] Control Animation
  ;;[1 1 1] OnLanded
  (if (> (`self.HP`) 0.0)
    (set `self.IsJumping` false)))

(event `DirectionStart`
  ;[0.1362 0.1893 1] Facing Control
  (if (`self.isFacingLeft`)
    (`SceneComponent.K2_SetWorldRotation` :`self` (`self.CapsuleComponent`))
    (else
      (`SceneComponent.K2_SetWorldRotation` (`self.CapsuleComponent`) (struct :`Yaw` 180.0) false false))))

(event `UpdateAnimations`
  ;[0.07908 0.1965 1] UpdateAnimations
  (switch `/Game/Blueprints/Enemies/Goblin/EnemyGoblinStates` (`self.GoblinStates`)
    (:`NewEnumerator0`
      (`PaperFlipbookComponent.SetFlipbook` (`self.Sprite`) "/Game/Sprites/Enemies/Goblin/GoblinLost1.GoblinLost1"))
    (:`NewEnumerator1`
      (`PaperFlipbookComponent.SetFlipbook` (`self.Sprite`) "/Game/Sprites/Enemies/Goblin/GoblinWalk.GoblinWalk"))
    (:`NewEnumerator3`
      (`PaperFlipbookComponent.SetFlipbook` (`self.Sprite`) "/Game/Sprites/Enemies/Goblin/GoblinJump1.GoblinJump1"))
    (:`NewEnumerator5`
      (`PaperFlipbookComponent.SetFlipbook` (`self.Sprite`) "/Game/Sprites/Enemies/Goblin/GoblinChase11.GoblinChase11"))
    (:`NewEnumerator6`
      (`PaperFlipbookComponent.SetFlipbook` (`self.Sprite`) "/Game/Sprites/Enemies/Goblin/GoblinAlert1.GoblinAlert1"))
    (:`NewEnumerator7`
      (`PaperFlipbookComponent.SetFlipbook` (`self.Sprite`) "/Game/Sprites/Enemies/Goblin/GoblinIdle1.GoblinIdle1"))))

(event `WarCry`
  ;[1 0.3304 0] DEFAULT
  (if (`self.isChase`)
    (`KismetSystemLibrary.Delay` (`KismetMathLibrary.RandomFloatInRange` 0.0 1.0))
    (`GameplayStatics.PlaySound2D` "/Game/Sound/SFXs/sfx_Goblin_Cue.sfx_Goblin_Cue" (`KismetMathLibrary.RandomFloatInRange` 0.2 1.0) 1.0 0.0 null null :!label _label_2)))

(event `CastPlayerRef`
  ;[1 1 1] CastPlayer
  (bind _asplayer_bp (cast `/Game/Blueprints/Player/Player_BP` (`GameplayStatics.GetPlayerCharacter` 0)))
  (set `self.PlayerRef` _asplayer_bp))

(event `self.ReceiveTick`
  (params (DeltaSeconds :type "Float (single-precision)"))
  ;[1 0.3304 0] DEFAULT
  (`self.ControlAnimation`)
  (`self.UpdateAnimations`)
  (`self.RunForward`))

(event `Patrol`
  (bind _returnvalue_x (`KismetMathLibrary.BreakVector` (`self.K2_GetActorLocation`)))
  (bind _startx (`self.StartX`))
  ;[1 1 1] Patrol
  (if (`self.isLost`)
    _
    (elif (`self.isChase`)
      _
      (elif (not (`self.isAlert`))
        (set `self.isIdle` true)
        (if (> _returnvalue_x _startx)
          (`KismetSystemLibrary.Delay` (`KismetMathLibrary.RandomFloatInRange` 0.5 3.0) :!label _label_3)
          (set `self.isIdle` false)
          (`self.TurnToStartX`)
          (elif (< _returnvalue_x _startx)
            (goto _label_3)))))))

(event `DirectionChange`
  ;[0.1362 0.1893 1] Facing Control
  (if (`self.isFacingLeft`)
    (`SceneComponent.K2_SetWorldRotation` (`self.CapsuleComponent`) (struct :`Yaw` 180.0) false false)
    (set `self.isFacingLeft` false)
    (else
      (`SceneComponent.K2_SetWorldRotation` :`self` (`self.CapsuleComponent`))
      (set `self.isFacingLeft` true))))

(event `self.ReceiveBeginPlay`
  ;[1 0.3304 0] DEFAULT
  (set `self.isFacingLeft` (`KismetMathLibrary.RandomBool`))
  (`self.RandomXY`)
  (`self.TurnToPlayer`)
  (`self.CastPlayerRef`)
  (`KismetSystemLibrary.K2_SetTimerDelegate` (delegate `Patrol`) (`KismetMathLibrary.RandomFloatInRange` 2.0 4.0) true)
  (`KismetSystemLibrary.K2_SetTimerDelegate` (delegate `CheckPlayerLocation`) 0.5 true)
  (`KismetSystemLibrary.K2_SetTimerDelegate` (delegate `CheckFront`) 0.1 true)
  (`KismetSystemLibrary.K2_SetTimerDelegate` (delegate `CheckFall`) 0.1 true)
  (`KismetSystemLibrary.K2_SetTimerDelegate` (delegate `CheckAlert`) (`KismetMathLibrary.RandomFloatInRange` 0.3 0.6) true)
  (`KismetSystemLibrary.K2_SetTimerDelegate` (delegate `AlertOthers`) 0.5 true)
  (`KismetSystemLibrary.K2_SetTimerDelegate` (delegate `WarCry`) (`KismetMathLibrary.RandomFloatInRange` 1.0 2.0) true))

(event `CheckPlayerLocation`
  ;[1 1 1] TurnToPlayer Prob
  (if (`self.isChase`)
    (if (`self.IsJumping`)
      _
      (elif (< (`KismetMathLibrary.RandomFloatInRange` 0.0 100.0) (`self.TurnToPlayerProb`))
        (`KismetSystemLibrary.Delay` (`KismetMathLibrary.RandomFloatInRange` 0.0 1.0))
        (`self.TurnToPlayer`)))))

(event `RunForward`
  ;[1 0.7887 0] RUN (Add Movement)
  (if (`self.isIdle`)
    _
    (elif (`self.isAlert`)
      _
      (elif (`self.isLost`)
        _
        (elif (`self.isFacingLeft`)
          (`self.AddMovementInput` (100.0 0.0 0.0) -1.0)
          (else
            (`self.AddMovementInput` (100.0 0.0 0.0))))))))

(event `CheckAlert`
  ;[1 0.01884 0] CheckAlert
  (if (`self.isChase`)
    (if (`/Game/Blueprints/Player/Player_BP.isInvisible` (`self.PlayerRef`))
      (`self.Lost`))
    (elif (`self.InSight`)
      (if (not (`/Game/Blueprints/Player/Player_BP.isInvisible` (`self.PlayerRef`)))
        (set `self.isIdle` false)
        (`self.Alert`)
        (goto _label_2)))))

(event `CheckFront`
  (bind _returnvalue_x (`KismetMathLibrary.BreakVector` (`self.K2_GetActorLocation`)))
  ;[1 1 1] CheckFront
  (if (`self.isLost`)
    _
    (elif (`self.isIdle`)
      _
      (elif (== (`self.LastX`) _returnvalue_x)
        (set `self.LastFacing` (`self.isFacingLeft`))
        (`self.Jump`)
        (else
          (set `self.LastX` _returnvalue_x))))))

(event `Alert`
  ;[1 0.01935 0] Alert & Lost
  (`self.AlertOthers`)
  (set `self.isAlert` true)
  (set `CharacterMovementComponent.MaxWalkSpeed` (`self.ChaseSpeed`) (`self.CharacterMovement`))
  (`KismetSystemLibrary.Delay` (`KismetMathLibrary.RandomFloatInRange` 0.3 0.6))
  (set `self.isAlert` false)
  (set `self.isChase` true)
  (`self.TurnToPlayer`))

(event `CheckFall`
  (bind _returnvalue_x (`KismetMathLibrary.BreakVector` (`self.K2_GetActorLocation`)))
  (bind (_returnvalue_x_2 _returnvalue_y _returnvalue_z) (`KismetMathLibrary.BreakVector` (`self.K2_GetActorLocation`)))
  (bind _startx (`self.StartX`))
  ;[1 1 1] CheckFall
  (if (`self.isIdle`)
    _
    (elif (not (`self.IsJumping`))
      (if (`self.isFacingLeft`)
        (set `self.StartX` (- _returnvalue_x 10.0))
        (else
          (set `self.StartX` (+ _returnvalue_x 10.0))))
      (bind _outhits (`KismetSystemLibrary.LineTraceMulti` (`KismetMathLibrary.MakeVector` _startx _returnvalue_y _returnvalue_z) (`KismetMathLibrary.MakeVector` _startx _returnvalue_y (- _returnvalue_z 15.0)) "TraceTypeQuery1"))
      (`/Engine/EditorBlueprintResources/StandardMacros.IsValid` (`.HitActor` (`GameplayStatics.BreakHitResult` (`|GetArrayItem` _outhits)))
        (:`Is Not Valid`
          (`self.Jump`)
          (set `self.IsJumping` true))))))

(event `Lost`
  ;[1 0.01935 0] Alert & Lost
  (set `self.isAlert` false)
  (set `self.isChase` false)
  (set `self.isLost` true)
  (`KismetSystemLibrary.Delay` 2.0)
  (set `CharacterMovementComponent.MaxWalkSpeed` (`self.WalkSpeed`) (`self.CharacterMovement`))
  (set `self.isLost` false)
  (set `self.isIdle` false))

(event `self.BoxColliderSight.OnComponentBeginOverlap`
  (params (OverlappedComponent :type "PrimitiveComponent Object Reference") (OtherActor :type "Actor Object Reference") (OtherComp :type "PrimitiveComponent Object Reference") (OtherBodyIndex :type Integer) (bFromSweep :type Boolean) (SweepResult :type "HitResult Structure (by ref)"))
  (cast `/Game/Blueprints/Player/Player_BP` OtherActor)
  (set `self.InSight` true))

(event `AlertOthers`
  ;[1 0.007289 0] Alert Others
  (if (`/Game/Blueprints/Player/Player_BP.isInvisible` (`self.PlayerRef`))
    _
    (elif (`self.isChase`)
      (set `self.GoblinsIndex` 0 :!label _label_4)
      (bind _outactors (`GameplayStatics.GetAllActorsOfClass` "EnemyGoblin_BP_C"))
      (bind _output (`|GetArrayItem` _outactors (`self.GoblinsIndex`)))
      (if (`/Game/Blueprints/Enemies/Goblin/EnemyGoblin_BP.isAlert` _output) :!label _label_5
        (if (< (`self.GoblinsIndex`) (- (`KismetArrayLibrary.Array_Length` _outactors) 1)) :!label _label_6
          (set `self.GoblinsIndex` (+ (`self.GoblinsIndex`) 1))
          (goto _label_5))
        (elif (`/Game/Blueprints/Enemies/Goblin/EnemyGoblin_BP.isChase` _output)
          (goto _label_6)
          (else
            (`KismetSystemLibrary.Delay` (`KismetMathLibrary.RandomFloatInRange` 0.0 0.2))
            (if (< (`KismetMathLibrary.Vector_Distance` (`self.K2_GetActorLocation` _output) (`self.K2_GetActorLocation`)) (`self.MaxAlertDistance`))
              (`self.Alert` _output)
              (goto _label_6)))))
      (elif (`self.isAlert`)
        (goto _label_4)))))

(event `self.BoxColliderSight.OnComponentEndOverlap`
  (params (OverlappedComponent :type "PrimitiveComponent Object Reference") (OtherActor :type "Actor Object Reference") (OtherComp :type "PrimitiveComponent Object Reference") (OtherBodyIndex :type Integer))
  (cast `/Game/Blueprints/Player/Player_BP` OtherActor)
  (set `self.InSight` false))

(fn `UserConstructionScript`)