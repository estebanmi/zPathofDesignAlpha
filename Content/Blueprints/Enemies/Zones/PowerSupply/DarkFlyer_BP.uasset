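; DarkFlyer is a flying enemy that homes on the player, deals contact damage and drops Bitcoin loot on death.
; It flies horizontally, periodically turning toward the player with a brief vertical nudge, and a shake Timeline stalls it when hit.
; Its tint is black or background-colored, depending on the player's VideoCard and PowerSupply flags, until damage reveals it.
; A distance timer and a ScreenCollider overlap gate destroy it off screen.
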(event `self.ReceiveAnyDamage`
  (params (Damage :type "Float (single-precision)") (DamageType :type "DamageType Object Reference") (InstigatedBy :type "Controller Object Reference") (DamageCauser :type "Actor Object Reference"))
  (bind _sprite (`self.Sprite`))
  (bind (_relativelocation_x _relativelocation_y _relativelocation_z) (`KismetMathLibrary.BreakVector` (`SceneComponent.RelativeLocation` _sprite)))
  ;[1 0.1458 0] ReceiveDamage
  (bind _output_get (set `self.HP` (- (`self.HP`) Damage)))
  (if (<= _output_get 0.0)
    (`PrimitiveComponent.SetCollisionEnabled` (`self.CapsuleComponent`) "NoCollision"))
  (set `self.isHit` true)
  (`GameplayStatics.PlaySound2D` "/Game/Sound/SFXs/sfx_BlopHit_Cue.sfx_BlopHit_Cue" 1.0 1.0 0.0 null null)
  (`MovementComponent.StopMovementImmediately` (`self.CharacterMovement`))
  (set `CharacterMovementComponent.MaxWalkSpeed` 0.0 (`self.CharacterMovement`))
  (bind (_direction _horizontalshake) (`Timeline|Timeline_0` :!via `PlayFromStart`)
    (:`Update`
      (`SceneComponent.K2_SetRelativeLocation` _sprite (`KismetMathLibrary.MakeVector` _horizontalshake _relativelocation_y _relativelocation_z) false false))
    (:`Finished`
      (if (<= (`self.HP`) 0.0)
        (set `self.isDead` true)
        (`/Engine/EditorBlueprintResources/StandardMacros.DoOnce` false
          (:`Completed`
            (`KismetSystemLibrary.Delay` 0.2)
            (`GameplayStatics.PlaySound2D` "/Game/Sound/SFXs/sfx_BlopDeath_Cue.sfx_BlopDeath_Cue" 1.0 1.0 0.0 null null)
            (`self.DropLoot`)
            (`KismetSystemLibrary.Delay` 0.2)
            (`self.K2_DestroyActor`)))
        (else
          (set `self.isHit` false)
          (set `CharacterMovementComponent.MaxWalkSpeed` 125.0 (`self.CharacterMovement`)))))))

(event `OverlappingDamage`
  (bind _output (`|GetArrayItem` (`PrimitiveComponent.GetOverlappingActors` (`self.CapsuleComponent`) "/Game/Blueprints/Player/Player_BP.Player_BP_C")))
  ;[1 0.1458 0] ReceiveDamage
  ;;[1 0 0.1066] Overlapping Damage
  (`/Engine/EditorBlueprintResources/StandardMacros.IsValid` _output
    (:`Is Valid`
      (`GameplayStatics.ApplyDamage` _output (`self.DamageContact`) null self))))

(event `DropLoot`
  (bind (_returnvalue_x _returnvalue_y _returnvalue_z) (`KismetMathLibrary.BreakVector` (`self.K2_GetActorLocation`)))
  ;[1 0.1458 0] ReceiveDamage
  ;;[1 1 1] Drop Loot
  (`|SpawnActorFromClass` "/Game/Blueprints/Collectibles/Loot/BitCoinLoot_BP.BitCoinLoot_BP_C" (`KismetMathLibrary.MakeTransform` (`KismetMathLibrary.MakeVector` _returnvalue_x 1.0 _returnvalue_z)) "Undefined" "OverrideRootScale" null null))

(event `self.ReceiveBeginPlay`
  ;[1 0.4825 0] DEFAULT
  (bind _asplayer_bp (cast `/Game/Blueprints/Player/Player_BP` (`GameplayStatics.GetPlayerCharacter` 0)))
  (set `self.PlayerRef` _asplayer_bp)
  (`self.VerticalFlight`)
  (`self.ColorControl`)
  (`KismetSystemLibrary.K2_SetTimerDelegate` (delegate `CheckOutOfScreen`) 0.5 true))

(event `ControlAnimation`
  ;[0 0.1759 0.4271] Control Animation
  (if (`self.isDead`)
    (set `self.DarkStates` "NewEnumerator4")
    (`/Engine/EditorBlueprintResources/StandardMacros.DoOnce` false
      (:`Completed`
        (`KismetSystemLibrary.Delay` 1.0)
        (`PaperFlipbookComponent.Stop` (`self.Sprite`))))
    (elif (`self.isHit`)
      (set `self.DarkStates` "NewEnumerator0")
      (else
        (set `self.DarkStates` "NewEnumerator1")))))

(event `self.ReceiveTick`
  (params (DeltaSeconds :type "Float (single-precision)"))
  ;[1 0.4825 0] DEFAULT
  (`self.OverlappingDamage`)
  (`self.flying`)
  (`self.Vertical`)
  (`self.ControlAnimation`)
  (`self.UpdateAnimations`)
  (`self.PowerSupply`))

(event `CheckOutOfScreen`
  (bind _returnvalue_x (`KismetMathLibrary.BreakVector` (`self.K2_GetActorLocation`)))
  ;[1 1 1] Destroy if Out of Screen
  (bind _outactors (`GameplayStatics.GetAllActorsOfClass` "/Game/Blueprints/Level/ScreenCollider_BP.ScreenCollider_BP_C"))
  (bind _returnvalue_x_2 (`KismetMathLibrary.BreakVector` (`self.K2_GetActorLocation` (`|GetArrayItem` _outactors))))
  (if (> (- _returnvalue_x_2 400.0) _returnvalue_x)
    (`self.K2_DestroyActor` :!label _label)
    (elif (<= (+ _returnvalue_x_2 400.0) _returnvalue_x)
      (goto _label))))

(event `UpdateAnimations`
  ;[1 0 0.5704] UpdateAnimations
  (switch `/Game/Blueprints/Enemies/Zones/PowerSupply/DarkEnemyStates` (`self.DarkStates`)
    (:`NewEnumerator0`
      (`PaperFlipbookComponent.SetFlipbook` (`self.Sprite`) "/Game/Sprites/Enemies/Zones/PowerSupply/Moa_Fly.Moa_Fly"))
    (:`NewEnumerator4`
      (`PaperFlipbookComponent.SetFlipbook` (`self.Sprite`) "/Game/Sprites/Enemies/Zones/PowerSupply/Moa_Fly.Moa_Fly"))
    (:`NewEnumerator5`
      (`PaperFlipbookComponent.SetFlipbook` (`self.Sprite`) "/Game/Sprites/Enemies/Zones/PowerSupply/Moa_Fly.Moa_Fly"))
    (:`NewEnumerator1`
      (`PaperFlipbookComponent.SetFlipbook` (`self.Sprite`) "/Game/Sprites/Enemies/Zones/PowerSupply/Moa_Fly.Moa_Fly"))))

(event `PowerSupply`
  (bind _sprite (`self.Sprite`))
  ;[1 1 1] Visibility
  (if (`self.isDead`)
    (if (`/Game/Blueprints/Player/Player_BP.VideoCardON` (`self.PlayerRef`))
      (`PaperFlipbookComponent.SetSpriteColor` _sprite (`self.ColorEnemy`) :!label _label_2)
      (else
        (`PaperFlipbookComponent.SetSpriteColor` _sprite (struct :`R` 1.0 :`G` 1.0 :`B` 1.0 :`A` 1.0) :!label _label_3)))
    (elif (`self.isHit`)
      (if (`/Game/Blueprints/Player/Player_BP.VideoCardON` (`self.PlayerRef`))
        (goto _label_2)
        (else
          (goto _label_3)))
      (elif (`/Game/Blueprints/Player/Player_BP.VideoCardON` (`self.PlayerRef`))
        (if (`/Game/Blueprints/Player/Player_BP.PowerSupplyON` (`self.PlayerRef`))
          (`PaperFlipbookComponent.SetSpriteColor` _sprite (`self.ColorBG`))
          (else
            (`PaperFlipbookComponent.SetSpriteColor` _sprite (struct :`A` 1.0) :!label _label_4)))
        (else
          (goto _label_4))))))

(event `ColorControl`
  (bind _returnvalue (`KismetMathLibrary.RandomFloatInRange` 0.6 1.0))
  ;[0 1 0.8393] Color Control
  (if (`/Game/Blueprints/Player/Player_BP.VideoCardON` (`self.PlayerRef`))
    (bind _outactors (`GameplayStatics.GetAllActorsOfClass` "/Game/Blueprints/Art/ColorController.ColorController_C"))
    (bind _returnvalue_2 (`|GetDataTableRow` "/Game/Blueprints/Art/ColorSchemeTable.ColorSchemeTable" (`/Game/Blueprints/Art/ColorController.ColorScheme` (`|GetArrayItem` _outactors)))
      (:`then`
        (set `self.ColorEnemy` (* (`.Enemies_33_D3933F8042CE8CB253100FB32ECD27F6` (break `/Game/Blueprints/Art/ColorScheme` _returnvalue_2)) (make `LinearColor` _returnvalue _returnvalue _returnvalue 1.0)))
        (if (`/Game/Blueprints/Player/Player_BP.PowerSupplyON` (`self.PlayerRef`))
          (set `self.ColorBG` (`.BackGround_32_1AA2CA3B45E8BFCCF9A3E3A6590E1CD1` (break `/Game/Blueprints/Art/ColorScheme` _returnvalue_2)))
          (else
            (set `self.ColorBG` (struct))))))))

(event `VerticalFlight`
  ;[0.3522 0 1] Movement
  ;;[1 1 1] Flight Control
  (`KismetSystemLibrary.Delay` (`KismetMathLibrary.RandomFloatInRange` 1.0 2.0) :!label _label_5)
  (`self.TurnToPlayer`)
  (set `self.FlyingVertical` true)
  (`KismetSystemLibrary.Delay` 0.15)
  (set `self.FlyingVertical` false)
  (goto _label_5))

(event `flying`
  ;[0.3522 0 1] Movement
  ;;[1 1 1] Vertical & Horizontal Flight
  (if (`self.isHit`)
    _
    (elif (`self.isFacingLeft`)
      (`self.AddMovementInput` (-1.0 0.0 0.0))
      (else
        (`self.AddMovementInput` (1.0 0.0 0.0))))))

(event `TurnToPlayer`
  (bind _returnvalue_x (`KismetMathLibrary.BreakVector` (`self.K2_GetActorLocation`)))
  (bind _returnvalue_x_2 (`KismetMathLibrary.BreakVector` (`self.K2_GetActorLocation` (`self.PlayerRef`))))
  ;[0.3522 0 1] Movement
  ;;[1 1 1] Turn
  (if (`self.isHit`)
    _
    (elif (`self.isDead`)
      _
      (elif (< _returnvalue_x _returnvalue_x_2)
        (if (`self.isFacingLeft`)
          (set `self.isFacingLeft` false)
          (`SceneComponent.K2_SetRelativeRotation` (`self.Sprite`) (struct :`Yaw` 180.0) false false))
        (elif (not (`self.isFacingLeft`))
          (set `self.isFacingLeft` true)
          (`SceneComponent.K2_SetRelativeRotation` :`self` (`self.Sprite`)))))))

(event `Vertical`
  (bind (_returnvalue_x _returnvalue_y _returnvalue_z) (`KismetMathLibrary.BreakVector` (`self.K2_GetActorLocation`)))
  (bind (_returnvalue_x_2 _returnvalue_y_2 _returnvalue_z_2) (`KismetMathLibrary.BreakVector` (`self.K2_GetActorLocation` (`self.PlayerRef`))))
  ;[0.3522 0 1] Movement
  ;;[1 1 1] Vertical & Horizontal Flight
  (if (`self.isHit`)
    _
    (elif (`self.FlyingVertical`)
      (if (> _returnvalue_z _returnvalue_z_2)
        (`self.K2_AddActorWorldOffset` (0.0 0.0 -0.5))
        (else
          (`self.K2_AddActorWorldOffset` (0.0 0.0 0.5)))))))

(event `self.Capsule.OnComponentBeginOverlap`
  (params (OverlappedComponent :type "PrimitiveComponent Object Reference") (OtherActor :type "Actor Object Reference") (OtherComp :type "PrimitiveComponent Object Reference") (OtherBodyIndex :type Integer) (bFromSweep :type Boolean) (SweepResult :type "HitResult Structure (by ref)"))
  ;[0 0 0] OnScreen or Not
  (cast `/Game/Blueprints/Level/ScreenCollider_BP` OtherActor)
  (goto _label_6 :!via `Close`))

(event `CloseGate`
  ;[0 0 0] OnScreen or Not
  (goto _label_6 :!via `Open`))

(event `self.Capsule.OnComponentEndOverlap`
  (params (OverlappedComponent :type "PrimitiveComponent Object Reference") (OtherActor :type "Actor Object Reference") (OtherComp :type "PrimitiveComponent Object Reference") (OtherBodyIndex :type Integer))
  ;[0 0 0] OnScreen or Not
  (cast `/Game/Blueprints/Level/ScreenCollider_BP` OtherActor)
  (`self.CloseGate`)
  (`KismetSystemLibrary.Delay` 2.0)
  (`/Engine/EditorBlueprintResources/StandardMacros.Gate` true :!label _label_6
    (:`Exit`
      (`self.K2_DestroyActor`))))

(fn `UserConstructionScript`)