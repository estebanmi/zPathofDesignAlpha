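; Exploding fragment projectile in the CoolingSystem enemy zone that damages the player on contact.
; Launch maps a numpad-style BulletDirection to one of eight XZ-plane directions and sets the physics Sphere's velocity scaled by BulletSpeed.
; Player overlap applies damage, spawns PlayerBulletExplosion_BP and destroys the fragment, while any hit explodes it without damage.
; Tick also applies damage to an overlapping player.
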(event `OverlappingDamage`
  (bind _output (`|GetArrayItem` (`PrimitiveComponent.GetOverlappingActors` (`self.Sphere`) "/Game/Blueprints/Player/Player_BP.Player_BP_C")))
  ;[1 1 1] Overlapping Damage
  (`/Engine/EditorBlueprintResources/StandardMacros.IsValid` _output
    (:`Is Valid`
      (`GameplayStatics.ApplyDamage` _output (`self.Damage`) null self))))

(event `self.ReceiveTick`
  (params (DeltaSeconds :type "Float (single-precision)"))
  (`self.OverlappingDamage`))

(event `Launch`
  (bind (_returnvalue_x _returnvalue_y _returnvalue_z) (`KismetMathLibrary.BreakVector` (* (select `int` (`self.Bullet Direction`) :`0` (0.0 0.0 0.0) :`1` (-0.707 0.0 -0.707) :`2` (0.0 0.0 -1.0) :`3` (0.707 0.0 -0.707) :`4` (-1.0 0.0 0.0) :`5` (0.0 0.0 0.0) :`6` (1.0 0.0 0.0) :`7` (-0.707 0.0 0.707) :`8` (0.0 0.0 1.0) :`9` (0.707 0.0 0.707) :!type "Vector Structure") (`self.BulletSpeed`))))
  (`PrimitiveComponent.SetPhysicsLinearVelocity` (`self.Sphere`) (`KismetMathLibrary.MakeVector` _returnvalue_x 0.0 _returnvalue_z) false "None"))

(event `self.ReceiveBeginPlay`
  (bind _asplayer_bp (cast `/Game/Blueprints/Player/Player_BP` (`GameplayStatics.GetPlayerCharacter` 0)))
  (set `self.PlayerRef` _asplayer_bp))

(event `self.Sphere.OnComponentHit`
  (params (HitComponent :type "PrimitiveComponent Object Reference") (OtherActor :type "Actor Object Reference") (OtherComp :type "PrimitiveComponent Object Reference") (NormalImpulse :type "Vector Structure") (Hit :type "HitResult Structure (by ref)"))
  (`|SpawnActorFromClass` "/Game/Blueprints/Player/ActionPlayer/PlayerBulletExplosion_BP.PlayerBulletExplosion_BP_C" (`KismetMathLibrary.MakeTransform` (`self.K2_GetActorLocation`)) "Undefined" "OverrideRootScale" null null)
  (`self.K2_DestroyActor`))

(event `self.Sphere.OnComponentBeginOverlap`
  (params (OverlappedComponent :type "PrimitiveComponent Object Reference") (OtherActor :type "Actor Object Reference") (OtherComp :type "PrimitiveComponent Object Reference") (OtherBodyIndex :type Integer) (bFromSweep :type Boolean) (SweepResult :type "HitResult Structure (by ref)"))
  (bind _asplayer_bp (cast `/Game/Blueprints/Player/Player_BP` OtherActor))
  (`GameplayStatics.ApplyDamage` _asplayer_bp (`self.Damage`) null self)
  (`|SpawnActorFromClass` "/Game/Blueprints/Player/ActionPlayer/PlayerBulletExplosion_BP.PlayerBulletExplosion_BP_C" (`KismetMathLibrary.MakeTransform` (`self.K2_GetActorLocation`)) "Undefined" "OverrideRootScale" null null)
  (`self.K2_DestroyActor`))

(fn `UserConstructionScript`)