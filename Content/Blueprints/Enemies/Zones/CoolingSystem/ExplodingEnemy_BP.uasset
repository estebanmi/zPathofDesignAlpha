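; Paper2D hopping enemy that damages the player on contact and explodes when its HP runs out or the player enters its trigger box.
; ToAttack starts a randomly timed loop of crouch-then-jump attacks toward the player, though nothing here calls it.
; Tick turns state flags into flipbook states, while timelines shake the sprite on hits and before spawning the explosion actor.
; Loot-drop logic exists but its only caller is unreachable.
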(event `DropLoot`
  (bind _returnvalue (`KismetMathLibrary.RandomFloatInRange` 0.0 100.0))
  ;[1 1 1] Drop Loot
  (switch `/Game/Blueprints/Enemies/EnemiesLoot` (`self.Loot`)
    (:`NewEnumerator1`
      (`self.Drop HP` :!label _label))
    (:`NewEnumerator2`
      (`self.Drop BitCoin` :!label _label_2))
    (:`NewEnumerator3`
      (if (> _returnvalue 60.0)
        (if (> _returnvalue 85.0)
          (goto _label)
          (else
            (goto _label_2)))))))

(event `Explode`
  (bind (_returnvalue_x _returnvalue_y _returnvalue_z) (`KismetMathLibrary.BreakVector` (`self.K2_GetActorLocation`)))
  (bind _sprite (`self.Sprite`))
  (bind _sprite_2 (`self.Sprite`))
  (bind (_relativelocation_x _relativelocation_y _relativelocation_z) (`KismetMathLibrary.BreakVector` (`SceneComponent.RelativeLocation` _sprite_2)))
  ;[1 1 1] Explode
  (`/Engine/EditorBlueprintResources/StandardMacros.DoOnce` false
    (:`Completed`
      (`self.TurnToPlayer`)
      (`ActorComponent.K2_DestroyComponent` (`self.Box`))
      (`PrimitiveComponent.SetCollisionEnabled` (`self.CapsuleComponent`) "NoCollision")
      (`self.Jump`)
      (`GameplayStatics.PlaySound2D` "/Game/Sound/SFXs/sfx_BlopJump_Cue.sfx_BlopJump_Cue" 1.0 1.0 0.0 null null)
      (set `self.isHit` false)
      (set `self.IsJumping` true)
      (`PaperFlipbookComponent.SetFlipbook` _sprite "/Game/Sprites/Enemies/Zones/CoolingSystem/ExplodingEnemy/ExplodingEnemy_Jump.ExplodingEnemy_Jump")
      (`KismetSystemLibrary.Delay` (`PaperFlipbookComponent.GetFlipbookLength` _sprite))
      (set `CharacterMovementComponent.GravityScale` 0.0 (`self.CharacterMovement`))
      (`MovementComponent.StopMovementImmediately` (`self.CharacterMovement`))
      (set `self.isDead` true)
      (bind (_direction _horizontalshake) (`Timeline|Timeline_1` :!via `PlayFromStart`)
        (:`Update`
          (`SceneComponent.K2_SetRelativeLocation` _sprite_2 (`KismetMathLibrary.MakeVector` _horizontalshake _relativelocation_y _relativelocation_z) false false))
        (:`Finished`
          (`|SpawnActorFromClass` "/Game/Blueprints/Enemies/Zones/CoolingSystem/ExplodingEnemyExplosion_BP.ExplodingEnemyExplosion_BP_C" (`KismetMathLibrary.MakeTransform` (`KismetMathLibrary.MakeVector` _returnvalue_x (+ _returnvalue_y 2.0) _returnvalue_z)) "Undefined" "OverrideRootScale" null null)
          (`/Game/Blueprints/Player/Player_BP.EmenyKilled` (`self.PlayerRef`))
          (`self.K2_DestroyActor`))))))

(event `Drop HP`
  (bind (_returnvalue_x _returnvalue_y _returnvalue_z) (`KismetMathLibrary.BreakVector` (`self.K2_GetActorLocation`)))
  ;[1 1 1] Drop Loot
  (`|SpawnActorFromClass` "/Game/Blueprints/Collectibles/Loot/BatteryLoot_BP.BatteryLoot_BP_C" (`KismetMathLibrary.MakeTransform` (`KismetMathLibrary.MakeVector` _returnvalue_x 1.0 _returnvalue_z)) "Undefined" "OverrideRootScale" null null))

(event `Drop BitCoin`
  (bind (_returnvalue_x _returnvalue_y _returnvalue_z) (`KismetMathLibrary.BreakVector` (`self.K2_GetActorLocation`)))
  ;[1 1 1] Drop Loot
  (`|SpawnActorFromClass` "/Game/Blueprints/Collectibles/Loot/BitCoinLoot_BP.BitCoinLoot_BP_C" (`KismetMathLibrary.MakeTransform` (`KismetMathLibrary.MakeVector` _returnvalue_x 1.0 _returnvalue_z)) "Undefined" "OverrideRootScale" null null))

(event `self.ReceiveAnyDamage`
  (params (Damage :type "Float (single-precision)") (DamageType :type "DamageType Object Reference") (InstigatedBy :type "Controller Object Reference") (DamageCauser :type "Actor Object Reference"))
  (bind _sprite (`self.Sprite`))
  (bind (_relativelocation_x _relativelocation_y _relativelocation_z) (`KismetMathLibrary.BreakVector` (`SceneComponent.RelativeLocation` _sprite)))
  ;[1 0.1155 0] ReceiveDamage
  (bind _output_get (set `self.HP` (- (`self.HP`) Damage)))
  (if (<= _output_get 0.0)
    (`PrimitiveComponent.SetCollisionEnabled` (`self.CapsuleComponent`) "NoCollision")
    (`MovementComponent.SetPlaneConstraintAxisSetting` (`self.CharacterMovement`) "Z"))
  (set `self.isHit` true)
  (`GameplayStatics.PlaySound2D` "/Game/Sound/SFXs/sfx_BlopHit_Cue.sfx_BlopHit_Cue" 1.0 1.0 0.0 null null)
  (bind (_direction _horizontalshake) (`Timeline|Timeline_0` :!via `PlayFromStart`)
    (:`Update`
      (`SceneComponent.K2_SetRelativeLocation` _sprite (`KismetMathLibrary.MakeVector` _horizontalshake _relativelocation_y _relativelocation_z) false false))
    (:`Finished`
      (if (<= (`self.HP`) 0.0)
        (`self.Explode`)
        (else
          (set `self.isHit` false)
          (`self.TurnToPlayer`))))))

(event `DeadZone`
  (params (OtherActor :type "Actor Object Reference"))
  ;[1 0.1155 0] ReceiveDamage
  ;;[1 1 1] Dead Zone
  (cast `/Game/Blueprints/Level/DeadZoneFalling_BP` OtherActor)
  (`GameplayStatics.PlaySound2D` "/Game/Sound/SFXs/sfx_BlopDeath_Cue.sfx_BlopDeath_Cue" 0.3 1.0 0.0 null null)
  (`self.K2_DestroyActor`))

(event `Attack`
  ;[1 0 0] Attack Jump
  (set `CharacterMovementComponent.MaxAcceleration` (`KismetMathLibrary.RandomFloatInRange` 0.0 20000.0) (`self.CharacterMovement`))
  (`self.TurnToPlayer`)
  (if (not (`self.isDead`))
    (set `self.isCrouching` true)
    (`KismetSystemLibrary.Delay` 1.0)
    (if (`self.isCrouching`)
      (set `self.isCrouching` false)
      (if (not (`self.isHit`))
        (set `self.IsJumping` true)
        (if (`self.isFacingLeft`)
          (`self.AddMovementInput` (-1.0 0.0 0.0))
          (else
            (`self.AddMovementInput` (1.0 0.0 0.0))))
        (`self.Jump`)
        (`GameplayStatics.PlaySound2D` "/Game/Sound/SFXs/sfx_BlopJump_Cue.sfx_BlopJump_Cue" 1.0 1.0 0.0 null null)
        (set `self.IsJumping` true)))))

(event `OverlappingDamage`
  (bind _output (`|GetArrayItem` (`PrimitiveComponent.GetOverlappingActors` (`self.CapsuleComponent`) "/Game/Blueprints/Player/Player_BP.Player_BP_C")))
  ;[1 0 0] Attack Jump
  ;;[1 1 1] Overlapping Damage
  (`/Engine/EditorBlueprintResources/StandardMacros.IsValid` _output
    (:`Is Valid`
      (`GameplayStatics.ApplyDamage` _output (`self.DamageContact`) null self))))

(event `self.CapsuleComponent.OnComponentBeginOverlap`
  (params (OverlappedComponent :type "PrimitiveComponent Object Reference") (OtherActor :type "Actor Object Reference") (OtherComp :type "PrimitiveComponent Object Reference") (OtherBodyIndex :type Integer) (bFromSweep :type Boolean) (SweepResult :type "HitResult Structure (by ref)"))
  ;[1 0 0] Attack Jump
  ;;[1 0.9688 0.9688] Apply Damage
  (bind _asplayer_bp (cast `/Game/Blueprints/Player/Player_BP` OtherActor)
    (:`then`
      (`GameplayStatics.ApplyDamage` _asplayer_bp (`self.DamageContact`) null self))
    (:`CastFailed`
      (`self.DeadZone` OtherActor))))

(event `ToAttack`
  ;[1 0 0] Attack Jump
  (`KismetSystemLibrary.K2_SetTimerDelegate` (delegate `Attack`) (`KismetMathLibrary.RandomFloatInRange` 2.0 4.0) true))

(event `ControlAnimation`
  ;[0.0133 0.4271 0] Control Animation
  (if (`self.isDead`)
    (set `self.ExplodingEnemyStates` "NewEnumerator4")
    (`/Engine/EditorBlueprintResources/StandardMacros.DoOnce` false
      (:`Completed`
        (`KismetSystemLibrary.Delay` 0.6)
        (`PaperFlipbookComponent.Stop` (`self.Sprite`))))
    (elif (`self.isHit`)
      (set `self.ExplodingEnemyStates` "NewEnumerator0")
      (elif (`self.isCrouching`)
        (set `self.ExplodingEnemyStates` "NewEnumerator2")
        (elif (`self.IsJumping`)
          (set `self.ExplodingEnemyStates` "NewEnumerator3" :!label _label_3)
          (elif (`NavMovementComponent.IsFalling` (`self.CharacterMovement`))
            (goto _label_3)
            (else
              (set `self.ExplodingEnemyStates` "NewEnumerator1"))))))))

(event `TurnToPlayer`
  (bind _returnvalue_x (`KismetMathLibrary.BreakVector` (`KismetMathLibrary.GetDirectionUnitVector` (`self.K2_GetActorLocation`) (`self.K2_GetActorLocation` (`self.PlayerRef`)))))
  ;[0 0.218 1] Turn To Player
  (if (`KismetSystemLibrary.IsValid` (`self.PlayerRef`))
    (if (> _returnvalue_x 0.0)
      (if (`self.isFacingLeft`)
        (if (not (`/Game/Blueprints/Player/Player_BP.isInvisible` (`self.PlayerRef`)))
          (`self.DirectionChange`)))
      (elif (`self.isFacingLeft`)
        _
        (elif (not (`/Game/Blueprints/Player/Player_BP.isInvisible` (`self.PlayerRef`)))
          (`self.DirectionChange`))))))

(event `self.OnLanded`
  (params (Hit :type "HitResult Structure (by ref)"))
  ;[0.0133 0.4271 0] Control Animation
  ;;[1 1 1] OnLanded
  (if (> (`self.HP`) 0.0)
    (set `self.IsJumping` false)
    (set `self.isCrouching` true)
    (`KismetSystemLibrary.Delay` 0.5)
    (set `self.isCrouching` false)))

(event `self.ReceiveBeginPlay`
  ;[0.9624 1 0.9789] DEFAULT
  (`self.CastPlayerRef`))

(event `DirectionChange`
  ;[0.1362 0.1893 1] Facing Control
  (if (`self.isFacingLeft`)
    (`SceneComponent.K2_SetWorldRotation` (`self.CapsuleComponent`) (struct :`Yaw` 180.0) false false)
    (set `self.isFacingLeft` false)
    (else
      (`SceneComponent.K2_SetWorldRotation` :`self` (`self.CapsuleComponent`))
      (set `self.isFacingLeft` true))))

(event `self.ReceiveTick`
  (params (DeltaSeconds :type "Float (single-precision)"))
  ;[0.9624 1 0.9789] DEFAULT
  (`self.ControlAnimation`)
  (`self.UpdateAnimations`)
  (`self.OverlappingDamage`))

(event `UpdateAnimations`
  ;[0.07908 0.1965 1] UpdateAnimations
  (switch `/Game/Blueprints/Enemies/Zones/CoolingSystem/ExplodingEnemyStates` (`self.ExplodingEnemyStates`)
    (:`NewEnumerator0`
      (`PaperFlipbookComponent.SetFlipbook` (`self.Sprite`) "/Game/Sprites/Enemies/Zones/CoolingSystem/ExplodingEnemy/ExplodingEnemy_Hit.ExplodingEnemy_Hit"))
    (:`NewEnumerator1`
      (`PaperFlipbookComponent.SetFlipbook` (`self.Sprite`) "/Game/Sprites/Enemies/Zones/CoolingSystem/ExplodingEnemy/ExplodingEnemy_Idle.ExplodingEnemy_Idle"))
    (:`NewEnumerator2`
      (`PaperFlipbookComponent.SetFlipbook` (`self.Sprite`) "/Game/Sprites/Enemies/Zones/CoolingSystem/ExplodingEnemy/ExplodingEnemy_ToJump.ExplodingEnemy_ToJump"))
    (:`NewEnumerator3`
      (`PaperFlipbookComponent.SetFlipbook` (`self.Sprite`) "/Game/Sprites/Enemies/Zones/CoolingSystem/ExplodingEnemy/ExplodingEnemy_Jump.ExplodingEnemy_Jump"))
    (:`NewEnumerator4`
      (`PaperFlipbookComponent.SetFlipbook` (`self.Sprite`) "/Game/Sprites/Enemies/Zones/CoolingSystem/ExplodingEnemy/ExplodingEnemy_ToExplode.ExplodingEnemy_ToExplode"))))

(event `CastPlayerRef`
  ;[0.9624 1 0.9789] DEFAULT
  ;;[1 1 1] CastPlayer
  (bind _asplayer_bp (cast `/Game/Blueprints/Player/Player_BP` (`GameplayStatics.GetPlayerCharacter` 0)))
  (set `self.PlayerRef` _asplayer_bp)
  (`self.TurnToPlayer`))

(event `self.Box.OnComponentBeginOverlap`
  (params (OverlappedComponent :type "PrimitiveComponent Object Reference") (OtherActor :type "Actor Object Reference") (OtherComp :type "PrimitiveComponent Object Reference") (OtherBodyIndex :type Integer) (bFromSweep :type Boolean) (SweepResult :type "HitResult Structure (by ref)"))
  (cast `/Game/Blueprints/Player/Player_BP` OtherActor)
  (`self.Explode`))

(fn `UserConstructionScript`)