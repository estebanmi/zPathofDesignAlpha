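; Short-lived explosion actor for the exploding enemy, with a Paper2D flipbook, sound, area damage and flying fragments.
; On BeginPlay it randomly flips the flipbook, plays the sound, and schedules its destruction for when the animation length elapses.
; After a brief delay it enlarges a sphere that damages overlapping actors, then shrinks it and disables collision.
; It also launches eight ExplodingFragment_BP actors, each with its own numbered direction, skipping 5 like a numpad layout.
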(event `Fragments`
  (bind (_returnvalue_x _returnvalue_y _returnvalue_z) (`KismetMathLibrary.BreakVector` (`self.K2_GetActorLocation`)))
  (bind (_returnvalue_x_2 _returnvalue_y_2 _returnvalue_z_2) (`KismetMathLibrary.BreakVector` (`self.K2_GetActorLocation`)))
  (bind (_returnvalue_x_3 _returnvalue_y_3 _returnvalue_z_3) (`KismetMathLibrary.BreakVector` (`self.K2_GetActorLocation`)))
  (bind (_returnvalue_x_4 _returnvalue_y_4 _returnvalue_z_4) (`KismetMathLibrary.BreakVector` (`self.K2_GetActorLocation`)))
  (bind (_returnvalue_x_5 _returnvalue_y_5 _returnvalue_z_5) (`KismetMathLibrary.BreakVector` (`self.K2_GetActorLocation`)))
  (bind (_returnvalue_x_6 _returnvalue_y_6 _returnvalue_z_6) (`KismetMathLibrary.BreakVector` (`self.K2_GetActorLocation`)))
  (bind (_returnvalue_x_7 _returnvalue_y_7 _returnvalue_z_7) (`KismetMathLibrary.BreakVector` (`self.K2_GetActorLocation`)))
  (bind (_returnvalue_x_8 _returnvalue_y_8 _returnvalue_z_8) (`KismetMathLibrary.BreakVector` (`self.K2_GetActorLocation`)))
  (bind _returnvalue (`|SpawnActorFromClass` "/Game/Blueprints/Enemies/Zones/CoolingSystem/ExplodingFragment_BP.ExplodingFragment_BP_C" (`KismetMathLibrary.MakeTransform` (`KismetMathLibrary.MakeVector` _returnvalue_x_5 (- _returnvalue_y_5 1.0) _returnvalue_z_5)) "Undefined" "OverrideRootScale" null null))
  (set `/Game/Blueprints/Enemies/Zones/CoolingSystem/ExplodingFragment_BP.Bullet Direction` 1 _returnvalue)
  (`/Game/Blueprints/Enemies/Zones/CoolingSystem/ExplodingFragment_BP.Launch` _returnvalue)
  (bind _returnvalue_2 (`|SpawnActorFromClass` "/Game/Blueprints/Enemies/Zones/CoolingSystem/ExplodingFragment_BP.ExplodingFragment_BP_C" (`KismetMathLibrary.MakeTransform` (`KismetMathLibrary.MakeVector` _returnvalue_x_6 (- _returnvalue_y_6 1.0) _returnvalue_z_6)) "Undefined" "OverrideRootScale" null null))
  (set `/Game/Blueprints/Enemies/Zones/CoolingSystem/ExplodingFragment_BP.Bullet Direction` 2 _returnvalue_2)
  (`/Game/Blueprints/Enemies/Zones/CoolingSystem/ExplodingFragment_BP.Launch` _returnvalue_2)
  (bind _returnvalue_3 (`|SpawnActorFromClass` "/Game/Blueprints/Enemies/Zones/CoolingSystem/ExplodingFragment_BP.ExplodingFragment_BP_C" (`KismetMathLibrary.MakeTransform` (`KismetMathLibrary.MakeVector` _returnvalue_x_7 (- _returnvalue_y_7 1.0) _returnvalue_z_7)) "Undefined" "OverrideRootScale" null null))
  (set `/Game/Blueprints/Enemies/Zones/CoolingSystem/ExplodingFragment_BP.Bullet Direction` 3 _returnvalue_3)
  (`/Game/Blueprints/Enemies/Zones/CoolingSystem/ExplodingFragment_BP.Launch` _returnvalue_3)
  (bind _returnvalue_4 (`|SpawnActorFromClass` "/Game/Blueprints/Enemies/Zones/CoolingSystem/ExplodingFragment_BP.ExplodingFragment_BP_C" (`KismetMathLibrary.MakeTransform` (`KismetMathLibrary.MakeVector` _returnvalue_x_8 (- _returnvalue_y_8 1.0) _returnvalue_z_8)) "Undefined" "OverrideRootScale" null null))
  (set `/Game/Blueprints/Enemies/Zones/CoolingSystem/ExplodingFragment_BP.Bullet Direction` 4 _returnvalue_4)
  (`/Game/Blueprints/Enemies/Zones/CoolingSystem/ExplodingFragment_BP.Launch` _returnvalue_4)
  (bind _returnvalue_5 (`|SpawnActorFromClass` "/Game/Blueprints/Enemies/Zones/CoolingSystem/ExplodingFragment_BP.ExplodingFragment_BP_C" (`KismetMathLibrary.MakeTransform` (`KismetMathLibrary.MakeVector` _returnvalue_x (- _returnvalue_y 1.0) _returnvalue_z)) "Undefined" "OverrideRootScale" null null))
  (set `/Game/Blueprints/Enemies/Zones/CoolingSystem/ExplodingFragment_BP.Bullet Direction` 6 _returnvalue_5)
  (`/Game/Blueprints/Enemies/Zones/CoolingSystem/ExplodingFragment_BP.Launch` _returnvalue_5)
  (bind _returnvalue_6 (`|SpawnActorFromClass` "/Game/Blueprints/Enemies/Zones/CoolingSystem/ExplodingFragment_BP.ExplodingFragment_BP_C" (`KismetMathLibrary.MakeTransform` (`KismetMathLibrary.MakeVector` _returnvalue_x_2 (- _returnvalue_y_2 1.0) _returnvalue_z_2)) "Undefined" "OverrideRootScale" null null))
  (set `/Game/Blueprints/Enemies/Zones/CoolingSystem/ExplodingFragment_BP.Bullet Direction` 7 _returnvalue_6)
  (`/Game/Blueprints/Enemies/Zones/CoolingSystem/ExplodingFragment_BP.Launch` _returnvalue_6)
  (bind _returnvalue_7 (`|SpawnActorFromClass` "/Game/Blueprints/Enemies/Zones/CoolingSystem/ExplodingFragment_BP.ExplodingFragment_BP_C" (`KismetMathLibrary.MakeTransform` (`KismetMathLibrary.MakeVector` _returnvalue_x_3 (- _returnvalue_y_3 1.0) _returnvalue_z_3)) "Undefined" "OverrideRootScale" null null))
  (set `/Game/Blueprints/Enemies/Zones/CoolingSystem/ExplodingFragment_BP.Bullet Direction` 8 _returnvalue_7)
  (`/Game/Blueprints/Enemies/Zones/CoolingSystem/ExplodingFragment_BP.Launch` _returnvalue_7)
  (bind _returnvalue_8 (`|SpawnActorFromClass` "/Game/Blueprints/Enemies/Zones/CoolingSystem/ExplodingFragment_BP.ExplodingFragment_BP_C" (`KismetMathLibrary.MakeTransform` (`KismetMathLibrary.MakeVector` _returnvalue_x_4 (- _returnvalue_y_4 1.0) _returnvalue_z_4)) "Undefined" "OverrideRootScale" null null))
  (set `/Game/Blueprints/Enemies/Zones/CoolingSystem/ExplodingFragment_BP.Bullet Direction` 9 _returnvalue_8)
  (`/Game/Blueprints/Enemies/Zones/CoolingSystem/ExplodingFragment_BP.Launch` _returnvalue_8))

(event `DelayDestroy`
  (`KismetSystemLibrary.Delay` (`PaperFlipbookComponent.GetFlipbookLength` (`self.PaperFlipbook`)))
  (`self.K2_DestroyActor`))

(event `self.ReceiveBeginPlay`
  (bind _sphere (`self.Sphere`))
  (`SceneComponent.K2_SetRelativeRotation` (`self.PaperFlipbook`) (`KismetMathLibrary.SelectRotator` (struct) (struct :`Yaw` 180.0) (`KismetMathLibrary.RandomBool`)) false false)
  (`GameplayStatics.PlaySound2D` "/Game/Sound/SFXs/sfx_CodeBlockExplosion_Cue.sfx_CodeBlockExplosion_Cue" 1.0 1.0 0.0 null null)
  (`self.DelayDestroy`)
  (`KismetSystemLibrary.Delay` 0.1)
  (`SphereComponent.SetSphereRadius` (`self.Sphere`) 15.0 true)
  (`self.Fragments`)
  (`KismetSystemLibrary.Delay` 0.1)
  (`SphereComponent.SetSphereRadius` _sphere 1.0 true)
  (`PrimitiveComponent.SetCollisionEnabled` _sphere "NoCollision"))

(event `self.Sphere.OnComponentBeginOverlap`
  (params (OverlappedComponent :type "PrimitiveComponent Object Reference") (OtherActor :type "Actor Object Reference") (OtherComp :type "PrimitiveComponent Object Reference") (OtherBodyIndex :type Integer) (bFromSweep :type Boolean) (SweepResult :type "HitResult Structure (by ref)"))
  (`GameplayStatics.ApplyDamage` OtherActor 20.0 null self))

(fn `UserConstructionScript`)