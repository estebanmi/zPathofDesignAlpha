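; EnemyRunner_BP is a 2D flipbook enemy that runs continuously and damages the player sword character on contact.
; Looping timers randomly turn it toward the player, turn or jump it when stuck, and jump it at ledges found by downward traces.
; Hits freeze movement and shake the sprite via timeline before recovery or delayed destruction.
; Tick drives running and state-based flipbooks; a randomized jump attack exists, but nothing here starts it.
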(event `self.ReceiveAnyDamage`
  (params (Damage :type "Float (single-precision)") (DamageType :type "DamageType Object Reference") (InstigatedBy :type "Controller Object Reference") (DamageCauser :type "Actor Object Reference"))
  (bind _sprite (`self.Sprite`))
  (bind (_relativelocation_x _relativelocation_y _relativelocation_z) (`KismetMathLibrary.BreakVector` (`SceneComponent.RelativeLocation` _sprite)))
  ;[1 0.1155 0] ReceiveDamage
  (bind _output_get (set `self.HP` (- (`self.HP`) Damage)))
  (if (<= _output_get 0.0)
    (`PrimitiveComponent.SetCollisionEnabled` (`self.CapsuleComponent`) "NoCollision"))
  (set `self.isHit` true)
  (`GameplayStatics.PlaySound2D` "/Game/Sound/SFXs/sfx_BlopHit_Cue.sfx_BlopHit_Cue" 1.0 1.0 0.0 null null)
  (set `CharacterMovementComponent.GravityScale` 0.0 (`self.CharacterMovement`))
  (`MovementComponent.StopMovementImmediately` (`self.CharacterMovement`))
  (bind (_direction _horizontalshake) (`Timeline|Timeline_0` :!via `PlayFromStart`)
    (:`Update`
      (`SceneComponent.K2_SetRelativeLocation` _sprite (`KismetMathLibrary.MakeVector` _horizontalshake _relativelocation_y _relativelocation_z) false false))
    (:`Finished`
      (if (<= (`self.HP`) 0.0)
        (set `self.isDead` true)
        (`/Engine/EditorBlueprintResources/StandardMacros.DoOnce` false
          (:`Completed`
            (`KismetSystemLibrary.Delay` 0.3)
            (`GameplayStatics.PlaySound2D` "/Game/Sound/SFXs/sfx_BlopDeath_Cue.sfx_BlopDeath_Cue" 1.0 1.0 0.0 null null)
            (`KismetSystemLibrary.Delay` 0.7)
            (`self.K2_DestroyActor`)))
        (else
          (set `CharacterMovementComponent.GravityScale` 2.0 (`self.CharacterMovement`))
          (set `self.isHit` false))))))

(event `Attack`
  ;[1 0 0] Attack Jump
  (set `CharacterMovementComponent.MaxAcceleration` (`KismetMathLibrary.RandomFloatInRange` 0.0 20000.0) (`self.CharacterMovement`))
  (`self.TurnToPlayer`)
  (if (not (`self.isDead`))
    (`KismetSystemLibrary.Delay` 1.0)
    (if (not (`self.isHit`))
      (set `self.IsJumping` true)
      (if (`self.isFacingLeft`)
        (`self.AddMovementInput` (-1.0 0.0 0.0))
        (else
          (`self.AddMovementInput` (1.0 0.0 0.0))))
      (`self.Jump`)
      (`GameplayStatics.PlaySound2D` "/Game/Sound/SFXs/sfx_BlopJump_Cue.sfx_BlopJump_Cue" 1.0 1.0 0.0 null null)
      (set `self.IsJumping` true))))

(event `self.CapsuleComponent.OnComponentHit`
  (params (HitComponent :type "PrimitiveComponent Object Reference") (OtherActor :type "Actor Object Reference") (OtherComp :type "PrimitiveComponent Object Reference") (NormalImpulse :type "Vector Structure") (Hit :type "HitResult Structure (by ref)"))
  ;[1 0 0] Attack Jump
  ;;[1 0.9688 0.9688] Apply Damage
  (bind _asplayer_sword_bp (cast `/Game/Blueprints/Player/PlayerSword_BP` OtherActor))
  (`GameplayStatics.ApplyDamage` _asplayer_sword_bp (`self.DamageContact`) null self))

(event `ToAttack`
  ;[1 0 0] Attack Jump
  (`KismetSystemLibrary.K2_SetTimerDelegate` (delegate `Attack`) (`KismetMathLibrary.RandomFloatInRange` 2.0 4.0) true))

(event `ControlAnimation`
  ;[0.0133 0.4271 0] Control Animation
  (if (`self.isDead`)
    (set `self.RunnerStates` "NewEnumerator4")
    (`/Engine/EditorBlueprintResources/StandardMacros.DoOnce` false
      (:`Completed`
        (`KismetSystemLibrary.Delay` 1.0)
        (`PaperFlipbookComponent.Stop` (`self.Sprite`))))
    (elif (`self.isHit`)
      (set `self.RunnerStates` "NewEnumerator0")
      (elif (`self.IsJumping`)
        (set `self.RunnerStates` "NewEnumerator3" :!label _label)
        (elif (`NavMovementComponent.IsFalling` (`self.CharacterMovement`))
          (goto _label)
          (else
            (set `self.RunnerStates` "NewEnumerator1")))))))

(event `TurnToPlayer`
  (bind _returnvalue_x (`KismetMathLibrary.BreakVector` (`KismetMathLibrary.GetDirectionUnitVector` (`self.K2_GetActorLocation`) (`self.K2_GetActorLocation` (`self.PlayerRef`)))))
  ;[0 0.218 1] Turn To Player
  (if (`KismetSystemLibrary.IsValid` (`self.PlayerRef`))
    (if (> _returnvalue_x 0.0)
      (if (`self.isFacingLeft`)
        (`self.DirectionChange`))
      (elif (not (`self.isFacingLeft`))
        (`self.DirectionChange`)))))

(event `self.OnLanded`
  (params (Hit :type "HitResult Structure (by ref)"))
  ;[0.0133 0.4271 0] Control Animation
  ;;[1 1 1] OnLanded
  (if (> (`self.HP`) 0.0)
    (set `self.IsJumping` false)))

(event `self.ReceiveBeginPlay`
  ;[0.9624 1 0.9789] DEFAULT
  (`self.TurnToPlayer`)
  (`self.CastPlayerRef`)
  (`KismetSystemLibrary.K2_SetTimerDelegate` (delegate `CheckPlayerLocation`) 0.5 true)
  (`KismetSystemLibrary.K2_SetTimerDelegate` (delegate `CheckFront`) 0.1 true)
  (`KismetSystemLibrary.K2_SetTimerDelegate` (delegate `CheckFall`) 0.1 true))

(event `DirectionStart`
  ;[0.1362 0.1893 1] Facing Control
  (if (`self.isFacingLeft`)
    (`SceneComponent.K2_SetWorldRotation` :`self` (`self.CapsuleComponent`))
    (else
      (`SceneComponent.K2_SetWorldRotation` (`self.CapsuleComponent`) (struct :`Yaw` 180.0) false false))))

(event `self.ReceiveTick`
  (params (DeltaSeconds :type "Float (single-precision)"))
  ;[0.9624 1 0.9789] DEFAULT
  (`self.ControlAnimation`)
  (`self.UpdateAnimations`)
  (`self.RunForward`))

(event `UpdateAnimations`
  ;[0.07908 0.1965 1] UpdateAnimations
  (switch `/Game/Blueprints/Enemies/Runner/EnemyRunnerStates` (`self.RunnerStates`)
    (:`NewEnumerator0`
      (`PaperFlipbookComponent.SetFlipbook` (`self.Sprite`) "/Game/Sprites/Enemies/Runner/EnemyRunnerHit1.EnemyRunnerHit1"))
    (:`NewEnumerator1`
      (`PaperFlipbookComponent.SetFlipbook` (`self.Sprite`) "/Game/Sprites/Enemies/Runner/EnemyRunnerRun.EnemyRunnerRun"))
    (:`NewEnumerator3`
      (`PaperFlipbookComponent.SetFlipbook` (`self.Sprite`) "/Game/Sprites/Enemies/Runner/EnemyRunnerJump1.EnemyRunnerJump1"))
    (:`NewEnumerator4`
      (`PaperFlipbookComponent.SetFlipbook` (`self.Sprite`) "/Game/Sprites/Enemies/Runner/Death/EnemyRunnerDeath1.EnemyRunnerDeath1"))))

(event `CastPlayerRef`
  ;[0.9624 1 0.9789] DEFAULT
  ;;[1 1 1] CastPlayer
  (bind _asplayer_sword_bp (cast `/Game/Blueprints/Player/PlayerSword_BP` (`GameplayStatics.GetPlayerCharacter` 0)))
  (set `self.PlayerRef` _asplayer_sword_bp))

(event `CheckFront`
  (bind _returnvalue_x (`KismetMathLibrary.BreakVector` (`self.K2_GetActorLocation`)))
  (if (`self.isDead`)
    _
    (elif (`self.isHit`)
      _
      (elif (== (`self.LastX`) _returnvalue_x)
        (set `self.LastFacing` (`self.isFacingLeft`))
        (`self.TurnToPlayer`)
        (`KismetSystemLibrary.Delay` 0.1)
        (if (== (`self.isFacingLeft`) (`self.LastFacing`))
          (`self.Jump`))
        (else
          (set `self.LastX` _returnvalue_x))))))

(event `DirectionChange`
  ;[0.1362 0.1893 1] Facing Control
  (if (`self.isFacingLeft`)
    (`SceneComponent.K2_SetWorldRotation` (`self.CapsuleComponent`) (struct :`Yaw` 180.0) false false)
    (set `self.isFacingLeft` false)
    (else
      (`SceneComponent.K2_SetWorldRotation` :`self` (`self.CapsuleComponent`))
      (set `self.isFacingLeft` true))))

(event `CheckPlayerLocation`
  ;[1 1 1] TurnToPlayer Prob
  (if (`self.isDead`)
    _
    (elif (`self.IsJumping`)
      _
      (elif (< (`KismetMathLibrary.RandomFloatInRange` 0.0 100.0) (`self.TurnToPlayerProb`))
        (`self.TurnToPlayer`)))))

(event `CheckFall`
  (bind _returnvalue_x (`KismetMathLibrary.BreakVector` (`self.K2_GetActorLocation`)))
  (bind (_returnvalue_x_2 _returnvalue_y _returnvalue_z) (`KismetMathLibrary.BreakVector` (`self.K2_GetActorLocation`)))
  (bind _startx (`self.StartX`))
  (if (`self.isDead`)
    _
    (elif (not (`self.IsJumping`))
      (if (`self.isFacingLeft`)
        (set `self.StartX` (- _returnvalue_x 10.0))
        (else
          (set `self.StartX` (+ _returnvalue_x 10.0))))
      (bind _outhits (`KismetSystemLibrary.LineTraceMulti` (`KismetMathLibrary.MakeVector` _startx _returnvalue_y _returnvalue_z) (`KismetMathLibrary.MakeVector` _startx _returnvalue_y (- _returnvalue_z 15.0)) "TraceTypeQuery1"))
      (`/Engine/EditorBlueprintResources/StandardMacros.IsValid` (`.HitActor` (`GameplayStatics.BreakHitResult` (`|GetArrayItem` _outhits)))
        (:`Is Not Valid`
          (`self.Jump`)
          (set `self.IsJumping` true))))))

(event `RunForward`
  (if (`self.isHit`)
    _
    (elif (`self.isFacingLeft`)
      (`self.AddMovementInput` (100.0 0.0 0.0) -1.0)
      (else
        (`self.AddMovementInput` (100.0 0.0 0.0))))))

(fn `UserConstructionScript`)