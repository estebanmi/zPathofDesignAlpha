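; Background art controller that creates ambient lightning and brief white screen flashes.
; On BeginPlay, LightningIntensity sets the maximum random delay for an endless CastLightning loop.
; Each strike spawns Lightning_BP at a random offset from the ScreenCollider_BP, randomly flipped, with a small chance of recursively chaining another strike.
; FlashBG spawns WhiteBG_BP if missing and briefly unhides it, using a DoOnce to block overlapping flashes.
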(event `self.ReceiveBeginPlay`
  (switch `/Game/Blueprints/Art/LightningIntensity` (`self.LightningIntensity`)
    (:`NewEnumerator0`
      (set `self.MaxDelay` 6))
    (:`NewEnumerator1`
      (set `self.MaxDelay` 4))
    (:`NewEnumerator2`
      (set `self.MaxDelay` 2)))
  (`self.CastLightning` :!label _label)
  (`KismetSystemLibrary.Delay` (`KismetMathLibrary.RandomFloatInRange` 0.1 (`KismetMathLibrary.Conv_IntToDouble` (`self.MaxDelay`))))
  (goto _label))

(event `CastLightning`
  (bind _outactors (`GameplayStatics.GetAllActorsOfClass` "/Game/Blueprints/Level/ScreenCollider_BP.ScreenCollider_BP_C"))
  (bind _output (`|GetArrayItem` _outactors))
  (`/Engine/EditorBlueprintResources/StandardMacros.IsValid` _output
    (:`Is Valid`
      (if (`KismetMathLibrary.RandomBool`)
        (bind _returnvalue (`self.GetTransform` _output))
        (bind _returnvalue_2 (+ (.x (.location _returnvalue)) (`KismetMathLibrary.RandomFloatInRange` -150.0 150.0)))
        (bind _returnvalue_3 (+ (.z (.location _returnvalue)) (`KismetMathLibrary.RandomFloatInRange` 87.0 100.0)))
        (`|SpawnActorFromClass` "/Game/Blueprints/Art/Lightning_BP.Lightning_BP_C" (`KismetMathLibrary.MakeTransform` (`KismetMathLibrary.MakeVector` _returnvalue_2 -19.0 _returnvalue_3) (`KismetMathLibrary.MakeRotator` 0.0)) "Undefined" "OverrideRootScale" null null)
        (else
          (`|SpawnActorFromClass` "/Game/Blueprints/Art/Lightning_BP.Lightning_BP_C" (`KismetMathLibrary.MakeTransform` (`KismetMathLibrary.MakeVector` _returnvalue_2 -19.0 _returnvalue_3) (`KismetMathLibrary.MakeRotator` 0.0 0.0 180.0)) "Undefined" "OverrideRootScale" null null)))
      (if (< 90.0 (`KismetMathLibrary.RandomFloatInRange` 0.0 100.0))
        (`KismetSystemLibrary.Delay` 0.1)
        (`self.CastLightning`)))))

(event `FlashBG`
  (bind _outactors (`GameplayStatics.GetAllActorsOfClass` "/Game/Blueprints/Art/WhiteBG_BP.WhiteBG_BP_C"))
  (if (== (`KismetArrayLibrary.Array_Length` _outactors) 0)
    (`|SpawnActorFromClass` "/Game/Blueprints/Art/WhiteBG_BP.WhiteBG_BP_C" (`self.GetTransform`) "Undefined" "OverrideRootScale" null null))
  (`/Engine/EditorBlueprintResources/StandardMacros.DoOnce` false :!label _label_2
    (:`Completed`
      (bind _outactors_2 (`GameplayStatics.GetAllActorsOfClass` "/Game/Blueprints/Art/WhiteBG_BP.WhiteBG_BP_C"))
      (bind _output (`|GetArrayItem` _outactors_2))
      (`self.SetActorHiddenInGame` _output false)
      (`KismetSystemLibrary.Delay` 0.1)
      (`self.SetActorHiddenInGame` _output true)
      (goto _label_2 :!via `Reset`))))

(fn `UserConstructionScript`)