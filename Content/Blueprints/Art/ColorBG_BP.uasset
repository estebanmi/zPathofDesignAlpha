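; ColorBG_BP is a background sprite actor that keeps a solid backdrop behind the screen area.
; On BeginPlay it scales its Paper2D sprite up to cover a large area and caches the first ScreenCollider_BP found in the level.
; Each Tick it follows that collider's X and Z at a fixed depth, printing a warning if none is found.
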(event `self.ReceiveBeginPlay`
  (`SceneComponent.SetRelativeScale3D` (`self.PaperSprite`) (500.0 1.0 300.0))
  (bind _outactors (`GameplayStatics.GetAllActorsOfClass` "/Game/Blueprints/Level/ScreenCollider_BP.ScreenCollider_BP_C"))
  (bind _output (`|GetArrayItem` _outactors))
  (`/Engine/EditorBlueprintResources/StandardMacros.IsValid` _output
    (:`Is Valid`
      (set `self.ScreenColliderRef` _output))))

(event `self.ReceiveTick`
  (params (DeltaSeconds :type "Float (single-precision)"))
  (bind (_returnvalue_x _returnvalue_y _returnvalue_z) (`KismetMathLibrary.BreakVector` (`self.K2_GetActorLocation` (`self.ScreenColliderRef`))))
  (`/Engine/EditorBlueprintResources/StandardMacros.IsValid` (`self.ScreenColliderRef`)
    (:`Is Valid`
      (`self.K2_SetActorLocation` (`KismetMathLibrary.MakeVector` _returnvalue_x -25.0 _returnvalue_z)))
    (:`Is Not Valid`
      (`KismetSystemLibrary.PrintString` "White_BG: Screen Collider Missing"))))

(fn `UserConstructionScript`)