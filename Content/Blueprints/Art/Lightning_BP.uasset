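; Lightning_BP is a one-shot Paper2D lightning strike effect with a brief screen flash.
; On BeginPlay it picks one of six flipbook sets, plays IN, black and OUT phases timed by delays, then destroys itself.
; FlashScreen spawns WhiteBG_BP if none exists and briefly unhides it during the black phase.
; Position aligns to ScreenCollider_BP's X, but runs before BeginPlay assigns that reference.
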(event `FlashScreen`
  (bind _outactors (`GameplayStatics.GetAllActorsOfClass` "/Game/Blueprints/Art/WhiteBG_BP.WhiteBG_BP_C"))
  (if (== (`KismetArrayLibrary.Array_Length` _outactors) 0)
    (`|SpawnActorFromClass` "/Game/Blueprints/Art/WhiteBG_BP.WhiteBG_BP_C" (`self.GetTransform`) "Undefined" "OverrideRootScale" null null))
  (`/Engine/EditorBlueprintResources/StandardMacros.DoOnce` false :!label _label
    (:`Completed`
      (bind _outactors_2 (`GameplayStatics.GetAllActorsOfClass` "/Game/Blueprints/Art/WhiteBG_BP.WhiteBG_BP_C"))
      (bind _output (`|GetArrayItem` _outactors_2))
      (`self.SetActorHiddenInGame` _output false)
      (`KismetSystemLibrary.Delay` 0.1)
      (`self.SetActorHiddenInGame` _output true)
      (goto _label :!via `Reset`))))

(event `self.ReceiveBeginPlay`
  (bind _paperflipbook (`self.PaperFlipbook`))
  (bind _paperflipbook_2 (`self.PaperFlipbook`))
  (`self.SelectLightning`)
  (`self.Position`)
  (bind _outactors (`GameplayStatics.GetAllActorsOfClass` "/Game/Blueprints/Level/ScreenCollider_BP.ScreenCollider_BP_C"))
  (bind _output (`|GetArrayItem` _outactors))
  (`/Engine/EditorBlueprintResources/StandardMacros.IsValid` _output
    (:`Is Valid`
      (set `self.ScreenColliderRef` _output)
      (`PaperFlipbookComponent.SetFlipbook` _paperflipbook_2 (`self.LightningIN`))
      (`KismetSystemLibrary.Delay` (`PaperFlipbookComponent.GetFlipbookLength` _paperflipbook_2))
      (`PaperFlipbookComponent.SetFlipbook` (`self.PaperFlipbook`) (`self.LightningBlack`))
      (`self.FlashScreen`)
      (`KismetSystemLibrary.Delay` 0.1)
      (`PaperFlipbookComponent.SetFlipbook` _paperflipbook (`self.LightningOUT`))
      (`KismetSystemLibrary.Delay` (- (`PaperFlipbookComponent.GetFlipbookLength` _paperflipbook) 0.02))
      (`self.K2_DestroyActor`))))

(event `Position`
  (bind _returnvalue_x (`KismetMathLibrary.BreakVector` (`self.K2_GetActorLocation` (`self.ScreenColliderRef`))))
  (bind (_returnvalue_x_2 _returnvalue_y _returnvalue_z) (`KismetMathLibrary.BreakVector` (`self.K2_GetActorLocation` (`self.ScreenColliderRef`))))
  (`/Engine/EditorBlueprintResources/StandardMacros.IsValid` (`self.ScreenColliderRef`)
    (:`Is Valid`
      (`self.K2_SetActorLocation` (`KismetMathLibrary.MakeVector` _returnvalue_x_2 -19.0 900.0)))
    (:`Is Not Valid`
      (`/Engine/EditorBlueprintResources/StandardMacros.IsValid` (`self.ScreenColliderRef`)
        (:`Is Valid`
          (`self.K2_SetActorLocation` (`KismetMathLibrary.MakeVector` _returnvalue_x -19.0 900.0)))))))

(event `SelectLightning`
  (switch `int` (`KismetMathLibrary.RandomIntegerInRange` 0 5)
    (:`0`
      (set `self.LightningIN` "/Game/Sprites/Art/Lightning/Lightning1IN.Lightning1IN")
      (set `self.LightningBlack` "/Game/Sprites/Art/Lightning/Lightning1Black.Lightning1Black")
      (set `self.LightningOUT` "/Game/Sprites/Art/Lightning/Lightning1OUT.Lightning1OUT"))
    (:`1`
      (set `self.LightningIN` "/Game/Sprites/Art/Lightning/Lightning2IN.Lightning2IN")
      (set `self.LightningBlack` "/Game/Sprites/Art/Lightning/Lightning2Black.Lightning2Black")
      (set `self.LightningOUT` "/Game/Sprites/Art/Lightning/Lightning2OUT.Lightning2OUT"))
    (:`2`
      (set `self.LightningIN` "/Game/Sprites/Art/Lightning/Lightning3IN.Lightning3IN")
      (set `self.LightningBlack` "/Game/Sprites/Art/Lightning/Lightning3Black.Lightning3Black")
      (set `self.LightningOUT` "/Game/Sprites/Art/Lightning/Lightning3OUT.Lightning3OUT"))
    (:`3`
      (set `self.LightningIN` "/Game/Sprites/Art/Lightning/Lightning4IN.Lightning4IN")
      (set `self.LightningBlack` "/Game/Sprites/Art/Lightning/Lightning4Black.Lightning4Black")
      (set `self.LightningOUT` "/Game/Sprites/Art/Lightning/Lightning4OUT.Lightning4OUT"))
    (:`4`
      (set `self.LightningIN` "/Game/Sprites/Art/Lightning/Lightning5IN.Lightning5IN")
      (set `self.LightningBlack` "/Game/Sprites/Art/Lightning/Lightning5Black.Lightning5Black")
      (set `self.LightningOUT` "/Game/Sprites/Art/Lightning/Lightning5OUT.Lightning5OUT"))
    (:`5`
      (set `self.LightningIN` "/Game/Sprites/Art/Lightning/Lightning6IN.Lightning6IN")
      (set `self.LightningBlack` "/Game/Sprites/Art/Lightning/Lightning6Black.Lightning6Black")
      (set `self.LightningOUT` "/Game/Sprites/Art/Lightning/Lightning6OUT.Lightning6OUT"))))

(fn `UserConstructionScript`)