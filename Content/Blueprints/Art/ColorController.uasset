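; ColorController tints every Paper2D tile map actor in the level based on the player's power supply and video card states.
; After a short delay at BeginPlay, it darkens tiles to near black if power is off in one specific world type.
; Otherwise, and whenever ColorLevel fires, an active video card applies the Level color from the selected ColorSchemeTable row.
; Both recolor events use manual index loops over the tile map actors.
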(event `self.ReceiveBeginPlay`
  (`KismetSystemLibrary.Delay` 0.1)
  (bind _asplayer_bp (cast `/Game/Blueprints/Player/Player_BP` (`GameplayStatics.GetPlayerCharacter` 0)))
  (bind _output_get (set `self.PlayerRef` _asplayer_bp))
  (if (`|EnumEquality` (`/Game/Blueprints/Player/Player_BP.CurrentWorldType` _output_get) "NewEnumerator4")
    (if (`/Game/Blueprints/Player/Player_BP.PowerSupplyON` _output_get)
      (if (`/Game/Blueprints/Player/Player_BP.VideoCardON` _output_get) :!label _label
        (`self.TileSets`)
        (`KismetSystemLibrary.PrintString` "TileSets Colored" true true (struct :`R` 0.819336 :`B` 1.0 :`A` 1.0)))
      (else
        (`self.DarkenTileSets`)))
    (else
      (goto _label))))

(event `ColorLevel`
  (goto _label))

(event `TileSets`
  (set `self.Index` 0)
  (bind _outactors (`GameplayStatics.GetAllActorsOfClass` "/Script/Paper2D.PaperTileMapActor" :!label _label_2))
  (bind _returnvalue (`|GetDataTableRow` "/Game/Blueprints/Art/ColorSchemeTable.ColorSchemeTable" (`self.ColorScheme`))
    (:`then`
      (`PaperTileMapComponent.SetTileMapColor` (`PaperTileMapActor.RenderComponent` (`|GetArrayItem` _outactors (`self.Index`))) (`.Level_31_53E2F58345BAE2A33F5ED5BE59653F21` (break `/Game/Blueprints/Art/ColorScheme` _returnvalue)))
      (if (< (`self.Index`) (- (`KismetArrayLibrary.Array_Length` _outactors) 1))
        (set `self.Index` (+ (`self.Index`) 1))
        (goto _label_2)))))

(event `DarkenTileSets`
  (set `self.Index` 0)
  (bind _outactors (`GameplayStatics.GetAllActorsOfClass` "/Script/Paper2D.PaperTileMapActor" :!label _label_3))
  (`|GetDataTableRow` "/Game/Blueprints/Art/ColorSchemeTable.ColorSchemeTable" (`self.ColorScheme`)
    (:`then`
      (`PaperTileMapComponent.SetTileMapColor` (`PaperTileMapActor.RenderComponent` (`|GetArrayItem` _outactors (`self.Index`))) (struct :`R` 0.001 :`G` 0.001 :`B` 0.001 :`A` 1.0))
      (if (< (`self.Index`) (- (`KismetArrayLibrary.Array_Length` _outactors) 1))
        (set `self.Index` (+ (`self.Index`) 1))
        (goto _label_3)))))

(fn `UserConstructionScript`)