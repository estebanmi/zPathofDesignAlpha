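; Paper2D black tree prop that sets one of six tree sprites on BeginPlay, either randomly or by design.
; With Random set, it picks any sprite and, on a coin flip, both rotates the actor 180 degrees and lowers it by a small random amount.
; Otherwise, TreeType selects the sprite and FlipHorizontal controls the rotation.
; The construction script is empty, so the variation is applied only at runtime.
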(event `RandomTree`
  (bind (_returnvalue_x _returnvalue_y _returnvalue_z) (`KismetMathLibrary.BreakVector` (`self.K2_GetActorLocation`)))
  (if (`KismetMathLibrary.RandomBool`)
    (`self.K2_SetActorRelativeLocation` (`KismetMathLibrary.MakeVector` _returnvalue_x _returnvalue_y (- _returnvalue_z (`KismetMathLibrary.Conv_IntToDouble` (`KismetMathLibrary.RandomIntegerInRange` 0 8)))))
    (`self.K2_SetActorRotation` (struct :`Yaw` 180.0)))
  (switch `int` (`KismetMathLibrary.RandomIntegerInRange` 0 5)
    (:`0`
      (`PaperSpriteComponent.SetSprite` (`self.PaperSprite`) "/Game/Sprites/Art/Tree/BlackTree_Sprite_0.BlackTree_Sprite_0"))
    (:`1`
      (`PaperSpriteComponent.SetSprite` (`self.PaperSprite`) "/Game/Sprites/Art/Tree/BlackTree_Sprite_1.BlackTree_Sprite_1"))
    (:`2`
      (`PaperSpriteComponent.SetSprite` (`self.PaperSprite`) "/Game/Sprites/Art/Tree/BlackTree_Sprite_2.BlackTree_Sprite_2"))
    (:`3`
      (`PaperSpriteComponent.SetSprite` (`self.PaperSprite`) "/Game/Sprites/Art/Tree/BlackTree_Sprite_3.BlackTree_Sprite_3"))
    (:`4`
      (`PaperSpriteComponent.SetSprite` (`self.PaperSprite`) "/Game/Sprites/Art/Tree/BlackTree_Sprite_4.BlackTree_Sprite_4"))
    (:`5`
      (`PaperSpriteComponent.SetSprite` (`self.PaperSprite`) "/Game/Sprites/Art/Tree/BlackTree_Sprite_5.BlackTree_Sprite_5"))))

(event `self.ReceiveBeginPlay`
  (if (`self.Random`)
    (`self.RandomTree`)
    (else
      (if (`self.FlipHorizontal`)
        (`self.K2_SetActorRotation` (struct :`Yaw` 180.0)))
      (switch `/Game/Blueprints/Art/TreeTypes` (`self.TreeType`)
        (:`NewEnumerator0`
          (`PaperSpriteComponent.SetSprite` (`self.PaperSprite`) "/Game/Sprites/Art/Tree/BlackTree_Sprite_0.BlackTree_Sprite_0"))
        (:`NewEnumerator1`
          (`PaperSpriteComponent.SetSprite` (`self.PaperSprite`) "/Game/Sprites/Art/Tree/BlackTree_Sprite_1.BlackTree_Sprite_1"))
        (:`NewEnumerator2`
          (`PaperSpriteComponent.SetSprite` (`self.PaperSprite`) "/Game/Sprites/Art/Tree/BlackTree_Sprite_2.BlackTree_Sprite_2"))
        (:`NewEnumerator3`
          (`PaperSpriteComponent.SetSprite` (`self.PaperSprite`) "/Game/Sprites/Art/Tree/BlackTree_Sprite_3.BlackTree_Sprite_3"))
        (:`NewEnumerator4`
          (`PaperSpriteComponent.SetSprite` (`self.PaperSprite`) "/Game/Sprites/Art/Tree/BlackTree_Sprite_4.BlackTree_Sprite_4"))
        (:`NewEnumerator5`
          (`PaperSpriteComponent.SetSprite` (`self.PaperSprite`) "/Game/Sprites/Art/Tree/BlackTree_Sprite_5.BlackTree_Sprite_5"))))))

(fn `UserConstructionScript`)